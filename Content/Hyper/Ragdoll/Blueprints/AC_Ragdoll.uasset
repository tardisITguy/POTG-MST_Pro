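; Character component that handles replicated ragdolling and recovery to standing, with an optional get-up animation.
; OnRep handlers switch mesh physics, collision, movement and movement replication as the ragdoll state changes.
; While ragdolled, a ground trace and spring interpolation keep the capsule under the body; after a delay, a pose snapshot replaces simulation.
; Recovery detects back-lying, orients the capsule instantly or blended, and restores walking once standing.
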(event `self.ReceiveBeginPlay`
  (`self.Initialize Ragdoll Settings`))

(event `self.ReceiveTick`
  (params (DeltaSeconds :type "Float (single-precision)"))
  (bind _get_up_animation_blend_in_time (`self.Get Up Animation Blend In Time`))
  ;[0.05127 0.05127 0.05127] When ragdoll, the capsule location needs to be updated. This fixes camera location.
  (`|ExecutionSequence`
    (:`then_0`
      (if (and (`self.Rotate`) (`self.Blend Rotation On Getup`))
        ;;[0.05098 0.05098 0.05098] When the get up animation is blended in, the blend rotates the character to the original rotation, we add a counter rotation which makes sure the character stands up in a realistic orientation. The blend time can be found in the animation blueprint, since we use a regular lerp node, the blend mode(linear) must match for the animation to look right.
        (bind _output_get (set `self.Blend Timer` (+ (`self.Blend Timer`) DeltaSeconds)))
        (if (<= _output_get _get_up_animation_blend_in_time)
          (`SceneComponent.K2_SetWorldLocationAndRotation` (`/Game/Hyper/Core/Generic/BlueprintMacroLibrary/BML_Generic_Component.Get Capsule Component`) (`self.Mesh Location`) (`KismetMathLibrary.RLerp` (`self.Start Rotation`) (`self.Target Rotation`) (/ _output_get _get_up_animation_blend_in_time) true) false false)
          (else
            (set `self.Rotate` false)))))
    (:`then_1`
      (if (not (`self.Use Ragdoll Snapshot`))
        (`self.Update Capsule Location`)))))

(event `Initialize Ragdoll Settings`
  ;[0.05127 0.05127 0.05127] For ragdoll capsule component placement
  (`self.Initialize Physics Setup`)
  ;[0.05127 0.05127 0.05127] Set the tick group of the mesh to post physics. This is for the ragdolling snapshot. A snapshot is more accurate AFTER physics.
  ; https://dev.epicgames.com/community/learning/tutorials/mvvL/unreal-engine-ragdolling-and-how-to-recover-from-it 20:00
  (`self.SetTickGroup` (`/Game/Hyper/Core/Generic/BlueprintMacroLibrary/BML_Generic_Component.Get Character Mesh`) "TG_PostPhysics"))

(event `self.Server To Ragdoll`
  (params (Ragdolling :type Boolean))
  (if (not (xor (`self.Is Ragdolling`) (`self.Use Ragdoll Snapshot`)))
    (bind _output_get (set `self.Is Ragdolling` Ragdolling))
    (if _output_get
      (`KismetSystemLibrary.Delay` 3.0)
      (`self.Freeze Ragdoll`)
      (else
        (set `self.Use Ragdoll Snapshot` false)))))

(event `To Animation`
  ;[0.05098 0.05098 0.05098] There are three parts of the getup animation from ragdoll. We need to have some frames skipped so we are able to initialize some things before excecuting. We do this with delays.
  (if (`self.Use Getup Animation`)
    ;;[0.05098 0.05098 0.05098] Save snapshot for animation
    (`self.Save Pose Snapshot Ragdoll`))
  ;;[0.05098 0.05098 0.05098] Reset physics
  (`self.Reset Physics`)
  (`PrimitiveComponent.SetCollisionEnabled` (`/Game/Hyper/Core/Generic/BlueprintMacroLibrary/BML_Generic_Component.Get Capsule Component`) "QueryAndPhysics")
  ;;[0.05098 0.05098 0.05098] Re-enable movement replication (see To Ragdoll)
  (`Actor.SetReplicateMovement` (`/Game/Hyper/Core/Generic/BlueprintMacroLibrary/BML_Generic_Component.Get Character`) true)
  ;;[0.05098 0.05098 0.05098] When a getup animation is used, to animation final gets called from the animation blueprint
  (if (not (`self.Use Getup Animation`))
    (`self.To Animation Final`)))

(fn `Freeze Ragdoll`
  (if (`self.Is Ragdolling`)
    (set `self.Use Ragdoll Snapshot` true)))

(fn `Initialize Physics Setup`
  (set `self.Initial Character Mesh Offset` (`SceneComponent.RelativeLocation` (`/Game/Hyper/Core/Generic/BlueprintMacroLibrary/BML_Generic_Component.Get Character Mesh`))))

(fn `OnRep_Is Ragdolling Execution`
  (if (`self.Is Ragdolling`)
    (`self.To Ragdoll`)
    (else
      ;[0.05098 0.05098 0.05098] Align capsule with ragdolled body
      (`self.Set Getup Capsule Orientation`)
      ;[0.05098 0.05098 0.05098] Since we need to use delays, continue in the event graph
      (`self.To Animation`))))

(fn `OnRep_Use Ragdoll Snapshot Execution`
  (if (`self.Use Ragdoll Snapshot`)
    (`self.Save Pose Snapshot Ragdoll`)
    (`self.Reset Physics`)))

(fn `Reset Physics`
  (bind _mesh (`/Game/Hyper/Core/Generic/BlueprintMacroLibrary/BML_Generic_Component.Get Character Mesh`))
  (`SkeletalMeshComponent.SetAllBodiesSimulatePhysics` _mesh false)
  (`PrimitiveComponent.SetCollisionEnabled` _mesh "QueryOnly")
  (set `SkeletalMeshComponent.bUpdateJointsFromAnimation` false _mesh))

(fn `Save Pose Snapshot Ragdoll`
  (bind _returnvalue (`/Game/Hyper/Core/Generic/BlueprintMacroLibrary/BML_Generic_Component.Get Anim Instance`))
  ;[0.05127 0.05127 0.05127] Save Pose Snapshot. We use this in the Get_Up State machine
  (`/Engine/EditorBlueprintResources/StandardMacros.IsValid` _returnvalue
    (:`Is Valid`
      (`AnimInstance.SavePoseSnapshot` _returnvalue "Ragdoll_Final_Pose"))))

(fn `Set Getup Capsule Orientation`
  (locals (NewLocalVar :type "Rotator Structure" :default (struct)))
  (bind _mesh (`/Game/Hyper/Core/Generic/BlueprintMacroLibrary/BML_Generic_Component.Get Character Mesh`))
  (bind _capsule_component (`/Game/Hyper/Core/Generic/BlueprintMacroLibrary/BML_Generic_Component.Get Capsule Component`))
  (bind _returnvalue (- (`SceneComponent.GetSocketLocation` _mesh "head") (`SceneComponent.GetSocketLocation` _mesh (`self.Ragdoll Root Bone`))))
  ;[0.05127 0.05127 0.05127] To set the capsule orientation. We need to calculate the vector of the character. We do this by making a vector from the neck vs pelvis
  (`self.Set Is Character Laying On Back`)
  (`SceneComponent.K2_SetWorldLocation` _capsule_component (`self.Mesh Location`) false false)
  (set `self.Target Rotation` (`KismetMathLibrary.MakeRotFromZX` (`KismetMathLibrary.Vector_Up`) (`KismetMathLibrary.SelectVector` (* _returnvalue -1.0) _returnvalue (`self.Laying On Back`))))
  (if (`self.Blend Rotation On Getup`)
    (set `self.Start Rotation` (`SceneComponent.K2_GetComponentRotation` _capsule_component))
    (set `self.Blend Timer` 0.0)
    (set `self.Rotate` true)
    (else
      (`SceneComponent.K2_SetWorldRotation` _capsule_component (`self.Target Rotation`) false false))))

(fn `Set Is Character Laying On Back`
  (returns (`Laying on back` :type Boolean))
  (bind (_returnvalue_x _returnvalue_y _returnvalue_z) (`KismetMathLibrary.BreakVector` (`KismetMathLibrary.GetRightVector` (`SceneComponent.GetSocketRotation` (`/Game/Hyper/Core/Generic/BlueprintMacroLibrary/BML_Generic_Component.Get Character Mesh`) (`self.Ragdoll Root Bone`)))))
  ;[0.05127 0.05127 0.05127] If the Z vector of the pelvis is bigger then 0 (positive side) we are lying on our back
  (bind _output_get (set `self.Laying On Back` (> _returnvalue_z 0.0)))
  (return _output_get))

(fn `To Animation Final`
  ;[0.05127 0.05127 0.05127] Should be called when character is standing again. We call it at the event graph of the anim BP on anim notify standing
  (`CharacterMovementComponent.SetMovementMode` (`/Game/Hyper/Core/Generic/BlueprintMacroLibrary/BML_Generic_Component.Get Character Movement`) "MOVE_Walking" 0))

(fn `To Ragdoll`
  (bind _mesh (`/Game/Hyper/Core/Generic/BlueprintMacroLibrary/BML_Generic_Component.Get Character Mesh`))
  (`PrimitiveComponent.SetCollisionEnabled` _mesh "QueryAndPhysics")
  (`SkeletalMeshComponent.SetAllBodiesBelowSimulatePhysics` _mesh (`self.Ragdoll Root Bone`) true true)
  (`CharacterMovementComponent.DisableMovement` (`/Game/Hyper/Core/Generic/BlueprintMacroLibrary/BML_Generic_Component.Get Character Movement`))
  (`PrimitiveComponent.SetCollisionEnabled` (`/Game/Hyper/Core/Generic/BlueprintMacroLibrary/BML_Generic_Component.Get Capsule Component`) "NoCollision")
  (set `SkeletalMeshComponent.bUpdateJointsFromAnimation` true (`/Game/Hyper/Core/Generic/BlueprintMacroLibrary/BML_Generic_Component.Get Character Mesh`))
  ;[0.05098 0.05098 0.05098] Disable movement replication, this is a compremise, it means we dont teleport when we transition to the pose snapshot, but only when we choose to re-enable movement replication, in this case this is when we start the getup animation, see To Animation
  (`Actor.SetReplicateMovement` (`/Game/Hyper/Core/Generic/BlueprintMacroLibrary/BML_Generic_Component.Get Character`) false))

(fn `Update Capsule Location`
  (bind _returnvalue (`SceneComponent.GetSocketLocation` (`/Game/Hyper/Core/Generic/BlueprintMacroLibrary/BML_Generic_Component.Get Character Mesh`) (`self.Ragdoll Root Bone`)))
  (bind _capsulecomponent (`Character.CapsuleComponent` (`/Game/Hyper/Core/Generic/BlueprintMacroLibrary/BML_Generic_Component.Get Character`)))
  ;[0.05127 0.05127 0.05127] When ragdoll, the capsule location needs to be updated  to the location of the mesh. This fixes camera location.
  ;[0.05127 0.05127 0.05127] Only excecute when in ragdolling state:
  ; From the mesh, trace downwards and look for a hit. This is normally the ground
  (if (`self.Is Ragdolling`)
    (bind (_outhit _returnvalue_2) (`KismetSystemLibrary.LineTraceSingle` _returnvalue (- _returnvalue (0.0 0.0 200.0)) "TraceTypeQuery1"))
    (if _returnvalue_2
      ;[0.05127 0.05127 0.05127] If there is a hit from the mesh, update the location of the capsule to the hit location. Otherwise set it to the pelvis location
      (set `self.Local Target Ground Location` (`.Location` (`GameplayStatics.BreakHitResult` _outhit)))
      (else
        (set `self.Local Target Ground Location` (`SceneComponent.GetSocketLocation` (`/Game/Hyper/Core/Generic/BlueprintMacroLibrary/BML_Generic_Component.Get Character Mesh`) (`self.Ragdoll Root Bone`)))))
    ;;[0.05127 0.05127 0.05127] interpolate from mesh location to target so we don't get a snap
    (bind _returnvalue_3 (`KismetMathLibrary.VectorSpringInterp` (`self.Mesh Location`) (- (`self.Local Target Ground Location`) (`self.Initial Character Mesh Offset`)) (`self.Spring State`) 400.0 1.0 (`GameplayStatics.GetWorldDeltaSeconds`) 1.0 0.0))
    (bind _output_get (set `self.Mesh Location` _returnvalue_3))
    (`SceneComponent.K2_SetWorldLocation` (`Character.CapsuleComponent` (`/Game/Hyper/Core/Generic/BlueprintMacroLibrary/BML_Generic_Component.Get Character`)) _output_get false false)
    (else
      ;;[0.05127 0.05127 0.05127] Determines how fast the capsule is moving
      (set `self.Mesh Location` (`SceneComponent.K2_GetComponentLocation` _capsulecomponent))
      (bind _returnvalue_4 (`PrimitiveComponent.GetPhysicsLinearVelocity` _capsulecomponent "None"))
      (`KismetMathLibrary.SetVectorSpringStateVelocity` (`self.Spring State`) _returnvalue_4))))