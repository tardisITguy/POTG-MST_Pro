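; Hotbar component that links inventory and equipment items to numbered slots and runs each item's default action (equip, unequip, consume, place) on key press.
; Slots store hotbar link data back into the source item, and inventory slot updates refresh linked hotbar slots through a server event.
; Link, delink and swap run locally, then repeat on the server when remote.
; Key presses execute on the server, and an OnRep handler broadcasts slot updates.
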(fn `Delink Item From Hotbar`
  (params (`Inventory Slot Index` :type Integer) (`Hotbar Slot Index` :type Integer))
  (locals (`From Equipment` :type Boolean))
  (bind _component (`/Game/Hyper/Core/Inventory/BlueprintMacroLibrary/BML_Inventory_Component.Get Inventory Manager`))
  (bind _hotbar_slot_index (`local.Hotbar Slot Index`))
  (bind _hotbar_slots (`self.Hotbar Slots`))
  (bind _struct_inventory_slot_item (make `/Game/Hyper/Core/Inventory/Datamodel/Structures/Main_Item_Slot_Structs/Struct_Inventory_Slot_Item` (make `DataTableRowHandle` "/Game/Hyper/Core/Inventory/Datamodel/Datatables/DT_Items.DT_Items" "Empty") 1 0 false (struct :`CurrentDurability` 100.0 :`IsUseable` true) (struct :`Chanceofspawinginvendorinventory` 1.0 :`MinimalAmounttorestock` 1 :`MaximumAmounttorestock` 5 :`MaximumStock` 10) true null (struct :`Hotbarslotindex` 999 :`Inventoryslotindex` 999) (struct :`Linkedtothisequipmentslot` "NewEnumerator13" :`AmmoSlot` (struct :`AmmoDataTable` (struct :`DataTable` "/Script/Engine.DataTable'/Game/Hyper/Core/Equipment_Manager/Datamodel/Datatables/DT_Ammo.DT_Ammo'")))))
  (bind ((`IsEquipmentSlot_10_708619A24E0EDA334AD9F18F83591FD6` _isequipmentslot)) (break `/Game/Hyper/Core/Inventory/Datamodel/Structures/Main_Item_Slot_Structs/Struct_Slot_Hotbar` (`.HotbarDetails_43_3AFAE4AD4920879B80FB18B92AABA698` (break `/Game/Hyper/Core/Inventory/Datamodel/Structures/Main_Item_Slot_Structs/Struct_Inventory_Slot_Item` (`|GetArrayItem` _hotbar_slots _hotbar_slot_index)))))
  ;[0.05098 0.05098 0.05098] Check if the hotbar slot is valid
  (if (`KismetArrayLibrary.Array_IsValidIndex` _hotbar_slots _hotbar_slot_index)
    ;[0.05098 0.05098 0.05098] Clear the hotbar data in the inventory item
    (set `local.From Equipment` _isequipmentslot)
    (bind _structout (setmembers `/Game/Hyper/Core/Inventory/Datamodel/Structures/Main_Item_Slot_Structs/Struct_Inventory_Slot_Item` :`StructRef` (`self.Get Item From Inventory` (`local.Inventory Slot Index`) _isequipmentslot) :`Hotbar Details` (make `/Game/Hyper/Core/Inventory/Datamodel/Structures/Main_Item_Slot_Structs/Struct_Slot_Hotbar` false)))
    ;[0.05098 0.05098 0.05098] Clear the hotbar slot
    (`KismetArrayLibrary.Array_Set` (`self.Hotbar Slots`) (`local.Hotbar Slot Index`) _struct_inventory_slot_item)
    (`self.Hotbar Slot Updated` _struct_inventory_slot_item (`local.Hotbar Slot Index`))
    (set `self.Hotbar Slots Previous` (`self.Hotbar Slots`))
    ;[0.05098 0.05098 0.05098] Update the inventory with the updated item info (hotbar data removed)
    (`/Game/Hyper/Core/Inventory/Blueprints/AC_Inventory_Abstract.Inventory Slot Updated` _component _structout (`local.Inventory Slot Index`) (select `bool` (`local.From Equipment`) :`false` (`/Game/Hyper/Core/Inventory/Blueprints/AC_Inventory_Abstract.Inventory Slots` _component) :`true` (`/Game/Hyper/Core/Equipment_Manager/Blueprints/AC_Equipment_Manager_Abstract.Equipment` (`/Game/Hyper/Core/Equipment_Manager/BlueprintMacroLibrary/BML_Equipment_Component.Get Equipment Manager`))))))

(fn `Execute Hotbar Default Action`
  (params (Index :type Integer))
  (bind _equipment (`/Game/Hyper/Core/Equipment_Manager/BlueprintMacroLibrary/BML_Equipment_Component.Get Equipment Manager`))
  (bind _component (`/Game/Hyper/Core/Inventory/BlueprintMacroLibrary/BML_Inventory_Component.Get Inventory Manager`))
  (bind ((`IsEquipmentSlot_10_708619A24E0EDA334AD9F18F83591FD6` _isequipmentslot) (`Inventoryslotindex_6_CB0A95B4425307CD729B6EB41D482243` _inventoryslotindex)) (break `/Game/Hyper/Core/Inventory/Datamodel/Structures/Main_Item_Slot_Structs/Struct_Slot_Hotbar` (`.HotbarDetails_43_3AFAE4AD4920879B80FB18B92AABA698` (break `/Game/Hyper/Core/Inventory/Datamodel/Structures/Main_Item_Slot_Structs/Struct_Inventory_Slot_Item` (`|GetArrayItem` (`self.Hotbar Slots`) (`local.Index`))))))
  (bind _item (`self.Get Item From Inventory` _inventoryslotindex _isequipmentslot))
  ;[0.05098 0.05098 0.05098] Excecute the default action for the pressed hotbar slot if valid
  (if (`KismetArrayLibrary.Array_IsValidIndex` (`self.Hotbar Slots`) (`local.Index`))
    (if (not (`/Game/Hyper/Core/Inventory/FunctionLibraries/BFL_InventoryCrafting.Is Item Empty?` _item))
      (switch `/Game/Hyper/Core/Inventory/Datamodel/Enumerations/Enum_Inventory_Actions` (select `bool` (`|EnumInequality` (`.Linkedtothisequipmentslot_12_328C4B4543785FE7767F57B8DD236BAA` (break `/Game/Hyper/Core/Equipment_Manager/Datamodel/Structures/Main_Structs/Struct_Equipment_Slot` (`.EquipmentSlot_46_2E425EF742BCF644C62CBE8FB44E9EF7` (break `/Game/Hyper/Core/Inventory/Datamodel/Structures/Main_Item_Slot_Structs/Struct_Inventory_Slot_Item` _item)))) "NewEnumerator13") :`false` (`.Defaultinventoryaction_29_7B535D824702D60E694A369E6360B1FF` (break `/Game/Hyper/Core/Inventory/Datamodel/Structures/Sub_Structs_Attributes/Struct_Attributes_Generic` (`.GenericAttributes_2_ECBA8D824275F3AB65EED8A7E46C293F` (break `/Game/Hyper/Core/Inventory/Datamodel/Structures/Main_Item_Slot_Structs/Struct_Item` (`/Game/Hyper/Core/Inventory/FunctionLibraries/BFL_InventoryCrafting.Get Inventory info from inventory slot` _item))))) :`true` "NewEnumerator16")
        (:`NewEnumerator0`
          (`/Game/Hyper/Core/Equipment_Manager/Blueprints/AC_Equipment_Manager_Abstract.Event: Equip` _equipment _item))
        (:`NewEnumerator16`
          (`/Game/Hyper/Core/Equipment_Manager/Blueprints/AC_Equipment_Manager_Abstract.Event: Unequip` _equipment _item))
        (:`NewEnumerator2`
          (`/Game/Hyper/Core/Inventory/Blueprints/AC_Inventory_Abstract.Event: Consume Item` _component _component _item (`.Inventoryslotindex_6_CB0A95B4425307CD729B6EB41D482243` (break `/Game/Hyper/Core/Inventory/Datamodel/Structures/Main_Item_Slot_Structs/Struct_Slot_Hotbar` (`.HotbarDetails_43_3AFAE4AD4920879B80FB18B92AABA698` (break `/Game/Hyper/Core/Inventory/Datamodel/Structures/Main_Item_Slot_Structs/Struct_Inventory_Slot_Item` _item)))) (`/Game/Hyper/Core/Inventory/Blueprints/AC_Inventory_Abstract.Inventory Slots` _component) true))
        (:`NewEnumerator5`
          (`/Game/Hyper/Core/Inventory/Blueprints/AC_Inventory_Abstract.TryStartBuildMode` (`/Game/Hyper/Core/Inventory/BlueprintMacroLibrary/BML_Inventory_Component.Get Inventory Manager`) _item))))))

(fn `Link Item To Hotbar`
  (params (`Inventory Slot Index` :type Integer) (`Hotbar Slot Index` :type Integer) (`Link To Equipment` :type Boolean))
  (locals (`Item To Link` :type "/Game/Hyper/Core/Inventory/Datamodel/Structures/Main_Item_Slot_Structs/Struct_Inventory_Slot_Item Structure") (NewLocalVar :type "/Game/Hyper/Core/Inventory/Datamodel/Structures/Main_Item_Slot_Structs/Struct_Inventory_Slot_Item Structure"))
  (bind _output (`|GetArrayItem` (`self.Hotbar Slots`) (`local.Hotbar Slot Index`)))
  (bind ((`IsLinkedtoHotbar_1_1B12971C4DF17EEE5AE386A403A84AF9` _islinkedtohotbar) (`Inventoryslotindex_6_CB0A95B4425307CD729B6EB41D482243` _inventoryslotindex)) (break `/Game/Hyper/Core/Inventory/Datamodel/Structures/Main_Item_Slot_Structs/Struct_Slot_Hotbar` (`.HotbarDetails_43_3AFAE4AD4920879B80FB18B92AABA698` (break `/Game/Hyper/Core/Inventory/Datamodel/Structures/Main_Item_Slot_Structs/Struct_Inventory_Slot_Item` _output))))
  ;[0.05098 0.05098 0.05098] Only certain items can be linked to the hotbar. That is why we check what the default action is, and based on that we choose if we can link the item to the hotbar
  (`|ExecutionSequence`
    (:`then_0`
      (if (`/Game/Hyper/Core/Inventory/FunctionLibraries/BFL_InventoryCrafting.check if inventory item is equal` _output (`self.Get Item From Inventory` (`local.Inventory Slot Index`) (`local.Link To Equipment`)))
        _
        (elif _islinkedtohotbar
          (`self.Delink Item From Hotbar` _inventoryslotindex (`local.Hotbar Slot Index`)))))
    (:`then_1`
      (switch `/Game/Hyper/Core/Inventory/Datamodel/Enumerations/Enum_Inventory_Actions` (`.Defaultinventoryaction_29_7B535D824702D60E694A369E6360B1FF` (break `/Game/Hyper/Core/Inventory/Datamodel/Structures/Sub_Structs_Attributes/Struct_Attributes_Generic` (`.GenericAttributes_2_ECBA8D824275F3AB65EED8A7E46C293F` (break `/Game/Hyper/Core/Inventory/Datamodel/Structures/Main_Item_Slot_Structs/Struct_Item` (`/Game/Hyper/Core/Inventory/FunctionLibraries/BFL_InventoryCrafting.Get Inventory info from inventory slot` (`self.Get Item From Inventory` (`local.Inventory Slot Index`) (`local.Link To Equipment`)))))))
        (:`NewEnumerator0`
          _)
        (:`NewEnumerator16`
          _)
        (:`NewEnumerator2`
          _)
        (:`NewEnumerator5`
          _))
      ;[0.05098 0.05098 0.05098] If the item on the hotbar isn't empty and we're swapping we add the item to the hotbar with the correct data
      (bind _structout (setmembers `/Game/Hyper/Core/Inventory/Datamodel/Structures/Main_Item_Slot_Structs/Struct_Inventory_Slot_Item` :`StructRef` (`self.Get Item From Inventory` (`local.Inventory Slot Index`) (`local.Link To Equipment`)) :`Hotbar Details` (make `/Game/Hyper/Core/Inventory/Datamodel/Structures/Main_Item_Slot_Structs/Struct_Slot_Hotbar` true (`local.Link To Equipment`) (`local.Hotbar Slot Index`) (`local.Inventory Slot Index`))))
      (`self.Event: Add Item To Hotbar` (`local.Hotbar Slot Index`) _structout)
      (`/Game/Hyper/Core/Inventory/Blueprints/AC_Inventory_Abstract.Inventory Slot Updated` (`/Game/Hyper/Core/Inventory/BlueprintMacroLibrary/BML_Inventory_Component.Get Inventory Manager`) _structout (`local.Inventory Slot Index`) (select `bool` (`local.Link To Equipment`) :`false` (`/Game/Hyper/Core/Inventory/Blueprints/AC_Inventory_Abstract.Inventory Slots` (`/Game/Hyper/Core/Inventory/BlueprintMacroLibrary/BML_Inventory_Component.Get Inventory Manager`)) :`true` (`/Game/Hyper/Core/Equipment_Manager/Blueprints/AC_Equipment_Manager_Abstract.Equipment` (`/Game/Hyper/Core/Equipment_Manager/BlueprintMacroLibrary/BML_Equipment_Component.Get Equipment Manager`)))))))

(fn `OnRep Hotbar Slots Execution`
  (locals (`Current Item` :type "/Game/Hyper/Core/Inventory/Datamodel/Structures/Main_Item_Slot_Structs/Struct_Inventory_Slot_Item Structure"))
  ;[0.05098 0.05098 0.05098] Update all slots when hotbar update is called
  (for (_array_element _array_index) (`self.Hotbar Slots`)
    (`self.Hotbar Slot Updated` _array_element _array_index)))

(fn `Swap Hotbar Slot`
  (params (`From Slot Index` :type Integer) (`To Slot Index` :type Integer))
  (bind _to_slot_index (`local.To Slot Index`))
  (bind _from_slot_index (`local.From slot index`))
  (bind _output (`|GetArrayItem` (`self.Hotbar Slots`) (`local.From slot index`)))
  (bind _output_2 (`|GetArrayItem` (`self.Hotbar Slots`) (`local.To Slot Index`)))
  (bind (_islinkedtohotbar _isequipmentslot _hotbarslotindex _inventoryslotindex) (break `/Game/Hyper/Core/Inventory/Datamodel/Structures/Main_Item_Slot_Structs/Struct_Slot_Hotbar` (`.HotbarDetails_43_3AFAE4AD4920879B80FB18B92AABA698` (break `/Game/Hyper/Core/Inventory/Datamodel/Structures/Main_Item_Slot_Structs/Struct_Inventory_Slot_Item` _output))))
  (bind (_islinkedtohotbar_2 _isequipmentslot_2 _hotbarslotindex_2 _inventoryslotindex_2) (break `/Game/Hyper/Core/Inventory/Datamodel/Structures/Main_Item_Slot_Structs/Struct_Slot_Hotbar` (`.HotbarDetails_43_3AFAE4AD4920879B80FB18B92AABA698` (break `/Game/Hyper/Core/Inventory/Datamodel/Structures/Main_Item_Slot_Structs/Struct_Inventory_Slot_Item` _output_2))))
  (bind _struct_slot_hotbar (make `/Game/Hyper/Core/Inventory/Datamodel/Structures/Main_Item_Slot_Structs/Struct_Slot_Hotbar` _islinkedtohotbar_2 _isequipmentslot_2 _to_slot_index _inventoryslotindex_2))
  (bind _struct_slot_hotbar_2 (make `/Game/Hyper/Core/Inventory/Datamodel/Structures/Main_Item_Slot_Structs/Struct_Slot_Hotbar` _islinkedtohotbar _isequipmentslot _from_slot_index _inventoryslotindex))
  ;[0.05098 0.05098 0.05098] Swap the hotbar slots in the array
  (`KismetArrayLibrary.Array_Swap` (`self.Hotbar Slots`) (`local.From slot index`) (`local.To slot index`))
  (`|ExecutionSequence`
    (:`then_0`
      ;[0.05098 0.05098 0.05098] Update the inventory slot and link the item to the new hotbar slot
      (if (not (`/Game/Hyper/Core/Inventory/FunctionLibraries/BFL_InventoryCrafting.Is Item Empty?` _output))
        (setmembers `/Game/Hyper/Core/Inventory/Datamodel/Structures/Main_Item_Slot_Structs/Struct_Inventory_Slot_Item` :`StructRef` _output :`Hotbar Details` _struct_slot_hotbar_2)
        (setmembers `/Game/Hyper/Core/Inventory/Datamodel/Structures/Main_Item_Slot_Structs/Struct_Inventory_Slot_Item` :`StructRef` (`self.Get Item From Inventory` _inventoryslotindex _isequipmentslot) :`Hotbar Details` _struct_slot_hotbar_2))
      (`self.Hotbar Slot Updated` (`|GetArrayItem` (`self.Hotbar Slots`) (`local.From slot index`)) _from_slot_index))
    (:`then_1`
      (if (not (`/Game/Hyper/Core/Inventory/FunctionLibraries/BFL_InventoryCrafting.Is Item Empty?` _output_2))
        (setmembers `/Game/Hyper/Core/Inventory/Datamodel/Structures/Main_Item_Slot_Structs/Struct_Inventory_Slot_Item` :`StructRef` _output_2 :`Hotbar Details` _struct_slot_hotbar)
        (setmembers `/Game/Hyper/Core/Inventory/Datamodel/Structures/Main_Item_Slot_Structs/Struct_Inventory_Slot_Item` :`StructRef` (`self.Get Item From Inventory` _inventoryslotindex_2 _isequipmentslot_2) :`Hotbar Details` _struct_slot_hotbar))
      (`self.Hotbar Slot Updated` (`|GetArrayItem` (`self.Hotbar Slots`) (`local.To Slot Index`)) _to_slot_index))))