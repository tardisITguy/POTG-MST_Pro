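; Master Blueprint for interactable, buildable inventory locations such as chests and workstations, with mesh, interact radius and build-state-dependent prompts.
; Server-controlled interaction on finished buildings sets the player as owner for inventory replication, then opens crafting or dual-inventory UI on that client.
; It blocks further interaction while open and clears ownership when the UI closes.
; A linked crafting component's on/off state spawns or destroys an effect actor, optionally starting switched on.
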(event `self.ReceiveBeginPlay`
  (`parent.ReceiveBeginPlay`)
  (bind (_crafting_component _is_valid) (`/Game/Hyper/Core/Inventory/Blueprints/AC_Inventory_Abstract.Get Linked Crafting Component` (`self.AC_Inventory_Advanced`)))
  (if _is_valid
    (`|ExecutionSequence`
      (:`then_0`
        ;[1 1 1] Switch particle effect when or or off
        (add `/Game/Hyper/Core/Crafting/Blueprints/AC_Crafting_Abstract.Workstation Switched On/Off` _crafting_component (delegate `Station turned on or off`))
        (`self.Station turned on or off` (`/Game/Hyper/Core/Crafting/Blueprints/AC_Crafting_Abstract.Is On` _crafting_component))
        (add `self.On Destructed` (delegate `Destroy Fire Effect`)))
      (:`then_1`
        ;[1 1 1] Turn on at spawn (After switch particle effect is binded)
        (if (`self.Should be turned on at spawn`)
          (`/Game/Hyper/Core/Crafting/Blueprints/AC_Crafting_Abstract.Event: Execute OnOff Logic` _crafting_component true))))))

(event `Station turned on or off`
  (params (`Is On` :type Boolean))
  ;[1 1 1] Switch particle effect when or or off
  (if (`self.Turn on Particle effect when on`)
    (if `Is On`
      (bind _returnvalue (`|SpawnActorFromClass` (`self.Actor class to spawn when turned on`) (`SceneComponent.K2_GetComponentToWorld` (`self.Particle Spawn Point`)) "AdjustIfPossibleButAlwaysSpawn" "OverrideRootScale" null null))
      (set `self.Actor Spawned when turned on` _returnvalue)
      (else
        (`self.Destroy Fire Effect`)))))

(event `Destroy Fire Effect`
  ;[1 1 1] Switch particle effect when or or off
  (bind _actor_spawned_when_turned_on (`self.Actor Spawned when turned on`)
    (:`then`
      (`self.K2_DestroyActor` _actor_spawned_when_turned_on))
    (:`else`)))

(event `self.ReceiveEndPlay`
  (params (EndPlayReason :type "EEndPlayReason Enum" :default "Destroyed"))
  ;[1 1 1] Switch particle effect when or or off
  (`self.Destroy Fire Effect`))

(event `Client Create Widget`
  (params (`Owning Controller` :type "Controller Object Reference"))
  (bind (_component _is_valid) (`/Game/Hyper/UI/Blueprints/BlueprintMacroLibrary/BML_HUD_Controller.Get HUD` `Owning Controller`))
  ;[0.05127 0.05127 0.05127] Open UI in interaction. This tries to do this properly for all childs. Can be overriden.
  ;;[0.05127 0.05127 0.05127] To prevent to need to set the interact in each child, we have setup the interaction in this master. We only see two types: With crafting or without crafting
  (bind (_crafting_component _is_valid_2) (`/Game/Hyper/Core/Inventory/Blueprints/AC_Inventory_Abstract.Get Linked Crafting Component` (`self.AC_Inventory_Advanced`)))
  (if _is_valid_2
    ;;[0.05127 0.05127 0.05127] If the inventory has crafting, show with crafting UI
    (if _is_valid
      (bind _returnvalue (`|CreateWidget` "/Game/Hyper/UI/Widgets/Specific/Inventory/Main_Widgets/UI_Crafting_With_World_Object.UI_Crafting_With_World_Object_C" (`/Game/Hyper/Core/Generic/BlueprintMacroLibrary/BML_Generic_ControllerInput.Get Player Controller` `Owning Controller`) (`/Game/Hyper/Core/Inventory/BlueprintMacroLibrary/BML_Inventory_Controller.Get Inventory Manager` `Owning Controller`) (`self.AC_Inventory_Advanced`)))
      (`/Game/Hyper/UI/Blueprints/HUD/HUD_Abstract.Create Interact Location Widget` _component _returnvalue)
      (add `/Game/Hyper/UI/Blueprints/HUD/HUD_Abstract.On Disable Interact Location Widget` _component (delegate `On Disable Interact Location Widget`) :!label _label)
      (add `self.On Destructed` (delegate `Destructed`)))
    (else
      ;;[0.05127 0.05127 0.05127] If the inventory has no crafting, show the dual inventories
      (if _is_valid
        (bind _returnvalue_2 (`|CreateWidget` "/Game/Hyper/UI/Widgets/Specific/Inventory/Main_Widgets/UI_Dual_Inventories.UI_Dual_Inventories_C" (`/Game/Hyper/Core/Generic/BlueprintMacroLibrary/BML_Generic_ControllerInput.Get Player Controller` `Owning Controller`) (`/Game/Hyper/Core/Inventory/BlueprintMacroLibrary/BML_Inventory_Controller.Get Inventory Manager` `Owning Controller`) (`self.AC_Inventory_Advanced`)))
        (`/Game/Hyper/UI/Blueprints/HUD/HUD_Abstract.Create Interact Location Widget` _component _returnvalue_2)
        (goto _label)))))

(event `/Game/Hyper/Core/Interaction/Interfaces/BPI_Interact.Interact`
  (params (`Owning Controller` :type "Controller Object Reference"))
  ;[0.05098 0.05098 0.05098] Server Interaction
  (`/Engine/EditorBlueprintResources/StandardMacros.IsValid` `Owning Controller`
    (:`Is Valid`
      (if (`self.Is Player Authorized` (cast `PlayerController` `Owning Controller` :!pure true))
        (if (`self.Is Building Finished`)
          (`parent.Interact` `Owning Controller`)
          (if (`self.Try Create UI on Interaction`)
            (set `self.Is Open` true)
            ;[0.05098 0.05098 0.05098] Own this location so the inventory is replicated to the player, we are on server so call a function on client to create the ui
            (`self.SetOwner` `Owning Controller`)
            (`self.Client Create Widget` `Owning Controller`))
          (else
            ;[0.05098 0.05098 0.05098] If we didnt finish the building before interacting with the parent we dont want to interact when if finishes, this will for example open a chest as soon as you add the last materials
            (`parent.Interact` `Owning Controller`)))))))

(event `On Disable Interact Location Widget`
  (`self.Clear Owner`)
  (remove `self.On Destructed` (delegate `Destructed`)))

(event `Destructed`
  (bind _returnvalue (`self.GetOwner`))
  ;[0.05098 0.05098 0.05098] Close UI when object is destroyed
  (`/Engine/EditorBlueprintResources/StandardMacros.IsValid` _returnvalue
    (:`Is Valid`
      (`/Game/Hyper/UI/Blueprints/ActorComponents/AC_UI_Manager_Abstract.Create Ingame HUD` (`/Game/Hyper/UI/Blueprints/BlueprintMacroLibrary/BML_UI_Manager_Controller.Get UI Manager ` (cast `PlayerController` _returnvalue :!pure true))))))

(event `Clear Owner`
  ;[0.05098 0.05098 0.05098] When we close the ui, we want to set this location to be owned by no one so the inventory isn't unnecessarily replicated
  (`self.SetOwner` null)
  (set `self.Is Open` false))

(fn `Can Interact`
  (params (`Owning Controller` :type "Controller Object Reference"))
  (returns (True :type Boolean))
  (bind _true (`parent.Can Interact` `Owning Controller`))
  (return (and _true (not (`self.Is Open`)))))

(fn `Get Interact Text`
  (params (`Owning Controller` :type "PlayerController Object Reference"))
  (returns (`Interact Text` :type Text) (`Secondary Interact Text` :type Text))
  (return (select `bool` (and (`self.Is Building Finished`) (not (`self.Currently_Upgrading`))) :`false` (`self.Interact Text Not Finished`) :`true` (`.CanInteractText_146_4F2B5CE046053ECBB1CF7DBE8B47675A` (break `/Game/Hyper/Core/BuildingSystem/Datamodel/Structures/Struct_Buildable_Info` (`self.Struct Buildable`)))) (select `bool` (and (`self.Is Building Finished`) (not (`self.Currently_Upgrading`))) :`false` (`self.Secondary Interact Text Not Finished`) :`true` (`self.Secondary Interact Text Finished`))))

(fn `Get Relative Interact Text Location`
  (returns (`Relative Location` :type "Vector Structure"))
  (return (`self.Relative Interact Location`)))

(fn `Should server control the interact`
  (returns (`Server should excecute interact call` :type Boolean))
  (return true))

(fn `UserConstructionScript`
  (`|ExecutionSequence`
    (:`then_0`
      ;[1 1 1] Sets the static mesh to the given variable input
      (`StaticMeshComponent.SetStaticMesh` (`self.StaticMeshComponent`) (`self.Static Mesh`)))
    (:`then_1`
      ;[1 1 1] Set Interaction Sphere Radius
      (`SphereComponent.SetSphereRadius` (`self.Can_Interact_Sphere`) (`self.pickupradius`) true))))