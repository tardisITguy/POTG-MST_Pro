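; Water interaction location, a child of the master interact location, that lets a player drink and refill bottles.
; Interacting raises a non-persistent attribute on the player's attribute manager.
; Dirty water adds a 50/50 chance of a sickness state effect through a server event.
; Clean water instead turns every empty bottle found in the inventory into a water bottle by editing the slot structs in place.
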(event `/Game/Hyper/Core/Interaction/Interfaces/BPI_Interact.Interact`
  (params (`Owning Controller` :type "Controller Object Reference"))
  (bind _component (`/Game/Hyper/Core/Attribute_System/BlueprintMacroLibrary/BML_Attribute__Controller.Get Attribute Manager` `Owning Controller`))
  (bind _component_2 (`/Game/Hyper/Core/Inventory/BlueprintMacroLibrary/BML_Inventory_Controller.Get Inventory Manager` `Owning Controller`))
  (bind _inventory_slots (`/Game/Hyper/Core/Inventory/Blueprints/AC_Inventory_Abstract.Inventory Slots` _component_2))
  (`parent.Interact` `Owning Controller`)
  (`|ExecutionSequence`
    (:`then_0`
      ;[1 1 1] Find attribute manager
      (`/Engine/EditorBlueprintResources/StandardMacros.IsValid` _component
        (:`Is Valid`
          (`/Game/Hyper/Core/Attribute_System/Blueprints/AC_Attribute_Manager_Abstact.Change By Amount Non-Persistant-Attribute` _component "NewEnumerator10" 50.0)
          ;[1 1 1] IF Dirty water, 50/50 chance of sick
          (if (`self.IsDirtyWater`)
            (if (> (`KismetMathLibrary.RandomFloatInRange` 0.0 1.0) 0.5)
              (`/Game/Hyper/Core/Attribute_System/Blueprints/AC_Attribute_Manager_Abstact.Event server: Add or Remove State Effect` _component "NewEnumerator1" false))))))
    (:`then_1`
      ;[1 1 1] Only fill bottles when it is clean water
      (if (not (`self.IsDirtyWater`))
        ;[1 1 1] Find all empty bottles in player inventory
        (bind (_slots_found_at_indexes _succes) (`/Game/Hyper/Core/Inventory/Blueprints/AC_Inventory_Abstract.Find Existing Slot Indexes Of Specified Inventory Item` _component_2 (make `/Game/Hyper/Core/Inventory/Datamodel/Structures/Main_Item_Slot_Structs/Struct_Inventory_Slot_Item` (make `DataTableRowHandle` "/Game/Hyper/Core/Inventory/Datamodel/Datatables/DT_Items.DT_Items" "Empty_Bottle") 1 0 false (struct :`CurrentDurability` 100.0 :`IsUseable` true) (struct :`Chanceofspawinginvendorinventory` 1.0 :`MinimalAmounttorestock` 1 :`MaximumAmounttorestock` 5 :`MaximumStock` 10) true null (struct :`Hotbarslotindex` 999 :`Inventoryslotindex` 999) (struct :`Linkedtothisequipmentslot` "NewEnumerator13" :`AmmoSlot` (struct :`AmmoDataTable` (struct :`DataTable` "/Script/Engine.DataTable'/Game/Hyper/Core/Equipment_Manager/Datamodel/Datatables/DT_Ammo.DT_Ammo'")))) _inventory_slots))
        (if _succes
          ;[1 1 1] For each found empty bottle, set the array element to water bottle
          (for _array_element _slots_found_at_indexes
            (setmembers `/Game/Hyper/Core/Inventory/Datamodel/Structures/Main_Item_Slot_Structs/Struct_Inventory_Slot_Item` :`StructRef` (`|GetArrayItem` _inventory_slots _array_element) :`Item` (make `DataTableRowHandle` "/Game/Hyper/Core/Inventory/Datamodel/Datatables/DT_Items.DT_Items" "Water_Bottle"))))))))

(fn `UserConstructionScript`
  (`parent.UserConstructionScript`))