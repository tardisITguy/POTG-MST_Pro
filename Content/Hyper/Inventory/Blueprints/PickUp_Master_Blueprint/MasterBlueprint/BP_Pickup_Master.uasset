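; Master pickup actor for inventory items, taking its mesh, physics (both overridable) and prompt text from item data.
; Interact passes the item and actor to the pawn's AC_Inventory_Abstract and pauses decay.
; Optional decay re-arms a roughly one-second randomized timer, reducing durability and amount until depleted.
; TryDestroyActor optionally respawns by stripping components, waiting, then spawning a durability-reset copy at the original transform or a random navmesh point before destroying itself.
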(fn `Can Interact`
  (params (`Owning Controller` :type "Controller Object Reference"))
  (returns (True :type Boolean))
  (return true))

(fn `Decay Item`
  (returns (`Durability is zero` :type Boolean) (`No Items left to decay` :type Boolean))
  (bind ((`Amount_5_3D501FFE494086BDD8C291A969150384` _amount) (`Durabilitydetails_24_1A7269D6428BC693FF3A859CFE819E71` _durabilitydetails)) (break `/Game/Hyper/Core/Inventory/Datamodel/Structures/Main_Item_Slot_Structs/Struct_Inventory_Slot_Item` (`self.Inventory Item`)))
  (bind ((`MaxDurability_5_588AF3324BF2FB2DF784D182F3F4E8B7` _maxdurability) (`Automaticdecayamountperinterval_34_5CC2F8974E545EA804A77FA418FD4BED` _automaticdecayamountperinterval) (`Hasdecayduetouse_33_678D5D5E4563A6B84A854689EB2E4443` _hasdecayduetouse) (`Decayamountperuse_37_13A5074448CEA280977E1F897FF5CDB5` _decayamountperuse)) (break `/Game/Hyper/Core/Inventory/Datamodel/Structures/Sub_Structs_Attributes/Struct_Attributes_Durability` (`.DurabilityAttributes_11_8BFC98204F44DCE1D7ADD68E766FA9F8` (break `/Game/Hyper/Core/Inventory/Datamodel/Structures/Main_Item_Slot_Structs/Struct_Item` (`/Game/Hyper/Core/Inventory/FunctionLibraries/BFL_InventoryCrafting.Get Inventory info from inventory slot` (`self.Inventory Item`))))))
  (bind _returnvalue (- (`.CurrentDurability_8_EAC98CE74E6B1BA6EBE8DC86CE9A5442` (break `/Game/Hyper/Core/Inventory/Datamodel/Structures/Main_Item_Slot_Structs/Struct_Slot_Durability` _durabilitydetails)) (select `bool` _hasdecayduetouse :`false` _automaticdecayamountperinterval :`true` _decayamountperuse)))
  (bind _returnvalue_2 (<= _returnvalue 0.0))
  (bind _returnvalue_3 (select `bool` _returnvalue_2 :`false` _amount :`true` (- _amount 1)))
  ;[0.05098 0.05098 0.05098] Is the new amount zero going to be zero?
  (if (<= _returnvalue_3 0)
    (return true true)
    (else
      ;[0.05098 0.05098 0.05098] Updating the durability value
      (bind _structout (setmembers `/Game/Hyper/Core/Inventory/Datamodel/Structures/Main_Item_Slot_Structs/Struct_Inventory_Slot_Item` :`StructRef` (`self.Inventory Item`) :`Amount` _returnvalue_3 :`Durability details` (make `/Game/Hyper/Core/Inventory/Datamodel/Structures/Main_Item_Slot_Structs/Struct_Slot_Durability` :`Current Durability` (select `bool` _returnvalue_2 :`false` _returnvalue :`true` _maxdurability))))
      (`|VariableSetRef` (`self.Inventory Item`) _structout)
      (return _returnvalue_2 false))))

(fn `Get Interact Animation`
  (params (`Owning Controller` :type "Controller Object Reference"))
  (returns (`Anim Montage` :type "AnimMontage Object Reference"))
  (return (`/Game/Hyper/Core/Interaction/FunctionLibraries/BFL_Interaction.Select Interaction Animation` `Owning Controller` (`self.Interact Montage Left`) (`self.Interact_Montage Right`))))

(fn `Get Interact Sound`
  (returns (`Interact Sound` :type "SoundBase Object Reference"))
  (return (`self.Interact Sound`)))

(fn `Get Interact Text`
  (params (`Owning Controller` :type "PlayerController Object Reference"))
  (returns (`Interact Text` :type Text) (`Secondary Interact Text` :type Text))
  (bind _inventory_item (`self.Inventory Item`))
  (bind ((`Amount_5_3D501FFE494086BDD8C291A969150384` _amount)) (break `/Game/Hyper/Core/Inventory/Datamodel/Structures/Main_Item_Slot_Structs/Struct_Inventory_Slot_Item` _inventory_item))
  (bind ((`ItemName_2_426F1C9A4BFBECD36658919EFE06663E` _itemname)) (break `/Game/Hyper/Core/Inventory/Datamodel/Structures/Sub_Structs_Attributes/Struct_Attributes_Generic` (`.GenericAttributes_2_ECBA8D824275F3AB65EED8A7E46C293F` (break `/Game/Hyper/Core/Inventory/Datamodel/Structures/Main_Item_Slot_Structs/Struct_Item` (`/Game/Hyper/Core/Inventory/FunctionLibraries/BFL_InventoryCrafting.Get Inventory info from inventory slot` _inventory_item)))))
  (return (`|FormatText` "Pickup {Itemname}" (select `bool` (== _amount 1) :`false` (`|FormatText` "{name}[{Amount}]" _itemname _amount) :`true` _itemname)) ""))

(fn `Get Relative Interact Text Location`
  (returns (`Relative Location` :type "Vector Structure"))
  (return (`self.Text Relative Location`)))

(fn `Initialize Item`
  (`|ExecutionSequence`
    (:`then_0`
      ;[0.05127 0.05127 0.05127] optionally Override static mesh
      (if (`self.Override static mesh`)
        (`StaticMeshComponent.SetStaticMesh` (`self.StaticMesh`) (`self.Overriden static mesh`))))
    (:`then_1`
      ;[0.04688 0.04688 0.04688] Determines if the pickup should simulate physics with the option to manually override
      (`PrimitiveComponent.SetSimulatePhysics` (`self.StaticMesh`) (select `bool` (`self.Override Simulate Physics?`) :`false` (`.ShouldSimulatePhysicsinWorld_31_9B3BD9FB4C72F4F8BE144D940E428EA2` (break `/Game/Hyper/Core/Inventory/Datamodel/Structures/Sub_Structs_Attributes/Struct_Attributes_Generic` (`.GenericAttributes_2_ECBA8D824275F3AB65EED8A7E46C293F` (break `/Game/Hyper/Core/Inventory/Datamodel/Structures/Main_Item_Slot_Structs/Struct_Item` (`/Game/Hyper/Core/Inventory/FunctionLibraries/BFL_InventoryCrafting.Get Inventory info from inventory slot` (`self.Inventory Item`)))))) :`true` (`self.Simulate Physics?`))))))

(fn `Should get other Actor to Interact with`
  (params (`Based on this Component` :type "PrimitiveComponent Object Reference"))
  (returns (True :type Boolean) (`Actor To Interact With` :type "Actor Object Reference"))
  (return false null))

(fn `Should server control the interact`
  (returns (`Server should excecute interact call` :type Boolean))
  (return false))

(fn `UserConstructionScript`
  ;[0.05098 0.05098 0.05098] Load and set static mesh
  (bind _object (`/Game/Hyper/Core/Generic/BlueprintMacroLibrary/BML_AssetLoading.Load Asset Blocking Checked` (`.Mesh_39_D54234E34E40EAD1251EACB012D1D572` (break `/Game/Hyper/Core/Inventory/Datamodel/Structures/Sub_Structs_Attributes/Struct_Attributes_Generic` (`.GenericAttributes_2_ECBA8D824275F3AB65EED8A7E46C293F` (break `/Game/Hyper/Core/Inventory/Datamodel/Structures/Main_Item_Slot_Structs/Struct_Item` (`/Game/Hyper/Core/Inventory/FunctionLibraries/BFL_InventoryCrafting.Get Inventory info from inventory slot` (`self.Inventory Item`)))))))
    (:`Is Valid`
      (bind _asstatic_mesh (cast `StaticMesh` _object))
      (`StaticMeshComponent.SetStaticMesh` (`self.StaticMesh`) _asstatic_mesh)
      (`self.Initialize Item`))))