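; Pickup pad that equips its configured inventory item on whoever overlaps it, displaying the item's async-loaded mesh.
; On authority, overlap is ignored during equip, unequip or montage playback; unarmed, fists or empty items trigger an unequip instead.
; Other items are first added to the inventory to obtain a slot index, then equipped from the first matching slot.
; Pickup then fires and plays a sound through the replication component.
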(event `self.Interact_Area_Sphere.OnComponentBeginOverlap`
  (params (OverlappedComponent :type "PrimitiveComponent Object Reference") (OtherActor :type "Actor Object Reference") (OtherComp :type "PrimitiveComponent Object Reference") (OtherBodyIndex :type Integer) (bFromSweep :type Boolean) (SweepResult :type "HitResult Structure (by ref)"))
  (bind _returnvalue (`self.GetInstigatorController` OtherActor))
  (bind _inventory_item (`self.Inventory Item`))
  (bind (_item _amount _slotindex _isbeingcrafted _durabilitydetails _tradingandlootdetails _shouldaddxpwhenpickedup _owningactor _hotbardetails _equipmentslot) (break `/Game/Hyper/Core/Inventory/Datamodel/Structures/Main_Item_Slot_Structs/Struct_Inventory_Slot_Item` (`self.Inventory Item`)))
  (bind _equipment (`/Game/Hyper/Core/Equipment_Manager/BlueprintMacroLibrary/BML_Equipment_Controller.Get Equipment Manager` _returnvalue))
  (bind _component (`/Game/Hyper/Core/Inventory/BlueprintMacroLibrary/BML_Inventory_Controller.Get Inventory Manager` _returnvalue))
  (bind (_equipment_2 _is_valid) (`/Game/Hyper/Core/Equipment_Manager/BlueprintMacroLibrary/BML_Equipment_Controller.Get Equipment Manager` _returnvalue))
  (`/Engine/EditorBlueprintResources/StandardMacros.IsValid` _returnvalue
    (:`Is Valid`
      (`/Engine/EditorBlueprintResources/ActorMacros.Switch Has Authority`
        (:`Authority`
          ;[0.05127 0.05127 0.05127] Does the actor has an equipment manager and is able to equip?
          (if _is_valid
            (if (not (or (`/Game/Hyper/Core/Equipment_Manager/Blueprints/AC_Equipment_Manager_Abstract.Is Equiping` _equipment_2) (`/Game/Hyper/Core/Equipment_Manager/Blueprints/AC_Equipment_Manager_Abstract.Is Unequiping` _equipment_2) (`AnimInstance.IsAnyMontagePlaying` (`/Game/Hyper/Core/Generic/BlueprintMacroLibrary/BML_Generic_ControllerInput.Get Anim Instance` _returnvalue))))
              ;[0.05127 0.05127 0.05127] When equipping an item, it is normally done via the inventory itself. The equip will peform a swap with the inventory item.
              ; However, if wanting to equip on overlap, we do not have the slot index. So we first add it to the inventory, so it creates the slot index to be able to be swapped.
              ; After that, we can peform the equip.
              (if (or (`/Game/Hyper/Core/Equipment_Manager/FunctionLibraries/BFL_Equipment.Is Slot Unarmed` _inventory_item) (`/Game/Hyper/Core/Equipment_Manager/FunctionLibraries/BFL_Equipment.Is Slot Fists` _inventory_item) (`/Game/Hyper/Core/Inventory/FunctionLibraries/BFL_InventoryCrafting.Is Item Empty?` _inventory_item))
                (`/Game/Hyper/Core/Equipment_Manager/Blueprints/AC_Equipment_Manager_Abstract.Event: Unequip` _equipment (`.item found in equipment slot` (`/Game/Hyper/Core/Equipment_Manager/Blueprints/AC_Equipment_Manager_Abstract.Get Equipment slot in equipment array` _equipment "NewEnumerator8")))
                (else
                  ;;[0.05127 0.05127 0.05127] Calling a function in the Inventory Abstract. It will excecute on the inventory component that has been assigned to the player. E.g. The basic, or the advanced. That will be determined by "Dynamic Dispatching"
                  (`/Game/Hyper/Core/Inventory/Blueprints/AC_Inventory_Abstract.Event: Try Add Item to inventory automatically` (`/Game/Hyper/Core/Inventory/BlueprintMacroLibrary/BML_Inventory_Controller.Get Inventory Manager` _returnvalue) (`self.Inventory Item`) false 0 true false true)
                  ;;[0.05127 0.05127 0.05127] Get the first found index of the item that was just added. Yes this means if you have two of the same weapons it will equip the first, not the most recent. Otherwise you need to manually find empty slot, and get that index
                  (bind (_slots_found_at_indexes _succes) (`/Game/Hyper/Core/Inventory/Blueprints/AC_Inventory_Abstract.Find Existing Slot Indexes Of Specified Inventory Item` _component (`self.Inventory Item`) (`/Game/Hyper/Core/Inventory/Blueprints/AC_Inventory_Abstract.Inventory Slots` _component)))
                  (if _succes
                    _
                    (else
                      _))
                  ;;[0.05127 0.05127 0.05127] Equip the items that has just been added to the inventory with on the specific slot index
                  (`/Game/Hyper/Core/Equipment_Manager/Blueprints/AC_Equipment_Manager_Abstract.Event: Equip` (`/Game/Hyper/Core/Equipment_Manager/BlueprintMacroLibrary/BML_Equipment_Controller.Get Equipment Manager` _returnvalue) (make `/Game/Hyper/Core/Inventory/Datamodel/Structures/Main_Item_Slot_Structs/Struct_Inventory_Slot_Item` _item _amount (select `bool` _succes :`true` (`|GetArrayItem` _slots_found_at_indexes)) _isbeingcrafted _durabilitydetails _tradingandlootdetails _shouldaddxpwhenpickedup _owningactor _hotbardetails _equipmentslot))
                  ;;[0.05127 0.05127 0.05127] Spawn sound and trigger item picked up
                  (`self.Item Picked Up`)
                  (`/Game/Hyper/Core/ReplicationSubSystem/Blueprints/AC_Replication_Abstract.Initialize Spawn Sound At Location` (`/Game/Hyper/Core/ReplicationSubSystem/BlueprintMacroLibrary/BML_Replication_Controller.Get Replication` _returnvalue) "/Game/Hyper/ResourcePack/Audio/MetaSounds/sfx_Interactable_WeaponPad_Collect_nl_metaPreset.sfx_Interactable_WeaponPad_Collect_nl_metaPreset" (`self.K2_GetActorLocation`) false 0.0 "/Game/Hyper/ResourcePack/Audio/AttenuationPresets/ATT_Default.ATT_Default" :!label _label))))))
        (:`Remote`
          (goto _label))))))

(event `self.ReceiveBeginPlay`
  (bind _object (`/Game/Hyper/Core/Generic/BlueprintMacroLibrary/BML_AssetLoading.Async Load Asset Checked` (`.Mesh_39_D54234E34E40EAD1251EACB012D1D572` (break `/Game/Hyper/Core/Inventory/Datamodel/Structures/Sub_Structs_Attributes/Struct_Attributes_Generic` (`.GenericAttributes_2_ECBA8D824275F3AB65EED8A7E46C293F` (break `/Game/Hyper/Core/Inventory/Datamodel/Structures/Main_Item_Slot_Structs/Struct_Item` (`/Game/Hyper/Core/Inventory/FunctionLibraries/BFL_InventoryCrafting.Get Inventory info from inventory slot` (`self.Inventory Item`)))))))
    (:`Completed`
      (bind _asstatic_mesh (cast `StaticMesh` _object))
      (set `self.Item Mesh` _asstatic_mesh)
      (`self.Initialize item`)
      (`self.Set relative location`))))

(fn `Initialize item`
  ;[1 1 1] Sets the static mesh to the given variable input
  (`StaticMeshComponent.SetStaticMesh` (`self.StaticMesh`) (`self.Item Mesh`)))

(fn `UserConstructionScript`
  (`self.Initialize item`)
  (`self.Set relative location`))