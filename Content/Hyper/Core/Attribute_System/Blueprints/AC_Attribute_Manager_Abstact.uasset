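; Abstract attribute manager component defining the interface for a character's attributes, states, damage, temperature and state effects.
; It declares getters and setters per attribute category, server events for attribute, effect and energy changes, and HUD value queries.
; Bodies are empty or return defaults, except the health and state-effect OnRep functions, which forward to empty Execution functions, presumably for child overrides.
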(event `self.ReceiveBeginPlay`)

(event `Event: Set Temperature State based on external temperature`
  (params (`External Temperature` :type "Float (double-precision)")))

(event `On Take Damage`
  (params (DamagedActor :type "Actor Object Reference") (Damage :type "Float (double-precision)") (`Damage Type` :type "DamageType Object Reference") (InstigatedBy :type "Controller Object Reference") (DamageCauser :type "Actor Object Reference")))

(event `Change By Amount Non-Persistant-Attribute`
  (params (`Non Persistant Attribute` :type "/Game/Hyper/Core/Attribute_System/Datamodel/Attribute_Effects/Enumerations/Enum_Non-Persistent_Character_Attributes Enum" :default "NewEnumerator13") (Amount :type "Float (double-precision)")))

(event `Server Remove or add all attribute values`
  (params (`Assigned Attributes` :type "/Game/Hyper/Core/Attribute_System/Datamodel/Attribute_Effects/Structures/Struct_Assigned_Attributes Structure") (Remove :type Boolean)))

(event `Event server: Add or Remove the attribute Value`
  (params (`Attribute Type` :type "/Game/Hyper/Core/Attribute_System/Datamodel/Attribute_Effects/Enumerations/Enum_Attribute_Types Enum" :default "NewEnumerator0") (`Is Removing` :type Boolean) (`Primary Attribute` :type "/Game/Hyper/Core/Attribute_System/Datamodel/Attribute_Effects/Enumerations/Enum_Persistent_Character_Primary_Attributes Enum" :default "NewEnumerator38") (`Survival Attribute` :type "/Game/Hyper/Core/Attribute_System/Datamodel/Attribute_Effects/Enumerations/Enum_Persistent_Character_Survival_Attributes Enum" :default "NewEnumerator19") (`Combat Attribute` :type "/Game/Hyper/Core/Attribute_System/Datamodel/Attribute_Effects/Enumerations/Enum_Persistant_Generic_Combat_Attributes Enum" :default "NewEnumerator16") (`Ranged Attribute` :type "/Game/Hyper/Core/Attribute_System/Datamodel/Attribute_Effects/Enumerations/Enum_Persistant_RangedCombat_Attributes Enum" :default "NewEnumerator13") (`Level Attribute` :type "/Game/Hyper/Core/Level_Manager/Datamodel/Enumerations/Enum_Skills Enum" :default "NewEnumerator29") (Base :type "Float (double-precision)") (Added :type "Float (double-precision)")))

(event `Event server: Add or Remove State Effect`
  (params (`State Effect` :type "/Game/Hyper/Core/Attribute_System/Datamodel/State_Effects/Enumerations/Enum_State_Effects Enum" :default "NewEnumerator0") (Remove :type Boolean)))

(event `Client: Show Damage Text`
  (params (`Damaged Actor` :type "Actor Object Reference") (Damage :type "Float (double-precision)") (Blocked :type Boolean)))

(event `Server Set Consume Energy`
  (params (`Consume Stamina` :type Boolean)))

(fn `Current Chill Temperature`
  (returns (`Current Chill Temperature` :type "Float (double-precision)"))
  (return 0.0))

(fn `Current Misc States`
  (returns (Wet :type Boolean) (Warmed :type Boolean) (`On Fire` :type Boolean))
  (return false false false))

(fn `Current TemperatureState`
  (returns (`Current Temperature State` :type "/Game/Hyper/Core/Attribute_System/Datamodel/State_Effects/Enumerations/Enum_TemperatureStates Enum"))
  (return "NewEnumerator0"))

(fn `CurrentHealthStates`
  (returns (`Is Healthy` :type Boolean) (`Is Wounded` :type Boolean) (`Is Sick` :type Boolean) (`Is Infected` :type Boolean) (`Is Poisoned` :type Boolean) (`Is Drunk` :type Boolean) (`Is Fatigued` :type Boolean) (`Is Bleeding` :type Boolean) (`Is Healthy time` :type Integer) (`Is WoundedTime` :type Integer) (`Is Sick Time` :type Integer) (`Is Infected Time` :type Integer) (`Is Poisoned Time` :type Integer) (`Is Drunk Time` :type Integer) (`Is Fatigued Time` :type Integer) (`Is Bleeding Time` :type Integer) (`Is Stunned` :type Boolean))
  (return false false false false false false false false 0 0 0 0 0 0 0 0 false))

(fn `energy_playerstates_hud_values`
  (returns (CurrentEnergy :type "Float (double-precision)") (MaxEnergy :type "Float (double-precision)"))
  (return 0.0 0.0))

(fn `Fatigue_playerstates_hud_values`
  (returns (`Current Fatigue` :type "Float (double-precision)") (`Maximum Fatigue` :type "Float (double-precision)"))
  (return 0.0 0.0))

(fn `Food_playerstates_hud_values`
  (returns (CurrentFood :type "Float (double-precision)") (MaxFood :type "Float (double-precision)"))
  (return 0.0 0.0))

(fn `Get Character Attribute State`
  (params (Attribute :type "/Game/Hyper/Core/Attribute_System/Datamodel/Attribute_Effects/Enumerations/Enum_Non-Persistent_Character_Attributes Enum" :default "NewEnumerator13"))
  (returns (`Is Zero` :type Boolean) (`Is In Low Range` :type Boolean) (`Is Max` :type Boolean))
  (return false false false))

(fn `Get Delta Seconds`
  (returns (Seconds :type "Float (double-precision)"))
  (return 0.0))

(fn `Get Generic Combat Attribute`
  (params (Attribute :type "/Game/Hyper/Core/Attribute_System/Datamodel/Attribute_Effects/Enumerations/Enum_Persistant_Generic_Combat_Attributes Enum" :default "NewEnumerator16"))
  (returns (Value :type "/Game/Hyper/Core/Attribute_System/Datamodel/Attribute_Effects/Structures/Struct_Float_Attribute Structure"))
  (return))

(fn `Get Non- Persistent Character Attribute`
  (params (Attribute :type "/Game/Hyper/Core/Attribute_System/Datamodel/Attribute_Effects/Enumerations/Enum_Non-Persistent_Character_Attributes Enum" :default "NewEnumerator13"))
  (returns (Value :type "Float (double-precision)"))
  (return 0.0))

(fn `Get Persistent Level Attribute`
  (params (Attribute :type "/Game/Hyper/Core/Level_Manager/Datamodel/Enumerations/Enum_Skills Enum" :default "NewEnumerator29"))
  (returns (Level :type Integer))
  (return 0))

(fn `Get Persistent Primary Character Attribute`
  (params (Attribute :type "/Game/Hyper/Core/Attribute_System/Datamodel/Attribute_Effects/Enumerations/Enum_Persistent_Character_Primary_Attributes Enum" :default "NewEnumerator38"))
  (returns (Value :type "/Game/Hyper/Core/Attribute_System/Datamodel/Attribute_Effects/Structures/Struct_Float_Attribute Structure"))
  (return))

(fn `Get Persistent Survival Character Attribute`
  (params (Attribute :type "/Game/Hyper/Core/Attribute_System/Datamodel/Attribute_Effects/Enumerations/Enum_Persistent_Character_Survival_Attributes Enum" :default "NewEnumerator19"))
  (returns (Value :type "/Game/Hyper/Core/Attribute_System/Datamodel/Attribute_Effects/Structures/Struct_Float_Attribute Structure"))
  (return))

(fn `Get Projectile Combat Attributes`
  (params (`Use Ammo` :type Boolean))
  (returns (Generic :type "Array of /Game/Hyper/Core/Attribute_System/Datamodel/Attribute_Effects/Structures/Struct_Persistant_Generic_Combat_Attributes Structure") (Ranged :type "Array of /Game/Hyper/Core/Attribute_System/Datamodel/Attribute_Effects/Structures/Struct_Persistant_RangedCombat_Attributes Structure") (`Ammo Damage Type` :type "DamageType Soft Class Reference"))
  (locals (`Generic Combat` :type "Array of /Game/Hyper/Core/Attribute_System/Datamodel/Attribute_Effects/Structures/Struct_Persistant_Generic_Combat_Attributes Structure") (`Ranged Combat` :type "Array of /Game/Hyper/Core/Attribute_System/Datamodel/Attribute_Effects/Structures/Struct_Persistant_RangedCombat_Attributes Structure"))
  (return _ _ null))

(fn `Get Ranged Combat Attribute`
  (params (Attribute :type "/Game/Hyper/Core/Attribute_System/Datamodel/Attribute_Effects/Enumerations/Enum_Persistant_RangedCombat_Attributes Enum" :default "NewEnumerator13"))
  (returns (Value :type "/Game/Hyper/Core/Attribute_System/Datamodel/Attribute_Effects/Structures/Struct_Float_Attribute Structure"))
  (return))

(fn `Get State Effect Time Left`
  (params (`State Effect` :type "/Game/Hyper/Core/Attribute_System/Datamodel/State_Effects/Enumerations/Enum_State_Effects Enum" :default "NewEnumerator0"))
  (returns (`Time Left` :type "Float (double-precision)") (`Is Active` :type Boolean))
  (return 0.0 false))

(fn `Get Variable Values Of Assigned Attributes`
  (params (`Attribute Type` :type "/Game/Hyper/Core/Attribute_System/Datamodel/Attribute_Effects/Enumerations/Enum_Attribute_Types Enum" :default "NewEnumerator0") (`Non persistant` :type "/Game/Hyper/Core/Attribute_System/Datamodel/Attribute_Effects/Enumerations/Enum_Non-Persistent_Character_Attributes Enum" :default "NewEnumerator13") (`Primary Attribute` :type "/Game/Hyper/Core/Attribute_System/Datamodel/Attribute_Effects/Enumerations/Enum_Persistent_Character_Primary_Attributes Enum" :default "NewEnumerator38") (`Survival Attribute` :type "/Game/Hyper/Core/Attribute_System/Datamodel/Attribute_Effects/Enumerations/Enum_Persistent_Character_Survival_Attributes Enum" :default "NewEnumerator19") (`Combat Attribute` :type "/Game/Hyper/Core/Attribute_System/Datamodel/Attribute_Effects/Enumerations/Enum_Persistant_Generic_Combat_Attributes Enum" :default "NewEnumerator16") (`Ranged Attribute` :type "/Game/Hyper/Core/Attribute_System/Datamodel/Attribute_Effects/Enumerations/Enum_Persistant_RangedCombat_Attributes Enum" :default "NewEnumerator13") (`Level Attribute` :type "/Game/Hyper/Core/Level_Manager/Datamodel/Enumerations/Enum_Skills Enum" :default "NewEnumerator29") (`Assigned Attributes` :type "/Game/Hyper/Core/Attribute_System/Datamodel/Attribute_Effects/Structures/Struct_Assigned_Attributes Structure"))
  (returns (Base :type "Float (double-precision)") (Added :type "Float (double-precision)") (Total :type "Float (double-precision)") (`Not Found` :type Boolean))
  (locals (`Local Found` :type Boolean))
  ;[0.05127 0.05127 0.05127] This function is used for returning the assinged atribute value of a specific assinged attirbute struct. So if you have a specific item, and want to return a specific attribute value, you can use this function
)

(fn `Get Variable Values of Attribute`
  (params (`Attribute Type` :type "/Game/Hyper/Core/Attribute_System/Datamodel/Attribute_Effects/Enumerations/Enum_Attribute_Types Enum" :default "NewEnumerator0") (`Primary Attribute` :type "/Game/Hyper/Core/Attribute_System/Datamodel/Attribute_Effects/Enumerations/Enum_Persistent_Character_Primary_Attributes Enum" :default "NewEnumerator38") (`Survival Attribute` :type "/Game/Hyper/Core/Attribute_System/Datamodel/Attribute_Effects/Enumerations/Enum_Persistent_Character_Survival_Attributes Enum" :default "NewEnumerator19") (`Combat Attribute` :type "/Game/Hyper/Core/Attribute_System/Datamodel/Attribute_Effects/Enumerations/Enum_Persistant_Generic_Combat_Attributes Enum" :default "NewEnumerator16") (`Ranged Attribute` :type "/Game/Hyper/Core/Attribute_System/Datamodel/Attribute_Effects/Enumerations/Enum_Persistant_RangedCombat_Attributes Enum" :default "NewEnumerator13") (`Level Attribute` :type "/Game/Hyper/Core/Level_Manager/Datamodel/Enumerations/Enum_Skills Enum" :default "NewEnumerator29") (`Non Persistent attributes` :type "/Game/Hyper/Core/Attribute_System/Datamodel/Attribute_Effects/Enumerations/Enum_Non-Persistent_Character_Attributes Enum" :default "NewEnumerator13"))
  (returns (Base :type "Float (double-precision)") (Added :type "Float (double-precision)") (Total :type "Float (double-precision)"))
  (locals (`Local Attribute Type Selection` :type "/Game/Hyper/Core/Attribute_System/Datamodel/Attribute_Effects/Enumerations/Enum_Attribute_Types Enum") (`Local Primary Attribute` :type "/Game/Hyper/Core/Attribute_System/Datamodel/Attribute_Effects/Enumerations/Enum_Persistent_Character_Primary_Attributes Enum") (`Local Survival Attribute` :type "/Game/Hyper/Core/Attribute_System/Datamodel/Attribute_Effects/Enumerations/Enum_Persistent_Character_Survival_Attributes Enum") (`Local Combat Attribute` :type "/Game/Hyper/Core/Attribute_System/Datamodel/Attribute_Effects/Enumerations/Enum_Persistant_Generic_Combat_Attributes Enum") (`Local Ranged Attribute` :type "/Game/Hyper/Core/Attribute_System/Datamodel/Attribute_Effects/Enumerations/Enum_Persistant_RangedCombat_Attributes Enum") (`Local Level Attrivute` :type "/Game/Hyper/Core/Level_Manager/Datamodel/Enumerations/Enum_Skills Enum") (`local non persistent attribute` :type "/Game/Hyper/Core/Attribute_System/Datamodel/Attribute_Effects/Enumerations/Enum_Non-Persistent_Character_Attributes Enum" :default "NewEnumerator13")))

(fn `health_playerstates_hud_values`
  (returns (CurrentHealth :type "Float (double-precision)") (MaxHealth :type "Float (double-precision)") (`Receive Damage` :type Boolean))
  (return 0.0 0.0 false))

(fn `Hydration_playerstates_hud_values`
  (returns (CurrentHydration :type "Float (double-precision)") (MaxHydration :type "Float (double-precision)"))
  (return 0.0 0.0))

(fn `Magic_playerstates_hud_values`
  (returns (`Current Magic` :type "Float (double-precision)") (`Maximum Magic` :type "Float (double-precision)"))
  (return 0.0 0.0))

(fn `OnRep_Current Health`
  (`self.OnRep_Current Health_Execution`))

(fn `OnRep_Current Health_Execution`)

(fn `OnRep_State Effects`
  (`self.OnRep_State Effects_Execution`))

(fn `OnRep_State Effects_Execution`)

(fn `oxygen_playerstates_hud_values`
  (returns (CurrentOxygen :type "Float (double-precision)") (MaxOxygen :type "Float (double-precision)") (`Consuming Oxygen` :type Boolean) (`Oxygen is max` :type Boolean))
  (return 0.0 0.0 false false))

(fn `Remove State Effect Object`
  (params (`State Effect` :type "/Game/Hyper/Core/Attribute_System/Datamodel/State_Effects/Enumerations/Enum_State_Effects Enum" :default "NewEnumerator0")))

(fn `Set Character Attribute State`
  (params (Attribute :type "/Game/Hyper/Core/Attribute_System/Datamodel/Attribute_Effects/Enumerations/Enum_Non-Persistent_Character_Attributes Enum" :default "NewEnumerator13") (`Is Zero` :type Boolean) (`Is In Low Range` :type Boolean) (`Is Max` :type Boolean)))

(fn `Set Generic Combat Attribute`
  (params (Attribute :type "/Game/Hyper/Core/Attribute_System/Datamodel/Attribute_Effects/Enumerations/Enum_Persistant_Generic_Combat_Attributes Enum" :default "NewEnumerator16") (Value :type "/Game/Hyper/Core/Attribute_System/Datamodel/Attribute_Effects/Structures/Struct_Float_Attribute Structure")))

(fn `Set Non- Persistent Character Attribute`
  (params (Attribute :type "/Game/Hyper/Core/Attribute_System/Datamodel/Attribute_Effects/Enumerations/Enum_Non-Persistent_Character_Attributes Enum" :default "NewEnumerator13") (Value :type "Float (double-precision)")))

(fn `Set Persistent Level Attribute`
  (params (Attribute :type "/Game/Hyper/Core/Level_Manager/Datamodel/Enumerations/Enum_Skills Enum" :default "NewEnumerator29") (Value :type Integer)))

(fn `Set Persistent Primary Character Attribute`
  (params (Attribute :type "/Game/Hyper/Core/Attribute_System/Datamodel/Attribute_Effects/Enumerations/Enum_Persistent_Character_Primary_Attributes Enum" :default "NewEnumerator38") (Value :type "/Game/Hyper/Core/Attribute_System/Datamodel/Attribute_Effects/Structures/Struct_Float_Attribute Structure")))

(fn `Set Persistent Survival Character Attribute`
  (params (Attribute :type "/Game/Hyper/Core/Attribute_System/Datamodel/Attribute_Effects/Enumerations/Enum_Persistent_Character_Survival_Attributes Enum" :default "NewEnumerator19") (Value :type "/Game/Hyper/Core/Attribute_System/Datamodel/Attribute_Effects/Structures/Struct_Float_Attribute Structure")))

(fn `Set Ranged Combat Attribute`
  (params (Attribute :type "/Game/Hyper/Core/Attribute_System/Datamodel/Attribute_Effects/Enumerations/Enum_Persistant_RangedCombat_Attributes Enum" :default "NewEnumerator13") (Value :type "/Game/Hyper/Core/Attribute_System/Datamodel/Attribute_Effects/Structures/Struct_Float_Attribute Structure")))

(fn `Weight_playerstates_hud_Values`
  (returns (`current weight` :type "Float (double-precision)") (`max weight` :type "Float (double-precision)")))