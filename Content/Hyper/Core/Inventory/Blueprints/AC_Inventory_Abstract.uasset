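; Abstract inventory component that declares the interface for item storage: adding, removing, moving, splitting, consuming, pickup, dropping and repair.
; Events and functions are almost all empty stubs or default returns, covering stack and slot handling, weight checks and durability.
; Inventory slot replication forwards its OnRep to an overridable execution function.
; Linked crafting, vendor, hotbar and allocator component getters report invalid by default.
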(event `Event: Transfer Item By TransferType`
  (params (TransferType :type "/Game/Hyper/Core/Inventory/Datamodel/Enumerations/Enum_Transfer_Types Enum" :default "NewEnumerator5") (`Inventory Item` :type "/Game/Hyper/Core/Inventory/Datamodel/Structures/Main_Item_Slot_Structs/Struct_Inventory_Slot_Item Structure") (`Custom amount` :type Integer) (`Source inventory component` :type "/Game/Hyper/Core/Inventory/Blueprints/AC_Inventory_Abstract Object Reference") (`Destination Inventory` :type "/Game/Hyper/Core/Inventory/Blueprints/AC_Inventory_Abstract Object Reference") (`Source Slot Index` :type Integer))
  ;[0 1 0.8906 1 113] Inventory Calls
  ;;[1 1 1 1 28] Transfer by type
)

(event `Event: Remove Item from inventory automaticly`
  (params (`Inventory Item to remove` :type "/Game/Hyper/Core/Inventory/Datamodel/Structures/Main_Item_Slot_Structs/Struct_Inventory_Slot_Item Structure") (`Amount to remove` :type Integer) (`Show Added Item Widget` :type Boolean))
  ;[0 1 0.8906 1 113] Inventory Calls
  ;;[1 1 1 1 28] Remove Item from inventory automaticly
)

(event `Event:Remove item at slot index`
  (params (`source inventory` :type "/Game/Hyper/Core/Inventory/Blueprints/AC_Inventory_Abstract Object Reference") (`Slot Index` :type Integer) (Amount :type Integer) (`Is equipment` :type Boolean) (`Item To Unequip` :type "/Game/Hyper/Core/Inventory/Datamodel/Structures/Main_Item_Slot_Structs/Struct_Inventory_Slot_Item Structure") (`Show Added Item Widget` :type Boolean))
  ;[0 1 0.8906 1 113] Inventory Calls
  ;;[1 1 1 1 28] Remove item at slot index
)

(event `Event: Try Transfer All to Destination Inventory`
  (params (`Source inventory` :type "/Game/Hyper/Core/Inventory/Blueprints/AC_Inventory_Abstract Object Reference") (`Destination Inventory` :type "/Game/Hyper/Core/Inventory/Blueprints/AC_Inventory_Abstract Object Reference"))
  ;[0 1 0.8906 1 113] Inventory Calls
  ;;[1 1 1 1 28] Try Transfer All to Destination Inventory
)

(event `Event: Split Inventory Stack by SplitType`
  (params (`Source inventory component` :type "/Game/Hyper/Core/Inventory/Blueprints/AC_Inventory_Abstract Object Reference") (`Split Type` :type "/Game/Hyper/Core/Inventory/Datamodel/Enumerations/Enum_split_types Enum" :default "NewEnumerator5") (`inventory item to be splitted` :type "/Game/Hyper/Core/Inventory/Datamodel/Structures/Main_Item_Slot_Structs/Struct_Inventory_Slot_Item Structure (by ref)") (`Custom Amount` :type Integer) (`Source Slot Index` :type Integer))
  ;[0 1 0.8906 1 113] Inventory Calls
  ;;[1 1 1 1 28] Splitting stacks
)

(event `Event: Move item to slot index`
  (params (`Inventory Item` :type "/Game/Hyper/Core/Inventory/Datamodel/Structures/Main_Item_Slot_Structs/Struct_Inventory_Slot_Item Structure (by ref)") (`Source inventory component` :type "/Game/Hyper/Core/Inventory/Blueprints/AC_Inventory_Abstract Object Reference (by ref)") (`Destination Inventory` :type "/Game/Hyper/Core/Inventory/Blueprints/AC_Inventory_Abstract Object Reference (by ref)") (`Source Slot Index` :type Integer) (`Destination Slot Index` :type Integer) (`Automatic placement` :type Boolean) (`Is from Equipment` :type Boolean))
  ;[0 1 0.8906 1 113] Inventory Calls
  ;;[1 1 1 1 28] Move
)

(event `Event: Try Add Item to inventory automatically`
  (params (`Inventory Item to be added` :type "/Game/Hyper/Core/Inventory/Datamodel/Structures/Main_Item_Slot_Structs/Struct_Inventory_Slot_Item Structure") (`Override Stack size` :type Boolean) (`Override max stack size` :type Integer) (`Override dynamic slot creation to true` :type Boolean) (`Use this function as check only` :type Boolean) (`Show Added Item Widget` :type Boolean))
  ;[0 1 0.8906 1 113] Inventory Calls
  ;;[1 1 1 1 28] Try Add Item to inventory automatically
)

(event `Event: Remove all empty slots from start index to end of array`
  (params (`Index to start removing` :type Integer) (TargetArray :type "Array of /Game/Hyper/Core/Inventory/Datamodel/Structures/Main_Item_Slot_Structs/Struct_Inventory_Slot_Item Structure (by ref)"))
  ;[0.3789 1 0 1 161] Utility
  ;;[1 1 1 1 28] Auto remove empty slots
)

(event `Event: Process Durability and decay logic by slot index for equipment`
  (params (`Slot Index` :type Integer))
  ;[0.3789 1 0 1 161] Utility
  ;;[1 1 1] Process durability and decay
)

(event `Event: Consume Item`
  (params (`Source inventory component` :type "/Game/Hyper/Core/Inventory/Blueprints/AC_Inventory_Abstract Object Reference") (`Inventory Item to consume` :type "/Game/Hyper/Core/Inventory/Datamodel/Structures/Main_Item_Slot_Structs/Struct_Inventory_Slot_Item Structure") (`Slot index` :type Integer) (`Target Array` :type "Array of /Game/Hyper/Core/Inventory/Datamodel/Structures/Main_Item_Slot_Structs/Struct_Inventory_Slot_Item Structure (by ref)") (`Is from hotbar` :type Boolean))
  ;[1 0.4981 0 1 123] Inventory Actions
  ;;[1 1 1 1 28] Consume
  ;;;[1 1 1] is possible to only replicate to owning client.
)

(event `Event owning client: Consume Item`
  (params (`Source inventory component` :type "/Game/Hyper/Core/Inventory/Blueprints/AC_Inventory_Abstract Object Reference") (`Inventory Item to consume` :type "/Game/Hyper/Core/Inventory/Datamodel/Structures/Main_Item_Slot_Structs/Struct_Inventory_Slot_Item Structure") (`Slot index` :type Integer) (`Target Array` :type "Array of /Game/Hyper/Core/Inventory/Datamodel/Structures/Main_Item_Slot_Structs/Struct_Inventory_Slot_Item Structure (by ref)") (`Is from hotbar` :type Boolean))
  ;[1 0.4981 0 1 123] Inventory Actions
  ;;[1 1 1 1 28] Consume
  ;;;[1 1 1] is possible to only replicate to owning client.
)

(event `Event: Pickup Item`
  (params (`inventory item` :type "/Game/Hyper/Core/Inventory/Datamodel/Structures/Main_Item_Slot_Structs/Struct_Inventory_Slot_Item Structure") (`Pickup BP interacting with` :type "/Game/Hyper/Core/Inventory/Blueprints/BP_Pickup_Abstract Object Reference"))
  ;[0.3789 1 0 1 161] Utility
  ;;[1 1 1] Pickup Item
)

(event `Event: Hotbar Update`
  (params (Item :type "/Game/Hyper/Core/Inventory/Datamodel/Structures/Main_Item_Slot_Structs/Struct_Inventory_Slot_Item Structure (by ref)"))
  ;[0.3789 1 0 1 161] Utility
  ;;[1 1 1] On call event, update the hotbar slot
)

(event `Event: Drop item by slot index`
  (params (`Slot Index` :type Integer) (Amount :type Integer) (`Inventory Item` :type "/Game/Hyper/Core/Inventory/Datamodel/Structures/Main_Item_Slot_Structs/Struct_Inventory_Slot_Item Structure"))
  ;[0.3789 1 0 1 161] Utility
  ;;[1 1 1 1 28] Dropping and spwaning
)

(event `Event: Destroy actor`
  (params (Target :type "Actor Object Reference"))
  ;[0.3789 1 0 1 161] Utility
  ;;[1 1 1 1 28] Destroy Actor
)

(event `Event: Destroy Pickup Actor`
  (params (Target :type "/Game/Hyper/Core/Inventory/Blueprints/BP_Pickup_Abstract Object Reference"))
  ;[0.3789 1 0 1 161] Utility
  ;;[1 1 1 1 28] Destroy Pickup actor
)

(event `Event: Try Repair Item by slot index`
  (params (`Slot Index` :type Integer) (`source inventory` :type "/Game/Hyper/Core/Inventory/Blueprints/AC_Inventory_Abstract Object Reference (by ref)") (`Target Array` :type "Array of /Game/Hyper/Core/Inventory/Datamodel/Structures/Main_Item_Slot_Structs/Struct_Inventory_Slot_Item Structure (by ref)"))
  ;[1 0.4981 0 1 123] Inventory Actions
  ;;[1 1 1 1 28] Repair
)

(event `Event: Server Spawn Item`
  (params (`Spawn Transform Location` :type "Transform Structure") (`Inventory Item` :type "/Game/Hyper/Core/Inventory/Datamodel/Structures/Main_Item_Slot_Structs/Struct_Inventory_Slot_Item Structure") (`Override Simulate Physics?` :type Boolean) (`Simulate Physics?` :type Boolean))
  ;[0.3789 1 0 1 161] Utility
  ;;[1 1 1 1 28] Dropping and spwaning
)

(event `Client: Reinitialize`)

(event `Add Or Remove Widget`
  (params (Widget :type "UserWidget Object Reference") (`Player Controller` :type "PlayerController Object Reference")))

(fn `Array Contains Item`
  (params (Array :type "Array of /Game/Hyper/Core/Inventory/Datamodel/Structures/Main_Item_Slot_Structs/Struct_Inventory_Slot_Item Structure") (`Item to find` :type "/Game/Hyper/Core/Inventory/Datamodel/Structures/Main_Item_Slot_Structs/Struct_Inventory_Slot_Item Structure"))
  (returns (`Item Found in array` :type Boolean))
  (locals (`local Item Found in array` :type Boolean :default false)))

(fn `Can all items be added`
  (params (`Items to add` :type "Array of /Game/Hyper/Core/Inventory/Datamodel/Structures/Main_Item_Slot_Structs/Struct_Inventory_Slot_Item Structure") (`Use Multiplier` :type Boolean) (`Amount Multiplier` :type Integer))
  (returns (`All items can be added` :type Boolean))
  (locals (`Local All items can be added` :type Boolean :default true) (`local Total Empty slots filled` :type Integer :default 0)))

(fn `Can item be added due to weight?`
  (params (item :type "/Game/Hyper/Core/Inventory/Datamodel/Structures/Main_Item_Slot_Structs/Struct_Inventory_Slot_Item Structure"))
  (returns (`All items can be added` :type Boolean) (`Amount that can be added` :type Integer) (`Amount that can not be added` :type Integer))
  (locals (`local weight to be added` :type "Float (double-precision)" :default 0.0) (`local amount of item that can be added due to weight` :type Integer :default 0)))

(fn `check if inventory item is equal`
  (params (`Struct_Inventory_Item 1` :type "/Game/Hyper/Core/Inventory/Datamodel/Structures/Main_Item_Slot_Structs/Struct_Inventory_Slot_Item Structure (by ref)") (`Struct_Inventory_Item 2` :type "/Game/Hyper/Core/Inventory/Datamodel/Structures/Main_Item_Slot_Structs/Struct_Inventory_Slot_Item Structure (by ref)"))
  (returns (True :type Boolean)))

(fn `Create Empty slot`
  (params (TargetArray :type "Array of /Game/Hyper/Core/Inventory/Datamodel/Structures/Main_Item_Slot_Structs/Struct_Inventory_Slot_Item Structure (by ref)"))
  (returns (`New slot index` :type Integer)))

(fn `Find Empty Slot`
  (params (Array :type "Array of /Game/Hyper/Core/Inventory/Datamodel/Structures/Main_Item_Slot_Structs/Struct_Inventory_Slot_Item Structure") (`Start Index` :type Integer))
  (returns (`Slot Index` :type Integer) (Success :type Boolean))
  (locals (`local Found Empty slot` :type Boolean :default false) (`local slot index of empty slot` :type Integer)))

(fn `Find Existing Slot Indexes Of Specified Inventory Item`
  (params (`Inventory Item` :type "/Game/Hyper/Core/Inventory/Datamodel/Structures/Main_Item_Slot_Structs/Struct_Inventory_Slot_Item Structure") (`Target Array` :type "Array of /Game/Hyper/Core/Inventory/Datamodel/Structures/Main_Item_Slot_Structs/Struct_Inventory_Slot_Item Structure"))
  (returns (`Slots found at indexes` :type "Array of Integer") (Succes :type Boolean))
  (locals (`Found Indexes` :type "Array of Integer")))

(fn `Get Inventory Item info`
  (params (`inventory item` :type "/Game/Hyper/Core/Inventory/Datamodel/Structures/Main_Item_Slot_Structs/Struct_Inventory_Slot_Item Structure (by ref)") (`Override Stack Size` :type Boolean) (`New Stack Size` :type Integer))
  (returns (Item :type "/Game/Hyper/Core/Inventory/Datamodel/Structures/Main_Item_Slot_Structs/Struct_Item Structure") (Stackable :type Boolean) (`Max stack size` :type Integer) (`Amount in slot` :type Integer) (`Room in slot` :type Integer))
  (return (struct) false 0 0 0))

(fn `Get Linked Allocator Component`
  (returns (`Allocator Component` :type "/Game/Hyper/Core/ItemAllocator/Blueprints/AC_Item_Allocator_Abstract Object Reference") (`Is Valid` :type Boolean))
  (return null false))

(fn `Get Linked Crafting Component`
  (returns (`Crafting Component` :type "/Game/Hyper/Core/Crafting/Blueprints/AC_Crafting_Abstract Object Reference") (`Is Valid` :type Boolean))
  (return null false))

(fn `Get Linked Hotbar Component`
  (returns (`Hotbar Component` :type "/Game/Hyper/Core/Inventory/Blueprints/AC_Hotbar_Abstract Object Reference") (`Is Valid` :type Boolean))
  (return null false))

(fn `Get Linked Vendor Component`
  (returns (`Vendor Component` :type "/Game/Hyper/Core/Vendor/Blueprints/AC_Vendor_Abstract Object Reference") (`Is Valid` :type Boolean))
  (return null false))

(fn `Get slot info by index`
  (params (Array :type "Array of /Game/Hyper/Core/Inventory/Datamodel/Structures/Main_Item_Slot_Structs/Struct_Inventory_Slot_Item Structure") (`Slot index` :type Integer) (`Override stack size` :type Boolean) (`New stack size` :type Integer))
  (returns (`Inventory Item data (slot)` :type "/Game/Hyper/Core/Inventory/Datamodel/Structures/Main_Item_Slot_Structs/Struct_Inventory_Slot_Item Structure (by ref)") (`Item data` :type "/Game/Hyper/Core/Inventory/Datamodel/Structures/Main_Item_Slot_Structs/Struct_Item Structure") (Stackable :type Boolean) (`Max stack size` :type Integer) (`Current Amount` :type Integer) (`Room in stack` :type Integer) (`Stack is full` :type Boolean)))

(fn `How many of item in inventory`
  (params (`Inventory Item` :type "/Game/Hyper/Core/Inventory/Datamodel/Structures/Main_Item_Slot_Structs/Struct_Inventory_Slot_Item Structure") (Array :type "Array of /Game/Hyper/Core/Inventory/Datamodel/Structures/Main_Item_Slot_Structs/Struct_Inventory_Slot_Item Structure (by ref)"))
  (returns (`amount of items found` :type Integer) (`of item` :type "/Game/Hyper/Core/Inventory/Datamodel/Structures/Main_Item_Slot_Structs/Struct_Inventory_Slot_Item Structure"))
  (locals (`local items found ` :type Integer :default 0)))

(fn `How many stacks should be created`
  (params (`inventory item` :type "/Game/Hyper/Core/Inventory/Datamodel/Structures/Main_Item_Slot_Structs/Struct_Inventory_Slot_Item Structure (by ref)") (`Amount to add` :type Integer) (`Override Stack Size` :type Boolean) (`New Stack Size` :type Integer))
  (returns (`amount of new stacks required` :type Integer)))

(fn `Move Item to slot index`
  (params (`Inventory Item` :type "/Game/Hyper/Core/Inventory/Datamodel/Structures/Main_Item_Slot_Structs/Struct_Inventory_Slot_Item Structure") (`Source inventory component` :type "/Game/Hyper/Core/Inventory/Blueprints/AC_Inventory_Abstract Object Reference") (`Destination Inventory` :type "/Game/Hyper/Core/Inventory/Blueprints/AC_Inventory_Abstract Object Reference") (`Source Slot Index` :type Integer) (`Destination Slot Index` :type Integer) (`Source Array` :type "Array of /Game/Hyper/Core/Inventory/Datamodel/Structures/Main_Item_Slot_Structs/Struct_Inventory_Slot_Item Structure (by ref)") (`Destination Array` :type "Array of /Game/Hyper/Core/Inventory/Datamodel/Structures/Main_Item_Slot_Structs/Struct_Inventory_Slot_Item Structure (by ref)") (`Automatic placement` :type Boolean) (`Is from equipment` :type Boolean))
  (returns (`All items added` :type Boolean))
  (locals (`local inventory item to be moved` :type "/Game/Hyper/Core/Inventory/Datamodel/Structures/Main_Item_Slot_Structs/Struct_Inventory_Slot_Item Structure" :default (struct :`Item` (struct :`DataTable` "/Script/Engine.DataTable'/Game/Hyper/Core/Inventory/Datamodel/Datatables/DT_Items.DT_Items'" :`RowName` "Empty") :`Amount` 1 :`Durabilitydetails` (struct) :`TradingandLootdetails` (struct :`Chanceofspawinginvendorinventory` 1.0 :`MinimalAmounttorestock` 1 :`MaximumAmounttorestock` 5 :`MaximumStock` 10) :`HotbarDetails` (struct) :`EquipmentSlot` (struct :`Linkedtothisequipmentslot` "NewEnumerator13" :`AmmoSlot` (struct :`AmmoDataTable` (struct :`DataTable` "/Script/Engine.DataTable'/Game/Hyper/Core/Equipment_Manager/Datamodel/Datatables/DT_Ammo.DT_Ammo'"))))) (`local destination inventory comp` :type "/Game/Hyper/Core/Inventory/Blueprints/AC_Inventory_Abstract Object Reference") (`local source slot index` :type Integer) (`local destination slot index` :type Integer) (`local source item` :type "/Game/Hyper/Core/Inventory/Datamodel/Structures/Main_Item_Slot_Structs/Struct_Inventory_Slot_Item Structure" :default (struct :`Item` (struct :`DataTable` "/Script/Engine.DataTable'/Game/Hyper/Core/Inventory/Datamodel/Datatables/DT_Items.DT_Items'" :`RowName` "Empty") :`Amount` 1 :`Durabilitydetails` (struct :`CurrentDurability` 100.0 :`IsUseable` true) :`TradingandLootdetails` (struct :`Chanceofspawinginvendorinventory` 1.0 :`MinimalAmounttorestock` 1 :`MaximumAmounttorestock` 5 :`MaximumStock` 10) :`HotbarDetails` (struct) :`EquipmentSlot` (struct :`Linkedtothisequipmentslot` "NewEnumerator13" :`AmmoSlot` (struct :`AmmoDataTable` (struct :`DataTable` "/Script/Engine.DataTable'/Game/Hyper/Core/Equipment_Manager/Datamodel/Datatables/DT_Ammo.DT_Ammo'"))))) (`local destination item` :type "/Game/Hyper/Core/Inventory/Datamodel/Structures/Main_Item_Slot_Structs/Struct_Inventory_Slot_Item Structure" :default (struct :`Item` (struct :`DataTable` "/Script/Engine.DataTable'/Game/Hyper/Core/Inventory/Datamodel/Datatables/DT_Items.DT_Items'" :`RowName` "Empty") :`Amount` 1 :`Durabilitydetails` (struct :`CurrentDurability` 100.0 :`IsUseable` true) :`TradingandLootdetails` (struct :`Chanceofspawinginvendorinventory` 1.0 :`MinimalAmounttorestock` 1 :`MaximumAmounttorestock` 5 :`MaximumStock` 10) :`HotbarDetails` (struct) :`EquipmentSlot` (struct :`Linkedtothisequipmentslot` "NewEnumerator13" :`AmmoSlot` (struct :`AmmoDataTable` (struct :`DataTable` "/Script/Engine.DataTable'/Game/Hyper/Core/Equipment_Manager/Datamodel/Datatables/DT_Ammo.DT_Ammo'"))))) (`local is an equipment move` :type Boolean) (`local source inventory component` :type "/Game/Hyper/Core/Inventory/Blueprints/AC_Inventory_Abstract Object Reference") (`Local Source Array` :type "Array of /Game/Hyper/Core/Inventory/Datamodel/Structures/Main_Item_Slot_Structs/Struct_Inventory_Slot_Item Structure") (`Local Destination Array` :type "Array of /Game/Hyper/Core/Inventory/Datamodel/Structures/Main_Item_Slot_Structs/Struct_Inventory_Slot_Item Structure") (`Local Is Automatic Placement` :type Boolean) (`Local to which equipment slot should this item to be added` :type "/Game/Hyper/Core/Equipment_Manager/Datamodel/Enumerations/Enum_Equipment_Slots Enum" :default "NewEnumerator13") (`Local Destination slot info` :type "/Game/Hyper/Core/Inventory/Datamodel/Structures/Main_Item_Slot_Structs/Struct_Inventory_Slot_Item Structure" :default (struct :`Item` (struct :`DataTable` "/Script/Engine.DataTable'/Game/Hyper/Core/Inventory/Datamodel/Datatables/DT_Items.DT_Items'" :`RowName` "Empty") :`Amount` 1 :`Durabilitydetails` (struct :`CurrentDurability` 100.0 :`IsUseable` true) :`TradingandLootdetails` (struct :`Chanceofspawinginvendorinventory` 1.0 :`MinimalAmounttorestock` 1 :`MaximumAmounttorestock` 5 :`MaximumStock` 10) :`ShouldAddXPwhenpickedup` true :`HotbarDetails` (struct) :`EquipmentSlot` (struct :`Linkedtothisequipmentslot` "NewEnumerator13" :`AmmoSlot` (struct :`AmmoDataTable` (struct :`DataTable` "/Script/Engine.DataTable'/Game/Hyper/Core/Equipment_Manager/Datamodel/Datatables/DT_Ammo.DT_Ammo'")))))))

(fn `OnRep_Inventory Slots`
  (`self.OnRep_Inventory Slots_Excecution`))

(fn `OnRep_Inventory Slots_Excecution`)

(fn `Remove item at slot index`
  (params (`Slot Index` :type Integer) (`Amount To Remove` :type Integer) (`Target Array` :type "Array of /Game/Hyper/Core/Inventory/Datamodel/Structures/Main_Item_Slot_Structs/Struct_Inventory_Slot_Item Structure") (`To Be Removed Item Is Equipped` :type Boolean) (`Show Added Item Widget` :type Boolean))
  (returns (Success :type Boolean) (`Empty slot` :type Boolean))
  (locals (`Local inventory slot item` :type "/Game/Hyper/Core/Inventory/Datamodel/Structures/Main_Item_Slot_Structs/Struct_Inventory_Slot_Item Structure" :default (struct :`Item` (struct :`DataTable` "/Script/Engine.DataTable'/Game/Hyper/Core/Inventory/Datamodel/Datatables/DT_Items.DT_Items'" :`RowName` "Empty") :`Amount` 1 :`Durabilitydetails` (struct) :`TradingandLootdetails` (struct :`Chanceofspawinginvendorinventory` 1.0 :`MinimalAmounttorestock` 1 :`MaximumAmounttorestock` 5 :`MaximumStock` 10) :`HotbarDetails` (struct) :`EquipmentSlot` (struct :`Linkedtothisequipmentslot` "NewEnumerator13" :`AmmoSlot` (struct :`AmmoDataTable` (struct :`DataTable` "/Script/Engine.DataTable'/Game/Hyper/Core/Equipment_Manager/Datamodel/Datatables/DT_Ammo.DT_Ammo'"))))) (`Local amount to remove` :type Integer) (`local slot index` :type Integer)))

(fn `Remove Item From Inventory Automatically`
  (params (`Inventory Item to remove` :type "/Game/Hyper/Core/Inventory/Datamodel/Structures/Main_Item_Slot_Structs/Struct_Inventory_Slot_Item Structure") (`Amount to remove` :type Integer) (`Target Array` :type "Array of /Game/Hyper/Core/Inventory/Datamodel/Structures/Main_Item_Slot_Structs/Struct_Inventory_Slot_Item Structure (by ref)") (`Show Added Item Widget` :type Boolean))
  (returns (Success :type Boolean) (`amount not removed` :type Integer))
  (locals (`local Amount to remove` :type Integer) (`local current amount in slot` :type Integer) (`local remainder to be removed` :type Integer :default 0) (`local found slot index` :type Integer) (`local existing slot found` :type "DataTableRowHandle Structure" :default (struct)) (`local amount removed` :type Integer)))

(fn `Set Inventory Slot to empty by index`
  (params (TargetArray :type "Array of /Game/Hyper/Core/Inventory/Datamodel/Structures/Main_Item_Slot_Structs/Struct_Inventory_Slot_Item Structure (by ref)") (Index :type Integer)))

(fn `Swap Item`
  (params (`Source Array` :type "Array of /Game/Hyper/Core/Inventory/Datamodel/Structures/Main_Item_Slot_Structs/Struct_Inventory_Slot_Item Structure") (`Destination Array` :type "Array of /Game/Hyper/Core/Inventory/Datamodel/Structures/Main_Item_Slot_Structs/Struct_Inventory_Slot_Item Structure") (`Source index` :type Integer) (`Destination Index` :type Integer) (`Source Inventory Component` :type "/Game/Hyper/Core/Inventory/Blueprints/AC_Inventory_Abstract Object Reference") (`Destination Inventory Component` :type "/Game/Hyper/Core/Inventory/Blueprints/AC_Inventory_Abstract Object Reference"))
  (returns (`Swap peformed` :type Boolean))
  (locals (`local source item` :type "/Game/Hyper/Core/Inventory/Datamodel/Structures/Main_Item_Slot_Structs/Struct_Inventory_Slot_Item Structure" :default (struct :`Item` (struct :`DataTable` "/Script/Engine.DataTable'/Game/Hyper/Core/Inventory/Datamodel/Datatables/DT_Items.DT_Items'" :`RowName` "Empty") :`Amount` 1 :`Durabilitydetails` (struct :`CurrentDurability` 100.0 :`IsUseable` true) :`TradingandLootdetails` (struct :`Chanceofspawinginvendorinventory` 1.0 :`MinimalAmounttorestock` 1 :`MaximumAmounttorestock` 5 :`MaximumStock` 10) :`HotbarDetails` (struct) :`EquipmentSlot` (struct :`Linkedtothisequipmentslot` "NewEnumerator13" :`AmmoSlot` (struct :`AmmoDataTable` (struct :`DataTable` "/Script/Engine.DataTable'/Game/Hyper/Core/Equipment_Manager/Datamodel/Datatables/DT_Ammo.DT_Ammo'"))))) (`local destination item` :type "/Game/Hyper/Core/Inventory/Datamodel/Structures/Main_Item_Slot_Structs/Struct_Inventory_Slot_Item Structure" :default (struct :`Item` (struct :`DataTable` "/Script/Engine.DataTable'/Game/Hyper/Core/Inventory/Datamodel/Datatables/DT_Items.DT_Items'" :`RowName` "Empty") :`Amount` 1 :`Durabilitydetails` (struct :`CurrentDurability` 100.0 :`IsUseable` true) :`TradingandLootdetails` (struct :`Chanceofspawinginvendorinventory` 1.0 :`MinimalAmounttorestock` 1 :`MaximumAmounttorestock` 5 :`MaximumStock` 10) :`HotbarDetails` (struct) :`EquipmentSlot` (struct :`Linkedtothisequipmentslot` "NewEnumerator13" :`AmmoSlot` (struct :`AmmoDataTable` (struct :`DataTable` "/Script/Engine.DataTable'/Game/Hyper/Core/Equipment_Manager/Datamodel/Datatables/DT_Ammo.DT_Ammo'"))))) (`local source index` :type Integer) (`local destination index` :type Integer) (`local is swapping equipment` :type Boolean)))

(fn `Try Add Item to Inventory Automatically`
  (params (`Inventory Item to be added` :type "/Game/Hyper/Core/Inventory/Datamodel/Structures/Main_Item_Slot_Structs/Struct_Inventory_Slot_Item Structure") (`Target Array` :type "Array of /Game/Hyper/Core/Inventory/Datamodel/Structures/Main_Item_Slot_Structs/Struct_Inventory_Slot_Item Structure (by ref)") (`Override Stack size` :type Boolean) (`Override max stack size` :type Integer) (`Override dynamic slot creation to true` :type Boolean) (`Use this function as check only` :type Boolean) (`Show Added Item Widget` :type Boolean))
  (returns (`All items added` :type Boolean) (`Amount not added` :type Integer) (`Empty slots filled` :type Integer))
  (locals (`local amount that could not be added into existing stacks` :type Integer :default 0) (`Local inventory item to be added` :type "/Game/Hyper/Core/Inventory/Datamodel/Structures/Main_Item_Slot_Structs/Struct_Inventory_Slot_Item Structure" :default (struct :`Item` (struct :`DataTable` "/Script/Engine.DataTable'/Game/Hyper/Core/Inventory/Datamodel/Datatables/DT_Items.DT_Items'" :`RowName` "Empty") :`Amount` 1 :`Durabilitydetails` (struct) :`TradingandLootdetails` (struct :`Chanceofspawinginvendorinventory` 1.0 :`MinimalAmounttorestock` 1 :`MaximumAmounttorestock` 5 :`MaximumStock` 10) :`HotbarDetails` (struct) :`EquipmentSlot` (struct :`Linkedtothisequipmentslot` "NewEnumerator13" :`AmmoSlot` (struct :`AmmoDataTable` (struct :`DataTable` "/Script/Engine.DataTable'/Game/Hyper/Core/Equipment_Manager/Datamodel/Datatables/DT_Ammo.DT_Ammo'"))))) (`local already added into new stack in other loop` :type Integer :default 0) (`Number of loops required` :type Integer :default 0) (`local amount that could not be added due to weight` :type Integer :default 0)))

(fn `Try Add Items To Empty And New Slots Automatically`
  (params (`inventory item to be added` :type "/Game/Hyper/Core/Inventory/Datamodel/Structures/Main_Item_Slot_Structs/Struct_Inventory_Slot_Item Structure") (`Amount to add` :type Integer) (`Target Array` :type "Array of /Game/Hyper/Core/Inventory/Datamodel/Structures/Main_Item_Slot_Structs/Struct_Inventory_Slot_Item Structure (by ref)") (`Override Stack Size` :type Boolean) (`New Stack Size` :type Integer) (`Override dynamic slot creation` :type Boolean) (`Use this function as check only` :type Boolean))
  (returns (`All items added` :type Boolean) (`Amount not added` :type Integer) (`Empty slots filled` :type Integer))
  (locals (`local amount to add` :type Integer) (`Local inventory item to be added` :type "/Game/Hyper/Core/Inventory/Datamodel/Structures/Main_Item_Slot_Structs/Struct_Inventory_Slot_Item Structure" :default (struct :`Item` (struct :`DataTable` "/Script/Engine.DataTable'/Game/Hyper/Core/Inventory/Datamodel/Datatables/DT_Items.DT_Items'" :`RowName` "Empty") :`Amount` 1 :`Durabilitydetails` (struct) :`TradingandLootdetails` (struct :`Chanceofspawinginvendorinventory` 1.0 :`MinimalAmounttorestock` 1 :`MaximumAmounttorestock` 5 :`MaximumStock` 10) :`HotbarDetails` (struct) :`EquipmentSlot` (struct :`Linkedtothisequipmentslot` "NewEnumerator13" :`AmmoSlot` (struct :`AmmoDataTable` (struct :`DataTable` "/Script/Engine.DataTable'/Game/Hyper/Core/Equipment_Manager/Datamodel/Datatables/DT_Ammo.DT_Ammo'"))))) (`local amount added into empty stacks` :type Integer)))

(fn `Try Add Items to Existing Stacks Automatically`
  (params (`Inventory Item` :type "/Game/Hyper/Core/Inventory/Datamodel/Structures/Main_Item_Slot_Structs/Struct_Inventory_Slot_Item Structure") (`Target Array` :type "Array of /Game/Hyper/Core/Inventory/Datamodel/Structures/Main_Item_Slot_Structs/Struct_Inventory_Slot_Item Structure (by ref)") (`Override Stack size` :type Boolean) (`Override max stack size` :type Integer) (`Use this function as check only` :type Boolean))
  (returns (`No existing stacks found` :type Boolean) (`All Items added` :type Boolean) (`Amount that could not be added into existing stacks` :type Integer))
  (locals (`local inventory item` :type "/Game/Hyper/Core/Inventory/Datamodel/Structures/Main_Item_Slot_Structs/Struct_Inventory_Slot_Item Structure" :default (struct :`Item` (struct :`DataTable` "/Script/Engine.DataTable'/Game/Hyper/Core/Inventory/Datamodel/Datatables/DT_Items.DT_Items'" :`RowName` "Empty") :`Amount` 1 :`Durabilitydetails` (struct) :`TradingandLootdetails` (struct :`Chanceofspawinginvendorinventory` 1.0 :`MinimalAmounttorestock` 1 :`MaximumAmounttorestock` 5 :`MaximumStock` 10) :`HotbarDetails` (struct) :`EquipmentSlot` (struct :`Linkedtothisequipmentslot` "NewEnumerator13" :`AmmoSlot` (struct :`AmmoDataTable` (struct :`DataTable` "/Script/Engine.DataTable'/Game/Hyper/Core/Equipment_Manager/Datamodel/Datatables/DT_Ammo.DT_Ammo'"))))) (`Local Amount previously added` :type Integer)))

(fn `Try Add items to stack`
  (params (Struct_Inventory_Item :type "/Game/Hyper/Core/Inventory/Datamodel/Structures/Main_Item_Slot_Structs/Struct_Inventory_Slot_Item Structure") (`Slot Index` :type Integer) (`Amount to be added` :type Integer) (`Amount in slot` :type Integer) (`Room in slot` :type Integer) (TargetArray :type "Array of /Game/Hyper/Core/Inventory/Datamodel/Structures/Main_Item_Slot_Structs/Struct_Inventory_Slot_Item Structure (by ref)") (`Use this function as check only` :type Boolean))
  (returns (`Amount added` :type Integer) (`All items added` :type Boolean) (`Amount left to be added` :type Integer)))

(fn `Try Move Item Automatically`
  (params (`Destination Inventory` :type "/Game/Hyper/Core/Inventory/Blueprints/AC_Inventory_Abstract Object Reference") (`Inventory Item To Be Moved` :type "/Game/Hyper/Core/Inventory/Datamodel/Structures/Main_Item_Slot_Structs/Struct_Inventory_Slot_Item Structure") (`Source Inventory` :type "/Game/Hyper/Core/Inventory/Blueprints/AC_Inventory_Abstract Object Reference"))
  (returns (Success :type Boolean)))

(fn `Try Process item to existing stack`
  (params (`Slot Index` :type Integer) (`Item to add` :type "/Game/Hyper/Core/Inventory/Datamodel/Structures/Main_Item_Slot_Structs/Struct_Inventory_Slot_Item Structure") (`correction of amount previously added` :type Integer) (Array :type "Array of /Game/Hyper/Core/Inventory/Datamodel/Structures/Main_Item_Slot_Structs/Struct_Inventory_Slot_Item Structure (by ref)") (`Override Stack size` :type Boolean) (`Override max stack size` :type Integer) (`Use this function as check only` :type Boolean))
  (returns (`amount added` :type Integer) (Success :type Boolean))
  (locals (`local amount added` :type Integer) (`local slot index` :type Integer) (`local item to add` :type "/Game/Hyper/Core/Inventory/Datamodel/Structures/Main_Item_Slot_Structs/Struct_Inventory_Slot_Item Structure" :default (struct :`Item` (struct :`DataTable` "/Script/Engine.DataTable'/Game/Hyper/Core/Inventory/Datamodel/Datatables/DT_Items.DT_Items'" :`RowName` "Empty") :`Amount` 1 :`Durabilitydetails` (struct) :`TradingandLootdetails` (struct :`Chanceofspawinginvendorinventory` 1.0 :`MinimalAmounttorestock` 1 :`MaximumAmounttorestock` 5 :`MaximumStock` 10) :`HotbarDetails` (struct) :`EquipmentSlot` (struct :`Linkedtothisequipmentslot` "NewEnumerator13" :`AmmoSlot` (struct :`AmmoDataTable` (struct :`DataTable` "/Script/Engine.DataTable'/Game/Hyper/Core/Equipment_Manager/Datamodel/Datatables/DT_Ammo.DT_Ammo'"))))) (`local current amount in slot` :type Integer :default 0) (`local max stack size` :type Integer :default 0) (`local amount to be added` :type Integer) (`Local Room in stack` :type Integer :default 0) (`local override Stack size` :type Boolean) (`local override max stack size` :type Integer :default 0)))

(fn `Whole array of items can be found in inventory?`
  (params (Array :type "Array of /Game/Hyper/Core/Inventory/Datamodel/Structures/Main_Item_Slot_Structs/Struct_Inventory_Slot_Item Structure"))
  (returns (`Sufficient items found` :type Boolean))
  (locals (`Sufficient items` :type Boolean :default true)))