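; Abstract base for farmable plant actors in the farming system, declaring an overridable API for growth stages, decay, water and fertilizer, seasons, quality, harvest and saving.
; Nearly all gameplay functions and events are empty stubs or return fixed defaults.
; OnRep handlers forward to separate execution functions, letting children supply replication responses.
; Implemented logic covers lazy GUID creation, linked pluckable yield cleanup and server-controlled interaction gated by CanBeHarvested.
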(event `Remove Active sprinkler`
  (params (Sprinkler :type "Actor Object Reference")))

(event `Add Active sprinkler`
  (params (Sprinkler :type "Actor Object Reference")))

(event `Event: Initialize Plant`)

(event `Event: pause Growth`)

(event `Event: Unpause Growth`)

(event `Event: Initiliaze Growing Timer`)

(event `TimerEvent: Grow`)

(event `Event: stop decay`)

(event `Event: Unpause decay`)

(event `Event: Initialize Decay Timer`)

(event `Event: Switch Plant Sickness`
  (params (Sick :type Boolean)))

(fn `Calculate_Crop_Quality`
  (returns (Quality :type "/Game/Hyper/Core/FarmingSystem/Datamodel/Enumerations/Enum_Crop_Quality Enum") (`Quality Factor` :type "Float (double-precision)")))

(fn `Calculate_Percentage_Of_Growing_Process_With_Fertilizer`
  (returns (Percentage :type "Float (double-precision)")))

(fn `Can Interact`
  (params (`Owning Controller` :type "Controller Object Reference"))
  (returns (True :type Boolean))
  (return (`self.Can_Be_Harvested`)))

(fn `Check and set if is watered via sprinkler`
  (returns (`Is Watered By Sprinkler` :type Boolean))
  (return false))

(fn `Check_If_Is_In_Growing_Season`
  (returns (In_Correct_Season :type Boolean)))

(fn `Check_If_should_decay_In_Season`
  (returns (Should_Decay :type Boolean))
  (return false))

(fn `Check_Tilled_Soil`
  (returns (Tilled_Soil_Present :type Boolean))
  (return true))

(fn `Check_UV`
  (returns (UV_Present :type Boolean)))

(fn `Deal and process damage`
  (params (Damage :type "Float (double-precision)"))
  (returns (`has zero durability` :type Boolean)))

(fn `Destroy_Connected_Yield`
  (bind _linked_pluckable_yield (`self.Linked_Pluckable_Yield`))
  ;[1 1 1] destroy all connected meshes
  (if (`KismetArrayLibrary.Array_IsValidIndex` _linked_pluckable_yield)
    (for _array_element _linked_pluckable_yield
      (`self.K2_DestroyActor` _array_element))
    ;;[1 1 1] Clear the arrays
    (`KismetArrayLibrary.Array_Clear` (`self.Linked_Pluckable_Yield`))
    (`KismetArrayLibrary.Array_Clear` (`self.Linked_Pluckable_Yield_GUIDS`))))

(fn `Does_Plant_Meet_Requirements_To_Grow`
  (returns (`Requirements Met` :type Boolean))
  (locals (`Consumed Oxygen` :type Boolean :default false) (`Consumed Fertilizer` :type Boolean :default false) (`Consumed Water` :type Boolean :default false)))

(fn `Get Interact Animation`
  (params (`Owning Controller` :type "Controller Object Reference"))
  (returns (`Anim Montage` :type "AnimMontage Object Reference"))
  (return (`/Game/Hyper/Core/Interaction/FunctionLibraries/BFL_Interaction.Select Interaction Animation` `Owning Controller` (`self.Interact Anim Montage Left`) (`self.Interact Anim Montage Right`))))

(fn `Get Interact Sound`
  (returns (`Interact Sound` :type "SoundBase Object Reference"))
  (return (`self.Interact Sound`)))

(fn `Get Interact Text`
  (params (`Owning Controller` :type "PlayerController Object Reference"))
  (returns (`Interact Text` :type Text) (`Secondary Interact Text` :type Text))
  (return (`|FormatText` "{Interact Text} {ItemName}" (`self.Interact Text`) (`.Name_2_3DE19FA64157CA393A5581947AAA309E` (break `/Game/Hyper/Core/FarmingSystem/Datamodel/Structures/Substructs/Struct_PlantAttributes_Generic` (`.Generic_82_923D547C4DB182B1CF7DC4917D8485DA` (break `/Game/Hyper/Core/FarmingSystem/Datamodel/Structures/Struct_Plant` (`self.Struct_Plant`)))))) ""))

(fn `Get Relative Interact Text Location`
  (returns (`Relative Location` :type "Vector Structure"))
  (return (`self.Relative Location`)))

(fn `Get_Buildable_Actor`
  (returns (Actor :type "/Game/Hyper/Core/BuildingSystem/Blueprints/BP_Buildable_Abstract Object Reference"))
  (return null))

(fn `Get_Current_Season`
  (returns (Season :type "/Game/Hyper/Core/FarmingSystem/Datamodel/Enumerations/Enum_Seasons Enum"))
  (return "NewEnumerator0"))

(fn `Get_Guid_Farmable`
  (returns (Output_Get :type String))
  ;[1 1 1] Stores the GUID if GUID is empty
  (if (not (`KismetStringLibrary.IsEmpty` (`self.GUID_Farmable`)))
    (return (`self.GUID_Farmable`))
    (else
      (bind _output_get (set `self.GUID_Farmable` (`KismetGuidLibrary.Conv_GuidToString` (`KismetGuidLibrary.NewGuid`))))
      (return _output_get))))

(fn `Get_Relative_Widget_Position`
  (returns (`Relactive Location` :type "Vector Structure"))
  (return (0.0 0.0 0.0)))

(fn `Is the current growth sufficient for the next stage`
  (returns (ReturnValue :type Boolean)))

(fn `Is_Plant_In_Last_Stage`
  (returns (ReturnValue :type Boolean))
  (return false))

(fn `Manually_Place_In_World`)

(fn `OnRep_Current Amount of Fertilizer`
  (`self.OnRep_Current Amount of Fertilizer Execution`))

(fn `OnRep_Current Amount of Fertilizer Execution`)

(fn `OnRep_Current Amount of Water`
  (`self.OnRep_Current Amount of Water Excecution`))

(fn `OnRep_Current Amount of Water Excecution`)

(fn `OnRep_Current Decay Percentage`
  (`self.OnRep_Current_Decay_Time Excecution`))

(fn `OnRep_Current Decay Percentage Excecution`)

(fn `OnRep_Current_Decay_Time`
  (`self.OnRep_Current_Decay_Time Excecution`))

(fn `OnRep_Current_Decay_Time Excecution`)

(fn `OnRep_Current_Durability`
  (`self.OnRep_Current_Durability Execution`))

(fn `OnRep_Current_Durability Execution`)

(fn `OnRep_Current_Growth_Time`
  (`self.OnRep_Current_Growth_Time Excecution`))

(fn `OnRep_Current_Growth_Time Excecution`)

(fn `OnRep_Farmable_Is_Ghost`
  (`self.OnRep_Farmable_Is_Ghost Excecution`))

(fn `OnRep_Farmable_Is_Ghost Excecution`)

(fn `Remove_Farmable_From_Save`)

(fn `Save_Farming_Actor`
  (locals (`local save object ` :type "SaveGame Object Reference")))

(fn `Set Plant to decayed`)

(fn `Set Statbar Visibility based on full health`
  (params (`Override to visible` :type Boolean) (`Override to Hidden` :type Boolean)))

(fn `Set_Plant_To_Stage_Index`
  (params (`Stage Index` :type Integer)))

(fn `Set_Plant_To_Yield_Stage`)

(fn `Should get other Actor to Interact with`
  (params (`Based on this Component` :type "PrimitiveComponent Object Reference"))
  (returns (True :type Boolean) (`Actor To Interact With` :type "Actor Object Reference"))
  (return false null))

(fn `Should server control the interact`
  (returns (`Server should excecute interact call` :type Boolean))
  (return true))

(fn `Should_Receive_Buildable_Info`
  (returns (True :type Boolean))
  (return false))

(fn `Try Spawn Pluckable Yield`
  (params (`Is Initializing from save` :type Boolean)))

(fn `Try_Consume_Fertilizer`
  (params (Amount :type "Float (double-precision)"))
  (returns (Consumed_Succesfully :type Boolean)))

(fn `Try_Consume_Oxygen`
  (params (Amount :type "Float (double-precision)"))
  (returns (Consumed_Succesfully :type Boolean))
  (return true))

(fn `Try_Consume_Water`
  (params (Amount :type "Float (double-precision)"))
  (returns (Consumed_Succesfully :type Boolean)))

(fn `Try_Harvest`
  (params (Controller :type "Controller Object Reference")))

(fn `Try_Regrow`
  (returns (`Plant Regrows` :type Boolean)))

(fn `Update_Statbar_Farmable`)

(fn `UserConstructionScript`)