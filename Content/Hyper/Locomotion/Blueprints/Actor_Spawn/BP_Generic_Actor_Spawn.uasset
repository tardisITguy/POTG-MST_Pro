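; A generic spawnable actor for replicated visuals and audio, configurable with a static mesh, skeletal mesh, Niagara system and sound.
; On BeginPlay it applies each valid asset to its component, setting relative transforms for all but the audio.
; Niagara sits under the skeletal mesh so systems can sample the parent's mesh locations.
; Setter events change RepNotify flags, whose OnRep functions switch the Niagara and audio components on or off.
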(event `self.ReceiveBeginPlay`
  ;[0.05127 0.05127 0.05127] Initialize any static mesh, skeletal mesh, niagara effect and/or sound component with its relative location.
  ; This actor can be used to spawn generic actors which needs to be replicated.
  (`|ExecutionSequence`
    (:`then_0`
      (bind _static_mesh (`self.Static Mesh`)
        (:`then`
          (`StaticMeshComponent.SetStaticMesh` (`self.StaticMeshComponent`) _static_mesh)
          (`SceneComponent.K2_SetRelativeTransform` (`self.StaticMeshComponent`) (`self.Static Mesh Relative Transform`) false false))
        (:`else`)))
    (:`then_1`
      (bind _skeletalmesh (`self.SkeletalMesh`)
        (:`then`
          (`SkinnedMeshComponent.SetSkinnedAssetAndUpdate` (`self.SkeletalMeshComponent`) _skeletalmesh true)
          ;;[0.05127 0.05127 0.05127] Not that the niagara is attached under the skeletal mesh. This is for when using the parent as input for skeletal mesh locations in an niagara system
          (`SceneComponent.K2_SetRelativeTransform` (`self.SkeletalMeshComponent`) (`self.Skeletal Mesh Relative Transform`) false false))
        (:`else`)))
    (:`then_2`
      (bind _niagara_system (`self.Niagara_System`)
        (:`then`
          (`NiagaraComponent.SetAsset` (`self.NiagaraComponent`) _niagara_system true)
          (`SceneComponent.K2_SetRelativeTransform` (`self.NiagaraComponent`) (`self.Niagara Relative Transform`) false false))
        (:`else`)))
    (:`then_3`
      (bind _sound (`self.Sound`)
        (:`then`
          (`AudioComponent.SetSound` (`self.AudioComponent`) _sound))
        (:`else`)))))

(event `Set Niagara Active`
  (params (bNewActive :type Boolean))
  ;[0.05127 0.05127 0.05127] Switch active state of niagara and audio
  (set `self.Niagara Active` bNewActive))

(event `Set Audio Active`
  (params (bNewActive :type Boolean))
  ;[0.05127 0.05127 0.05127] Switch active state of niagara and audio
  (set `self.Audio Active` bNewActive))

(fn `OnRep_Audio Active`
  (`ActorComponent.SetActive` (`self.AudioComponent`) (`self.Audio Active`) false))

(fn `OnRep_Niagara Active`
  (`ActorComponent.SetActive` (`self.NiagaraComponent`) (`self.Niagara Active`) false))

(fn `UserConstructionScript`)