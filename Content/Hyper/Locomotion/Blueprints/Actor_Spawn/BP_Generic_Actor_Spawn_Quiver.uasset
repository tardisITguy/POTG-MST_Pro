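; Quiver actor that visually shows the number of available arrows.
; On BeginPlay it assigns the arrow mesh to the static mesh child of each placeholder under ArrowPlaceholders, up to the available count and capped at nine.
; UpdateQuiver stores a new count, clears all placeholder meshes and refills them, so existing components are reused rather than spawned.
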(event `self.ReceiveBeginPlay`
  (`parent.ReceiveBeginPlay`)
  (`self.Set Arrows in quiver` :!label _label))

(event `Update Quiver`
  (params (`Arrows Available` :type Integer))
  ;[0.05127 0.05127 0.05127] Set new arrow amount, clear all arrow meshes and fill them again
  (set `self.Arrows available` `Arrows Available`)
  (`self.Clear Arrow Meshes`)
  (goto _label))

(fn `Clear Arrow Meshes`
  (for _array_element (`SceneComponent.GetChildrenComponents` (`self.Arrow_Placeholders`) true)
    (bind _asstatic_mesh_component (cast `StaticMeshComponent` (`SceneComponent.GetChildComponent` _array_element 0)))
    (`StaticMeshComponent.SetStaticMesh` _asstatic_mesh_component null)))

(fn `Set Arrows in quiver`
  (for (_array_element _array_index) (`SceneComponent.GetChildrenComponents` (`self.Arrow_Placeholders`) true)
    (if (or (>= _array_index 9) (>= _array_index (`self.Arrows available`)))
      (break)
      (else
        (bind _asstatic_mesh_component (cast `StaticMeshComponent` (`SceneComponent.GetChildComponent` _array_element 0)))
        (`StaticMeshComponent.SetStaticMesh` _asstatic_mesh_component (`self.Arrow mesh`))))))

(fn `UserConstructionScript`
  (`parent.UserConstructionScript`))