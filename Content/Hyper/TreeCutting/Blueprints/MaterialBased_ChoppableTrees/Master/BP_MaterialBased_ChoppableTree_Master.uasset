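; Master actor for a replicated choppable tree that shows each valid equipment hit as a growing material mask.
; At the hit threshold, RepNotify slices a procedural mesh copy at mask height into a stump and physics-driven falling top.
; The top becomes spawned logs after a delay or ground trace, or goes straight to the instigator's inventory.
; The stump takes separate damage and can drop an item when destroyed.
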(event `self.ReceiveBeginPlay`
  (`self.Initialize`)
  (bind _dynamic_material_instance (`self.Dynamic Material Instance`)
    (:`then`
      (`MaterialInstanceDynamic.SetScalarParameterValue` _dynamic_material_instance "Mask_Alpha" (`self.Total Hit Amount Registrered`))
      (`self.Apply Initial Mask` (`self.Damage Causer`))
      (`PrimitiveComponent.SetCollisionEnabled` (`self.Capsule`) "QueryAndPhysics")
      (if (`self.Has Broken`)
        (`self.OnRep_Has Broken_Execution` true)
        (`self.Destroy Top`)))
    (:`else`)))

(event `Initialize Mask`
  (params (`Damage Causer` :type "Actor Object Reference"))
  ;[0.05127 0.05127 0.05127] Rep notify the initialization of the mask via the damage causer variable
  (set `self.Damage Causer` `Damage Causer`))

(event `Process Hit`
  (params (`Forward Vector` :type "Vector Structure") (Instigator :type "Controller Object Reference"))
  (bind (_component _is_valid) (`/Game/Hyper/Core/Inventory/BlueprintMacroLibrary/BML_Inventory_Controller.Get Inventory Manager` Instigator))
  (if (>= (`self.Total Hit Amount Registrered`) (`self.Total Hit Amount Break Threshold`))
    (`self.Split Tree` `Forward Vector`)
    (if (`self.Directly add to inventory instead of spawning logs in world`)
      (if _is_valid
        (bind _asbp_pickup_abstract (castclass `/Game/Hyper/Core/Inventory/Blueprints/BP_Pickup_Abstract` (`self.Log To Spawn`)))
        (`/Game/Hyper/Core/Inventory/Blueprints/AC_Inventory_Abstract.Event: Try Add Item to inventory automatically` _component (make `/Game/Hyper/Core/Inventory/Datamodel/Structures/Main_Item_Slot_Structs/Struct_Inventory_Slot_Item` (`.Item_2_C7967C054AE750B79BB1FDB9058FE0B3` (break `/Game/Hyper/Core/Inventory/Datamodel/Structures/Main_Item_Slot_Structs/Struct_Inventory_Slot_Item` (defaults `Object` _asbp_pickup_abstract))) (`self.Amount of logs to spawn`) 0 false (struct :`CurrentDurability` 100.0 :`IsUseable` true) (struct :`Chanceofspawinginvendorinventory` 1.0 :`MinimalAmounttorestock` 1 :`MaximumAmounttorestock` 5 :`MaximumStock` 10) true null (struct :`Hotbarslotindex` 999 :`Inventoryslotindex` 999) (struct :`Linkedtothisequipmentslot` "NewEnumerator13" :`AmmoSlot` (struct :`AmmoDataTable` (struct :`DataTable` "/Script/Engine.DataTable'/Game/Hyper/Core/Equipment_Manager/Datamodel/Datatables/DT_Ammo.DT_Ammo'")))) false 0 false false false)
        (`KismetSystemLibrary.Delay` (`self.Duration Before Logs Spawning`))
        (if (`self.Use Tree Falling Sound`) :!label _label
          (`/Game/Hyper/Core/ReplicationSubSystem/Blueprints/AC_Replication_Abstract.Initialize Spawn Sound At Location` (`/Game/Hyper/Core/ReplicationSubSystem/BlueprintMacroLibrary/BML_Replication_Controller.Get Replication` Instigator) "/Game/Hyper/ResourcePack/Sounds/Tree/Tree_Fall_Cue.Tree_Fall_Cue" (`KismetSystemLibrary.GetComponentBounds` (`self.ProceduralMesh`)) false 0.0 "/Game/Hyper/ResourcePack/Audio/AttenuationPresets/ATT_Default.ATT_Default"))
        (`self.Destroy Actor And Check Respawn`)
        (else
          (if (`self.Use Ground Hit Detection for Destroy`) :!label _label_2
            (bind _returnvalue (`KismetSystemLibrary.K2_SetTimerDelegate` (delegate `Trace Ground`) 0.025 true))
            (else
              (`KismetSystemLibrary.Delay` (`self.Duration Before Logs Spawning`))
              (`self.Spawn Logs` :!label _label_3)
              (goto _label)))))
      (else
        (goto _label_2)))
    (else
      (`self.Apply Hit to Tree and adapt Mask`))))

(event `Destroy Top`
  (bind _proceduralmesh (`self.ProceduralMesh`)
    (:`then`
      (`ActorComponent.K2_DestroyComponent` _proceduralmesh))
    (:`else`
      _))
  (bind _capsule (`self.Capsule`)
    (:`then`
      (`ActorComponent.K2_DestroyComponent` _capsule))
    (:`else`)))

(event `Trace Ground`
  (bind _origin (`KismetSystemLibrary.GetComponentBounds` (`self.ProceduralMesh`)))
  (bind (_outhit _returnvalue) (`KismetSystemLibrary.BoxTraceSingle` _origin (- _origin (`KismetMathLibrary.MakeVector` 0.0 0.0 (`self.Distance to trace down for ground`))) (100.0 100.0 200.0) (struct) "TraceTypeQuery1"))
  (if _returnvalue
    (`KismetSystemLibrary.K2_ClearAndInvalidateTimerHandle` (stale `Process Hit` _returnvalue))
    (set `self.Has hit ground` true)
    (`KismetSystemLibrary.Delay` (`self.How long to delay after hit ground`))
    (goto _label_3)
    (else
      (`KismetSystemLibrary.Delay` 6.75)
      (if (not (`self.Has hit ground`))
        (goto _label_3)))))

(event `self.ReceivePointDamage`
  (params (Damage :type "Float (single-precision)") (DamageType :type "DamageType Object Reference") (HitLocation :type "Vector Structure") (HitNormal :type "Vector Structure") (HitComponent :type "PrimitiveComponent Object Reference") (BoneName :type Name) (ShotFromDirection :type "Vector Structure") (InstigatedBy :type "Controller Object Reference") (DamageCauser :type "Actor Object Reference") (HitInfo :type "HitResult Structure (by ref)"))
  (bind _returnvalue (`self.GetComponentByClass` DamageCauser "/Game/Hyper/Core/Equipment_Manager/Blueprints/AC_Equipment_Manager_Abstract.AC_Equipment_Manager_Abstract_C"))
  ;[0.05127 0.05127 0.05127] On damage, the first time initlize the mask. That determines the height.
  ; After that, just register and process the hit
  (if (`self.Has Broken`)
    (`self.Trunk Logic` HitComponent Damage)
    (else
      ;;[0.05127 0.05127 0.05127] Does the instigator has the required equipment to inflict damage?
      (`/Engine/EditorBlueprintResources/StandardMacros.IsValid` _returnvalue
        (:`Is Valid`
          (if (`/Game/Hyper/Core/Equipment_Manager/Blueprints/AC_Equipment_Manager_Abstract.Does actor has required equipmenttype in slot?` _returnvalue (`self.Accepted Equipment Type to inflict Damage`) "NewEnumerator8")
            (`|ExecutionSequence`
              (:`then_0`
                (`/Engine/EditorBlueprintResources/StandardMacros.DoOnce` false
                  (:`Completed`
                    (`self.Initialize Mask` DamageCauser))))
              (:`then_1`
                (`self.Process Hit` (`self.GetActorForwardVector` DamageCauser) InstigatedBy)))))))))

(event `Destroy TreecuttingActor`)

(fn `Apply Hit to Tree and adapt Mask`
  ;[0.03689 0.03689 0.03689 0.5922] Add hit amount registered
  ;;[0.05127 0.05127 0.05127] set the hardness of the mask in the rep notify
  (set `self.Total Hit Amount Registrered` (+ (`self.Total Hit Amount Registrered`) (`self.Hit amount increase per hit`))))

(fn `Apply Initial Mask`
  (params (`Damage Causer` :type "Actor Object Reference"))
  (bind (_returnvalue_x _returnvalue_y _returnvalue_z) (`KismetMathLibrary.BreakVector` (`self.K2_GetActorLocation`)))
  (bind _dynamic_material_instance (`self.Dynamic Material Instance`))
  (`/Engine/EditorBlueprintResources/ActorMacros.Switch Has Authority`
    (:`Authority`
      (if (`KismetSystemLibrary.IsStandalone`)
        ;[0.05127 0.05127 0.05127] Determines the start location of the mask. Use the XY from the mesh itself, but add a fixed value from the damage causer height so it always is in the same position even though the tree can be hidden a part in the landscape
        (`MaterialInstanceDynamic.SetVectorParameterValue` _dynamic_material_instance "StartLocation" (`KismetMathLibrary.Conv_VectorToLinearColor` (`KismetMathLibrary.MakeVector` (+ _returnvalue_x (`self.Relative X stat`)) (+ _returnvalue_y (`self.Relative Y Start`)) (+ _returnvalue_z (`self.Mask_Height`)))) :!label _label)
        ;[0.05127 0.05127 0.05127] Determines the bounds of the mask to apply on and a tiling for the inside texture. Make sure to have the bounds bigger than the widt and lenght  the tree (XY)
        (`MaterialInstanceDynamic.SetVectorParameterValue` _dynamic_material_instance "Bounds" (`KismetMathLibrary.Conv_VectorToLinearColor` (`self.Mask Bounds`)))
        (`MaterialInstanceDynamic.SetScalarParameterValue` _dynamic_material_instance "Inside_Tiling" (`self.Inside_Tiling`))
        (`MaterialInstanceDynamic.SetScalarParameterValue` _dynamic_material_instance "Edge_Fallof" (`self.Edge_Fallof`))
        (elif (`KismetSystemLibrary.IsServer`)
          (goto _label))))
    (:`Remote`
      (goto _label))))

(fn `Calculate Damage To Trunk`
  (params (Damage :type "Float (double-precision)"))
  (returns (`Met damage threshold` :type Boolean))
  ;[0.05098 0.05098 0.05098] Add the damage to the total trunk damage
  (bind _output_get (set `self.Damage done to trunk` (+ (`self.Damage done to trunk`) Damage)))
  (return (>= _output_get (`self.Damage required to destroy trunk`))))

(fn `Enable Physics on Procedural Mesh and add force`
  (params (`Procedural Mesh` :type "ProceduralMeshComponent Object Reference") (`Forward Vector of Hit` :type "Vector Structure") (`Ignore this Actor collision` :type "Actor Object Reference") (`Set collision to` :type "ECollisionEnabled Enum" :default "QueryAndPhysics"))
  ;[0.05127 0.05127 0.05127] After the mesh is splitted, make sure to enable physics and gravity and add a impulse into the direction of the forward vector from the damage causer
  (`PrimitiveComponent.SetSimulatePhysics` `Procedural Mesh` true)
  (`PrimitiveComponent.SetEnableGravity` `Procedural Mesh` true)
  (`PrimitiveComponent.AddImpulse` `Procedural Mesh` (* `Forward Vector of Hit` (`self.Impulse factor after break`)) "None" true)
  (`PrimitiveComponent.SetCollisionEnabled` `Procedural Mesh` (`local.Set collision to`))
  (`/Engine/EditorBlueprintResources/StandardMacros.IsValid` `Ignore this Actor collision`
    (:`Is Valid`
      (`PrimitiveComponent.IgnoreActorWhenMoving` `Procedural Mesh` `Ignore this Actor collision` true))))

(fn `Initialize`
  (bind _returnvalue (`PrimitiveComponent.GetMaterial` (`self.BaseMesh`) (`self.Choppable Material Index`)))
  (`StaticMeshComponent.SetStaticMesh` (`self.BaseMesh`) (`self.Static Mesh`))
  ;[0.05127 0.05127 0.05127] Copy a procedural mesh from the origingal static mesh component
  (`KismetProceduralMeshLibrary.CopyProceduralMeshFromStaticMeshComponent` (`self.BaseMesh`) (select `bool` (> (`StaticMesh.GetNumLODs` (`StaticMeshComponent.StaticMesh` (`self.BaseMesh`))) 0) :`true` (`self.LOD to use for procedural mesh`)) (`self.ProceduralMesh`))
  ;[0.05127 0.05127 0.05127] Make sure to enable collision on the procedural mesh
  (`PrimitiveComponent.SetCollisionEnabled` (`self.ProceduralMesh`) "QueryAndPhysics")
  ;[0.05127 0.05127 0.05127] Create a material instance and make sure to apply it on the mesh. It used the specified index of the material index that should be the same as the base mesh that we are trying to hit
  (set `self.Original Material` _returnvalue)
  (`/Engine/EditorBlueprintResources/ActorMacros.Switch Has Authority`
    (:`Authority`
      (if (`KismetSystemLibrary.IsStandalone`)
        (bind _returnvalue_2 (`KismetMaterialLibrary.CreateDynamicMaterialInstance` _returnvalue :!label _label))
        (bind _output_get (set `self.Dynamic Material Instance` _returnvalue_2))
        (`PrimitiveComponent.SetMaterial` (`self.BaseMesh`) (`self.Choppable Material Index`) _output_get)
        (set `self.Initialized` true)
        (elif (`KismetSystemLibrary.IsServer`)
          (goto _label))))
    (:`Remote`
      (goto _label))))

(fn `OnRep_Damage Causer`
  (if (`self.Initialized`)
    (`self.Apply Initial Mask` (`self.Damage Causer`))))

(fn `OnRep_Destroyed Top`
  (if (`self.Destroyed Top`)
    ;[0.05098 0.05098 0.05098] Destroy Top if initialized, the actor is not initialized if coming into rep range
    (if (`self.Initialized`)
      (`self.Destroy Top`))))

(fn `OnRep_Has Broken_Execution`
  (params (`Override Initialization Check` :type Boolean))
  (locals (`Original Trunk Rotation` :type "Rotator Structure") (`Skip Falling Down` :type Boolean))
  (bind _basemesh (`self.BaseMesh`))
  (bind _trunk_mesh (`self.Trunk Mesh`))
  (bind _trunk_mesh_2 (`self.Trunk Mesh`))
  (bind _box (`self.Box`))
  (bind _proceduralmesh (`self.ProceduralMesh`))
  (bind (_origin _boxextent) (`KismetSystemLibrary.GetComponentBounds` _trunk_mesh_2))
  (bind (_returnvalue_x _returnvalue_y _returnvalue_z) (`KismetMathLibrary.BreakVector` (`SceneComponent.K2_GetComponentLocation` (`self.BaseMesh`))))
  (bind _z (.z (`SceneComponent.K2_GetComponentScale` (`self.DefaultSceneRoot`))))
  (if (or `Override Initialization Check` (`self.Initialized`))
    (set `local.Skip Falling Down` (> (- (`GameStateBase.GetServerWorldTimeSeconds` (`GameplayStatics.GetGameState`)) (`self.Tree Broken Server Time`)) 10.0))
    (if (`self.Has Broken`)
      ;[0.05127 0.05127 0.05127] When tree can break, disable static mesh and enable the procedural mesh
      (`SceneComponent.SetVisibility` _basemesh false false)
      (`PrimitiveComponent.SetCollisionEnabled` _basemesh "NoCollision")
      (`SceneComponent.SetVisibility` (`self.ProceduralMesh`) true false)
      ;[0.05127 0.05127 0.05127] Slice the procedural mesh
      (bind _outotherhalfprocmesh (`KismetProceduralMeshLibrary.SliceProceduralMesh` (`self.ProceduralMesh`) (`KismetMathLibrary.MakeVector` _returnvalue_x _returnvalue_y (+ _returnvalue_z (`self.Mask_Height`))) (`self.Split Plane Normal`) true "CreateNewSectionForCap" (`self.Ring Material`)))
      (bind _output_get (set `self.Trunk Mesh` _outotherhalfprocmesh))
      (`self.Set Procedrual Trunk Materials` _output_get)
      (`|ExecutionSequence`
        (:`then_0`
          (if (`local.Skip Falling Down`)
            (`ActorComponent.K2_DestroyComponent` _proceduralmesh)
            (else
              (`self.Set Procedural TopMesh Materials` _proceduralmesh)
              (`self.Enable Physics on Procedural Mesh and add force` (`self.ProceduralMesh`) (`self.Forward Vector of instigating hit`))
              (bind _returnvalue (`GameplayStatics.SpawnSoundAtLocation` (`self.Tree Fall Sound`) (`self.K2_GetActorLocation`) (struct) 1.0 1.0 0.0 "/Game/Hyper/ResourcePack/Audio/AttenuationPresets/ATT_Default.ATT_Default" null))
              (set `self.Active Tree Fall sound` _returnvalue))))
        (:`then_1`
          ;[0.05098 0.05098 0.05098] Disable the convex trunk collider
          (if (not (`self.Use Convex Trunk Collision`))
            (`PrimitiveComponent.SetCollisionEnabled` (`self.Trunk Mesh`) "NoCollision")
            ;[0.05098 0.05098 0.05098] Temporary set the trunk location. This is required if you want the correct box collision location.
            (bind _output_get_2 (set `local.Original Trunk Rotation` (`SceneComponent.K2_GetComponentRotation` _trunk_mesh)))
            (`SceneComponent.K2_SetWorldRotation` _trunk_mesh (`KismetMathLibrary.MakeRotator` 0.0 0.0 (.yaw _output_get_2)) false false)
            ;[0.05098 0.05098 0.05098] Calculate the correct location and box extent for the trunk
            (`PrimitiveComponent.SetCollisionEnabled` _box "QueryAndPhysics")
            (`SceneComponent.K2_SetRelativeLocation` _box (`KismetMathLibrary.MakeVector` (.x (`SceneComponent.RelativeLocation` (`self.Box`))) (.y (`SceneComponent.RelativeLocation` (`self.Box`))) (/ (.z (- _origin (`SceneComponent.K2_GetComponentLocation` _trunk_mesh_2))) _z)) false true)
            (`BoxComponent.SetBoxExtent` _box (`KismetMathLibrary.MakeVector` (.x (`BoxComponent.BoxExtent` (`self.Box`))) (.y (`BoxComponent.BoxExtent` (`self.Box`))) (* (/ (.z _boxextent) _z) (`self.Box Collision Z Scale Multiplier`))) true)
            ;[0.05098 0.05098 0.05098] Reset the trunk rotation.
            (`SceneComponent.K2_SetWorldRotation` (`self.Trunk Mesh`) (`local.Original Trunk Rotation`) false false)))))))

(fn `OnRep_Has hit ground`
  (bind _active_tree_fall_sound (`self.Active Tree Fall sound`))
  (`/Engine/EditorBlueprintResources/StandardMacros.IsValid` _active_tree_fall_sound
    (:`Is Valid`
      (`AudioComponent.Stop` _active_tree_fall_sound)
      (`ActorComponent.K2_DestroyComponent` _active_tree_fall_sound)
      (bind _capsule (`self.Capsule`)
        (:`then`
          (`PrimitiveComponent.SetCollisionEnabled` _capsule "NoCollision")
          (`ActorComponent.K2_DestroyComponent` _capsule))
        (:`else`)))))

(fn `OnRep_Total Hit Amount Registrered`
  (if (`self.Initialized`)
    (bind _dynamic_material_instance (`self.Dynamic Material Instance`)
      (:`then`
        (`MaterialInstanceDynamic.SetScalarParameterValue` _dynamic_material_instance "Mask_Alpha" (`self.Total Hit Amount Registrered`)))
      (:`else`))))

(fn `Set Procedrual Trunk Materials`
  (params (`Procedural Trunk` :type "ProceduralMeshComponent Object Reference"))
  (bind _returnvalue (- (`PrimitiveComponent.GetNumMaterials` `Procedural Trunk`) 1))
  ;[0.05127 0.05127 0.05127] Check how many materials are assigned to the trunk that is left. Loop over all the indexes
  (for _index (range (+ _returnvalue 1))
    ;[0.05127 0.05127 0.05127] When the trunk is split. We need to set the materials of that trunk.
    ; In most cases only one material is assinged to the trunk and the trunk material is on index 0, however it occurs that in some tree meshes the default trunk material is set to index 2,3 or something else.
    ;
    ; After we split the tree, it will set the material on the trunk to the first index it finds on the original mesh. But if the first material of the mesh is not the trunk material, it will be displayed wrong. E.g. the trunk uses the leaves material.
    ;
    ; So what we do here is:
    ; 1. getting the original static mesh
    ; 2. Get the material index that has the trunk material (You need to customly check it and set the index if it is not on zero)
    ; 3. Set the first index found of the procedural generated trunk to that specific trunk material
    (if (== _index 0)
      (`PrimitiveComponent.SetMaterial` (`local.Procedural Trunk`) 0 (`StaticMesh.GetMaterial` (`self.Static Mesh`) (`self.First Trunk Material Index`)))
      (else
        ;[0.05127 0.05127 0.05127] The last index of the trunk is the added CAP. This should be the tree ring material
        (if (== _index _returnvalue)
          (`PrimitiveComponent.SetMaterial` (`local.Procedural Trunk`) _returnvalue (`self.Ring Material`))
          (else
            ;[0.05127 0.05127 0.05127] If index 1 =! to the last material on the procedrual trunk. It means that the trunk has two materials assigned.
            ; Just the same as at index 0, we set the trunk material custom based on the orginal static mesh material
            (if (== _index 1)
              (`PrimitiveComponent.SetMaterial` (`local.Procedural Trunk`) 1 (`StaticMesh.GetMaterial` (`self.Static Mesh`) (`self.Second Trunk Material Index`)))))))))
  (return))

(fn `Set Procedural TopMesh Materials`
  (params (`Procedural Mesh` :type "PrimitiveComponent Object Reference"))
  (if (`self.Set Top trunk Mesh Manually`)
    (`PrimitiveComponent.SetMaterial` `Procedural Mesh` 0 (`self.Top Material Mesh Index 0`))
    (if (> (`PrimitiveComponent.GetNumMaterials` `Procedural Mesh`) 0)
      (bind _top_material_mesh_index_01 (`self.Top Material Mesh Index 01`)
        (:`then`
          (`PrimitiveComponent.SetMaterial` `Procedural Mesh` 1 _top_material_mesh_index_01)
          (if (> (`PrimitiveComponent.GetNumMaterials` `Procedural Mesh`) 1)
            (bind _top_material_mesh_index_02 (`self.Top Material Mesh Index 02`)
              (:`then`
                (`PrimitiveComponent.SetMaterial` `Procedural Mesh` 2 _top_material_mesh_index_02)
                (if (> (`PrimitiveComponent.GetNumMaterials` `Procedural Mesh`) 2)
                  (bind _top_material_mesh_index_03 (`self.Top Material Mesh Index 03`)
                    (:`then`
                      (`PrimitiveComponent.SetMaterial` `Procedural Mesh` 3 _top_material_mesh_index_03))
                    (:`else`
                      _))))
              (:`else`
                _))))
        (:`else`
          _))))
  ;[0.05127 0.05127 0.05127] The last index is the ring/cap material. Set it.
  (`PrimitiveComponent.SetMaterial` `Procedural Mesh` (- (`PrimitiveComponent.GetNumMaterials` `Procedural Mesh`) 1) (`self.Ring Material`))
  (return))

(fn `Spawn Logs`
  ;[1 1 1] Loop over child components and spawn log on location of scene components under Tree Top
  (bind _proceduralmesh (`self.ProceduralMesh`)
    (:`then`
      (for _array_element (`SceneComponent.GetChildrenComponents` _proceduralmesh false)
        ;;[1 1 1] Check how man logs are spawned
        (bind _output_get (set `self.Logs spawned` (+ (`self.Logs spawned`) 1)))
        (if (not (>= (- _output_get 1) (`self.Amount of logs to spawn`)))
          (bind (_returnvalue_location _returnvalue_rotation _returnvalue_scale) (`KismetMathLibrary.BreakTransform` (`SceneComponent.K2_GetComponentToWorld` _array_element)))
          (`|SpawnActorFromClass` (`self.Log To Spawn`) (`KismetMathLibrary.MakeTransform` _returnvalue_location _returnvalue_rotation (select `bool` (`self.Use Actor Scale for log Scale`) :`false` (1.0 1.0 1.0) :`true` _returnvalue_scale)) "AlwaysSpawn" "SelectDefaultAtRuntime" null null)))
      (set `self.Destroyed Top` true)
      (`self.Destroy Top`))
    (:`else`)))

(fn `Split Tree`
  (params (`Forward Vector` :type "Vector Structure"))
  ;[0.05127 0.05127 0.05127] On break, excecute via rep notify
  (set `self.Forward Vector of instigating hit` `Forward Vector`)
  (set `self.Tree Broken Server Time` (`GameStateBase.GetServerWorldTimeSeconds` (`GameplayStatics.GetGameState`)))
  (set `self.Has Broken` true))

(fn `Trunk Logic`
  (params (a :type "Object Object Reference") (Damage :type "Float (double-precision)"))
  ;[0.05098 0.05098 0.05098] I would prefer to use an CHAOS based trunk. However I do not seem to be able to set the "Object State" dynamicly. This is a proper alternative for now.
  ;;[0.05098 0.05098 0.05098] Check if the trunk is hit, if so, destroy it
  (if (and (== a (`self.Trunk Mesh`)) (`self.Has Broken`))
    ;;[0.05098 0.05098 0.05098] If trunk has met damage threshold, destroy the trunk component and call the destroy treeecutting actor
    (bind _met_damage_threshold (`self.Calculate Damage To Trunk` (`local.Damage`)))
    (if _met_damage_threshold
      (set `self.Trunk is destroyed` true)
      ;;[0.05098 0.05098 0.05098] Spawn item when trunk is destroyed
      (if (`self.Spawn item when trunk is destroyed`)
        (`|SpawnActorFromClass` (`self.Spawn this item when trunk is destroyed`) (`SceneComponent.K2_GetComponentToWorld` (`self.Trunk Mesh`)) "AdjustIfPossibleButAlwaysSpawn" "SelectDefaultAtRuntime" null null)
        ;;[0.05098 0.05098 0.05098] Spawn trunk sound
        (`GameplayStatics.PlaySoundAtLocation` (`self.Trunk destruct sound`) (`self.K2_GetActorLocation`) (struct) 1.0 1.0 0.0 null null null null))
      (`ActorComponent.K2_DestroyComponent` (`self.Trunk Mesh`))
      (`self.Destroy Actor And Check Respawn`))))

(fn `UserConstructionScript`
  (`StaticMeshComponent.SetStaticMesh` (`self.BaseMesh`) (`self.Static Mesh`))
  (if (`self.Override World Scale`)
    (`SceneComponent.SetWorldScale3D` (`self.BaseMesh`) (`self.New Scale`))))