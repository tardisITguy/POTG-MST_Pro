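; Master Blueprint for a tree that breaks instantly, bursting into physics-driven pieces instead of being felled as one.
; Outside dedicated servers, the HasBroken OnRep hides the static mesh, slices the procedural mesh twice with capped cuts, and launches three pieces in randomized directions with a fall sound.
; Breaks older than a few seconds by server time only hide the tree, skipping the effect.
; DestroyTop removes the pieces after a delay.
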(event `self.ReceiveBeginPlay`
  (`parent.ReceiveBeginPlay`))

(event `self.Destroy Top`
  (`KismetSystemLibrary.Delay` 2.0)
  ;[0.05098 0.05098 0.05098] Because we split the instant breakable trees into more than 1 piece, we need to remove the additional meshes
  (bind _proceduralmesh (`self.ProceduralMesh`)
    (:`then`
      (`ActorComponent.K2_DestroyComponent` _proceduralmesh)
      (`|ExecutionSequence`
        (:`then_0`
          (bind _out_other_half_proc_mesh (`self.Out Other Half Proc Mesh`)
            (:`then`
              _)
            (:`else`)))
        (:`then_1`
          (bind _trunk_mesh (`self.Trunk Mesh`)
            (:`then`
              _)
            (:`else`))))
      (`ActorComponent.K2_DestroyComponent` _out_other_half_proc_mesh)
      (`ActorComponent.K2_DestroyComponent` _trunk_mesh))
    (:`else`)))

(event `Delay Procedural Mesh Physics`
  (`KismetSystemLibrary.DelayUntilNextTick`)
  (`/Engine/EditorBlueprintResources/StandardMacros.IsValid` (`self.ProceduralMesh`)
    (:`Is Valid`
      (`self.Enable Physics on Procedural Mesh and add force` (`self.ProceduralMesh`) (`self.Get Random Unit Direction` (`self.Forward Vector of instigating hit`)) self "PhysicsOnly"))))

(fn `Get Random Unit Direction`
  (params (Direction :type "Vector Structure"))
  (returns (`Randomized Direction` :type "Vector Structure"))
  (return (`KismetMathLibrary.Normal` (+ Direction (`KismetMathLibrary.RandomUnitVector`)))))

(fn `OnRep_Has Broken_Execution`
  (params (`Override Initialization Check` :type Boolean))
  (locals (`Skip Falling Down` :type Boolean))
  (bind _out_other_half_proc_mesh (`self.Out Other Half Proc Mesh`))
  (bind _trunk_mesh (`self.Trunk Mesh`))
  (bind _proceduralmesh (`self.ProceduralMesh`))
  (bind _basemesh (`self.BaseMesh`))
  (bind (_returnvalue_x _returnvalue_y _returnvalue_z) (`KismetMathLibrary.BreakVector` (`SceneComponent.K2_GetComponentLocation` (`self.BaseMesh`))))
  (bind (_returnvalue_x_2 _returnvalue_y_2 _returnvalue_z_2) (`KismetMathLibrary.BreakVector` (`SceneComponent.K2_GetComponentLocation` (`self.BaseMesh`))))
  ;[0.05098 0.05098 0.05098] Only run when on client
  (if (not (`KismetSystemLibrary.IsDedicatedServer`))
    (set `local.Skip Falling Down` (> (- (`GameStateBase.GetServerWorldTimeSeconds` (`GameplayStatics.GetGameState`)) (`self.Tree Broken Server Time`)) 5.0))
    (if (`self.Initialized`)
      (if (`self.Has broken`)
        ;[0.05127 0.05127 0.05127] When tree can break, disable static mesh and enable the procedural mesh
        (`PrimitiveComponent.SetCollisionEnabled` (`self.Capsule`) "NoCollision")
        (`SceneComponent.SetVisibility` _basemesh false false)
        (`PrimitiveComponent.SetCollisionEnabled` _basemesh "NoCollision")
        ;;[0.05098 0.05098 0.05098] If we skip the breaking of the tree because enough time has passed, we only have to hide the static mesh
        (if (not (`local.Skip Falling Down`))
          (`SceneComponent.SetVisibility` (`self.ProceduralMesh`) true false)
          ;[0.05127 0.05127 0.05127] Slice the procedural mesh
          (bind _outotherhalfprocmesh (`KismetProceduralMeshLibrary.SliceProceduralMesh` (`self.ProceduralMesh`) (`KismetMathLibrary.MakeVector` _returnvalue_x _returnvalue_y (+ _returnvalue_z (`self.Mask_Height`))) (`self.Split Plane Normal`) true "CreateNewSectionForCap" (`self.Ring Material`)))
          (set `self.Trunk Mesh` _outotherhalfprocmesh)
          (`PrimitiveComponent.SetCollisionObjectType` _proceduralmesh "ECC_WorldDynamic")
          (`PrimitiveComponent.SetCollisionResponseToChannel` _proceduralmesh "ECC_Pawn" "ECR_Ignore")
          (`PrimitiveComponent.SetCollisionResponseToChannel` _proceduralmesh "ECC_WorldDynamic" "ECR_Ignore")
          (`PrimitiveComponent.SetCollisionResponseToChannel` _proceduralmesh "ECC_Destructible" "ECR_Ignore")
          (`PrimitiveComponent.SetCollisionObjectType` _trunk_mesh "ECC_WorldDynamic")
          (`PrimitiveComponent.SetCollisionResponseToChannel` _trunk_mesh "ECC_Pawn" "ECR_Ignore")
          (`PrimitiveComponent.SetCollisionResponseToChannel` _trunk_mesh "ECC_WorldDynamic" "ECR_Ignore")
          (`PrimitiveComponent.SetCollisionResponseToChannel` _trunk_mesh "ECC_Destructible" "ECR_Ignore")
          (`self.Set Procedrual Trunk Materials` (`self.Trunk Mesh`))
          (`self.Enable Physics on Procedural Mesh and add force` (`self.Trunk Mesh`) (`self.Get Random Unit Direction` (`self.Forward Vector of instigating hit`)) self "PhysicsOnly")
          (`self.Set Procedural TopMesh Materials` (`self.ProceduralMesh`))
          (`self.Delay Procedural Mesh Physics`)
          ;[0.05127 0.05127 0.05127] Second slice
          (bind _outotherhalfprocmesh_2 (`KismetProceduralMeshLibrary.SliceProceduralMesh` (`self.ProceduralMesh`) (`KismetMathLibrary.MakeVector` _returnvalue_x_2 _returnvalue_y_2 (+ _returnvalue_z_2 (* (`self.Mask_Height`) 2.0))) (`self.Split Plane Normal`) true "CreateNewSectionForCap" (`self.Ring Material`)))
          (set `self.Out Other Half Proc Mesh` _outotherhalfprocmesh_2)
          (`PrimitiveComponent.SetCollisionObjectType` _out_other_half_proc_mesh "ECC_WorldDynamic")
          (`PrimitiveComponent.SetCollisionResponseToChannel` _out_other_half_proc_mesh "ECC_Pawn" "ECR_Ignore")
          (`PrimitiveComponent.SetCollisionResponseToChannel` _out_other_half_proc_mesh "ECC_WorldDynamic" "ECR_Ignore")
          (`PrimitiveComponent.SetCollisionResponseToChannel` _out_other_half_proc_mesh "ECC_Destructible" "ECR_Ignore")
          (`self.Enable Physics on Procedural Mesh and add force` (`self.Out Other Half Proc Mesh`) (`self.Get Random Unit Direction` (`self.Forward Vector of instigating hit`)) self "PhysicsOnly")
          (`GameplayStatics.PlaySoundAtLocation` (`self.Tree Fall Sound`) (`self.K2_GetActorLocation`) (struct) 1.0 1.0 0.0 "/Game/Hyper/ResourcePack/Audio/AttenuationPresets/ATT_Default.ATT_Default" null null null))))))

(fn `UserConstructionScript`
  (`parent.UserConstructionScript`))