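; Master choppable tree whose Chaos geometry middle breaks under hits from actors with the required equipment, felling the top.
; Point damage spawns damage-scaled Chaos impact actors; the server totals broken mass until a threshold triggers multicast falling.
; It then removes the costly geometry and, after a delay, swaps the top for logs at its child components.
; The non-Chaos trunk takes damage after breaking, optionally drops an item, and calls destroy-and-respawn handling.
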(event `LetTreeFallOnClients`
  ;[0.05127 0.05127 0.05127] Logic for letting tree break
  (`self.Let Tree Fall`))

(event `Destroy Top`
  ;[0.05127 0.05127 0.05127] Logic for letting tree break
  (`ActorComponent.K2_DestroyComponent` (`self.Top_Mesh`)))

(event `Destroy geometry`
  ;[0.05127 0.05127 0.05127] Logic for letting tree break
  (`KismetSystemLibrary.DelayUntilNextTick`)
  (bind _middlegeometrycollection (`self.MiddleGeometryCollection`)
    (:`then`
      (`ActorComponent.K2_DestroyComponent` _middlegeometrycollection))
    (:`else`)))

(event `self.MiddleGeometryCollection.OnChaosBreakEvent`
  (params (BreakEvent :type "ChaosBreakEvent Structure (by ref)"))
  ;[0.05127 0.05127 0.05127] Logic for letting tree break
  (`/Engine/EditorBlueprintResources/ActorMacros.Switch Has Authority`
    (:`Authority`
      (bind _mass_chopped_has_reached_threshold (`self.Calculate mass chopped and check if has met threshold` BreakEvent))
      (if _mass_chopped_has_reached_threshold
        (`/Engine/EditorBlueprintResources/StandardMacros.DoOnce` false
          (:`Completed`
            (set `self.Has Broken` true)
            (`PrimitiveComponent.SetSimulatePhysics` (`self.Top_Mesh`) true)
            (`self.LetTreeFallOnClients`)
            (`|ExecutionSequence`
              (:`then_0`
                (`self.Destroy geometry`))
              (:`then_1`
                (`KismetSystemLibrary.Delay` (`self.Duration Before Logs Spawning`))
                (`self.Spawn Logs`)
                (`self.Destroy Actor And Check Respawn`)))))))))

(event `self.ReceivePointDamage`
  (params (Damage :type "Float (single-precision)") (DamageType :type "DamageType Object Reference") (HitLocation :type "Vector Structure") (HitNormal :type "Vector Structure") (HitComponent :type "PrimitiveComponent Object Reference") (BoneName :type Name) (ShotFromDirection :type "Vector Structure") (InstigatedBy :type "Controller Object Reference") (DamageCauser :type "Actor Object Reference") (HitInfo :type "HitResult Structure (by ref)"))
  (bind _returnvalue (`self.GetComponentByClass` DamageCauser "/Game/Hyper/Core/Equipment_Manager/Blueprints/AC_Equipment_Manager_Abstract.AC_Equipment_Manager_Abstract_C"))
  (bind _returnvalue_2 (+ (* Damage 0.01) 1.0))
  ;[0.05127 0.05127 0.05127] On damage
  ;;[0.05127 0.05127 0.05127] Does the instigator has the required equipment to inflict damage?
  (`/Engine/EditorBlueprintResources/StandardMacros.IsValid` DamageCauser
    (:`Is Valid`
      (`/Engine/EditorBlueprintResources/StandardMacros.IsValid` _returnvalue
        (:`Is Valid`
          (if (`/Game/Hyper/Core/Equipment_Manager/Blueprints/AC_Equipment_Manager_Abstract.Does actor has required equipmenttype in slot?` _returnvalue (`self.Accepted Equipment Type to inflict Damage`) "NewEnumerator8")
            (`self.Set Dynamic`)
            ;;[0.05127 0.05127 0.05127] This checks if it is the trunk that is hit and if it may be hit. If so, calculate trunk logic, if not, do nothing.
            (`self.Trunk Logic` HitComponent Damage)
            (`|SpawnActorFromClass` "/Game/Hyper/ResourcePack/Chaos/BP_Chaos_WeaponImpact.BP_Chaos_WeaponImpact_C" (`KismetMathLibrary.MakeTransform` (`.Location` (`GameplayStatics.BreakHitResult` HitInfo))) "Undefined" "MultiplyWithRoot" null (* (* 2500.0 _returnvalue_2) (`self.Force Mutliplier`)) (* (* 1.0 _returnvalue_2) (`self.Force Mutliplier`)) true null)
            ;[0.05127 0.05127 0.05127] on hit, make sure to start inactivity timer from the start
            (`self.Start inactivity timer`)))))))

(event `Set Dynamic`
  ;[0.05127 0.05127 0.05127] The "Set Dynamic" node sometimes makes a sphere that is larger than the geometry. So when it was set as dynamic it immediately falls through the world as it has no remaining static pieces to anchor the parts that are set as dynamic.  Try making that set dynamic size smaller to test. If it falls through, change the bounds and multiply by .a lower value to ensure the sphere size for the set bounds always leaves some as static for the anchor.
  (bind _middlegeometrycollection (`self.MiddleGeometryCollection`)
    (:`then`
      (`GeometryCollectionComponent.ApplyKinematicField` _middlegeometrycollection (`.SphereRadius` (`KismetSystemLibrary.GetComponentBounds` _middlegeometrycollection)) (`SceneComponent.K2_GetComponentLocation` _middlegeometrycollection)))
    (:`else`)))

(event `self.ReceiveBeginPlay`
  ;[0.05127 0.05127 0.05127] When spawning the tree dynamicly, the construction script does not seem to be excecuted properly and the anchor does not work. The geometry will move unless it is static. So we made the geometry static by default, and make it dynamic on begin play
  ;;[0.05127 0.05127 0.05127] Start inactivity timer
  (`self.Start Inactivity Timer`))

(fn `Calculate damage done to trunk`
  (params (Damage :type "Float (double-precision)"))
  (returns (`Met damage threshold` :type Boolean))
  (bind _output_get (set `self.Damage done to trunk` (+ (`self.Damage done to trunk`) Damage)))
  (return (>= _output_get (`self.Damage required to destroy trunk`))))

(fn `Calculate mass chopped and check if has met threshold`
  (params (ChaosBreakEvent :type "ChaosBreakEvent Structure (by ref)"))
  (returns (`Mass chopped has reached threshold` :type Boolean))
  ;[1 1 1] Get mass from break event and add it to total mass variable
  (bind _output_get (set `self.Total Mass Broken` (+ (`self.Total Mass Broken`) (`.Mass` (break `ChaosBreakEvent` ChaosBreakEvent)))))
  ;[1 1 1] Optionally print total mass chopped down
  (if (`self.Print Mass Chopped Down`)
    (`KismetSystemLibrary.PrintString` (`KismetStringLibrary.Concat_StrStr` "Total mass chopped down: " (`KismetStringLibrary.Conv_DoubleToString` _output_get)) true true (struct :`G` 0.66 :`B` 1.0 :`A` 1.0) 5.0))
  (return (>= _output_get (`self.Mass required to be chopped before falling`))))

(fn `Let Tree Fall`
  (`PrimitiveComponent.SetSimulatePhysics` (`self.Top_Mesh`) true)
  (`GameplayStatics.PlaySoundAtLocation` (`self.Tree Break Sound`) (`self.K2_GetActorLocation`) (struct) 1.0 1.0 0.0 null null null null))

(fn `Spawn Logs`
  ;[1 1 1] Loop over child components and spawn log on location of scene components under Tree Top
  (for _array_element (`SceneComponent.GetChildrenComponents` (`self.Top_Mesh`) false)
    ;;[1 1 1] Check how man logs are spawned
    (bind _output_get (set `self.Logs spawned` (+ (`self.Logs spawned`) 1)))
    (if (not (>= (- _output_get 1) (`self.Amount of logs to spawn`)))
      (`|SpawnActorFromClass` (`self.Log To Spawn`) (`SceneComponent.K2_GetComponentToWorld` _array_element) "Undefined" "SelectDefaultAtRuntime" null null)))
  (`self.Destroy Top`))

(fn `Trunk Logic`
  (params (A :type "Object Object Reference") (Damage :type "Float (double-precision)"))
  ;[1 1 1] I would prefer to use an CHAOS based trunk. However I do not seem to be able to set the "Object State" dynamicly. This is a proper alternative for now.
  ;;[1 1 1] Check if the trunk is hit, if so, destroy it
  (if (and (== A (`self.Trunk_Mesh`)) (`self.Has Broken`))
    ;;[1 1 1] If trunk has met damage threshold, destroy the trunk component and call the destroy treeecutting actor
    (bind _met_damage_threshold (`self.Calculate damage done to trunk` Damage))
    (if _met_damage_threshold
      (set `self.Trunk is destroyed` true)
      ;;[1 1 1] Spawn item when trunk is destroyed
      (if (`self.Spawn item when trunk is destroyed`)
        (`|SpawnActorFromClass` (`self.Spawn this item when trunk is destroyed`) (`SceneComponent.K2_GetComponentToWorld` (`self.Trunk_Mesh`)) "AdjustIfPossibleButAlwaysSpawn" "SelectDefaultAtRuntime" null null)
        ;;[1 1 1] Spawn trunk sound
        (`GameplayStatics.PlaySoundAtLocation` (`self.Trunk destruct sound`) (`self.K2_GetActorLocation`) (struct) 1.0 1.0 0.0 null null null null))
      (`ActorComponent.K2_DestroyComponent` (`self.Trunk_Mesh`))
      (`self.Destroy Actor And Check Respawn`))))

(fn `UserConstructionScript`
  (`self.Set Dynamic`))