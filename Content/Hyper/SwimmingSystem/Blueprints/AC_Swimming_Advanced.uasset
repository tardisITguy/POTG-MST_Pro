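; Character component for advanced swimming, adding surface swimming, toggled diving, sprint swimming and drowning state.
; Physics-volume overlaps flag water entry, while movement-mode changes swap the swimming input context, orientation and rotation rate with splash effects.
; Each tick, a trace above a head-attached breathing point detects submersion, driving oxygen consumption, underwater audio and timed bubble particles.
; Strafe swimming smoothly interpolates rotation toward the control rotation and replicates it.
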(event `EnhancedInput|/Game/Hyper/Locomotion/Input/Movement/IA_MoveForward`
  (params (ActionValue :type "Float (double-precision)") (ElapsedSeconds :type "Float (double-precision)") (TriggeredSeconds :type "Float (double-precision)") (InputAction :type "InputAction Object Reference" :default "/Game/Hyper/Locomotion/Input/Movement/IA_MoveForward.IA_MoveForward"))
  (bind _component (`/Game/Hyper/Core/Locomotion/BlueprintMacroLibrary/Generic/BML_ExtendedMovement_Component.Get ExtendedMovement`))
  (:`Triggered`
    ;[0.05127 0.05127 0.05127] Is disabling movement?
    (if (not (or (`/Game/Hyper/Core/Locomotion/Blueprints/AC_Extended_Movement_Abstract.Disable Forward Input` _component) (`/Game/Hyper/Core/Locomotion/Blueprints/AC_Extended_Movement_Abstract.Disable Movement` _component)))
      ;[0.05127 0.05127 0.05127] Is Swimming?
      (if (`NavMovementComponent.IsSwimming` (`/Game/Hyper/Core/Generic/BlueprintMacroLibrary/BML_Generic_Component.Get Character Movement`))
        (if (`self.Is Diving`)
          (`self.Swim forward while diving` ActionValue)
          (else
            (`self.Swim Forward while not diving` ActionValue)))))))

(event `EnhancedInput|/Game/Hyper/Locomotion/Input/Movement/IA_Sprint`
  (params (ActionValue :type Boolean) (ElapsedSeconds :type "Float (double-precision)") (TriggeredSeconds :type "Float (double-precision)") (InputAction :type "InputAction Object Reference" :default "/Game/Hyper/Locomotion/Input/Movement/IA_Sprint.IA_Sprint"))
  (:`Started`
    (`self.Event Sprint swim`))
  (:`Completed`
    (`self.Event normal swim`)))

(event `EnhancedInput|/Game/Hyper/Locomotion/Input/Swimming/IA_Dive`
  (params (ActionValue :type Boolean) (ElapsedSeconds :type "Float (double-precision)") (TriggeredSeconds :type "Float (double-precision)") (InputAction :type "InputAction Object Reference" :default "/Game/Hyper/Locomotion/Input/Swimming/IA_Dive.IA_Dive"))
  (:`Started`
    (`self.Event switch diving mode`)))

(event `EnhancedInput|/Game/Hyper/Locomotion/Input/Swimming/IA_SwimVerticalUp`
  (params (ActionValue :type "Float (double-precision)") (ElapsedSeconds :type "Float (double-precision)") (TriggeredSeconds :type "Float (double-precision)") (InputAction :type "InputAction Object Reference" :default "/Game/Hyper/Locomotion/Input/Swimming/IA_SwimVerticalUp.IA_SwimVerticalUp"))
  (:`Triggered`
    (`self.DiveMovementLogic` ActionValue)))

(event `EnhancedInput|/Game/Hyper/Locomotion/Input/Swimming/IA_SwimVerticalDown`
  (params (ActionValue :type "Float (double-precision)") (ElapsedSeconds :type "Float (double-precision)") (TriggeredSeconds :type "Float (double-precision)") (InputAction :type "InputAction Object Reference" :default "/Game/Hyper/Locomotion/Input/Swimming/IA_SwimVerticalDown.IA_SwimVerticalDown"))
  (:`Triggered`
    (`self.DiveMovementLogic` ActionValue)))

(fn `CheckIfIsUnderwater`
  (returns (`Is underwater` :type Boolean) (ImpactPoint :type "Vector Structure"))
  (bind (_returnvalue_x _returnvalue_y _returnvalue_z) (`KismetMathLibrary.BreakVector` (`SceneComponent.K2_GetComponentLocation` (`self.Breathing point reference`))))
  (bind _returnvalue (`SceneComponent.K2_GetComponentLocation` (`self.Breathing point reference`)))
  ;[0.05098 0.05098 0.05098] Only check if is swimming
  (if (`NavMovementComponent.IsSwimming` (`/Game/Hyper/Core/Generic/BlueprintMacroLibrary/BML_Generic_Component.Get Character Movement`))
    ;[0.05098 0.05098 0.05098] Trace for world dynamic. If you encounter bugs  because you use a dynamic object somewhere else while swimming to trigger this hit, you are able to add an own object type in the project "water"
    (bind (_outhit _returnvalue_2) (`KismetSystemLibrary.LineTraceSingleForObjects` (+ _returnvalue (0.0 0.0 25.0)) (+ _returnvalue (0.0 0.0 15.0)) (`|MakeArray` "ObjectTypeQuery2" :!type "EObjectTypeQuery Enum")))
    ;[0.05098 0.05098 0.05098] Only continue if there was a hit
    (if _returnvalue_2
      (bind (_bblockinghit _binitialoverlap _time _distance _location _impactpoint) (`GameplayStatics.BreakHitResult` _outhit))
      (if (> (.z _location) _returnvalue_z)
        (bind _output_get (set `self.Is underwater` true))
        (return _output_get _impactpoint)
        (else
          (bind _output_get_2 (set `self.Is underwater` false))
          (return _output_get_2 _impactpoint)))
      (else
        (bind _output_get_3 (set `self.Is underwater` false))
        (return _output_get_3 (0.0 0.0 0.0))))
    (else
      (set `self.Is underwater` false)
      (return false (0.0 0.0 0.0)))))

(fn `Create and Attach BreathingPoint Reference`
  (bind _returnvalue (`|AddComponentByClass` :`self` (`/Game/Hyper/Core/Generic/BlueprintMacroLibrary/BML_Generic_Component.Get Character`) :`Class` "/Script/Engine.SceneComponent" :`bManualAttachment` true))
  (bind _output_get (set `self.Breathing Point Reference` _returnvalue))
  (`SceneComponent.K2_AttachToComponent` _output_get (`/Game/Hyper/Core/Generic/BlueprintMacroLibrary/BML_Generic_Component.Get Character Mesh`) "head" "SnapToTarget" "SnapToTarget" "SnapToTarget" true))

(fn `DiveMovementLogic`
  (params (ScaleValue :type "Float (double-precision)"))
  (if (`self.Is Diving`)
    ;[0.05098 0.05098 0.05098] Only continue if the character is swimming
    (if (`NavMovementComponent.IsSwimming` (`/Game/Hyper/Core/Generic/BlueprintMacroLibrary/BML_Generic_Component.Get Character Movement`))
      (`Pawn.AddMovementInput` (`/Game/Hyper/Core/Generic/BlueprintMacroLibrary/BML_Generic_Component.Get Character`) (`KismetMathLibrary.GetUpVector` (`KismetMathLibrary.MakeRotator` 0.0 (.pitch (`Pawn.GetControlRotation` (`/Game/Hyper/Core/Generic/BlueprintMacroLibrary/BML_Generic_Component.Get Character`))))) (`local.ScaleValue`) false))))

(fn `OnRep_Desired Rotation`
  (`Actor.K2_SetActorRotation` (`/Game/Hyper/Core/Generic/BlueprintMacroLibrary/BML_Generic_Component.Get Character`) (`self.Desired Rotation`) true))

(fn `Set to Swimming Global Orientation`
  (bind _component (`/Game/Hyper/Core/Locomotion/BlueprintMacroLibrary/Generic/BML_ExtendedMovement_Component.Get ExtendedMovement`))
  ;[0.05127 0.05127 0.05127] Set to forward facing or strafe movement
  (if (`self.Strafe Movement swimming?`)
    (`/Game/Hyper/Core/Locomotion/Blueprints/AC_Extended_Movement_Abstract.Set to Strafe Movement` _component)
    (else
      (`/Game/Hyper/Core/Locomotion/Blueprints/AC_Extended_Movement_Abstract.Set to forward Facing Movement` _component))))

(fn `SetSmoothCharacterRotationOnStrafeMovement`
  (if (and (`self.Is in Water`) (`NavMovementComponent.IsSwimming` (`/Game/Hyper/Core/Generic/BlueprintMacroLibrary/BML_Generic_Component.Get Character Movement`)))
    (if (`self.Is not Drowned`)
      ;[0.05098 0.05098 0.05098] Only excecute on client
      (if (`Pawn.IsLocallyControlled` (`/Game/Hyper/Core/Generic/BlueprintMacroLibrary/BML_Generic_Component.Get Character`))
        ;[0.05098 0.05098 0.05098] Only continue if strafe movement is true
        (if (`self.Strafe Movement swimming?`)
          (set `self.From Rot` (`Pawn.GetControlRotation` (`/Game/Hyper/Core/Generic/BlueprintMacroLibrary/BML_Generic_Component.Get Character`)))
          (set `self.To Rot` (select `bool` (and (`NavMovementComponent.IsSwimming` (`/Game/Hyper/Core/Generic/BlueprintMacroLibrary/BML_Generic_Component.Get Character Movement`)) (`self.Is Diving`)) :`false` (`KismetMathLibrary.MakeRotator` (.roll (`self.From Rot`)) 0.0 (.yaw (`self.From Rot`))) :`true` (`self.From Rot`)))
          ;[0.05098 0.05098 0.05098] Smoothly interps to target
          (set `self.Current Control Rot` (`KismetMathLibrary.RInterpTo` (select `bool` (== (`self.Current Control Rot`) (struct) :`ErrorTolerance` 1.0) :`false` (`self.Current Control Rot`) :`true` (`self.From Rot`)) (`self.To Rot`) (`GameplayStatics.GetWorldDeltaSeconds`)))
          ;[0.05098 0.05098 0.05098] Set the rotation on the client and then replicate to server
          (`Actor.K2_SetActorRotation` (`/Game/Hyper/Core/Generic/BlueprintMacroLibrary/BML_Generic_Component.Get Character`) (`self.Current Control Rot`) false)
          (`self.ReplicateRotationToServer` (`self.Current Control Rot`) (`/Game/Hyper/Core/Generic/BlueprintMacroLibrary/BML_Generic_Component.Get Character`)))))))

(fn `Swim forward while diving`
  (params (ScaleValue :type "Float (double-precision)"))
  ;[0.05098 0.05098 0.05098] When diving mode is enabled. Make the forward vector of the camera the movement direction
  ;;[0.05098 0.05098 0.05098] Makes sure is not excevuted when not alive
  (if (`self.Is not Drowned`)
    (`Pawn.AddMovementInput` (`/Game/Hyper/Core/Generic/BlueprintMacroLibrary/BML_Generic_Component.Get Character`) (`KismetMathLibrary.GetForwardVector` (`Pawn.GetControlRotation` (`/Game/Hyper/Core/Generic/BlueprintMacroLibrary/BML_Generic_Component.Get Character`))) (`local.ScaleValue`) false)))

(fn `Swim Forward while not diving`
  (params (ScaleValue :type "Float (single-precision)"))
  (`Pawn.AddMovementInput` (`/Game/Hyper/Core/Generic/BlueprintMacroLibrary/BML_Generic_Component.Get Character`) (`KismetMathLibrary.GetForwardVector` (`KismetMathLibrary.MakeRotator` 0.0 0.0 (.yaw (`Pawn.GetControlRotation` (`/Game/Hyper/Core/Generic/BlueprintMacroLibrary/BML_Generic_Component.Get Character`))))) (`local.ScaleValue`) false))