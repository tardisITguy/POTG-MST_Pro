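; BP_Pluckable_Yield is a farming system master Blueprint for a pluckable yield, displayed as a static mesh.
; On BeginPlay it applies its stored mesh to the mesh component and sets StaticMeshSet, whose RepNotify reapplies the mesh for replication.
; A GUID getter lazily generates and caches a string ID on first request, then returns the same value.
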(event `self.ReceiveBeginPlay`
  (`StaticMeshComponent.SetStaticMesh` (`self.StaticMesh`) (`self.Static Mesh`))
  (set `self.Static mesh set` true))

(fn `Get_Guid`
  (returns (Output_Get :type String))
  ;[1 1 1] Stores the GUID if GUID is empty
  (if (> (`KismetStringLibrary.Len` (`self.GUID`)) 0)
    (return (`self.GUID`))
    (else
      (bind _output_get (set `self.GUID` (`KismetGuidLibrary.Conv_GuidToString` (`KismetGuidLibrary.NewGuid`))))
      (return _output_get))))

(fn `OnRep_Static mesh set`
  (`StaticMeshComponent.SetStaticMesh` (`self.StaticMesh`) (`self.Static Mesh`)))

(fn `UserConstructionScript`)