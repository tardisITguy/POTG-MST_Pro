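; BP_Sprinkler is an interactable farming sprinkler that players switch on or off, turning on only when HasWater is set.
; The server owns the state and registers or removes the sprinkler on BP_Farming_Abstract actors inside its sphere on toggle, overlap and destroy.
; Clients mirror IsOn in audio and particles through a RepNotify, also applied on BeginPlay for late joiners.
; A GUID is generated once on the server if empty.
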(event `self.ReceiveBeginPlay`
  (bind _is_on (`self.Is_On`))
  (`/Engine/EditorBlueprintResources/ActorMacros.Switch Has Authority`
    (:`Authority`
      ;[0.05098 0.05098 0.05098] We need to wait for the actors to be initilialized
      (`KismetSystemLibrary.DelayUntilNextTick`)
      ;[0.05098 0.05098 0.05098] At initialize, store GUID and set the sprinkler on or off and also propegate this to the overlapping farming masters
      (`self.Get GUID`)
      (set `self.Is_On` _is_on)
      (if _is_on
        (`self.Set is watered by sprinkler in sprinkler radius` true)
        (else
          (`self.Set is watered by sprinkler in sprinkler radius` false))))
    (:`Remote`
      ;[0.05098 0.05098 0.05098] On client, initialily set it on or off due to rep notify not calling when just joining (no changed state)
      (if (`self.Is_On`)
        (`ActorComponent.SetActive` (`self.Audio`) true false)
        (`ActorComponent.SetActive` (`self.ParticleSystem`) true false)
        (else
          (`ActorComponent.SetActive` (`self.ParticleSystem`) false false)
          (`ActorComponent.SetActive` (`self.Audio`) false false))))))

(event `self.Sphere.OnComponentBeginOverlap`
  (params (OverlappedComponent :type "PrimitiveComponent Object Reference") (OtherActor :type "Actor Object Reference") (OtherComp :type "PrimitiveComponent Object Reference") (OtherBodyIndex :type Integer) (bFromSweep :type Boolean) (SweepResult :type "HitResult Structure (by ref)"))
  ;[0.05098 0.05098 0.05098] When new farmables are getting placed, check again to set sprinkler to true
  (if (`self.Is_On`)
    (`self.Set is watered by sprinkler in sprinkler radius` true)))

(event `Switch On/Of Sprinkler`
  ;[0.05098 0.05098 0.05098] Check if the sprinkler is on. If so, turn of.
  ; If trying to turn on, check first if the sprinkler has water. If not, don't do anything.
  ;
  ; The "has water" can be used for things like a storage of water, or is it connected to an automated system, is there water in the pipes or whatever implementation you desire
  (`/Engine/EditorBlueprintResources/ActorMacros.Switch Has Authority` :!label _label
    (:`Authority`
      (if (`self.Is_On`)
        (set `self.Is_On` false)
        ;;[1 1 1] Check all in radius to switch is watered by this sprinkler
        (`self.Set is watered by sprinkler in sprinkler radius` false)
        (elif (`self.Has_Water`)
          (set `self.Is_On` true)
          (`self.Set is watered by sprinkler in sprinkler radius` true))))))

(event `/Game/Hyper/Core/Interaction/Interfaces/BPI_Interact.Interact`
  (params (`Owning Controller` :type "Controller Object Reference"))
  (goto _label))

(event `Destroy`
  ;[0.05098 0.05098 0.05098] If destroy, set is watered by sprinkler to false so the reference gets removed by linked farming masters
  (`self.Set is watered by sprinkler in sprinkler radius` false))

(fn `Can Interact`
  (params (`Owning Controller` :type "Controller Object Reference"))
  (returns (True :type Boolean))
  (return true))

(fn `Get GUID`
  (returns (Output_Get :type String))
  ;[1 1 1] Stores the GUID if GUID is empty
  (if (> (`KismetStringLibrary.Len` (`self.GUID`)) 0)
    (return (`self.GUID`))
    (else
      (bind _output_get (set `self.GUID` (`KismetGuidLibrary.Conv_GuidToString` (`KismetGuidLibrary.NewGuid`))))
      (return _output_get))))

(fn `Get Interact Animation`
  (params (`Owning Controller` :type "Controller Object Reference"))
  (returns (`Anim Montage` :type "AnimMontage Object Reference"))
  (return (`/Game/Hyper/Core/Interaction/FunctionLibraries/BFL_Interaction.Select Interaction Animation` `Owning Controller` (`self.Anim Montage Left`) (`self.Anim Montage Right`))))

(fn `Get Interact Sound`
  (returns (`Interact Sound` :type "SoundBase Object Reference"))
  (return null))

(fn `Get Interact Text`
  (params (`Owning Controller` :type "PlayerController Object Reference"))
  (returns (`Interact Text` :type Text) (`Secondary Interact Text` :type Text))
  (return (select `bool` (`self.Has_Water`) :`false` (`self.No Water Text`) :`true` (select `bool` (`self.Is_On`) :`false` (`self.Interact Text Off`) :`true` (`self.Interact Text On`))) ""))

(fn `Get Relative Interact Text Location`
  (returns (`Relative Location` :type "Vector Structure"))
  (return (`self.Relative Location`)))

(fn `OnRep_Is_On`
  (if (`self.Is_On`)
    (`ActorComponent.SetActive` (`self.Audio`) true false)
    (`ActorComponent.SetActive` (`self.ParticleSystem`) true false)
    (else
      (`ActorComponent.SetActive` (`self.ParticleSystem`) false false)
      (`ActorComponent.SetActive` (`self.Audio`) false false))))

(fn `Set is watered by sprinkler in sprinkler radius`
  (params (`Is watered by sprinkler` :type Boolean))
  (for _array_element (`PrimitiveComponent.GetOverlappingActors` (`self.Sphere`) "/Game/Hyper/Core/FarmingSystem/Blueprints/BP_Farming_Abstract.BP_Farming_Abstract_C")
    (bind _asbp_farming_abstract (cast `/Game/Hyper/Core/FarmingSystem/Blueprints/BP_Farming_Abstract` _array_element))
    (if `Is watered by sprinkler`
      (`/Game/Hyper/Core/FarmingSystem/Blueprints/BP_Farming_Abstract.Add Active sprinkler` _asbp_farming_abstract self)
      (else
        (`/Game/Hyper/Core/FarmingSystem/Blueprints/BP_Farming_Abstract.Remove Active sprinkler` _asbp_farming_abstract self))))
  (return))

(fn `Should get other Actor to Interact with`
  (params (`Based on this Component` :type "PrimitiveComponent Object Reference"))
  (returns (True :type Boolean) (`Actor To Interact With` :type "Actor Object Reference"))
  (return false null))

(fn `Should server control the interact`
  (returns (`Server should excecute interact call` :type Boolean))
  (return true))

(fn `UserConstructionScript`)