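; Player farming component that handles looking at, tending and restoring BP_Farming_Abstract plants.
; A looping camera trace shows the stat bar only on the farmable in view.
; Equipment manager events handle cure, water and fertilizer attempts, with camera traces passing the hit actor to server events that message it.
; On load, the server respawns non-manually-placed plants from the FarmSave slot, then relinks their pluckable yields by GUID.
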(event `self.ReceiveBeginPlay`
  ;[1 1 1] Load farming
  (`self.Load Farming`)
  (`self.Initialize Equipment Binds`)
  (`self.Start Farming Trace`))

(event `Initialize Equipment Binds`
  (bind (_equipment _is_valid) (`/Game/Hyper/Core/Equipment_Manager/BlueprintMacroLibrary/BML_Equipment_Component.Get Equipment Manager`))
  ;[0.05127 0.05127 0.05127] Assign events from equipmentmanager. The equipment manager determines if we want to try one of these events
  (if _is_valid
    (add `/Game/Hyper/Core/Equipment_Manager/Blueprints/AC_Equipment_Manager_Abstract.Try Cure Plant` _equipment (`|CreateDelegate` :!event `Initialize Try Cure Plant`))
    (add `/Game/Hyper/Core/Equipment_Manager/Blueprints/AC_Equipment_Manager_Abstract.Try Add Water` _equipment (`|CreateDelegate` :!event `Initialize Try add Water`))
    (add `/Game/Hyper/Core/Equipment_Manager/Blueprints/AC_Equipment_Manager_Abstract.Try Add Fertilizer` _equipment (`|CreateDelegate` :!event `Initialize Try add Fertilizer`))))

(event `Event: Spawn Plants from save`
  (`self.Spawn_Plants_From_Save`))

(event `Load Farming_1`
  (if (and (`KismetSystemLibrary.IsServer`) (`Pawn.IsControlled` (`/Game/Hyper/Core/Generic/BlueprintMacroLibrary/BML_Generic_Component.Get Character`)))
    (`/Engine/EditorBlueprintResources/StandardMacros.IsValid` (`GameplayStatics.GetPlayerCharacter` 0) :!label _label
      (:`Is Valid`
        (`self.Event: Spawn Plants from save`)))
    (elif (`KismetSystemLibrary.IsDedicatedServer`)
      (goto _label))))

(event `self.Initialize Try Cure Plant`
  (bind _asplayer_controller (`/Game/Hyper/Core/Generic/BlueprintMacroLibrary/BML_Generic_Component.Get Player Controller`))
  (bind (_outhit _hit _hitactor) (`/Game/Hyper/Core/Generic/FunctionLibraries/BFL_Generic.Trace From Active Camera` _asplayer_controller "TraceTypeQuery3" (`|MakeArray` (`/Game/Hyper/Core/Generic/BlueprintMacroLibrary/BML_Generic_Component.Get Character`) :!type "Actor Object Reference")))
  ;[0.07888 1 0] All interactions with the plants. All logic is done on the server
  ; When try to peform the action, do a simple trace forward and check if there is a hit and use the farmable interface
  (if _hit
    (`self.Server Try Cure Plan` _hitactor _asplayer_controller)))

(event `Server Try Cure Plan`
  (params (`Target Farmeable` :type "Object Object Reference") (`Instrigating Controller` :type "PlayerController Object Reference"))
  ;[0.07888 1 0] All interactions with the plants. All logic is done on the server
  ; When try to peform the action, do a simple trace forward and check if there is a hit and use the farmable interface
  (message `/Game/Hyper/Core/FarmingSystem/Interfaces/BPI_Farming.Try_Cure_Plant` `Target Farmeable` `Instrigating Controller`))

(event `Server Try add Fertilizer`
  (params (`Target Farmeable` :type "Object Object Reference") (`Instrigating Controller` :type "PlayerController Object Reference"))
  ;[0.07888 1 0] All interactions with the plants. All logic is done on the server
  ; When try to peform the action, do a simple trace forward and check if there is a hit and use the farmable interface
  (message `/Game/Hyper/Core/FarmingSystem/Interfaces/BPI_Farming.Try_Add_Fertilizer` `Target Farmeable` 25.0 `Instrigating Controller`))

(event `self.Initialize Try add Fertilizer`
  (bind _asplayer_controller (`/Game/Hyper/Core/Generic/BlueprintMacroLibrary/BML_Generic_Component.Get Player Controller`))
  (bind (_outhit _hit _hitactor) (`/Game/Hyper/Core/Generic/FunctionLibraries/BFL_Generic.Trace From Active Camera` _asplayer_controller "TraceTypeQuery3" (`|MakeArray` (`/Game/Hyper/Core/Generic/BlueprintMacroLibrary/BML_Generic_Component.Get Character`) :!type "Actor Object Reference")))
  ;[0.07888 1 0] All interactions with the plants. All logic is done on the server
  ; When try to peform the action, do a simple trace forward and check if there is a hit and use the farmable interface
  (if _hit
    (`self.Server Try add Fertilizer` _hitactor _asplayer_controller)))

(event `Server Try add Water`
  (params (`Target Farmeable` :type "Object Object Reference") (`Instrigating Controller` :type "PlayerController Object Reference"))
  ;[0.07888 1 0] All interactions with the plants. All logic is done on the server
  ; When try to peform the action, do a simple trace forward and check if there is a hit and use the farmable interface
  (message `/Game/Hyper/Core/FarmingSystem/Interfaces/BPI_Farming.Try_Add_Water` `Target Farmeable` 25.0 `Instrigating Controller`))

(event `self.Initialize Try add Water`
  (bind _asplayer_controller (`/Game/Hyper/Core/Generic/BlueprintMacroLibrary/BML_Generic_Component.Get Player Controller`))
  (bind (_outhit _hit _hitactor) (`/Game/Hyper/Core/Generic/FunctionLibraries/BFL_Generic.Trace From Active Camera` _asplayer_controller "TraceTypeQuery3" (`|MakeArray` (`/Game/Hyper/Core/Generic/BlueprintMacroLibrary/BML_Generic_Component.Get Character`) :!type "Actor Object Reference")))
  ;[0.07888 1 0] All interactions with the plants. All logic is done on the server
  ; When try to peform the action, do a simple trace forward and check if there is a hit and use the farmable interface
  (if _hit
    (`self.Server Try add Water` _hitactor _asplayer_controller)))

(event `Start Farming Trace`
  ;[0.05098 0.05098 0.05098] Trace for the farmable that you're looking at and only activate that widget
  (`KismetSystemLibrary.K2_SetTimerDelegate` (delegate `Farming Trace Tick`) 0.1 true))

(event `Farming Trace Tick`
  (bind (_outhit _hit _hitactor) (`/Game/Hyper/Core/Generic/FunctionLibraries/BFL_Generic.Trace From Active Camera` (`/Game/Hyper/Core/Generic/BlueprintMacroLibrary/BML_Generic_Component.Get Player Controller`) "TraceTypeQuery3"))
  ;[0.05098 0.05098 0.05098] Trace for the farmable that you're looking at and only activate that widget
  (if _hit
    (`self.Looking At Farmable`
      (:`then`
        (if (== _hitactor (`self.Looking At Farmable`))
          (bind _asbp_farming_abstract (cast `/Game/Hyper/Core/FarmingSystem/Blueprints/BP_Farming_Abstract` _hitactor :!label _label))
          (`|ExecutionSequence`
            (:`then_0`
              (bind _looking_at_farmable (`self.Looking At Farmable` :!label _label_2)
                (:`then`
                  (`/Game/Hyper/Core/FarmingSystem/Blueprints/BP_Farming_Abstract.Set Statbar Visibility based on full health` _looking_at_farmable false true)
                  (set `self.Looking At Farmable` null))
                (:`else`)))
            (:`then_1`
              (bind _output_get (set `self.Looking At Farmable` _asbp_farming_abstract))
              (`/Game/Hyper/Core/FarmingSystem/Blueprints/BP_Farming_Abstract.Set Statbar Visibility based on full health` _output_get true false)))
          (else
            (goto _label_2))))
      (:`else`
        (goto _label)))
    (else
      (goto _label_2))))

(fn `Spawn_Plants_From_Save`
  (locals (`Local Save` :type "/Game/Hyper/FarmingSystem/Save/BP_Save_Plants Object Reference") (`Local  Spawned Plants` :type "Array of /Game/Hyper/Core/FarmingSystem/Blueprints/BP_Farming_Abstract Object Reference") (Local_GUID_To_Actor :type "Map of String to Actor Object Reference"))
  (bind _returnvalue (`GameplayStatics.DoesSaveGameExist` "FarmSave"))
  (if _returnvalue
    (bind _returnvalue_2 (`GameplayStatics.LoadGameFromSlot` "FarmSave"))
    (bind _asbp_save_plants (cast `/Game/Hyper/FarmingSystem/Save/BP_Save_Plants` _returnvalue_2))
    (set `local.Local Save` _asbp_save_plants)
    (for _array_element (`/Game/Hyper/FarmingSystem/Save/BP_Save_Plants.Plants` _asbp_save_plants)
      (bind (_guid_farmable _plantdatatablerow _transform _currentdurabilityfarmable _is_regrowing _can_be_harvested _current_growth_stage _current_growth_time _currentamountoffertilizer _currentamountofwater _is_destructed _current_decay_time _is_decayed _is_decaying _is_sick _fertilizerconsumed _linkedpluckableyield _current_growth_percentage _actor _ismanuallyplacedinworld) (break `/Game/Hyper/FarmingSystem/Save/Struct_Saved_Plants` _array_element))
      (if (not _ismanuallyplacedinworld)
        (bind _asbp_farming_abstract (castclass `/Game/Hyper/Core/FarmingSystem/Blueprints/BP_Farming_Abstract` _actor))
        (bind _returnvalue_3 (`|SpawnActorFromClass` :`Class` _asbp_farming_abstract :`SpawnTransform` _transform :`CollisionHandlingOverride` "AlwaysSpawn" :`TransformScaleMethod` "SelectDefaultAtRuntime" :`Current_Growth_Time` _current_growth_time :`Current_Growth_Stage` _current_growth_stage :`Current_Growth_Percentage` _current_growth_percentage :`Plant` _plantdatatablerow :`Can_Be_Harvested` _can_be_harvested :`Is_Regrowing` _is_regrowing :`Is_Farmable_Destructed` _is_destructed :`Current_Durability_Farmable` _currentdurabilityfarmable :`GUID_Farmable` _guid_farmable :`Current_Decay_Time` _current_decay_time :`Current Amount of Fertilizer` _currentamountoffertilizer :`Current Amount of Water` _currentamountofwater :`Is_Decayed` _is_decayed :`Is_Sick` _is_sick :`Is_Decaying` _is_decaying :`Fertilizer Consumed` _fertilizerconsumed :`Linked_Pluckable_Yield_GUIDS` _linkedpluckableyield :`Is_Farmable_Spawned_From_Save` true :`Is Manually placed in world` _ismanuallyplacedinworld :`Password` "0000" :`Build By Player` null :`Instigator` null))
        (`BlueprintMapLibrary.Map_Add` (`local.Local_GUID_To_Actor`) _guid_farmable _returnvalue_3)
        (`KismetArrayLibrary.Array_Add` (`local.Local  Spawned Plants`) _returnvalue_3)))
    (for _array_element_2 (`local.Local  Spawned Plants`)
      (for _array_element_3 (`/Game/Hyper/Core/FarmingSystem/Blueprints/BP_Farming_Abstract.Linked_Pluckable_Yield_GUIDS` _array_element_2)
        (bind (_value _returnvalue_4) (`BlueprintMapLibrary.Map_Find` (`local.Local_GUID_To_Actor`) _array_element_3))
        (if _returnvalue_4
          (`KismetArrayLibrary.Array_Add` (`/Game/Hyper/Core/FarmingSystem/Blueprints/BP_Farming_Abstract.Linked_Pluckable_Yield` _array_element_2) _value))))))