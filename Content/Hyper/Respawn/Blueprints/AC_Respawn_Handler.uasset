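; Respawn handler component that adds an open-world or arena respawn component to its owner by game type and respawns players.
; SpawnPlayer caches inventory, spawn locations and arena spawn type, destroys the old pawn to avoid overlaps, then spawns and possesses that game type's character.
; It restores the cached data, with inventory only if KeepInventory is set.
; It manually reinitializes interaction, equipment, UI and inventory managers to rebind references, inputs and HUD.
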(event `Initialize Game Mode`
  (bind _returnvalue (`self.GetOwner`))
  ;[0.05098 0.05098 0.05098] Add the second respawn component based on the game type
  (switch `/Game/Hyper/Core/Respawn/Datamodel/Enumerations/Enum_Game_Type` (`self.Game Type`)
    (:`NewEnumerator0`
      (`|AddComponentByClass` _returnvalue "/Game/Hyper/Respawn/Blueprints/OpenWorldRespawn/AC_Respawn_GameMode_OpenWorld.AC_Respawn_GameMode_OpenWorld_C"))
    (:`NewEnumerator1`
      (`|AddComponentByClass` _returnvalue "/Game/Hyper/Respawn/Blueprints/ArenaRespawn/AC_Respawn_GameMode_Arena.AC_Respawn_GameMode_Arena_C" :!label _label))
    (:`NewEnumerator2`
      (goto _label))))

(fn `Get Player By Game Type`
  (returns (Character :type "Character Class Reference"))
  (switch `/Game/Hyper/Core/Respawn/Datamodel/Enumerations/Enum_Game_Type` (`self.Game Type`)
    (:`NewEnumerator0`
      (return (`self.Open World Character`)))
    (:`NewEnumerator1`
      (return (`self.Team Character`)))
    (:`NewEnumerator2`
      (return (`self.Free For All Character`)))))

(fn `Spawn Player`
  (params (`Player Controller` :type "PlayerController Object Reference") (`Spawn Location` :type "Transform Structure"))
  (locals (`Old Inventory` :type "Array of /Game/Hyper/Core/Inventory/Datamodel/Structures/Main_Item_Slot_Structs/Struct_Inventory_Slot_Item Structure") (`Old Respawn Locations` :type "Array of /Game/Hyper/Core/Respawn/Blueprints/AC_Respawn_Location_Abstract Object Reference") (`Old Spawn Type` :type "/Game/Hyper/Core/Respawn/Datamodel/Enumerations/Enum_Player_Spawn_Type Enum"))
  (bind _returnvalue (`Controller.K2_GetPawn` `Player Controller`))
  (bind _component (`/Game/Hyper/Core/Inventory/BlueprintMacroLibrary/BML_Inventory_Controller.Get Inventory Manager` `Player Controller`))
  (bind _component_2 (`/Game/Hyper/Core/Respawn/BlueprintMacroLibrary/BML_Respawn_Controller.Get Respawn Manager` `Player Controller`))
  (bind _player_controller (`local.Player Controller`))
  (bind _component_3 (`/Game/Hyper/Core/Interaction/BlueprintMacroLibrary/BML_Interact_Controller.Get Interact Manager` (`local.Player Controller`)))
  (bind _component_4 (`/Game/Hyper/Core/Respawn/BlueprintMacroLibrary/BML_Respawn_Controller.Get Respawn Manager` (`local.Player Controller`)))
  (`/Engine/EditorBlueprintResources/StandardMacros.IsValid` _returnvalue
    (:`Is Valid`
      (`/Engine/EditorBlueprintResources/StandardMacros.IsValid` _component
        (:`Is Valid`
          (set `local.Old Inventory` (`/Game/Hyper/Core/Inventory/Blueprints/AC_Inventory_Abstract.Inventory Slots` _component)))
        (:`Is Not Valid`
          _))
      (`/Engine/EditorBlueprintResources/StandardMacros.IsValid` _component_2
        (:`Is Valid`
          (set `local.Old Respawn Locations` (`/Game/Hyper/Core/Respawn/Blueprints/AC_Respawn_Manager_Abstract.Spawn Locations` _component_2)))
        (:`Is Not Valid`
          _))
      (bind _asac_respawn_manager_arena (cast `/Game/Hyper/Respawn/Blueprints/ArenaRespawn/AC_Respawn_Manager_Arena` _component_2)
        (:`then`
          (set `local.Old Spawn Type` (`/Game/Hyper/Core/Respawn/Blueprints/AC_Respawn_Manager_Abstract.Spawn Type` _asac_respawn_manager_arena)))
        (:`CastFailed`
          _))
      ;[0.05098 0.05098 0.05098] We're destroying the old actor before spawning in the new one. This is because otherwise it could cause overlapping errors
      (`Actor.K2_DestroyActor` _returnvalue))
    (:`Is Not Valid`
      _))
  (bind _character (`self.Get Player By Game Type`))
  (bind _returnvalue_2 (`|SpawnActorFromClass` _character (`KismetMathLibrary.MakeTransform` (.location `Spawn Location`) (.rotation `Spawn Location`)) "AdjustIfPossibleButAlwaysSpawn" "MultiplyWithRoot" null null))
  (`Controller.Possess` (`local.Player Controller`) _returnvalue_2)
  ;[0.05098 0.05098 0.05098] We initialize the interaction system again. This is because the objects that are interacted with have a reference to the old interaction component
  (`/Engine/EditorBlueprintResources/StandardMacros.IsValid` _component_3
    (:`Is Valid`
      (`/Game/Hyper/Core/Interaction/Blueprints/AC_Interact_Abstract.Initialize` _component_3))
    (:`Is Not Valid`
      _))
  ;[0.05098 0.05098 0.05098] Keep the respawn location data
  (set `/Game/Hyper/Core/Respawn/Blueprints/AC_Respawn_Manager_Abstract.Spawn Locations` (`local.Old Respawn Locations`) _component_4)
  ;[0.05098 0.05098 0.05098] We transfer the inventory from the old character to the new one if wanted.
  (if (`/Game/Hyper/Core/Respawn/Blueprints/AC_Respawn_Manager_Abstract.Keep Inventory` _component_4)
    (`self.Transfer Inventory Items to New Player` (`local.Old Inventory`) (`/Game/Hyper/Core/Inventory/BlueprintMacroLibrary/BML_Inventory_Controller.Get Inventory Manager` (`local.Player Controller`))))
  ;[0.05098 0.05098 0.05098] If the respawn manager is from an arena, we want to set the saved spawn type
  (bind _asac_respawn_manager_arena_2 (cast `/Game/Hyper/Respawn/Blueprints/ArenaRespawn/AC_Respawn_Manager_Arena` (`/Game/Hyper/Core/Respawn/BlueprintMacroLibrary/BML_Respawn_Controller.Get Respawn Manager` (`local.Player Controller`)))
    (:`then`
      (`/Game/Hyper/Core/Respawn/Blueprints/AC_Respawn_Manager_Abstract.Set Spawn Type` _asac_respawn_manager_arena_2 (`local.Old Spawn Type`)))
    (:`CastFailed`
      _))
  ;[0.05098 0.05098 0.05098] Initialize the starting equipment manually. We do this because the player doesn't have a local controller when spawned.
  (`/Engine/EditorBlueprintResources/StandardMacros.IsValid` (`/Game/Hyper/Core/Generic/BlueprintMacroLibrary/BML_Generic_ControllerInput.Get Character` _player_controller)
    (:`Is Valid`
      (`/Game/Hyper/Core/Equipment_Manager/Blueprints/AC_Equipment_Manager_Abstract.Client: Reinitialize` (`/Game/Hyper/Core/Equipment_Manager/BlueprintMacroLibrary/BML_Equipment_Controller.Get Equipment Manager` _player_controller))
      ;[0.05098 0.05098 0.05098] Reinitializing the UI manager to recouple the inputs and HUD
      (`/Game/Hyper/UI/Blueprints/ActorComponents/AC_UI_Manager_Abstract.Reinitialize` (`/Game/Hyper/UI/Blueprints/BlueprintMacroLibrary/BML_UI_Manager_Controller.Get UI Manager ` (`local.Player Controller`)))
      ;[0.05098 0.05098 0.05098] Reinitializing the Inventory Manager to recouple the inputs
      (`/Game/Hyper/Core/Inventory/Blueprints/AC_Inventory_Abstract.Client: Reinitialize` (`/Game/Hyper/Core/Inventory/BlueprintMacroLibrary/BML_Inventory_Controller.Get Inventory Manager` (`local.Player Controller`))))))

(fn `Transfer Inventory Items To New Player`
  (params (Array :type "Array of /Game/Hyper/Core/Inventory/Datamodel/Structures/Main_Item_Slot_Structs/Struct_Inventory_Slot_Item Structure") (Target :type "/Game/Hyper/Core/Inventory/Blueprints/AC_Inventory_Abstract Object Reference"))
  (for _array_element Array
    (`/Game/Hyper/Core/Inventory/Blueprints/AC_Inventory_Abstract.Try Add Item to Inventory Automatically` Target _array_element (`/Game/Hyper/Core/Inventory/Blueprints/AC_Inventory_Abstract.Inventory Slots` Target) false 0 true false false)))