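; Game mode component that handles open-world respawning, letting players pick a spawn zone before spawning.
; On initialization it caches zone-flagged respawn location actors once, then places a temporary dummy character at a random start camera view actor.
; The controller possesses that dummy, which receives a respawn manager component to show the selection UI.
; A lookup returns a random spawn transform among cached locations matching the chosen zone type.
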(fn `Get Random Spawn Location`
  (params (InputPin :type "/Game/Hyper/Core/Respawn/Datamodel/Enumerations/Enum_Zone_Name Enum" :default "NewEnumerator0"))
  (returns (`Spawn Transform` :type "Transform Structure"))
  (locals (`Possible Spawn Locations` :type "Array of /Game/Hyper/Respawn/Blueprints/OpenWorldRespawn/BP_Respawn_Location_OpenWorld Object Reference"))
  (bind _returnvalue (`KismetArrayLibrary.Array_Length` (`local.Possible Spawn Locations`)))
  ;[0.05098 0.05098 0.05098] Create a list of spawn locations that are valid for the pressed button
  (for _array_element (`self.Zone Spawn Locations`)
    (if (`|EnumEquality` InputPin (`/Game/Hyper/Respawn/Blueprints/OpenWorldRespawn/AC_Respawn_Location_OpenWorld.Respawn Zone Type` (`/Game/Hyper/Respawn/Blueprints/OpenWorldRespawn/BP_Respawn_Location_OpenWorld.AC_Respawn_Location_OpenWorld` _array_element)))
      (`KismetArrayLibrary.Array_Add` (`local.Possible Spawn Locations`) _array_element)))
  ;[0.05098 0.05098 0.05098] Choose a random spawn location from your type
  (if (> _returnvalue 0)
    (return (`/Game/Hyper/Core/Respawn/Blueprints/AC_Respawn_Location_Abstract.Get Respawn Transform` (`/Game/Hyper/Respawn/Blueprints/OpenWorldRespawn/BP_Respawn_Location_OpenWorld.AC_Respawn_Location_OpenWorld` (`|GetArrayItem` (`local.Possible Spawn Locations`) (`KismetMathLibrary.RandomIntegerInRange` 0 (- _returnvalue 1))))))
    (else
      (`KismetSystemLibrary.PrintString` "No spawn location available of selected type"))))

(fn `Initialize Spawn`
  (params (`Player Controller` :type "PlayerController Object Reference") (`Game Type` :type "/Game/Hyper/Core/Respawn/Datamodel/Enumerations/Enum_Game_Type Enum" :default "NewEnumerator0"))
  (locals (`Dummy Transform` :type "Transform Structure" :default "0.000000,0.000000,500.000000|0.000000,0.000000,0.000000|1.000000,1.000000,1.000000"))
  (if (not (`self.Zone Locations Loaded`))
    (`self.Save Spawn Locations`))
  ;[0.05127 0.05127 0.05127] Determine start location view
  (bind _outactors (`GameplayStatics.GetAllActorsOfClass` "/Game/Hyper/Respawn/Blueprints/OpenWorldRespawn/BP_StartCameraViewOnStart.BP_StartCameraViewOnStart_C"))
  (if (`KismetArrayLibrary.Array_IsEmpty` _outactors)
    (`KismetSystemLibrary.PrintString` "No Start Camera view actor in the world. Will choose spawn location screen 0,0,0" false)
    (else
      (set `local.Dummy Transform` (`Actor.GetTransform` (`KismetArrayLibrary.Array_Random` _outactors)))))
  ;[0.05098 0.05098 0.05098] We're spawning a temporary character when open world. This way we can show the UI for respawning.
  (bind _returnvalue (`|SpawnActorFromClass` "/Game/Hyper/Respawn/Blueprints/BP_DummyChar_SpawnPointSelection.BP_DummyChar_SpawnPointSelection_C" (`local.Dummy Transform`) "AdjustIfPossibleButAlwaysSpawn" "MultiplyWithRoot" null null))
  (`Controller.Possess` (`local.Player Controller`) _returnvalue)
  (bind _returnvalue_2 (`|AddComponentByClass` _returnvalue "/Game/Hyper/Respawn/Blueprints/OpenWorldRespawn/AC_Respawn_Manager_OpenWorld.AC_Respawn_Manager_OpenWorld_C"))
  (`/Game/Hyper/Core/Respawn/Blueprints/AC_Respawn_Manager_Abstract.Initialize Respawn UI` _returnvalue_2))

(fn `Save Spawn Locations`
  (bind _outactors (`GameplayStatics.GetAllActorsOfClass` "/Game/Hyper/Respawn/Blueprints/OpenWorldRespawn/BP_Respawn_Location_OpenWorld.BP_Respawn_Location_OpenWorld_C"))
  (for _array_element _outactors
    (if (`/Game/Hyper/Respawn/Blueprints/OpenWorldRespawn/AC_Respawn_Location_OpenWorld.Is Part Of Zone` (`/Game/Hyper/Respawn/Blueprints/OpenWorldRespawn/BP_Respawn_Location_OpenWorld.AC_Respawn_Location_OpenWorld` _array_element))
      (`KismetArrayLibrary.Array_Add` (`self.Zone Spawn Locations`) _array_element)))
  (set `self.Zone Locations Loaded` true))