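; Loot bag actor for the open-world respawn system that fills its inventory from InventoryItems and despawns after DespawnTime.
; The server starts the despawn timer on BeginPlay, and interacting pauses it, with interaction blocked in the final second to avoid timing issues.
; A client-side binding to the HUD's interact widget closing has AC_Respawn_Manager_OpenWorld resume the timer and destroy the bag if empty.
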(event `self.ReceiveBeginPlay`
  (bind _ac_inventory_advanced (`self.AC_Inventory_Advanced`))
  (`parent.ReceiveBeginPlay`)
  ;[0.05098 0.05098 0.05098] Add all of the given items to the inventory of the loot bag.
  (for _array_element (`self.Inventory Items`)
    (if (not (`/Game/Hyper/Core/Inventory/FunctionLibraries/BFL_InventoryCrafting.Is Item Empty?` _array_element))
      (`/Game/Hyper/Core/Inventory/Blueprints/AC_Inventory_Abstract.Try Add Item to Inventory Automatically` _ac_inventory_advanced _array_element (`/Game/Hyper/Core/Inventory/Blueprints/AC_Inventory_Abstract.Inventory Slots` _ac_inventory_advanced) false 0 true false false)))
  ;[0.05098 0.05098 0.05098] We're creating a timer for the lootbag. When this timer is over, we destroy the object.
  (`/Engine/EditorBlueprintResources/ActorMacros.Switch Has Authority`
    (:`Authority`
      (bind _returnvalue (`KismetSystemLibrary.K2_SetTimerDelegate` (delegate `On Timer Finished`) (`self.Despawn Time`)))
      (set `self.Timer Handle` _returnvalue))))

(event `On Timer Finished`
  ;[0.05098 0.05098 0.05098] We're creating a timer for the lootbag. When this timer is over, we destroy the object.
  (`self.K2_DestroyActor`))

(event `/Game/Hyper/Core/Interaction/Interfaces/BPI_Interact.Interact`
  (params (`Owning Controller` :type "Controller Object Reference"))
  (if (not (<= (`KismetSystemLibrary.K2_GetTimerRemainingTimeHandle` (`self.Timer Handle`)) 1.0))
    (`parent.Interact` `Owning Controller`)
    (`KismetSystemLibrary.K2_PauseTimerHandle` (`self.Timer Handle`))
    (`self.Bind On Disable Interact Location Widget` `Owning Controller`)))

(event `On Disable Interact Location Widget_Event`
  (remove `/Game/Hyper/UI/Blueprints/HUD/HUD_Abstract.On Disable Interact Location Widget` (`/Game/Hyper/UI/Blueprints/BlueprintMacroLibrary/BML_HUD_Controller.Get HUD` (stale `Bind On Disable Interact Location Widget` Controller)) (delegate `On Disable Interact Location Widget_Event`))
  (bind (_component _is_valid) (`/Game/Hyper/Core/Respawn/BlueprintMacroLibrary/BML_Respawn_Controller.Get Respawn Manager` (stale `Bind On Disable Interact Location Widget` Controller)))
  (bind (_asac_respawn_manager_open_world _bsuccess) (cast `/Game/Hyper/Respawn/Blueprints/OpenWorldRespawn/AC_Respawn_Manager_OpenWorld` _component :!pure true))
  (if (and _bsuccess _is_valid)
    (`/Game/Hyper/Respawn/Blueprints/OpenWorldRespawn/AC_Respawn_Manager_OpenWorld.Unpause Lootbag Timer` _asac_respawn_manager_open_world self)
    (if (`/Game/Hyper/Core/Inventory/FunctionLibraries/BFL_InventoryCrafting.Is Inventory Array Empty` (`/Game/Hyper/Core/Inventory/Blueprints/AC_Inventory_Abstract.Inventory Slots` (`self.AC_Inventory_Advanced`)))
      (`/Game/Hyper/Respawn/Blueprints/OpenWorldRespawn/AC_Respawn_Manager_OpenWorld.Destroy Lootbag` _asac_respawn_manager_open_world self))))

(event `Bind On Disable Interact Location Widget`
  (params (Controller :type "Controller Object Reference"))
  (add `/Game/Hyper/UI/Blueprints/HUD/HUD_Abstract.On Disable Interact Location Widget` (`/Game/Hyper/UI/Blueprints/BlueprintMacroLibrary/BML_HUD_Controller.Get HUD` Controller) (delegate `On Disable Interact Location Widget_Event`)))

(fn `UserConstructionScript`
  (`parent.UserConstructionScript`))