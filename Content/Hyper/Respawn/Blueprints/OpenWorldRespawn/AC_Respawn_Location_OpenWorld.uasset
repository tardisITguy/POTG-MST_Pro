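; Actor component that marks its owner as an open-world respawn location, supplying the spawn transform from the owner's capsule, or the actor transform as fallback.
; Deactivating it starts a looping timer that counts down the respawn timeout and reactivates it once, with every state change broadcast.
; It also tracks authorised players by unique ID, optionally limiting the location to a single player.
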(event `self.Set Active`
  (params (`New Active` :type Boolean))
  ;[0.05098 0.05098 0.05098] Active a timer when event is called. This timer will handle the time left for that location to be active
  (bind _output_get (set `self.Is Active` `New Active`))
  (`self.On Set Active` _output_get self)
  (if _output_get
    ;[0.05098 0.05098 0.05098] When active we clear the timer so it can be set again later.
    (`KismetSystemLibrary.K2_ClearAndInvalidateTimerHandle` (`self.Timer Handle`))
    (set `self.Respawn Time` 0.0)
    (`self.Reset Respawn Timeout`)
    (else
      ;;[0.05098 0.05098 0.05098] When the location is set to not active, we start a timer.
      (bind _returnvalue (`KismetSystemLibrary.K2_SetTimerDelegate` (delegate `Respawn Timer`) 0.01 true))
      (set `self.Timer Handle` _returnvalue)
      (set `self.Respawn Time` (`self.Respawn Timeout`)))))

(event `Respawn Timer`
  ;[0.05098 0.05098 0.05098] Activate this respawn location when the time is finished.
  (bind _output_get (set `self.Respawn Time` (- (`self.Respawn Time`) 0.01)))
  (if (<= _output_get 0.0)
    (`/Engine/EditorBlueprintResources/StandardMacros.DoOnce` false :!label _label
      (:`Completed`
        (`self.Set Active` true)))))

(event `Reset Respawn Timeout`
  ;[0.05098 0.05098 0.05098] Activate this respawn location when the time is finished.
  (goto _label :!via `Reset`))

(fn `Add or Remove Authorised Player`
  (params (Controller :type "Controller Object Reference") (`Use Authorisation Check` :type Boolean :default true) (Add :type Boolean :default true))
  (returns (`Player Added Or Removed` :type Boolean))
  (bind _returnvalue (`PlayerState.BP_GetUniqueId` (`Controller.PlayerState` Controller)))
  ;[0.05098 0.05098 0.05098] Add unique player to the authorised list
  (if Add
    (if `Use Authorisation Check`
      (if (> (`KismetArrayLibrary.Array_Length` (`self.Authorised Players`)) 0)
        (if (`self.Can Have Multiple Authorised Players`)
          _
          (else
            (return false)))))
    (`KismetArrayLibrary.Array_AddUnique` (`self.Authorised Players`) _returnvalue)
    (return true)
    (else
      ;[0.05098 0.05098 0.05098] Remove player from list
      (bind _returnvalue_2 (`KismetArrayLibrary.Array_RemoveItem` (`self.Authorised Players`) _returnvalue))
      (return _returnvalue_2))))

(fn `Get Respawn Transform`
  (returns (`Spawn Transform` :type "Transform Structure"))
  (bind _returnvalue (`self.GetOwner`))
  (bind _returnvalue_2 (`Actor.GetComponentByClass` _returnvalue "/Script/Engine.CapsuleComponent"))
  ;[0.05098 0.05098 0.05098] Return the actor location as location to spawn at. This will check if the location has a capsule component. This is because that will give us a place where we know we can respawn.
  (`/Engine/EditorBlueprintResources/StandardMacros.IsValid` _returnvalue_2
    (:`Is Valid`
      (return (`SceneComponent.K2_GetComponentToWorld` _returnvalue_2)))
    (:`Is Not Valid`
      (return (`Actor.GetTransform` _returnvalue)))))