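; Player-buildable open-world respawn point that tracks which players are authorized through its ACRespawnLocationOpenWorld component.
; When construction finishes, the server automatically authorizes the builder, bypassing the authorization check.
; If multiple authorized players are allowed, server-controlled interaction with the finished building toggles the interacting player's authorization, with the check applied.
; Interact text reflects authorization by player unique ID, falling back to parent text during construction.
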(event `/Game/Hyper/Core/Interaction/Interfaces/BPI_Interact.Interact`
  (params (`Owning Controller` :type "Controller Object Reference"))
  (bind _ac_respawn_location_openworld (`self.AC_Respawn_Location_OpenWorld`))
  ;[0.05098 0.05098 0.05098] On interact we want to add this player to the authorised player list. This will only add unique players
  (`parent.Interact` `Owning Controller`)
  (if (and (`/Game/Hyper/Respawn/Blueprints/OpenWorldRespawn/AC_Respawn_Location_OpenWorld.Can Have Multiple Authorised Players` _ac_respawn_location_openworld) (`self.Is Building Finished`))
    (`/Game/Hyper/Respawn/Blueprints/OpenWorldRespawn/AC_Respawn_Location_OpenWorld.Add or Remove Authorised Player` _ac_respawn_location_openworld `Owning Controller` true (not (`KismetArrayLibrary.Array_Contains` (`/Game/Hyper/Respawn/Blueprints/OpenWorldRespawn/AC_Respawn_Location_OpenWorld.Authorised Players` (`self.AC_Respawn_Location_OpenWorld`)) (`PlayerState.BP_GetUniqueId` (`Controller.PlayerState` `Owning Controller`)))))))

(fn `Can Interact`
  (params (`Owning Controller` :type "Controller Object Reference"))
  (returns (True :type Boolean))
  ;[0.05098 0.05098 0.05098] Save the client player controller for the authorization check in get interact text
  (bind _asplayer_controller (cast `PlayerController` `Owning Controller`)
    (:`then`
      (set `self.Client Player Controller` _asplayer_controller))
    (:`CastFailed`
      _))
  (bind _true (`parent.Can Interact` `Owning Controller`))
  (return _true))

(fn `Get Interact Text`
  (params (`Owning Controller` :type "PlayerController Object Reference"))
  (returns (`Interact Text` :type Text) (`Secondary Interact Text` :type Text))
  ;[0.05098 0.05098 0.05098] Change the text based on if the player is authorized
  (if (`self.Is Building Finished`)
    (return (select `bool` (`KismetArrayLibrary.Array_Contains` (`/Game/Hyper/Respawn/Blueprints/OpenWorldRespawn/AC_Respawn_Location_OpenWorld.Authorised Players` (`self.AC_Respawn_Location_OpenWorld`)) (`PlayerState.BP_GetUniqueId` (`Controller.PlayerState` (`local.Owning Controller`)))) :`false` "Interact to authorize yourself" :`true` "You are authorized" :!type "Text") "")
    (else
      (bind (_interact_text _secondary_interact_text) (`parent.Get Interact Text` (`local.Owning Controller`)))
      (return _interact_text _secondary_interact_text))))

(fn `OnRep_Is Building Finished_Excecution`
  (bind _build_by_player (`self.Build By Player`))
  (`parent.OnRep_Is Building Finished_Excecution`)
  ;[0.05098 0.05098 0.05098] Make sure the owner only updates when the building is complete
  (if (`self.Is Building Finished`)
    (`/Engine/EditorBlueprintResources/ActorMacros.Switch Has Authority`
      (:`Authority`
        (`/Engine/EditorBlueprintResources/StandardMacros.IsValid` _build_by_player
          (:`Is Valid`
            (`/Game/Hyper/Respawn/Blueprints/OpenWorldRespawn/AC_Respawn_Location_OpenWorld.Add or Remove Authorised Player` (`self.AC_Respawn_Location_OpenWorld`) _build_by_player false true)))))))

(fn `Should server control the interact`
  (returns (`Server should excecute interact call` :type Boolean))
  (return true))

(fn `UserConstructionScript`
  (`parent.UserConstructionScript`))