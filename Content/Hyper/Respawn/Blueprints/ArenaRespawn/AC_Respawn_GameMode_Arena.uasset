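; Arena respawn component for the game mode that handles a player's initial spawn in Team or Free for All games.
; It caches arena spawn location actors on first initialization.
; Team players possess a dummy character at a random start-camera view, which receives a respawn manager component to show spawn selection UI.
; Free for All picks a random type-matching location and spawns through a server event that forwards to AC_Respawn_Handler.
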(event `Server: Spawn Player`
  (params (`Player Controller` :type "PlayerController Object Reference") (`Spawn Transform` :type "Transform Structure"))
  (`/Game/Hyper/Respawn/Blueprints/AC_Respawn_Handler.Spawn Player` (`Actor.GetComponentByClass` (`GameplayStatics.GetGameMode`) "/Game/Hyper/Respawn/Blueprints/AC_Respawn_Handler.AC_Respawn_Handler_C") `Player Controller` `Spawn Transform`))

(fn `Get Random Spawn Location By Type`
  (params (`Player Spawn Type` :type "/Game/Hyper/Core/Respawn/Datamodel/Enumerations/Enum_Player_Spawn_Type Enum" :default "NewEnumerator0"))
  (returns (`Has Spawn Location` :type Boolean) (`Spawn Transform` :type "Transform Structure"))
  (locals (`Possible Spawn Locations` :type "Array of /Game/Hyper/Respawn/Blueprints/ArenaRespawn/BP_Respawn_Location_Arena Object Reference"))
  (bind _possible_spawn_locations (`local.Possible Spawn Locations`))
  (bind _returnvalue (`KismetArrayLibrary.Array_Length` _possible_spawn_locations))
  ;[0.05098 0.05098 0.05098] Gathering all of the possible spawn locations for that specific player based on the spawn type (E.G. Free for all, team01 etc.)
  (for _array_element (`self.Spawn Locations`)
    (if (`|EnumEquality` `Player Spawn Type` (`/Game/Hyper/Core/Respawn/Blueprints/AC_Respawn_Location_Abstract.Spawn Type` (`/Game/Hyper/Respawn/Blueprints/ArenaRespawn/BP_Respawn_Location_Arena.AC_Respawn_Location_Arena` _array_element)))
      (`KismetArrayLibrary.Array_Add` (`local.Possible Spawn Locations`) _array_element)))
  ;[0.05098 0.05098 0.05098] Choosing a random location out of the given locations
  (if (> _returnvalue 0)
    (return true (`/Game/Hyper/Core/Respawn/Blueprints/AC_Respawn_Location_Abstract.Get Respawn Transform` (`/Game/Hyper/Respawn/Blueprints/ArenaRespawn/BP_Respawn_Location_Arena.AC_Respawn_Location_Arena` (`|GetArrayItem` _possible_spawn_locations (`KismetMathLibrary.RandomIntegerInRange` 0 (- _returnvalue 1))))))
    (else
      (`KismetSystemLibrary.PrintString` "You do not have any respawn locations for this game type")
      (return false))))

(fn `Initialize Spawn`
  (params (`Player Controller` :type "PlayerController Object Reference") (`Game Type` :type "/Game/Hyper/Core/Respawn/Datamodel/Enumerations/Enum_Game_Type Enum" :default "NewEnumerator0"))
  (locals (`Dummy Transform` :type "Transform Structure"))
  ;[0.05098 0.05098 0.05098] Saving the spawn locations when not saved
  (if (not (`self.Spawn Locations Loaded`))
    (`self.Save Spawn Locations`))
  ;[0.05098 0.05098 0.05098] Checking the game type, and running different logic based on the that
  (switch `/Game/Hyper/Core/Respawn/Datamodel/Enumerations/Enum_Game_Type` `Game Type`
    (:`NewEnumerator1`
      ;[0.05098 0.05098 0.05098] We're spawning a temporary character when open world. This way we can show the UI for respawning.
      ;;[0.05127 0.05127 0.05127] Determine start location view
      (bind _outactors (`GameplayStatics.GetAllActorsOfClass` "/Game/Hyper/Respawn/Blueprints/OpenWorldRespawn/BP_StartCameraViewOnStart.BP_StartCameraViewOnStart_C"))
      (if (`KismetArrayLibrary.Array_IsEmpty` _outactors)
        (`KismetSystemLibrary.PrintString` "No Start Camera view actor in the world. Will choose spawn location screen 0,0,0" false)
        (else
          (set `local.Dummy Transform` (`Actor.GetTransform` (`KismetArrayLibrary.Array_Random` _outactors)))))
      (bind _returnvalue (`|SpawnActorFromClass` "/Game/Hyper/Respawn/Blueprints/BP_DummyChar_SpawnPointSelection.BP_DummyChar_SpawnPointSelection_C" (`local.Dummy Transform`) "AdjustIfPossibleButAlwaysSpawn" "MultiplyWithRoot" null null))
      (`Controller.Possess` (`local.Player Controller`) _returnvalue)
      (bind _returnvalue_2 (`|AddComponentByClass` _returnvalue "/Game/Hyper/Respawn/Blueprints/ArenaRespawn/AC_Respawn_Manager_Arena.AC_Respawn_Manager_Arena_C"))
      (`/Game/Hyper/Core/Respawn/Blueprints/AC_Respawn_Manager_Abstract.Initialize Respawn UI` _returnvalue_2))
    (:`NewEnumerator2`
      ;[0.05098 0.05098 0.05098] We're getting a location to spawn on, and then spawning a character on that location
      (bind (_has_spawn_location _spawn_transform) (`self.Get Random Spawn Location By Type` "NewEnumerator0"))
      (if _has_spawn_location
        (`self.Server: Spawn Player` (`local.Player Controller`) _spawn_transform)
        (else
          (`KismetSystemLibrary.PrintString` "You don't have any spawn locations set up for free for all. This way it's not possible to spawn."))))))

(fn `Save Spawn Locations`
  (bind _outactors (`GameplayStatics.GetAllActorsOfClass` "/Game/Hyper/Respawn/Blueprints/ArenaRespawn/BP_Respawn_Location_Arena.BP_Respawn_Location_Arena_C"))
  (set `self.Spawn Locations` _outactors)
  (set `self.Spawn Locations Loaded` true))