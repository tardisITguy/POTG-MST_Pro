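; Arena respawn manager component that handles a player's death, respawn menus and spawn requests.
; On authority it binds to the attribute manager's death event, which opens the respawn widget if respawning is allowed.
; Spawning is delegated to GameMode components using a random location by spawn type, falling back to team selection when none exists.
; Menus reapply UI-only input after HUD initialization, and a server-to-client RPC reinitializes the HUD.
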(event `self.ReceiveBeginPlay`
  (bind (_component _is_valid) (`/Game/Hyper/Core/Attribute_System/BlueprintMacroLibrary/BML_Attribute_Component.Get Attribute Manager`))
  ;[0.05098 0.05098 0.05098] Bind the on die event.
  ; Currently in attribute manager. If you do not have an attribute manager, please implement a Die event your own
  (`/Engine/EditorBlueprintResources/ActorComponentMacros.Switch Has Authority`
    (:`Authority`
      (if _is_valid
        (add `/Game/Hyper/Core/Attribute_System/Blueprints/AC_Attribute_Manager_Abstact.On Die` _component (delegate `On Die`))
        (else
          (`KismetSystemLibrary.PrintString` "You do not have an attribute manager, please implement a Die event Dispatcher on your own." false))))))

(event `self.Initiate Respawn`
  (bind _asplayer_controller (`/Game/Hyper/Core/Generic/BlueprintMacroLibrary/BML_Generic_Component.Get Player Controller`))
  (bind _asplayer_controller_2 (`/Game/Hyper/Core/Generic/BlueprintMacroLibrary/BML_Generic_Component.Get Player Controller`))
  ;[0.05098 0.05098 0.05098] When dead: initialize the hud after a certain delay.
  (if (`self.Can Respawn`) :!label _label
    (`/Engine/EditorBlueprintResources/StandardMacros.IsValid` _asplayer_controller
      (:`Is Valid`
        (bind _returnvalue (`|CreateWidget` "/Game/Hyper/UI/Widgets/Specific/Respawn/ArenaBased/UI_RespawnSelection_Arena.UI_RespawnSelection_Arena_C" _asplayer_controller))
        (`UserWidget.AddToViewport` _returnvalue 0)
        (add `/Game/Hyper/UI/Blueprints/HUD/HUD_Abstract.On HUD Initialized` (`/Game/Hyper/UI/Blueprints/BlueprintMacroLibrary/BML_HUD_Component.Get HUD`) (delegate `On HUD Initialized`))
        (`WidgetBlueprintLibrary.SetInputMode_UIOnlyEx` _asplayer_controller_2 _returnvalue "LockAlways" true :!label _label_2)
        (set `PlayerController.bShowMouseCursor` true _asplayer_controller_2)))))

(event `On Die`
  ;[0.05098 0.05098 0.05098] When dead: initialize the hud after a certain delay.
  (goto _label))

(event `On HUD Initialized`
  ;[0.05098 0.05098 0.05098] When dead: initialize the hud after a certain delay.
  (goto _label_2))

(event `self.Spawn Player Arena`
  (params (`Player Controller` :type "PlayerController Object Reference"))
  (bind _returnvalue (`GameplayStatics.GetGameMode`))
  ;[0.05098 0.05098 0.05098] Run the spawning of the player on the gamemode. This is because the gamemode should be in control of the spawning.
  (bind (_has_spawn_location _spawn_transform) (`/Game/Hyper/Respawn/Blueprints/ArenaRespawn/AC_Respawn_GameMode_Arena.Get Random Spawn Location By Type` (`Actor.GetComponentByClass` _returnvalue "/Game/Hyper/Respawn/Blueprints/ArenaRespawn/AC_Respawn_GameMode_Arena.AC_Respawn_GameMode_Arena_C") (`self.Spawn Type`)))
  (if _has_spawn_location
    (`/Game/Hyper/Respawn/Blueprints/AC_Respawn_Handler.Spawn Player` (`Actor.GetComponentByClass` _returnvalue "/Game/Hyper/Respawn/Blueprints/AC_Respawn_Handler.AC_Respawn_Handler_C") `Player Controller` _spawn_transform)
    (else
      (`self.Initialize Respawn UI`))))

(event `self.Server: Reinitialize HUD`
  ;[0.05098 0.05098 0.05098] Create a call to the client. We only want to reinitialize the HUD on the client, and not the server.
  (`self.Client: Reinitialize HUD`))

(event `self.Client: Reinitialize HUD`
  ;[0.05098 0.05098 0.05098] Call the reinitialization of the HUD on the client
  (bind _ashud_master (cast `/Game/Hyper/UI/Blueprints/HUD/HUD_Master` (`PlayerController.GetHUD` (`/Game/Hyper/Core/Generic/BlueprintMacroLibrary/BML_Generic_Component.Get Player Controller`)))
    (:`then`
      (`/Game/Hyper/UI/Blueprints/HUD/HUD_Master.Reinitialize` _ashud_master))
    (:`CastFailed`
      (`KismetSystemLibrary.PrintString` "Your HUD doesn't derive from 'HUD_Master'. This way the HUD can not be initialized." false))))

(event `self.Initialize Respawn UI`
  (bind _asplayer_controller (`/Game/Hyper/Core/Generic/BlueprintMacroLibrary/BML_Generic_Component.Get Player Controller`))
  ;[0.05098 0.05098 0.05098] Initializing menu where you can choose the team that you're on. This will only trigger for the team gamemode. Free for all will automatically spawn a player.
  (`/Engine/EditorBlueprintResources/StandardMacros.IsValid` _asplayer_controller
    (:`Is Valid`
      (bind _returnvalue (`|CreateWidget` "/Game/Hyper/UI/Widgets/Specific/Respawn/ArenaBased/UI_Team_Selection.UI_Team_Selection_C" _asplayer_controller))
      (`UserWidget.AddToViewport` _returnvalue 0)
      (add `/Game/Hyper/UI/Blueprints/HUD/HUD_Abstract.On HUD Initialized` (`/Game/Hyper/UI/Blueprints/BlueprintMacroLibrary/BML_HUD_Component.Get HUD`) (delegate `On HUD Initialized_Event`))
      (`WidgetBlueprintLibrary.SetInputMode_UIOnlyEx` _asplayer_controller _returnvalue "DoNotLock" true :!label _label_3)
      (set `PlayerController.bShowMouseCursor` true _asplayer_controller))))

(event `On HUD Initialized_Event`
  ;[0.05098 0.05098 0.05098] Initializing menu where you can choose the team that you're on. This will only trigger for the team gamemode. Free for all will automatically spawn a player.
  ;;[0.05098 0.05098 0.05098] Sometimes the HUD is initialized after this. It will then reset the input
  (goto _label_3))

(event `self.Set Spawn Type`
  (params (`New Spawn Type` :type "/Game/Hyper/Core/Respawn/Datamodel/Enumerations/Enum_Player_Spawn_Type Enum" :default "NewEnumerator0"))
  ;[0.05098 0.05098 0.05098] Setting the spawn type for the player to spawn on
  (set `self.Spawn Type` `New Spawn Type`))