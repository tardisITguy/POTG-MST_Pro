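; Example respawn component for a character that shows a death screen intended to simply restart the level.
; On BeginPlay, a locally controlled character binds to the attribute manager's OnDie event.
; On death, standalone or non-dedicated-server instances clear all widgets and display UI_OnDieSimpleRespawn above other UI.
; Otherwise it only prints a notice that no respawn screen is shown.
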(event `self.ReceiveBeginPlay`
  ;[0.05127 0.05127 0.05127] This respawn is for example only. It simply restarts the level.
  (if (`Pawn.IsLocallyControlled` (`/Game/Hyper/Core/Generic/BlueprintMacroLibrary/BML_Generic_Component.Get Character`))
    (add `/Game/Hyper/Core/Attribute_System/Blueprints/AC_Attribute_Manager_Abstact.On Die` (`/Game/Hyper/Core/Attribute_System/BlueprintMacroLibrary/BML_Attribute_Component.Get Attribute Manager`) (delegate `On Die_Event`))))

(event `On Die_Event`
  ;[0.05127 0.05127 0.05127] This respawn is for example only. It simply restarts the level.
  (if (or (not (`KismetSystemLibrary.IsDedicatedServer`)) (`KismetSystemLibrary.IsStandalone`))
    (`WidgetLayoutLibrary.RemoveAllWidgets`)
    (bind _returnvalue (`|CreateWidget` "/Game/Hyper/UI/Widgets/Specific/Respawn/OnDie/UI_OnDieSimpleRespawn.UI_OnDieSimpleRespawn_C" (`/Game/Hyper/Core/Generic/BlueprintMacroLibrary/BML_Generic_Component.Get Player Controller`)))
    (`UserWidget.AddToViewport` _returnvalue 1000)
    (`KismetSystemLibrary.PrintString` "This respawn simply restarts the level, just as an example.")
    (else
      (`KismetSystemLibrary.PrintString` "You are currently playing as client. No respawn screen will be shown since it is only here as an example."))))