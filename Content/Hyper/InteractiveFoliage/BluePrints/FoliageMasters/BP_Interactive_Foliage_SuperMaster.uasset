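; Base stand-in actor for interactive foliage that displays a configured static mesh and swaps itself for a damageable foliage actor when hit.
; Point damage only counts when the damage causer's equipment manager reports an accepted equipment type in a specific slot.
; On authority, it spawns the replacement at its transform, passing along its mesh and class.
; After a short delay, it forwards the hit to the new actor and destroys itself.
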(event `self.ReceiveBeginPlay`
  (`StaticMeshComponent.SetStaticMesh` (`self.StaticMesh`) (`self.Original Static Mesh`)))

(event `self.ReceivePointDamage`
  (params (Damage :type "Float (single-precision)") (DamageType :type "DamageType Object Reference") (HitLocation :type "Vector Structure") (HitNormal :type "Vector Structure") (HitComponent :type "PrimitiveComponent Object Reference") (BoneName :type Name) (ShotFromDirection :type "Vector Structure") (InstigatedBy :type "Controller Object Reference") (DamageCauser :type "Actor Object Reference") (HitInfo :type "HitResult Structure (by ref)"))
  (bind _returnvalue (`self.GetComponentByClass` DamageCauser "/Game/Hyper/Core/Equipment_Manager/Blueprints/AC_Equipment_Manager_Abstract.AC_Equipment_Manager_Abstract_C"))
  ;[0.05127 0.05127 0.05127] Does the instigator has the required equipment to inflict damage?
  (`/Engine/EditorBlueprintResources/StandardMacros.IsValid` DamageCauser
    (:`Is Valid`
      (`/Engine/EditorBlueprintResources/StandardMacros.IsValid` _returnvalue
        (:`Is Valid`
          (if (`/Game/Hyper/Core/Equipment_Manager/Blueprints/AC_Equipment_Manager_Abstract.Does actor has required equipmenttype in slot?` _returnvalue (`self.Accepted Equipment Type to inflict Damage`) "NewEnumerator8")
            ;[0.05127 0.05127 0.05127] Spawn the actual damageable actor
            (`/Engine/EditorBlueprintResources/ActorMacros.Switch Has Authority`
              (:`Authority`
                (bind _spawned_actor (`self.Spawn Foilage` (`self.GetTransform`) (`GameplayStatics.GetObjectClass` self)))
                (`/Engine/EditorBlueprintResources/StandardMacros.IsValid` _spawned_actor
                  (:`Is Valid`
                    (`KismetSystemLibrary.Delay` (`self.Damage Delay`))
                    (`GameplayStatics.ApplyPointDamage` _spawned_actor Damage HitLocation HitInfo InstigatedBy DamageCauser)
                    (`self.K2_DestroyActor`))
                  (:`Is Not Valid`
                    (`KismetSystemLibrary.PrintString` "Failed To Spawn Interactive Foilage")))))))))))

(fn `Spawn Foilage`
  (params (Transform :type "Transform Structure") (`Super Master Class` :type "/Game/Hyper/Core/InteractiveFoliage/Blueprints/BP_Interactive_Foliage_SuperMaster_Abstract Class Reference"))
  (returns (`Spawned Actor` :type "Actor Object Reference"))
  (bind _returnvalue (`|SpawnActorFromClass` (`self.Foilage To Spawn`) (`local.Transform`) "AlwaysSpawn" "SelectDefaultAtRuntime" null (`self.Original Static Mesh`) (`local.Super Master Class`) null))
  (return _returnvalue))

(fn `UserConstructionScript`
  (`StaticMeshComponent.SetStaticMesh` (`self.StaticMesh`) (`self.Original Static Mesh`)))