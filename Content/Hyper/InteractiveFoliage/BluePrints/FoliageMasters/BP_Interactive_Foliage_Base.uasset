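; Base actor for interactive foliage, handling inactivity cleanup and respawning after a player or other source interacts with it.
; On authority, a retriggerable inactivity timer respawns or destroys idle, unbroken instances to favor lighter performance classes.
; Destruction either triggers a delayed respawn, optionally blocked when the base mesh is destroyed, or delayed removal.
; Respawn spawns the SuperMaster class with this class and mesh, then destroys itself; the broken-state replication hook is empty here.
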(event `self.ReceiveBeginPlay`
  ;[0.05127 0.05127 0.05127] When activated, there was interaction with this actor. So we start the inactivity timer
  (`/Engine/EditorBlueprintResources/ActorMacros.Switch Has Authority`
    (:`Authority`
      (`self.Start Inactivity Timer`))))

(event `Start Inactivity Timer`
  ;[0.05127 0.05127 0.05127] Inactivity is for cleaning up to keep the peformance classes alive above the full interactive ones after x time
  (`KismetSystemLibrary.RetriggerableDelay` (`self.Max Inactivity`))
  ;;[0.05127 0.05127 0.05127] If the respawn timer is active OR is in the process of breaking, just let it be. If not, destroy the actor
  (if (or (`self.Respawn Timer is active`) (`self.Has Broken`))
    _
    (elif (`self.Does Respawn`)
      (`self.Respawn`)
      (else
        (`self.K2_DestroyActor`)))))

(event `Destroy Actor And Check Respawn`
  ;[0.05127 0.05127 0.05127] On Destroy, check if should respawn or not
  (if (`self.Does Respawn`)
    (if (`self.When base mesh is destroyed do not respawn`)
      (if (`self.Base Mesh is destroyed`)
        (`self.K2_DestroyActor`)
        (else
          (set `self.Respawn Timer Is Active` true :!label _label)
          (`KismetSystemLibrary.Delay` (`self.Respawn Time`))
          (`self.Respawn`)))
      (else
        (goto _label)))
    (else
      (`KismetSystemLibrary.RetriggerableDelay` (`self.Delay To Destroy Actor If Not Respawning`))
      (`self.K2_DestroyActor`))))

(event `Respawn`
  ;[0.05127 0.05127 0.05127] Respawn supermaster class after that destroy self
  (`|SpawnActorFromClass` (`self.Super Master Class`) (`self.GetTransform`) "AdjustIfPossibleButDontSpawnIfColliding" "MultiplyWithRoot" null (`GameplayStatics.GetObjectClass` self) (`self.Static Mesh`) null)
  (`self.K2_DestroyActor`))

(fn `OnRep_Has Broken`
  (`self.OnRep_Has Broken_Execution` false))

(fn `OnRep_Has Broken_Execution`
  (params (`Override Initialization Check` :type Boolean)))

(fn `UserConstructionScript`)