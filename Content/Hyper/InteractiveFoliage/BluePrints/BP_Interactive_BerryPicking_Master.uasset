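; Master Blueprint for an interactive berry bush that populates itself with berry actors, with its mesh set in the construction script.
; On BeginPlay, only the server runs SpawnBerries, which uses the direct child components of BushMesh as spawn points.
; It spawns the configured berry class at each point's world transform with decay disabled, stopping once AmountToSpawn is reached or the points run out.
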(event `self.ReceiveBeginPlay`
  (`/Engine/EditorBlueprintResources/ActorMacros.Switch Has Authority`
    (:`Authority`
      (`self.Spawn Berries Event`))))

(event `Spawn Berries Event`
  (`self.SpawnBerries`))

(fn `SpawnBerries`
  ;[1 1 1] Loop over child components and spawn on location of scene components under root
  (for _array_element (`SceneComponent.GetChildrenComponents` (`self.BushMesh`) false)
    (`|SpawnActorFromClass` (`self.BerryToSpawn`) (`SceneComponent.K2_GetComponentToWorld` _array_element) "AlwaysSpawn" "SelectDefaultAtRuntime" null false 5.0 0.3 true false (struct) 30.0 10.0 125.0 false false 1000.0 null)
    (`/Engine/EditorBlueprintResources/StandardMacros.IncrementInt` (`self.AmountOfSpawns`)
      (:`  `
        (if (>= (`self.AmountOfSpawns`) (`self.AmountToSpawn`))
          (break)))))
  (return))

(fn `UserConstructionScript`
  (`StaticMeshComponent.SetStaticMesh` (`self.BushMesh`) (`self.Static Mesh`)))