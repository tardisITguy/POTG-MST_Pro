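; BP_Hit_Damage_Text is a short-lived floating text actor that displays hit damage through a widget component.
; On BeginPlay it passes its Text and TextColor variables to the UI_Hit_Damage_Text widget, then picks random X, Y and upward Z targets.
; The LerpToLocation timeline adds the lerped values as relative offsets every update, so movement accumulates rather than ending at those targets, and destroys the actor when finished.
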(event `self.ReceiveBeginPlay`
  ;[0.05127 0.05127 0.05127] Set values in the widget:
  ; Replicate the text value
  (bind _asui_hit_damage_text (cast `/Game/Hyper/Attribute_System/Hit_Damage_Text/UI_Hit_Damage_Text` (`WidgetComponent.GetUserWidgetObject` (`self.Widget`))))
  (`/Game/Hyper/Attribute_System/Hit_Damage_Text/UI_Hit_Damage_Text.Set Values` _asui_hit_damage_text (`self.Text`) (`self.Text Color`))
  ;[1 1 1] Lerps the widget to a random location in range
  (set `self.Random X Target` (`KismetMathLibrary.RandomFloatInRange` -5.0 5.0))
  (set `self.Random Z Target` (`KismetMathLibrary.RandomFloatInRange` 0.0 5.0))
  (set `self.Random Y Target` (`KismetMathLibrary.RandomFloatInRange` -5.0 5.0))
  (bind (_direction _alpha) (`Timeline|Lerp to Location`)
    (:`Update`
      (`SceneComponent.K2_AddRelativeLocation` (`self.Widget`) (`KismetMathLibrary.MakeVector` (`KismetMathLibrary.Lerp` 0.0 (`self.Random X Target`) _alpha) (`KismetMathLibrary.Lerp` 0.0 (`self.Random Y Target`) _alpha) (`KismetMathLibrary.Lerp` 0.0 (`self.Random Z Target`) _alpha)) false false))
    (:`Finished`
      ;[1 1 1] Destroy after finished
      (`self.K2_DestroyActor`))))

(fn `UserConstructionScript`)