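; Example interaction pad that switches an attribute feature on or off when an actor overlaps its sphere.
; It finds the Attribute Manager through the overlapping actor's instigator controller and flips the Use flag for the attribute chosen in WhichAttribute.
; Health toggles regeneration instead, while Weight toggles the Inventory Manager's weight use along with the Attribute Manager's weight HUD flag.
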(event `self.Interact_Area_Sphere.OnComponentBeginOverlap`
  (params (OverlappedComponent :type "PrimitiveComponent Object Reference") (OtherActor :type "Actor Object Reference") (OtherComp :type "PrimitiveComponent Object Reference") (OtherBodyIndex :type Integer) (bFromSweep :type Boolean) (SweepResult :type "HitResult Structure (by ref)"))
  (bind _returnvalue (`self.GetInstigatorController` OtherActor))
  (bind _component (`/Game/Hyper/Core/Inventory/BlueprintMacroLibrary/BML_Inventory_Controller.Get Inventory Manager` _returnvalue))
  (bind (_component_2 _is_valid) (`/Game/Hyper/Core/Attribute_System/BlueprintMacroLibrary/BML_Attribute__Controller.Get Attribute Manager` _returnvalue))
  (if _is_valid
    (switch `string` (`self.which attribute`)
      (:`stamina`
        ;[0.05127 0.05127 0.05127] stamina
        (set `/Game/Hyper/Core/Attribute_System/Blueprints/AC_Attribute_Manager_Abstact.Use Stamina` (not (`/Game/Hyper/Core/Attribute_System/Blueprints/AC_Attribute_Manager_Abstact.Use Stamina` _component_2)) _component_2))
      (:`energy`
        ;[0.05127 0.05127 0.05127] fatigue
        (set `/Game/Hyper/Core/Attribute_System/Blueprints/AC_Attribute_Manager_Abstact.Use Energy` (not (`/Game/Hyper/Core/Attribute_System/Blueprints/AC_Attribute_Manager_Abstact.Use Energy` _component_2)) _component_2))
      (:`magic`
        ;[0.05127 0.05127 0.05127] magic
        (if (`/Game/Hyper/Core/Attribute_System/Blueprints/AC_Attribute_Manager_Abstact.Use Mana` _component_2)
          (set `/Game/Hyper/Core/Attribute_System/Blueprints/AC_Attribute_Manager_Abstact.Use Mana` false _component_2)
          (else
            (set `/Game/Hyper/Core/Attribute_System/Blueprints/AC_Attribute_Manager_Abstact.Use Mana` true _component_2))))
      (:`oxygen`
        ;[0.05127 0.05127 0.05127] oxygen
        (if (`/Game/Hyper/Core/Attribute_System/Blueprints/AC_Attribute_Manager_Abstact.Use Oxygen` _component_2)
          (set `/Game/Hyper/Core/Attribute_System/Blueprints/AC_Attribute_Manager_Abstact.Use Oxygen` false _component_2)
          (else
            (set `/Game/Hyper/Core/Attribute_System/Blueprints/AC_Attribute_Manager_Abstact.Use Oxygen` true _component_2))))
      (:`food`
        ;[0.05127 0.05127 0.05127] food
        (if (`/Game/Hyper/Core/Attribute_System/Blueprints/AC_Attribute_Manager_Abstact.Use Food` _component_2)
          (set `/Game/Hyper/Core/Attribute_System/Blueprints/AC_Attribute_Manager_Abstact.Use Food` false _component_2)
          (else
            (set `/Game/Hyper/Core/Attribute_System/Blueprints/AC_Attribute_Manager_Abstact.Use Food` true _component_2))))
      (:`hydration`
        ;[0.05127 0.05127 0.05127] hydration
        (if (`/Game/Hyper/Core/Attribute_System/Blueprints/AC_Attribute_Manager_Abstact.Use Hydration` _component_2)
          (set `/Game/Hyper/Core/Attribute_System/Blueprints/AC_Attribute_Manager_Abstact.Use Hydration` false _component_2)
          (else
            (set `/Game/Hyper/Core/Attribute_System/Blueprints/AC_Attribute_Manager_Abstact.Use Hydration` true _component_2))))
      (:`health`
        ;[0.05127 0.05127 0.05127] Health regen
        (if (`/Game/Hyper/Core/Attribute_System/Blueprints/AC_Attribute_Manager_Abstact.Has Health Regen` _component_2)
          (set `/Game/Hyper/Core/Attribute_System/Blueprints/AC_Attribute_Manager_Abstact.Has Health Regen` false _component_2)
          (else
            (set `/Game/Hyper/Core/Attribute_System/Blueprints/AC_Attribute_Manager_Abstact.Has Health Regen` true _component_2))))
      (:`weight`
        (if (`/Game/Hyper/Core/Inventory/Blueprints/AC_Inventory_Abstract.Use Weight` _component)
          (set `/Game/Hyper/Core/Inventory/Blueprints/AC_Inventory_Abstract.Use Weight` false _component)
          (set `/Game/Hyper/Core/Attribute_System/Blueprints/AC_Attribute_Manager_Abstact.Use Weight in HUD` false _component_2)
          (else
            (set `/Game/Hyper/Core/Inventory/Blueprints/AC_Inventory_Abstract.Use Weight` true _component)
            (set `/Game/Hyper/Core/Attribute_System/Blueprints/AC_Attribute_Manager_Abstact.Use Weight in HUD` true _component_2)))))))

(fn `UserConstructionScript`
  (`parent.UserConstructionScript`))