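; Example interaction pad from the Attribute System that deals continuous damage to characters standing inside its interact sphere.
; Sphere overlap begin and end events add and remove characters from a tracked actor list.
; A looping 0.1-second timer started on BeginPlay applies a matching fraction of DamagePerSecond to each listed actor, with the pad as damage causer.
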(event `self.ReceiveBeginPlay`
  (`KismetSystemLibrary.K2_SetTimerDelegate` (delegate `Damage Actor`) 0.1 true))

(event `Damage Actor`
  (for _array_element (`self.DamageActors`)
    (`GameplayStatics.ApplyDamage` _array_element (* (`self.Damage per second`) 0.1) null self)))

(event `self.Interact_Area_Sphere.OnComponentBeginOverlap`
  (params (OverlappedComponent :type "PrimitiveComponent Object Reference") (OtherActor :type "Actor Object Reference") (OtherComp :type "PrimitiveComponent Object Reference") (OtherBodyIndex :type Integer) (bFromSweep :type Boolean) (SweepResult :type "HitResult Structure (by ref)"))
  (cast `Character` OtherActor)
  (`KismetArrayLibrary.Array_AddUnique` (`self.DamageActors`) OtherActor))

(event `self.Interact_Area_Sphere.OnComponentEndOverlap`
  (params (OverlappedComponent :type "PrimitiveComponent Object Reference") (OtherActor :type "Actor Object Reference") (OtherComp :type "PrimitiveComponent Object Reference") (OtherBodyIndex :type Integer))
  (cast `Character` OtherActor)
  (`KismetArrayLibrary.Array_RemoveItem` (`self.DamageActors`) OtherActor))

(fn `UserConstructionScript`
  (`parent.UserConstructionScript`))