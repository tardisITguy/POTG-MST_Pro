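; Example interaction pad that adds or removes an attribute system state effect on whoever steps into its sphere.
; On overlap, the server finds the overlapping actor's instigator controller and gets its Attribute Manager component.
; It then passes the configured Effect and Remove flag to that component's server event for adding or removing state effects.
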(event `self.Interact_Area_Sphere.OnComponentBeginOverlap`
  (params (OverlappedComponent :type "PrimitiveComponent Object Reference") (OtherActor :type "Actor Object Reference") (OtherComp :type "PrimitiveComponent Object Reference") (OtherBodyIndex :type Integer) (bFromSweep :type Boolean) (SweepResult :type "HitResult Structure (by ref)"))
  (bind _returnvalue (`self.GetInstigatorController` OtherActor))
  (bind (_component _is_valid) (`/Game/Hyper/Core/Attribute_System/BlueprintMacroLibrary/BML_Attribute__Controller.Get Attribute Manager` _returnvalue))
  (`/Engine/EditorBlueprintResources/ActorMacros.Switch Has Authority`
    (:`Authority`
      (`/Engine/EditorBlueprintResources/StandardMacros.IsValid` _returnvalue
        (:`Is Valid`
          (if _is_valid
            (`/Game/Hyper/Core/Attribute_System/Blueprints/AC_Attribute_Manager_Abstact.Event server: Add or Remove State Effect` _component (`self.Effect`) (`self.Remove?`))))))))

(fn `UserConstructionScript`
  (`parent.UserConstructionScript`))