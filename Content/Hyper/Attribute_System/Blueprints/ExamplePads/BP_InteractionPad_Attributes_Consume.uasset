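; Example interaction pad that makes an overlapping actor consume one attribute, Stamina, Energy, Magic or Oxygen, for as long as it stays in the pad's sphere.
; On begin overlap, it finds the Attribute Manager through the actor's instigator controller and switches on WhichAttribute to set the matching Consume flag.
; End overlap clears that flag; the pad only toggles flags and does no draining itself.
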(event `self.Interact_Area_Sphere.OnComponentBeginOverlap`
  (params (OverlappedComponent :type "PrimitiveComponent Object Reference") (OtherActor :type "Actor Object Reference") (OtherComp :type "PrimitiveComponent Object Reference") (OtherBodyIndex :type Integer) (bFromSweep :type Boolean) (SweepResult :type "HitResult Structure (by ref)"))
  (bind (_component _is_valid) (`/Game/Hyper/Core/Attribute_System/BlueprintMacroLibrary/BML_Attribute__Controller.Get Attribute Manager` (`self.GetInstigatorController` OtherActor)))
  (if _is_valid
    (switch `string` (`self.which attribute`)
      (:`stamina`
        (set `/Game/Hyper/Core/Attribute_System/Blueprints/AC_Attribute_Manager_Abstact.ConsumeStamina` true _component))
      (:`energy`
        (set `/Game/Hyper/Core/Attribute_System/Blueprints/AC_Attribute_Manager_Abstact.Consume Energy` true _component))
      (:`magic`
        (set `/Game/Hyper/Core/Attribute_System/Blueprints/AC_Attribute_Manager_Abstact.Consume Mana` true _component))
      (:`oxygen`
        (set `/Game/Hyper/Core/Attribute_System/Blueprints/AC_Attribute_Manager_Abstact.ConsumeOxygen` true _component)))))

(event `self.Interact_Area_Sphere.OnComponentEndOverlap`
  (params (OverlappedComponent :type "PrimitiveComponent Object Reference") (OtherActor :type "Actor Object Reference") (OtherComp :type "PrimitiveComponent Object Reference") (OtherBodyIndex :type Integer))
  (bind (_component _is_valid) (`/Game/Hyper/Core/Attribute_System/BlueprintMacroLibrary/BML_Attribute__Controller.Get Attribute Manager` (`self.GetInstigatorController` OtherActor)))
  (if _is_valid
    (switch `string` (`self.which attribute`)
      (:`stamina`
        (set `/Game/Hyper/Core/Attribute_System/Blueprints/AC_Attribute_Manager_Abstact.ConsumeStamina` false _component))
      (:`energy`
        (set `/Game/Hyper/Core/Attribute_System/Blueprints/AC_Attribute_Manager_Abstact.Consume Energy` false _component))
      (:`magic`
        (set `/Game/Hyper/Core/Attribute_System/Blueprints/AC_Attribute_Manager_Abstact.Consume Mana` false _component))
      (:`oxygen`
        (set `/Game/Hyper/Core/Attribute_System/Blueprints/AC_Attribute_Manager_Abstact.ConsumeOxygen` false _component)))))

(fn `UserConstructionScript`
  (`parent.UserConstructionScript`))