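; Actor for one data-driven state effect on a character, applied on BeginPlay and reverted when destroyed.
; The server handles montage, particles, sound, temperature state and chained effect changes, restoring Healthy on removal when allowed.
; Timers deal interval damage or, for temporary and auto-recover effects, request removal through the attribute manager.
; Remote instances toggle camera modifiers, and the OnRep for remaining time notifies the manager.
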(event `self.ReceiveBeginPlay`
  (bind ((`Istemporary?_17_4F02E9EE47699524112793913C63CFCC` _istemporary_) (`Hasaautorecoverchance_35_E7694F3941275B1DCE4923BCF663DFD5` _hasaautorecoverchance) (`ApplyIntervalDamage?_50_EC97E3F34E89BE79DE92DAA499198B22` _applyintervaldamage_)) (break `/Game/Hyper/Core/Attribute_System/Datamodel/State_Effects/Structures/Struct_State_Effects` (`self.State Effect`)))
  (`/Engine/EditorBlueprintResources/ActorMacros.Switch Has Authority`
    (:`Authority`
      (`|ExecutionSequence`
        (:`then_0`
          ;[0.05098 0.05098 0.05098] Start timers if needed. Tempory and auto recover will remove the effect once finished. Interval damage starts a looping timer, doing damage over time.
          (`|ExecutionSequence`
            (:`then_0`
              (if _istemporary_
                (`self.Start Temporary Timer`)))
            (:`then_1`
              (if _hasaautorecoverchance
                (`self.Start Auto Recover Timer`)))
            (:`then_2`
              (if _applyintervaldamage_
                (`self.Start Interval Damage Timer`)))))
        (:`then_1`
          ;[0.05098 0.05098 0.05098] Apply all the elements defined in the state effect datatable
          (`|ExecutionSequence`
            (:`then_0`
              (`self.Try Toggle Animation Montage` true)
              (`self.Try Toggle Particles` true)
              (`self.Try Play Sound` true))
            (:`then_1`
              (`self.Update State Effects` true)
              (`self.Try Update Temperature`))))))
    (:`Remote`
      (`self.Try Toggle Camera Modifiers` true))))

(event `self.ReceiveDestroyed`
  (`/Engine/EditorBlueprintResources/ActorMacros.Switch Has Authority`
    (:`Authority`
      (`|ExecutionSequence`
        (:`then_0`
          ;[0.05098 0.05098 0.05098] Stop all timers
          (`KismetSystemLibrary.K2_ClearAndInvalidateTimerHandle` (`self.Temporary Timer Handle`))
          (`KismetSystemLibrary.K2_ClearAndInvalidateTimerHandle` (`self.Recover Timer Handle`))
          (`KismetSystemLibrary.K2_ClearAndInvalidateTimerHandle` (`self.Damage Timer Handle`)))
        (:`then_1`
          ;[0.05098 0.05098 0.05098] Revert all the elements we enabled when the effect started.
          (`|ExecutionSequence`
            (:`then_0`
              (`self.Try Toggle Animation Montage` false)
              (`self.Try Toggle Particles` false)
              (`self.Try Play Sound` false))
            (:`then_1`
              (`self.Update State Effects` false)
              (`self.Try Set Healthy`))))))
    (:`Remote`
      (`self.Try Toggle Camera Modifiers` false))))

(event `Start Temporary Timer`
  (bind _returnvalue (`KismetSystemLibrary.K2_SetTimerDelegate` (delegate `On Temporary Tick`) 1.0 true))
  (set `self.Temporary Timer Handle` _returnvalue)
  (set `self.Temporary Time Remaining` (`.Duration_14_B01A8E1A44DFF39DDAE4E0A47C4F245B` (break `/Game/Hyper/Core/Attribute_System/Datamodel/State_Effects/Structures/Struct_State_Effects` (`self.State Effect`)))))

(event `On Temporary Tick`
  (bind _result (`/Engine/EditorBlueprintResources/StandardMacros.DecrementFloat` (`self.Temporary Time Remaining`))
    (:`  `
      (if (not (> _result 0.0))
        (`self.Initialize Remove Effect`)))))

(event `Start Auto Recover Timer`
  (bind ((`Chanceforautorecover_40_A67D4B104F717C43F9C306A34EA541CD` _chanceforautorecover) (`Timetoautorecover_79_4914D289457CF8ABEDE338B3939D54C8` _timetoautorecover) (`Recoversautomaticlyafterthistimeifautorecoverwasnotsuceeded_86_F5B1D0E44DAC6CF31EF65B9E55B6C975` _recoversautomaticlyafterthistimeifautorecoverwasnotsuceeded)) (break `/Game/Hyper/Core/Attribute_System/Datamodel/State_Effects/Structures/Struct_State_Effects` (`self.State Effect`)))
  (bind _returnvalue (`KismetSystemLibrary.K2_SetTimerDelegate` (delegate `On Auto Recover Finished`) (select `bool` (< (`KismetMathLibrary.RandomFloatInRange` 0.0 1.0) _chanceforautorecover) :`false` _recoversautomaticlyafterthistimeifautorecoverwasnotsuceeded :`true` _timetoautorecover)))
  (set `self.Recover Timer Handle` _returnvalue))

(event `On Auto Recover Finished`
  (`self.Initialize Remove Effect`))

(event `Start Interval Damage Timer`
  (bind _returnvalue (`KismetSystemLibrary.K2_SetTimerDelegate` (delegate `On Damage Tick`) (`.IntervalDamageInterval_88_38B050384BFF3C8F7C2615B12BEC6A0F` (break `/Game/Hyper/Core/Attribute_System/Datamodel/State_Effects/Structures/Struct_State_Effects` (`self.State Effect`))) true))
  (set `self.Damage Timer Handle` _returnvalue))

(event `On Damage Tick`
  (bind ((`IntervalDamage_70_A68CCD0842D3B5CBFD815882AA362FD8` _intervaldamage) (`IntervalDamageInterval_88_38B050384BFF3C8F7C2615B12BEC6A0F` _intervaldamageinterval) (`IntervalDamageType_128_71EBBEE84690EA3E40F8F0A5466AE3E9` _intervaldamagetype)) (break `/Game/Hyper/Core/Attribute_System/Datamodel/State_Effects/Structures/Struct_State_Effects` (`self.State Effect`)))
  (`GameplayStatics.ApplyDamage` (`self.GetOwner`) _intervaldamage null null _intervaldamagetype))

(fn `Get Temporary Timer Remaining`
  (returns (`Time Remaining` :type "Float (double-precision)"))
  (return (`self.Temporary Time Remaining`)))

(fn `Initialize Remove Effect`
  ;[0.05098 0.05098 0.05098] Call Remove State Effect, this will eventually destroy this object which will remove all the elements which were applied
  (`/Game/Hyper/Core/Attribute_System/Blueprints/AC_Attribute_Manager_Abstact.Event server: Add or Remove State Effect` (`/Game/Hyper/Core/Attribute_System/BlueprintMacroLibrary/BML_Attribute_Actor.Get Attribute Manager`) (`.EffectState_44_1E571E154B3959C0B073E4904B6F13B4` (break `/Game/Hyper/Core/Attribute_System/Datamodel/State_Effects/Structures/Struct_State_Effects` (`self.State Effect`))) true))

(fn `OnRep_Temporary Time Remaining`
  (`/Game/Hyper/Core/Attribute_System/Blueprints/AC_Attribute_Manager_Abstact.Any Effect Timer Updated` (`/Game/Hyper/Core/Attribute_System/BlueprintMacroLibrary/BML_Attribute_Actor.Get Attribute Manager`)))

(fn `Try Play Sound`
  (params (Activated :type Boolean))
  (bind ((`OnActivatedPlaySound_90_E48792754E961D911A6F2D94CAAAB12A` _onactivatedplaysound) (`ActivatedSound_97_EB90D78F45D935C2E7E20DB810416FAD` _activatedsound) (`OnUnactivatedplaysound_92_E34CF30240D0FF15CEDBD09FD7176CDE` _onunactivatedplaysound) (`UnactivatedSound_98_0C4794E64EB6296E8C27A297E5C6D0EB` _unactivatedsound)) (break `/Game/Hyper/Core/Attribute_System/Datamodel/State_Effects/Structures/Struct_State_Effects` (`self.State Effect`)))
  (bind _rootcomponent (`Actor.RootComponent` (`/Game/Hyper/Core/Generic/BlueprintMacroLibrary/BML_Generic_Actor.Get Pawn`)))
  (bind _returnvalue (select `bool` (`local.Activated`) :`false` _unactivatedsound :`true` _activatedsound))
  (if (and (select `bool` (`local.Activated`) :`false` _onunactivatedplaysound :`true` _onactivatedplaysound) (`KismetSystemLibrary.IsValid` _returnvalue))
    (`/Engine/EditorBlueprintResources/StandardMacros.IsValid` _rootcomponent
      (:`Is Valid`
        (`/Game/Hyper/Core/ReplicationSubSystem/Blueprints/AC_Replication_Abstract.Initialize Spawn Sound At Location On Owning Client` (`/Game/Hyper/Core/ReplicationSubSystem/BlueprintMacroLibrary/BML_Replication_Actor.Get Replication`) _returnvalue (+ (`SceneComponent.K2_GetComponentLocation` _rootcomponent) (0.0 0.0 100.0)) false 0.0 "/Game/Hyper/ResourcePack/Audio/AttenuationPresets/ATT_Default.ATT_Default")))))

(fn `Try Set Healthy`
  (bind _asac_attribute_manager_advanced (cast `/Game/Hyper/Attribute_System/Blueprints/AC_Attribute_Manager_Advanced` (`/Game/Hyper/Core/Attribute_System/BlueprintMacroLibrary/BML_Attribute_Actor.Get Attribute Manager`) :!pure true))
  (bind _can_be_set_to_healthy (`/Game/Hyper/Attribute_System/Blueprints/AC_Attribute_Manager_Advanced.Check if can be set to Healthy Sate` _asac_attribute_manager_advanced))
  (if _can_be_set_to_healthy
    (`/Game/Hyper/Attribute_System/Blueprints/AC_Attribute_Manager_Advanced.Add or Remove State Effect` _asac_attribute_manager_advanced "NewEnumerator0" false)))

(fn `Try Toggle Animation Montage`
  (params (Active :type Boolean))
  (bind _component (`/Game/Hyper/Core/ReplicationSubSystem/BlueprintMacroLibrary/BML_Replication_Actor.Get Replication`))
  (bind ((`PlayAnimation_123_8F043BD6489254C15EEF20B1B6C294F4` _playanimation) (`PlayAnimaton_124_00F18AFF4507BB8595EA5B9261230A36` _playanimaton)) (break `/Game/Hyper/Core/Attribute_System/Datamodel/State_Effects/Structures/Struct_State_Effects` (`self.State Effect`)))
  (if (and _playanimation (`KismetSystemLibrary.IsValid` _playanimaton))
    (`/Engine/EditorBlueprintResources/StandardMacros.IsValid` (`/Game/Hyper/Core/Generic/BlueprintMacroLibrary/BML_Generic_Actor.Get Anim Instance`)
      (:`Is Valid`
        (if (`local.Active`)
          (`/Game/Hyper/Core/ReplicationSubSystem/Blueprints/AC_Replication_Abstract.Initialize Multicast Latent Montage` :`self` _component :`Montage To Play` _playanimaton)
          (else
            (`/Game/Hyper/Core/ReplicationSubSystem/Blueprints/AC_Replication_Abstract.Initialize Stop Multicast Montage` _component)))))))

(fn `Try Toggle Camera Modifiers`
  (params (Active :type Boolean))
  (bind ((`HasaCameraModifier_132_E3CA8D16413DDF9320528DB3C587A555` _hasacameramodifier) (`CameraModfierToApply_133_99D6B3C64DAD35118F91F9A5B90D094B` _cameramodfiertoapply)) (break `/Game/Hyper/Core/Attribute_System/Datamodel/State_Effects/Structures/Struct_State_Effects` (`self.State Effect`)))
  (bind _player_camera_manager (`/Game/Hyper/Core/Generic/BlueprintMacroLibrary/BML_Generic_ControllerInput.Get Player Camera Manager` (`/Game/Hyper/Core/Generic/BlueprintMacroLibrary/BML_Generic_Actor.Get Controller`)))
  (if _hasacameramodifier
    (if (`local.Active`)
      (bind _returnvalue (`PlayerCameraManager.AddNewCameraModifier` _player_camera_manager _cameramodfiertoapply))
      (`CameraModifier.EnableModifier` _returnvalue)
      (else
        (bind _returnvalue_2 (`PlayerCameraManager.FindCameraModifierByClass` _player_camera_manager _cameramodfiertoapply))
        (`PlayerCameraManager.RemoveCameraModifier` _player_camera_manager _returnvalue_2)))))

(fn `Try Toggle Particles`
  (params (Active :type Boolean))
  (bind _mesh (`/Game/Hyper/Core/Generic/BlueprintMacroLibrary/BML_Generic_Actor.Get Character Mesh`))
  (bind ((`PlayParticleEffect_106_47CE9BBB4AAF58D2FAE076BD30D3B612` _playparticleeffect) (`ParticleEffect_111_37D0E589429716B177F2E28E64259560` _particleeffect)) (break `/Game/Hyper/Core/Attribute_System/Datamodel/State_Effects/Structures/Struct_State_Effects` (`self.State Effect`)))
  (bind (_returnvalue_location _returnvalue_rotation _returnvalue_scale) (`KismetMathLibrary.BreakTransform` (`SceneComponent.K2_GetComponentToWorld` _mesh)))
  (if (and _playparticleeffect (`KismetSystemLibrary.IsValidClass` _particleeffect))
    (if (`local.Active`)
      (`/Engine/EditorBlueprintResources/StandardMacros.IsValid` _mesh
        (:`Is Valid`
          (bind _returnvalue (`|SpawnActorFromClass` (`.ParticleEffect_111_37D0E589429716B177F2E28E64259560` (break `/Game/Hyper/Core/Attribute_System/Datamodel/State_Effects/Structures/Struct_State_Effects` (`self.State Effect`))) (`KismetMathLibrary.MakeTransform` (+ _returnvalue_location (0.0 0.0 100.0)) _returnvalue_rotation _returnvalue_scale) "AlwaysSpawn" "MultiplyWithRoot" null null))
          (bind _output_get (set `self.Particle Effect` _returnvalue))
          (`self.K2_AttachToComponent` _output_get (`/Game/Hyper/Core/Generic/BlueprintMacroLibrary/BML_Generic_Actor.Get Character Mesh`) "None" "KeepWorld" "KeepWorld" "KeepWorld" true)))
      (else
        (`/Engine/EditorBlueprintResources/StandardMacros.IsValid` (`self.Particle Effect`)
          (:`Is Valid`
            (`self.K2_DestroyActor` (`self.Particle Effect`))))))))

(fn `Try Update Temperature`
  (bind _component (`/Game/Hyper/Core/Attribute_System/BlueprintMacroLibrary/BML_Attribute_Actor.Get Attribute Manager`))
  (bind ((`EffectCatagory_65_5553019840797655381E7D91410C45B4` _effectcatagory) (`EffectState_44_1E571E154B3959C0B073E4904B6F13B4` _effectstate)) (break `/Game/Hyper/Core/Attribute_System/Datamodel/State_Effects/Structures/Struct_State_Effects` (`self.State Effect`)))
  (if (`|EnumEquality` _effectcatagory "NewEnumerator1")
    ;[0.05098 0.05098 0.05098] Map the temperature state effect to its temperature state equivalent
    (switch `/Game/Hyper/Core/Attribute_System/Datamodel/State_Effects/Enumerations/Enum_State_Effects` _effectstate
      (:`NewEnumerator7`
        (set `/Game/Hyper/Core/Attribute_System/Blueprints/AC_Attribute_Manager_Abstact.Current Temperature State` "NewEnumerator0" _component))
      (:`NewEnumerator8`
        (set `/Game/Hyper/Core/Attribute_System/Blueprints/AC_Attribute_Manager_Abstact.Current Temperature State` "NewEnumerator1" _component))
      (:`NewEnumerator9`
        (set `/Game/Hyper/Core/Attribute_System/Blueprints/AC_Attribute_Manager_Abstact.Current Temperature State` "NewEnumerator2" _component))
      (:`NewEnumerator10`
        (set `/Game/Hyper/Core/Attribute_System/Blueprints/AC_Attribute_Manager_Abstact.Current Temperature State` "NewEnumerator3" _component))
      (:`NewEnumerator11`
        (set `/Game/Hyper/Core/Attribute_System/Blueprints/AC_Attribute_Manager_Abstact.Current Temperature State` "NewEnumerator4" _component)))))

(fn `Update State Effects`
  (params (Active :type Boolean))
  (locals (`Local Attribute Manager` :type "/Game/Hyper/Attribute_System/Blueprints/AC_Attribute_Manager_Advanced Object Reference"))
  (bind ((`Onactivatedremovetheseeffects_62_2DC782E7448A8D54699A8B970CD89AC2` _onactivatedremovetheseeffects) (`Onactivatedaddtheseeffects_63_C975C3604211BC4C850A76BACA83E06D` _onactivatedaddtheseeffects)) (break `/Game/Hyper/Core/Attribute_System/Datamodel/State_Effects/Structures/Struct_State_Effects` (`self.State Effect`)))
  (set `local.Local Attribute Manager` (cast `/Game/Hyper/Attribute_System/Blueprints/AC_Attribute_Manager_Advanced` (`/Game/Hyper/Core/Attribute_System/BlueprintMacroLibrary/BML_Attribute_Actor.Get Attribute Manager`) :!pure true))
  (if Active
    (`|ExecutionSequence`
      (:`then_0`
        (for _array_element _onactivatedremovetheseeffects
          (`/Game/Hyper/Attribute_System/Blueprints/AC_Attribute_Manager_Advanced.Add or Remove State Effect` (`local.Local Attribute Manager`) _array_element true)))
      (:`then_1`
        (for _array_element_2 _onactivatedaddtheseeffects
          (`/Game/Hyper/Attribute_System/Blueprints/AC_Attribute_Manager_Advanced.Add or Remove State Effect` (`local.Local Attribute Manager`) _array_element_2 false))))
    (else
      (for _array_element_3 (`.Onremovedactivatetheseeffects_121_A0734BD64912AB2F72BFB79BB1C692FE` (break `/Game/Hyper/Core/Attribute_System/Datamodel/State_Effects/Structures/Struct_State_Effects` (`self.State Effect`)))
        (`/Game/Hyper/Attribute_System/Blueprints/AC_Attribute_Manager_Advanced.Add or Remove State Effect` (`local.Local Attribute Manager`) _array_element_3 false)))))

(fn `UserConstructionScript`)