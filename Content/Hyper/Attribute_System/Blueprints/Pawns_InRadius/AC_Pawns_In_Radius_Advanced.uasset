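; Character component that shows name widgets above nearby pawns, set up on authority for player-controlled characters.
; After a short delay for possession, a looping timer runs a sphere trace around the character instead of using Tick.
; Hits that pass BPI_PawnInRadius checks get an attached BP_PawnInRadius_Widget_Actor, tracked in a map to avoid duplicates.
; A cleanup pass destroys widgets whose pawns are missing from the in-radius list.
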(event `self.ReceiveBeginPlay`
  (`parent.ReceiveBeginPlay`)
  (`/Engine/EditorBlueprintResources/ActorComponentMacros.Switch Has Authority`
    (:`Authority`
      ;[0.05127 0.05127 0.05127] There seems to be no controller assinged on the start so a small delay
      (`KismetSystemLibrary.Delay` 0.2)
      (if (`Pawn.IsPlayerControlled` (`/Game/Hyper/Core/Generic/BlueprintMacroLibrary/BML_Generic_Component.Get Character`))
        (`self.Initialize Pawns in radius timer`)))))

(event `Initialize Pawns in radius timer`
  ;[0.05127 0.05127 0.05127] Get pawns in RADIUS. Continously is checking for potential pawns in a radius and set the PawnStats_Widget
  ;;[0.05127 0.05127 0.05127] Starts the timer by event on begin play. Not on tick, this is less expensive
  (`KismetSystemLibrary.K2_SetTimerDelegate` (delegate `Check Pawns in radius`) 0.1 true))

(event `Check Pawns in radius`
  ;[0.05127 0.05127 0.05127] Get pawns in RADIUS. Continously is checking for potential pawns in a radius and set the PawnStats_Widget
  ;;[0.05127 0.05127 0.05127] Traces hit actors by forward vector of the camera
  (`self.Check For Pawns In Radius`))

(fn `Check For Pawns In Radius`
  (locals (`Local Pawns in Radius` :type "Array of Actor Object Reference"))
  (bind _returnvalue (`Actor.K2_GetActorLocation` (`/Game/Hyper/Core/Generic/BlueprintMacroLibrary/BML_Generic_Component.Get Character`)))
  (bind (_outhits _returnvalue_2) (`KismetSystemLibrary.SphereTraceMultiForObjects` _returnvalue _returnvalue (`self.Check in this radius`) (`|MakeArray` "ObjectTypeQuery3" :!type "EObjectTypeQuery Enum") false (`|MakeArray` null :!type "Actor Object Reference")))
  (if _returnvalue_2
    (for _array_element _outhits
      (bind (_bblockinghit _binitialoverlap _time _distance _location _impactpoint _normal _impactnormal _physmat _hitactor) (`GameplayStatics.BreakHitResult` _array_element))
      (if (`KismetSystemLibrary.DoesImplementInterface` _hitactor "/Game/Hyper/Attribute_System/Blueprints/Pawns_InRadius/BPI_PawnInRadius.BPI_PawnInRadius_C")
        (bind _true (message `/Game/Hyper/Attribute_System/Blueprints/Pawns_InRadius/BPI_PawnInRadius.Should_Receive_Pawn_Info` _hitactor))
        (if _true
          (`KismetArrayLibrary.Array_AddUnique` (`local.Local Pawns in Radius`) _hitactor)
          (if (not (`BlueprintMapLibrary.Map_Contains` (`self.Actors that has In Pawn Widget attached`) _hitactor))
            (bind (_aspawn _bsuccess) (cast `Pawn` _hitactor :!pure true))
            (if _bsuccess
              (if true
                (bind _relative_location (message `/Game/Hyper/Attribute_System/Blueprints/Pawns_InRadius/BPI_PawnInRadius.Get_Relative_Widget_Position` _hitactor))
                (bind _pawnname (message `/Game/Hyper/Attribute_System/Blueprints/Pawns_InRadius/BPI_PawnInRadius.Get_PawnName` _hitactor))
                (bind _returnvalue_3 (`|SpawnActorFromClass` "/Game/Hyper/Attribute_System/Blueprints/Pawns_InRadius/UI/BP_PawnInRadius_Widget_Actor.BP_PawnInRadius_Widget_Actor_C" (`KismetMathLibrary.MakeTransform` _relative_location) "AlwaysSpawn" "OverrideRootScale" null _pawnname _aspawn null))
                (`BlueprintMapLibrary.Map_Add` (`self.Actors that has In Pawn Widget attached`) _hitactor _returnvalue_3)
                (`Actor.K2_AttachToActor` _returnvalue_3 _hitactor "None" "KeepRelative" "KeepRelative" "KeepRelative" true))))))))
  (bind _keys (`BlueprintMapLibrary.Map_Keys` (`self.Actors that has In Pawn Widget attached`)))
  (for _array_element_2 _keys
    (if (not (`KismetArrayLibrary.Array_Contains` (`local.Local Pawns in Radius`) _array_element_2))
      (bind (_value _returnvalue_4) (`BlueprintMapLibrary.Map_Find` (`self.Actors that has In Pawn Widget attached`) _array_element_2))
      (if _returnvalue_4
        (`/Engine/EditorBlueprintResources/StandardMacros.IsValid` _value
          (:`Is Valid`
            (`Actor.K2_DestroyActor` _value))
          (:`Is Not Valid`
            _))
        (`BlueprintMapLibrary.Map_Remove` (`self.Actors that has In Pawn Widget attached`) _array_element_2)))))