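; Crafting component for characters and workstations that turns learned recipes into queued, timed crafting jobs using the inventory manager.
; Crafting removes ingredients and fills queue slots; a polled server check starts slot 0's timer, then outputs items and grants XP, retrying on inventory updates when full.
; Optional on/off switching burns inventory fuel and pauses timers; cancelling refunds ingredients.
; Client actions are mirrored through server events, with OnRep handlers notifying queue and power changes.
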(fn `Add Item To Crafting Queue`
  (params (Item :type "/Game/Hyper/Core/Inventory/Datamodel/Structures/Main_Item_Slot_Structs/Struct_Inventory_Slot_Item Structure"))
  (`/Game/Hyper/Core/Inventory/Blueprints/AC_Inventory_Abstract.Try Add Item to Inventory Automatically` (`/Game/Hyper/Core/Inventory/BlueprintMacroLibrary/BML_Inventory_Component.Get Inventory Manager`) (`local.Item`) (`self.Crafting Queue`) true (`.MaxCraftingqueuestack_21_583E07854961FF3A065CF893E088BFDA` (break `/Game/Hyper/Core/Inventory/Datamodel/Structures/Sub_Structs_Attributes/Struct_Attributes_Crafting` (`.CraftingAttributes_5_DE64E5CE420D6916B14274B3EA0F2FB9` (break `/Game/Hyper/Core/Inventory/Datamodel/Structures/Main_Item_Slot_Structs/Struct_Item` (`/Game/Hyper/Core/Inventory/FunctionLibraries/BFL_InventoryCrafting.Get Inventory info from inventory slot` Item))))) false false false)
  (`self.Queue Updated`))

(fn `Check Amount Of Filled Slots In Queue`
  (returns (`Amount In Crafting Queue` :type Integer) (`All Queue Slots Used` :type Boolean))
  (locals (`Local Amount in crafting queue` :type Integer))
  (for _array_element (`self.Crafting Queue`)
    (if (not (`/Game/Hyper/Core/Inventory/FunctionLibraries/BFL_InventoryCrafting.Is Item Empty?` _array_element))
      (`/Engine/EditorBlueprintResources/StandardMacros.IncrementInt` (`local.Local Amount in crafting queue`))))
  (return (`local.Local Amount in crafting queue`) (select `bool` (`self.Create Crafting Queue Slots Dynamically`) :`false` (>= (`local.Local Amount in crafting queue`) (`KismetArrayLibrary.Array_Length` (`self.Crafting Queue`))))))

(fn `Check To Start Fuel Timer`
  (returns (`Found And Removed Fuel` :type Boolean))
  (locals (`Local Found Fuel In Inventory` :type Boolean))
  (bind _component (`/Game/Hyper/Core/Inventory/BlueprintMacroLibrary/BML_Inventory_Component.Get Inventory Manager`))
  (for _array_element (`self.Accepted Fuel`)
    (bind _success (`/Game/Hyper/Core/Inventory/Blueprints/AC_Inventory_Abstract.Remove Item From Inventory Automatically` _component _array_element 1 (`/Game/Hyper/Core/Inventory/Blueprints/AC_Inventory_Abstract.Inventory Slots` _component) false))
    (if _success
      (set `local.Local Found Fuel In Inventory` true)
      (set `self.Current Fuel` _array_element)
      (break)))
  (if (`local.Local Found Fuel In Inventory`)
    (set `self.Current Fuel Time` (* (`.Combustionratepersecond_7_8673B1C846CBC780F48869A0E65D2985` (break `/Game/Hyper/Core/Inventory/Datamodel/Structures/Sub_Structs_Attributes/Struct_Attributes_Combustibles` (`.CombustableAttributes_14_0DCA8AB044B6CB6BD18E98BC265BD16D` (break `/Game/Hyper/Core/Inventory/Datamodel/Structures/Main_Item_Slot_Structs/Struct_Item` (`/Game/Hyper/Core/Inventory/FunctionLibraries/BFL_InventoryCrafting.Get Inventory info from inventory slot` (`self.Current Fuel`)))))) (`self.Combustion Rate Multiplier`)))
    (return true)
    (else
      (return false))))

(fn `Craft Item by Action Type`
  (params (Item :type "/Game/Hyper/Core/Inventory/Datamodel/Structures/Main_Item_Slot_Structs/Struct_Inventory_Slot_Item Structure") (`Custom Amount` :type Integer) (`Action Type` :type "/Game/Hyper/Core/Crafting/Datamodel/Enumerations/Enum_CraftingAction_Types Enum" :default "NewEnumerator6"))
  (locals (`Local Craftable Amount` :type Integer :default 0))
  (bind _component (`/Game/Hyper/Core/Inventory/BlueprintMacroLibrary/BML_Inventory_Component.Get Inventory Manager`))
  (bind _max_craft_amount_override (`self.Max Craft Amount override`))
  (bind _local_craftable_amount (`local.Local Craftable Amount`))
  (bind _local_craftable_amount_2 (`local.Local Craftable Amount`))
  (bind _max_craft_amount_override_2 (`self.Max Craft Amount override`))
  (bind _custom_amount (`local.Custom Amount`))
  (bind ((`Item_2_C7967C054AE750B79BB1FDB9058FE0B3` _item) (`Durabilitydetails_24_1A7269D6428BC693FF3A859CFE819E71` _durabilitydetails) (`TradingandLootdetails_30_A4191A2D48AF499B2B301CAED61CB925` _tradingandlootdetails) (`Owningactor_40_506222B0483BEF8929F316B61301B204` _owningactor)) (break `/Game/Hyper/Core/Inventory/Datamodel/Structures/Main_Item_Slot_Structs/Struct_Inventory_Slot_Item` (`local.Item`)))
  (bind (_number_of_items_craftable _no_items_can_be_made _number_of_items_fit_in_crafting_queue) (`self.Get Max Amount Of Items Craftable` (`local.Item`) (`/Game/Hyper/Core/Inventory/Blueprints/AC_Inventory_Abstract.Inventory Slots` (`/Game/Hyper/Core/Inventory/BlueprintMacroLibrary/BML_Inventory_Component.Get Inventory Manager`))))
  (bind _returnvalue (select `bool` (>= _custom_amount _local_craftable_amount_2) :`false` _custom_amount :`true` _local_craftable_amount_2))
  (bind _returnvalue_2 (select `bool` (> _local_craftable_amount _number_of_items_fit_in_crafting_queue) :`false` _local_craftable_amount :`true` _number_of_items_fit_in_crafting_queue))
  (bind _returnvalue_3 (select `/Game/Hyper/Core/Crafting/Datamodel/Enumerations/Enum_CraftingAction_Types` (`local.Action Type`) :`NewEnumerator0` 1 :`NewEnumerator2` 5 :`NewEnumerator4` 10 :`NewEnumerator3` (select `bool` (> _returnvalue _max_craft_amount_override_2) :`false` _returnvalue :`true` _max_craft_amount_override_2) :`NewEnumerator1` (select `bool` (> _returnvalue_2 _max_craft_amount_override) :`false` _returnvalue_2 :`true` _max_craft_amount_override)))
  ;[0.05098 0.05098 0.05098] Only craft when we dont have a turn on off or when we do have turn on off, craft when its turned on
  (if (not (xor (`self.Has Turn On Off`) (`self.Is On`)))
    (set `local.Local Craftable Amount` _number_of_items_craftable)
    (if (and (>= _number_of_items_craftable 1) (not (<= _number_of_items_fit_in_crafting_queue 0)))
      (for _array_element (`.Recipe_13_58CFCD784A705C8DF5E133AA64AA5329` (break `/Game/Hyper/Core/Inventory/Datamodel/Structures/Sub_Structs_Attributes/Struct_Attributes_Crafting` (`.CraftingAttributes_5_DE64E5CE420D6916B14274B3EA0F2FB9` (break `/Game/Hyper/Core/Inventory/Datamodel/Structures/Main_Item_Slot_Structs/Struct_Item` (`/Game/Hyper/Core/Inventory/FunctionLibraries/BFL_InventoryCrafting.Get Inventory info from inventory slot` (`local.Item`))))))
        (`/Game/Hyper/Core/Inventory/Blueprints/AC_Inventory_Abstract.Remove Item From Inventory Automatically` _component _array_element (* (`.Amount_5_3D501FFE494086BDD8C291A969150384` (break `/Game/Hyper/Core/Inventory/Datamodel/Structures/Main_Item_Slot_Structs/Struct_Inventory_Slot_Item` _array_element)) _returnvalue_3) (`/Game/Hyper/Core/Inventory/Blueprints/AC_Inventory_Abstract.Inventory Slots` _component) false))
      (`self.Add Item To Crafting Queue` (make `/Game/Hyper/Core/Inventory/Datamodel/Structures/Main_Item_Slot_Structs/Struct_Inventory_Slot_Item` _item _returnvalue_3 0 false _durabilitydetails _tradingandlootdetails true _owningactor (struct :`Hotbarslotindex` 999 :`Inventoryslotindex` 999) (struct :`Linkedtothisequipmentslot` "NewEnumerator13" :`AmmoSlot` (struct :`AmmoDataTable` (struct :`DataTable` "/Script/Engine.DataTable'/Game/Hyper/Core/Equipment_Manager/Datamodel/Datatables/DT_Ammo.DT_Ammo'"))))))))

(fn `Execute on Off Logic`
  (params (`Switch State` :type Boolean))
  (returns (`Is On` :type Boolean))
  ;[0.05098 0.05098 0.05098] Only execute logic if we have turn on off
  (if (`self.Has Turn On Off`)
    (if (`local.Switch State`)
      (if (`self.Is On`)
        _
        (elif (`self.Consumes Fuel When On`)
          (bind _found_and_removed_fuel (`self.Check To Start Fuel Timer`))
          (if _found_and_removed_fuel
            (`self.Event: Start Fuel Timer`)
            (set `self.Is On` true :!label _label)
            (`KismetSystemLibrary.K2_UnPauseTimerHandle` (`self.Crafting Queue Timer Handle`))
            (`KismetSystemLibrary.K2_UnPauseTimerHandle` (`self.Fuel Timer Handle`))
            (return true)
            (else
              _))
          (else
            (goto _label))))
      (set `self.Is On` false)
      (`KismetSystemLibrary.K2_PauseTimerHandle` (`self.Crafting Queue Timer Handle`))
      (`KismetSystemLibrary.K2_PauseTimerHandle` (`self.Fuel Timer Handle`))
      (return false))))

(fn `Get Amount Of Filled Slots In Queue`
  (returns (`Amount in crafting queue` :type Integer) (`All queue slots used` :type Boolean))
  (locals (`Local Amount in crafting queue` :type Integer))
  (bind _crafting_queue (`self.Crafting Queue`))
  (bind _local_amount_in_crafting_queue (`local.Local Amount in crafting queue`))
  (for _array_element _crafting_queue
    (if (not (`/Game/Hyper/Core/Inventory/FunctionLibraries/BFL_InventoryCrafting.Is Item Empty?` _array_element))
      (set `local.Local Amount in crafting queue` (+ (`local.Local Amount in crafting queue`) 1))))
  (return _local_amount_in_crafting_queue (select `bool` (`self.Create Crafting Queue Slots Dynamically`) :`false` (>= _local_amount_in_crafting_queue (`KismetArrayLibrary.Array_Length` _crafting_queue)))))

(fn `Get Max Amount Of Items Craftable`
  (params (Recipe :type "/Game/Hyper/Core/Inventory/Datamodel/Structures/Main_Item_Slot_Structs/Struct_Inventory_Slot_Item Structure") (`Target Array` :type "Array of /Game/Hyper/Core/Inventory/Datamodel/Structures/Main_Item_Slot_Structs/Struct_Inventory_Slot_Item Structure (by ref)"))
  (returns (`Number of items craftable` :type Integer) (`No items can be made` :type Boolean) (`Number of items fit in crafting queue` :type Integer))
  (locals (`Local Recipe to be made` :type "Array of /Game/Hyper/Core/Inventory/Datamodel/Structures/Main_Item_Slot_Structs/Struct_Inventory_Slot_Item Structure") (`Lowest number of possible items to be crafted` :type Integer :default 999999))
  (bind _lowest_number_of_possible_items_to_be_crafted (`local.Lowest number of possible items to be crafted`))
  (bind _lowest_number_of_possible_items_to_be_crafted_2 (`local.Lowest number of possible items to be crafted`))
  (bind ((`Recipe_13_58CFCD784A705C8DF5E133AA64AA5329` _recipe) (`MaxCraftingqueuestack_21_583E07854961FF3A065CF893E088BFDA` _maxcraftingqueuestack)) (break `/Game/Hyper/Core/Inventory/Datamodel/Structures/Sub_Structs_Attributes/Struct_Attributes_Crafting` (`.CraftingAttributes_5_DE64E5CE420D6916B14274B3EA0F2FB9` (break `/Game/Hyper/Core/Inventory/Datamodel/Structures/Main_Item_Slot_Structs/Struct_Item` (`/Game/Hyper/Core/Inventory/FunctionLibraries/BFL_InventoryCrafting.Get Inventory info from inventory slot` Recipe)))))
  (bind _output_get (set `local.Local Recipe to be made` _recipe))
  (for _array_element _output_get
    (bind _returnvalue (`KismetMathLibrary.FFloor` (/ (`KismetMathLibrary.Conv_IntToDouble` (`/Game/Hyper/Core/Inventory/Blueprints/AC_Inventory_Abstract.How many of item in inventory` (`/Game/Hyper/Core/Inventory/BlueprintMacroLibrary/BML_Inventory_Component.Get Inventory Manager`) _array_element (`local.Target Array`))) (`KismetMathLibrary.Conv_IntToDouble` (`.Amount_5_3D501FFE494086BDD8C291A969150384` (break `/Game/Hyper/Core/Inventory/Datamodel/Structures/Main_Item_Slot_Structs/Struct_Inventory_Slot_Item` _array_element))))))
    (if (< _returnvalue (`local.Lowest number of possible items to be crafted`))
      (set `local.Lowest number of possible items to be crafted` _returnvalue)))
  (return _lowest_number_of_possible_items_to_be_crafted (or (<= _lowest_number_of_possible_items_to_be_crafted_2 0) (> _lowest_number_of_possible_items_to_be_crafted_2 9999)) (select `bool` (`self.Create Crafting Queue Slots Dynamically`) :`false` (* _maxcraftingqueuestack (- (`KismetArrayLibrary.Array_Length` (`self.Crafting Queue`)) (`self.Get Amount Of Filled Slots In Queue`))) :`true` _lowest_number_of_possible_items_to_be_crafted)))

(fn `Initialize Crafting Queue`
  (for _ (range 1 (+ (`self.Amount Of Crafting Queue Slots`) 1))
    (`KismetArrayLibrary.Array_Add` (`self.Crafting Queue`) (make `/Game/Hyper/Core/Inventory/Datamodel/Structures/Main_Item_Slot_Structs/Struct_Inventory_Slot_Item` :`Item` (make `DataTableRowHandle` "/Game/Hyper/Core/Inventory/Datamodel/Datatables/DT_Items.DT_Items" "Empty")))))

(fn `Learn Recipe`
  (params (`Recipe Item` :type "/Game/Hyper/Core/Inventory/Datamodel/Structures/Main_Item_Slot_Structs/Struct_Inventory_Slot_Item Structure") (`Source Slot Index` :type Integer) (`Target Array` :type "Array of /Game/Hyper/Core/Inventory/Datamodel/Structures/Main_Item_Slot_Structs/Struct_Inventory_Slot_Item Structure") (`Is From Hotbar` :type Boolean))
  (returns (Success :type Boolean))
  (locals (`Local Slots` :type "Array of /Game/Hyper/Core/Inventory/Datamodel/Structures/Main_Item_Slot_Structs/Struct_Inventory_Slot_Item Structure"))
  (bind _component (`/Game/Hyper/Core/Inventory/BlueprintMacroLibrary/BML_Inventory_Component.Get Inventory Manager`))
  (bind (_thisitemisarecipetolearn _whichitemtolearn) (break `/Game/Hyper/Core/Inventory/Datamodel/Structures/Sub_Structs_Attributes/Struct_Attributes_LearningRecipe` (`.RecipeAttributes_62_74D73B024863421BF2AA82A29D0C60EF` (break `/Game/Hyper/Core/Inventory/Datamodel/Structures/Main_Item_Slot_Structs/Struct_Item` (`/Game/Hyper/Core/Inventory/FunctionLibraries/BFL_InventoryCrafting.Get Inventory info from inventory slot` `Recipe Item`)))))
  (if _thisitemisarecipetolearn
    ;[0.05098 0.05098 0.05098] Check if we haven't already learned this recipe, we dont want to return success if we have already learned the item
    (bind _item_found_in_array (`/Game/Hyper/Core/Inventory/Blueprints/AC_Inventory_Abstract.Array Contains Item` (`/Game/Hyper/Core/Inventory/BlueprintMacroLibrary/BML_Inventory_Component.Get Inventory Manager`) (`self.Learned Recipes`) _whichitemtolearn))
    (if _item_found_in_array
      (return false)
      (elif (`.IsCraftable_1_CEC66577442A51DFD81DF1BDAE85A777` (break `/Game/Hyper/Core/Inventory/Datamodel/Structures/Sub_Structs_Attributes/Struct_Attributes_Crafting` (`.CraftingAttributes_5_DE64E5CE420D6916B14274B3EA0F2FB9` (break `/Game/Hyper/Core/Inventory/Datamodel/Structures/Main_Item_Slot_Structs/Struct_Item` (`/Game/Hyper/Core/Inventory/FunctionLibraries/BFL_InventoryCrafting.Get Inventory info from inventory slot` _whichitemtolearn)))))
        (`KismetArrayLibrary.Array_AddUnique` (`self.Learned Recipes`) _whichitemtolearn)
        (`|ExecutionSequence`
          (:`then_0`
            ;[0.05098 0.05098 0.05098] Choose from which slots we got the recipe, if we got the recipe from the hotbar we need to empty the hotbar slot
            (if (`local.Is From Hotbar`)
              (bind _hotbar_component (`/Game/Hyper/Core/Inventory/Blueprints/AC_Inventory_Abstract.Get Linked Hotbar Component` _component))
              (`/Game/Hyper/Core/Inventory/Blueprints/AC_Inventory_Abstract.Set Inventory Slot to empty by index` _component (`/Game/Hyper/Core/Inventory/Blueprints/AC_Hotbar_Abstract.Hotbar Slots` _hotbar_component) (`local.Source Slot Index`))
              (else
                (`/Game/Hyper/Core/Inventory/Blueprints/AC_Inventory_Abstract.Set Inventory Slot to empty by index` _component (`/Game/Hyper/Core/Inventory/Blueprints/AC_Inventory_Abstract.Inventory Slots` _component) (`local.Source Slot Index`)))))
          (:`then_1`
            (`/Game/Hyper/Core/Inventory/Blueprints/AC_Inventory_Abstract.Inventory Updated` (`/Game/Hyper/Core/Inventory/BlueprintMacroLibrary/BML_Inventory_Component.Get Inventory Manager`))
            (return true)))))))

(fn `OnRep_Crafting Queue_Execution`
  ;[0.05098 0.05098 0.05098] Notify clients of crafting queue update
  (`self.Queue Updated`))

(fn `OnRep_Is On_Execution`
  ;[0.05098 0.05098 0.05098] Notify clients of workstation toggle
  (`self.Workstation Switched On/Off` (`self.Is On`)))

(fn `Process Crafting Queue Slot 0 And Initialize Timer`
  ;[0.05098 0.05098 0.05098] Get the crafting queue at index 0
  (set `self.Current item being crafted` (`|GetArrayItem` (`self.Crafting Queue`)))
  ;[0.05098 0.05098 0.05098] Checks amount of slot
  ; if zero -> remove slot
  ; Remove slot at index 0,
  ; Get all other slots, and move to  current index -1 (by removing the item in the array)
  ; Create new empty slot in the end of the array
  (bind (_item _stackable _max_stack_size _amount_in_slot) (`/Game/Hyper/Core/Inventory/Blueprints/AC_Inventory_Abstract.Get Inventory Item info` (`/Game/Hyper/Core/Inventory/BlueprintMacroLibrary/BML_Inventory_Component.Get Inventory Manager`) (`self.Current Item Being Crafted`) false 0))
  (if (<= _amount_in_slot 0)
    (`KismetArrayLibrary.Array_Remove` (`self.Crafting Queue`))
    (`/Game/Hyper/Core/Inventory/Blueprints/AC_Inventory_Abstract.Create Empty slot` (`/Game/Hyper/Core/Inventory/BlueprintMacroLibrary/BML_Inventory_Component.Get Inventory Manager`) (`self.Crafting Queue`))
    (`self.Event: Reset crafting queue check`)
    (else
      (`self.Start Crafting queue Timer` (`self.Current Item Being Crafted`)))))

(fn `Remove All Items From Queue`
  (for (_array_element _array_index) (`self.Crafting Queue`)
    (`self.Remove Item Or Slot From Queue On Slot Index` _array_element true _array_index))
  (`self.Queue Updated`))

(fn `Remove Item Or Slot From Queue On Slot Index`
  (params (`Inventory Slot Item` :type "/Game/Hyper/Core/Inventory/Datamodel/Structures/Main_Item_Slot_Structs/Struct_Inventory_Slot_Item Structure") (`Remove All From Stack` :type Boolean) (`Slot Index` :type Integer))
  (locals (`Amount Multiplier` :type Integer))
  (bind _component (`/Game/Hyper/Core/Inventory/BlueprintMacroLibrary/BML_Inventory_Component.Get Inventory Manager`))
  (bind ((`Recipe_13_58CFCD784A705C8DF5E133AA64AA5329` _recipe)) (break `/Game/Hyper/Core/Inventory/Datamodel/Structures/Sub_Structs_Attributes/Struct_Attributes_Crafting` (`.CraftingAttributes_5_DE64E5CE420D6916B14274B3EA0F2FB9` (break `/Game/Hyper/Core/Inventory/Datamodel/Structures/Main_Item_Slot_Structs/Struct_Item` (`/Game/Hyper/Core/Inventory/FunctionLibraries/BFL_InventoryCrafting.Get Inventory info from inventory slot` (`local.Inventory Slot Item`))))))
  (if (not (`/Game/Hyper/Core/Inventory/FunctionLibraries/BFL_InventoryCrafting.Is Item Empty?` (`|GetArrayItem` (`self.Crafting Queue`) `Slot Index`)))
    (set `local.Amount Multiplier` (select `bool` (`local.Remove All From Stack`) :`false` 1 :`true` (`.Amount_5_3D501FFE494086BDD8C291A969150384` (break `/Game/Hyper/Core/Inventory/Datamodel/Structures/Main_Item_Slot_Structs/Struct_Inventory_Slot_Item` (`local.Inventory Slot Item`)))))
    ;[0.05098 0.05098 0.05098] Check if all the items in the recipe can be returned to the inventory
    (bind _all_items_can_be_added (`/Game/Hyper/Core/Inventory/Blueprints/AC_Inventory_Abstract.Can all items be added` (`/Game/Hyper/Core/Inventory/BlueprintMacroLibrary/BML_Inventory_Component.Get Inventory Manager`) _recipe (`local.Remove All From Stack`) (`local.Amount Multiplier`)))
    (if _all_items_can_be_added
      ;[0.05098 0.05098 0.05098] Return all resources to inventory
      (for _array_element _recipe
        (bind ((`Item_2_C7967C054AE750B79BB1FDB9058FE0B3` _item) (`Amount_5_3D501FFE494086BDD8C291A969150384` _amount) (`Isbeingcrafted_7_98AF152C4CD6A4BA93D3868E9782440B` _isbeingcrafted) (`Durabilitydetails_24_1A7269D6428BC693FF3A859CFE819E71` _durabilitydetails) (`TradingandLootdetails_30_A4191A2D48AF499B2B301CAED61CB925` _tradingandlootdetails)) (break `/Game/Hyper/Core/Inventory/Datamodel/Structures/Main_Item_Slot_Structs/Struct_Inventory_Slot_Item` _array_element))
        (`/Game/Hyper/Core/Inventory/Blueprints/AC_Inventory_Abstract.Try Add Item to Inventory Automatically` _component (make `/Game/Hyper/Core/Inventory/Datamodel/Structures/Main_Item_Slot_Structs/Struct_Inventory_Slot_Item` :`Item` _item :`Amount` (* _amount (`local.Amount Multiplier`)) :`Is being crafted` _isbeingcrafted :`Durability details` _durabilitydetails :`Trading and Loot details` _tradingandlootdetails) (`/Game/Hyper/Core/Inventory/Blueprints/AC_Inventory_Abstract.Inventory Slots` _component) false 0 false false true))
      ;[0.05098 0.05098 0.05098] Remove item from crafting queue and update the queue
      (bind (_success _empty_slot) (`/Game/Hyper/Core/Inventory/Blueprints/AC_Inventory_Abstract.Remove item at slot index` (`/Game/Hyper/Core/Inventory/BlueprintMacroLibrary/BML_Inventory_Component.Get Inventory Manager`) (`local.Slot Index`) (`local.Amount Multiplier`) (`self.Crafting Queue`) false false))
      (`self.Queue Updated`)
      ;[0.05098 0.05098 0.05098] Reset the queue timer if we removed an item from the first slot
      (if (and _empty_slot (== (`local.Slot Index`) 0))
        (`KismetSystemLibrary.K2_ClearAndInvalidateTimerHandle` (`self.Crafting Queue Timer Handle`))
        (`self.Reset Crafting Queue Ended Gate`)
        (`self.Event: Reset Crafting Queue Check`)))))

(fn `Set Default Known Crafting Recipes`
  ;[0.05098 0.05098 0.05098] Loop over all items and get each catagory
  (bind _outrownames (`DataTableFunctionLibrary.GetDataTableRowNames` "/Game/Hyper/Core/Inventory/Datamodel/Datatables/DT_Items.DT_Items"))
  (for _array_element _outrownames
    (bind _returnvalue (`|GetDataTableRow` "/Game/Hyper/Core/Inventory/Datamodel/Datatables/DT_Items.DT_Items" _array_element)
      (:`then`
        (if (`.CraftingRecipeisknownbydefault_24_908E47C34E93C1B9BF9ACCB808672515` (break `/Game/Hyper/Core/Inventory/Datamodel/Structures/Sub_Structs_Attributes/Struct_Attributes_Crafting` (`.CraftingAttributes_5_DE64E5CE420D6916B14274B3EA0F2FB9` (break `/Game/Hyper/Core/Inventory/Datamodel/Structures/Main_Item_Slot_Structs/Struct_Item` _returnvalue))))
          (`KismetArrayLibrary.Array_Add` (`self.Learned Recipes`) (make `/Game/Hyper/Core/Inventory/Datamodel/Structures/Main_Item_Slot_Structs/Struct_Inventory_Slot_Item` (make `DataTableRowHandle` "/Game/Hyper/Core/Inventory/Datamodel/Datatables/DT_Items.DT_Items" _array_element) 1 0 false (struct :`CurrentDurability` 100.0 :`IsUseable` true) (struct :`Chanceofspawinginvendorinventory` 1.0 :`MinimalAmounttorestock` 1 :`MaximumAmounttorestock` 5 :`MaximumStock` 10) true null (struct :`Hotbarslotindex` 999 :`Inventoryslotindex` 999) (struct :`Linkedtothisequipmentslot` "NewEnumerator13" :`AmmoSlot` (struct :`AmmoDataTable` (struct :`DataTable` "/Script/Engine.DataTable'/Game/Hyper/Core/Equipment_Manager/Datamodel/Datatables/DT_Ammo.DT_Ammo'"))))))))))