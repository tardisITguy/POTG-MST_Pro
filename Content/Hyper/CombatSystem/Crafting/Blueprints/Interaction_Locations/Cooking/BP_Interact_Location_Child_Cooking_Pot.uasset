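; Cooking pot interact location, a child Blueprint that applies a warmed state effect to nearby characters while the workstation is on.
; It binds to the advanced crafting component's on/off event to add or remove the effect for every character already inside the SphereWarmed volume.
; Sphere overlaps add it on entry only when switched on and always remove it on exit, via each character's attribute manager server event.
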(event `self.ReceiveBeginPlay`
  (`parent.ReceiveBeginPlay`)
  (add `/Game/Hyper/Core/Crafting/Blueprints/AC_Crafting_Abstract.Workstation Switched On/Off` (`self.AC_Crafting_Advanced`) (delegate `On/off`)))

(event `On/off`
  (params (`Is On` :type Boolean))
  (bind _overlappingactors (`PrimitiveComponent.GetOverlappingActors` (`self.Sphere_Warmed`) "/Script/Engine.Character"))
  ;[1 1 1] When this location is turned on or off, switch warmed state
  (if `Is On`
    (for _array_element _overlappingactors
      (bind _ascharacter (cast `Character` _array_element))
      (bind _returnvalue (`self.GetComponentByClass` _ascharacter "/Game/Hyper/Core/Attribute_System/Blueprints/AC_Attribute_Manager_Abstact.AC_Attribute_Manager_Abstact_C"))
      (`/Engine/EditorBlueprintResources/StandardMacros.IsValid` _returnvalue
        (:`Is Valid`
          (`/Game/Hyper/Core/Attribute_System/Blueprints/AC_Attribute_Manager_Abstact.Event server: Add or Remove State Effect` _returnvalue "NewEnumerator14" false))))
    (else
      (for _array_element_2 _overlappingactors
        (bind _ascharacter_2 (cast `Character` _array_element_2))
        (bind _returnvalue_2 (`self.GetComponentByClass` _ascharacter_2 "/Game/Hyper/Core/Attribute_System/Blueprints/AC_Attribute_Manager_Abstact.AC_Attribute_Manager_Abstact_C"))
        (`/Engine/EditorBlueprintResources/StandardMacros.IsValid` _returnvalue_2
          (:`Is Valid`
            (`/Game/Hyper/Core/Attribute_System/Blueprints/AC_Attribute_Manager_Abstact.Event server: Add or Remove State Effect` _returnvalue_2 "NewEnumerator14" true)))))))

(event `self.Sphere_Warmed.OnComponentBeginOverlap`
  (params (OverlappedComponent :type "PrimitiveComponent Object Reference") (OtherActor :type "Actor Object Reference") (OtherComp :type "PrimitiveComponent Object Reference") (OtherBodyIndex :type Integer) (bFromSweep :type Boolean) (SweepResult :type "HitResult Structure (by ref)"))
  (if (`/Game/Hyper/Core/Crafting/Blueprints/AC_Crafting_Abstract.Is On` (`self.AC_Crafting_Advanced`))
    (bind _ascharacter (cast `Character` OtherActor))
    (bind _returnvalue (`self.GetComponentByClass` _ascharacter "/Game/Hyper/Core/Attribute_System/Blueprints/AC_Attribute_Manager_Abstact.AC_Attribute_Manager_Abstact_C"))
    (`/Engine/EditorBlueprintResources/StandardMacros.IsValid` _returnvalue
      (:`Is Valid`
        (`/Game/Hyper/Core/Attribute_System/Blueprints/AC_Attribute_Manager_Abstact.Event server: Add or Remove State Effect` _returnvalue "NewEnumerator14" false)))))

(event `self.Sphere_Warmed.OnComponentEndOverlap`
  (params (OverlappedComponent :type "PrimitiveComponent Object Reference") (OtherActor :type "Actor Object Reference") (OtherComp :type "PrimitiveComponent Object Reference") (OtherBodyIndex :type Integer))
  (bind _ascharacter (cast `Character` OtherActor))
  (bind _returnvalue (`self.GetComponentByClass` _ascharacter "/Game/Hyper/Core/Attribute_System/Blueprints/AC_Attribute_Manager_Abstact.AC_Attribute_Manager_Abstact_C"))
  (`/Engine/EditorBlueprintResources/StandardMacros.IsValid` _returnvalue
    (:`Is Valid`
      (`/Game/Hyper/Core/Attribute_System/Blueprints/AC_Attribute_Manager_Abstact.Event server: Add or Remove State Effect` _returnvalue "NewEnumerator14" true))))

(fn `UserConstructionScript`
  (`parent.UserConstructionScript`))