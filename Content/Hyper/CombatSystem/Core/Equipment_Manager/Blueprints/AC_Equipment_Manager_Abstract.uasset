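; Abstract equipment manager component that defines the interface for a character's equipped items, weapons and ammo in the combat system.
; It declares stubbed events and functions for equipping, primary and secondary inputs, equipment slot lookup and ammo handling, with Server and Client naming marking the intended network side.
; Nearly everything is empty or returns defaults; only the equipment RepNotify has logic, forwarding to an empty execution function.
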(event `On Hit With Damage`)

(event `Server Add Ammo To Weapon`
  (params (`Equipment slot` :type "/Game/Hyper/Core/Equipment_Manager/Datamodel/Enumerations/Enum_Equipment_Slots Enum" :default "NewEnumerator13") (Ammo :type "DataTableRowHandle Structure") (Amount :type Integer)))

(event `Server Set Ammo Amount In Equipment`
  (params (`Which equipment slot to find` :type "/Game/Hyper/Core/Equipment_Manager/Datamodel/Enumerations/Enum_Equipment_Slots Enum" :default "NewEnumerator13") (Amount :type Integer) (`Overwrite ammo type` :type Boolean) (`Overwrite ammo to this` :type "DataTableRowHandle Structure")))

(event `Client: Start Update Arrow Rotation`)

(event `Server Update Quiver`)

(event `Server Unequip Ammo`
  (params (`Item Slot` :type "/Game/Hyper/Core/Inventory/Datamodel/Structures/Main_Item_Slot_Structs/Struct_Inventory_Slot_Item Structure")))

(event `Event: Equip Ammo`
  (params (`Item to find` :type "/Game/Hyper/Core/Inventory/Datamodel/Structures/Main_Item_Slot_Structs/Struct_Inventory_Slot_Item Structure")))

(event `Event: Equip`
  (params (`Inventory Slot` :type "/Game/Hyper/Core/Inventory/Datamodel/Structures/Main_Item_Slot_Structs/Struct_Inventory_Slot_Item Structure")))

(event `Event: Unequip`
  (params (`Item slot` :type "/Game/Hyper/Core/Inventory/Datamodel/Structures/Main_Item_Slot_Structs/Struct_Inventory_Slot_Item Structure")))

(event `Server: Set  Ammo In Ammo Slot`
  (params (`Ammo Amount` :type Integer)))

(event `Server: Add Ammo To Ammo Slot`
  (params (`Amount To Add` :type Integer)))

(event `Server: Destroy equipped weapon and set to unarmed`
  (params (Item :type "/Game/Hyper/Core/Inventory/Datamodel/Structures/Main_Item_Slot_Structs/Struct_Inventory_Slot_Item Structure (by ref)") (`Do not add to inventory` :type Boolean) (`Is Instigated by authority` :type Boolean)))

(event `Client: Reinitialize`)

(event `Event: Try Start Primary Action`
  ;[0.05127 0.05127 0.05127] Primary Action
)

(event `Event: Try Stop Primary Action`
  ;[0.05127 0.05127 0.05127] Primary Action
)

(event `Event: Try Start Secondary Action`
  ;[0.05127 0.05127 0.05127] Secondary action
)

(event `Event: Try Stop Secondary Action`
  ;[0.05127 0.05127 0.05127] Secondary action
)

(fn `Add Ammo to Ammo slot`
  (params (`Amount to Add` :type Integer)))

(fn `Check if Ammo Is Accepted in Equipment`
  (params (Equipment :type "/Game/Hyper/Core/Equipment_Manager/Datamodel/Structures/Main_Structs/Struct_Equipment Structure (by ref)") (`Ammo Data Table Row to check` :type "DataTableRowHandle Structure (by ref)"))
  (returns (Accepted :type Boolean))
  (return false))

(fn `Check if Current Equipped Ammo Is Accepted in Equipment`
  (params (Equipment :type "/Game/Hyper/Core/Equipment_Manager/Datamodel/Structures/Main_Structs/Struct_Equipment Structure (by ref)"))
  (returns (Accepted :type Boolean) (`Amount in slot` :type Integer) (Empty :type Boolean))
  (return false 0 false))

(fn `Does actor has required equipmenttype in slot?`
  (params (`Required Equipment Types` :type "Array of /Game/Hyper/Core/Equipment_Manager/Datamodel/Enumerations/Enum_Equipment_Type Enum") (`In slot` :type "/Game/Hyper/Core/Equipment_Manager/Datamodel/Enumerations/Enum_Equipment_Slots Enum" :default "NewEnumerator8"))
  (returns (True :type Boolean))
  (return true))

(fn `Find Attached Equipment slot in equipment array`
  (params (`Which equipment slot to find` :type "/Game/Hyper/Core/Equipment_Manager/Datamodel/Enumerations/Enum_Equipment_Slots Enum" :default "NewEnumerator0"))
  (returns (`Attached equipment found in slot` :type Boolean) (`index of found equipment slot in equipment array` :type Integer) (`The found slot is empty?` :type Boolean) (`attached struct found` :type "/Game/Hyper/Core/Equipment_Manager/Datamodel/Structures/Main_Structs/Struct_Attached_Equipment Structure"))
  (locals (`local equipment slot found` :type Boolean) (`Local index in equipment slot found` :type Integer) (`Local attached struct found` :type "/Game/Hyper/Core/Equipment_Manager/Datamodel/Structures/Main_Structs/Struct_Attached_Equipment Structure")))

(fn `Get Ammo Info in Equiped Weapon`
  (params (`Equipment slot` :type "/Game/Hyper/Core/Equipment_Manager/Datamodel/Enumerations/Enum_Equipment_Slots Enum" :default "NewEnumerator13"))
  (returns (`Max Rounds in Magazine` :type Integer) (`Max Magazines` :type Integer) (`Max total Ammo` :type Integer) (`Added Damage attributes` :type "/Game/Hyper/Core/Equipment_Manager/Datamodel/Structures/Sub_Structs/Struct_CombatAttributes_Damage Structure") (`Selected Ammo Row` :type Name) (`Amount of ammo in weapon` :type Integer) (`Room in weapon magzine` :type Integer) (`Full Magazine` :type Boolean) (Empty :type Boolean))
  (return 0 0 0 (struct) "None" 0 0 false false))

(fn `Get Equipment slot in equipment array`
  (params (`Which equipment slot to find` :type "/Game/Hyper/Core/Equipment_Manager/Datamodel/Enumerations/Enum_Equipment_Slots Enum" :default "NewEnumerator8"))
  (returns (`equipment slot found` :type Boolean) (`index of found equipment slot in equipment array` :type Integer) (`The found slot is empty or unarmed?` :type Boolean) (`item found in equipment slot` :type "/Game/Hyper/Core/Inventory/Datamodel/Structures/Main_Item_Slot_Structs/Struct_Inventory_Slot_Item Structure"))
  (locals (`local item found in equipment slot` :type "/Game/Hyper/Core/Inventory/Datamodel/Structures/Main_Item_Slot_Structs/Struct_Inventory_Slot_Item Structure") (`local equipment slot found` :type Boolean) (`Local index in equipment slot found` :type Integer))
  (return false 0 false))

(fn `Initialize Starting Equipment`)

(fn `OnRep_Equipment`
  (`self.OnRep_Equipment Execution`))

(fn `OnRep_Equipment Execution`)

(fn `Set  Ammo In Ammo Slot`
  (params (`Ammo Amount` :type Integer)))

(fn `Set  Equipment Array Elem By Index`
  (params (Index :type Integer) (`Item Slot` :type "/Game/Hyper/Core/Inventory/Datamodel/Structures/Main_Item_Slot_Structs/Struct_Inventory_Slot_Item Structure") (`Item Data Table Row` :type "DataTableRowHandle Structure") (Amount :type Integer) (Equipment_Slot :type "/Game/Hyper/Core/Equipment_Manager/Datamodel/Structures/Main_Structs/Struct_Equipment_Slot Structure")))

(fn `Set Ammo Amount In Equipment`
  (params (`Which equipment slot to find` :type "/Game/Hyper/Core/Equipment_Manager/Datamodel/Enumerations/Enum_Equipment_Slots Enum" :default "NewEnumerator8") (Amount :type Integer) (`Overwrite ammo type` :type Boolean) (`Overwrite ammo to this` :type "DataTableRowHandle Structure")))

(fn `Set Equipment Slot Data`
  (params (Struct_Inventory_Slot_Item :type "/Game/Hyper/Core/Inventory/Datamodel/Structures/Main_Item_Slot_Structs/Struct_Inventory_Slot_Item Structure (by ref)") (`Equipment Slot` :type "/Game/Hyper/Core/Equipment_Manager/Datamodel/Enumerations/Enum_Equipment_Slots Enum" :default "NewEnumerator13") (`Local Found Equipment Index` :type Integer)))