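; Abstract combat component that declares the shared interface for combat in the Hyper combat system, with nearly every body left as an empty stub.
; It covers aiming and zoom, fire mode, reload, blocking, target locking, crosshairs, projectiles, melee damage, hit reactions and impact effects.
; Aim and zoom OnReps only forward to empty Execution functions, and the default damage handler passes damage through unblocked.
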(event `Initialize hit additive animation`
  (params (`start Actor` :type "Actor Object Reference") (`target Actor` :type "Actor Object Reference") (`Die montgage` :type Boolean)))

(event `Event: Try Start Aiming`
  ;[0.05127 0.05127 0.05127] Aiming
)

(event `Set to ADS`
  (params (GameplayTag_IsADS :type Boolean) (`Should Zoom` :type Boolean :default true))
  ;[0.05127 0.05127 0.05127] Aiming
)

(event `Event: Try Stop Aiming`
  ;[0.05127 0.05127 0.05127] Aiming
)

(event `Event: Try Toggle Firemode`
  ;[0.05127 0.05127 0.05127] Toggle Fire mode
)

(event `Event: Try Reload`
  ;[0.05127 0.05127 0.05127] Reload
)

(event `Event: Try start Blocking`
  ;[0.05127 0.05127 0.05127] Defend/Block
)

(event `Event: Try stop Blocking`
  ;[0.05127 0.05127 0.05127] Defend/Block
)

(event `Event: Try Lock Target`
  ;[0.05127 0.05127 0.05127] Locking and unlocking Target
)

(event `Event: Unlock Target`
  ;[0.05127 0.05127 0.05127] Locking and unlocking Target
)

(event `Event: Initialize Attached Particle Multicast`
  (params (SystemTemplate :type "NiagaraSystem Object Reference") (AttachToComponent :type "SceneComponent Object Reference") (AttachPointName :type Name) (Location :type "Vector Structure") (`On attached equipment` :type Boolean) (Index :type Integer))
  ;[0.05127 0.05127 0.05127] play  localy, and than on Server
)

(event `Server: Spawn Projectile`
  (params (Class :type "Object Class Reference") (`Static Mesh` :type "StaticMesh Object Reference") (Weapon_Info :type "/Game/Hyper/Core/Equipment_Manager/Datamodel/Structures/Main_Structs/Struct_Equipment Structure") (`Initial Projectile Speed` :type "Float (single-precision)") (Time_Active :type "Float (double-precision)") (Transform :type "Transform Structure") (`Used Ammo` :type "DataTableRowHandle Structure") (Velocity :type "Vector Structure")))

(event `Event:Spawn Hit Damage Text`
  (params (`Spawn Transform Location` :type "Vector Structure") (`Hit Text` :type Text))
  ;[0.05127 0.05127 0.05127] Hit Text
)

(event `Event: Spawn Impact`
  (params (SpawnTransform :type "Transform Structure") (Hit :type "HitResult Structure") (Instigator :type "Pawn Object Reference") (Owner :type "Actor Object Reference"))
  ;[0.05127 0.05127 0.05127] Spawn impact effect via server call
)

(event `Event: Initialize Try Inflict Melee Damage`
  (params (`Attack Type` :type "/Game/Hyper/Core/Equipment_Manager/Datamodel/Enumerations/Enum_Melee_Attack_Types Enum" :default "NewEnumerator0")))

(event `Set to In Combat mode`)

(event `Initialize Try Apply Damage`
  (params (`Hit info` :type "HitResult Structure") (`Damage Causer` :type "Actor Object Reference") (`Is Heavy Attack` :type Boolean)))

(event `Start Crosshair Timer`)

(event `Stop Crosshair Timer`)

(event `Reset set original FOV Zoom`)

(event `Event: Start Aim Zoom`)

(event `Event: Reverse Aim Zoom`)

(fn `Add Secondary Offset To Equipped Weapon`
  (params (Revert :type Boolean)))

(fn `Apply_Damage`
  (params (`Hit Actor` :type "Actor Object Reference") (`Hit info` :type "HitResult Structure") (`Attack Type` :type "/Game/Hyper/Core/Equipment_Manager/Datamodel/Enumerations/Enum_Melee_Attack_Types Enum" :default "NewEnumerator0") (`Override Damage Amount` :type "Float (double-precision)"))
  (returns (`Damage Applied` :type "Float (single-precision)") (`health is zero after this hit` :type Boolean)))

(fn `Block Damage?`
  (params (`Hit Causing Actor` :type "Actor Object Reference"))
  (returns (Blocked :type Boolean)))

(fn `Can Peform Combat Action?`
  (returns (`Can Execute` :type Boolean))
  (return false))

(fn `Choose_Hit_Montage`
  (params (`Hit Direction` :type "/Game/Hyper/Locomotion/Chars/Mannequin_UE5/Anims/Enum_AnimEnum_CardinalDirection Enum" :default "NewEnumerator0") (`Die montgage` :type Boolean) (`Attack Type` :type "/Game/Hyper/Core/Equipment_Manager/Datamodel/Enumerations/Enum_Melee_Attack_Types Enum" :default "NewEnumerator0"))
  (returns (Montage :type "AnimMontage Object Reference"))
  (return null))

(fn `Get Hit Direction`
  (params (`start Actor` :type "Actor Object Reference") (`target Actor` :type "Actor Object Reference"))
  (returns (`Hit Direction` :type "/Game/Hyper/Locomotion/Chars/Mannequin_UE5/Anims/Enum_AnimEnum_CardinalDirection Enum") (`Hit Direction in degrees` :type "Float (single-precision)")))

(fn `Get Locking Attributes Of Equipment`
  (params (Equipment :type "/Game/Hyper/Core/Equipment_Manager/Datamodel/Enumerations/Enum_Equipment_Slots Enum" :default "NewEnumerator8"))
  (returns (`Can lock onto target with this weapon` :type Boolean) (`Rotate to locked target` :type Boolean) (`Use outliner` :type Boolean) (`Lose Lock after this distance` :type "Float (double-precision)"))
  (return false false false 0.0))

(fn `Get_Active_Camera_Component`
  (returns (`active camera` :type "CameraComponent Object Reference"))
  (locals (`local active camera` :type "CameraComponent Object Reference")))

(fn `Handle Take Damage`
  (params (`Damage In` :type "Float (double-precision)") (`Damage Type` :type "DamageType Object Reference") (`Instigated By` :type "Controller Object Reference") (`Damage Causer` :type "Actor Object Reference"))
  (returns (`Damage Out` :type "Float (double-precision)") (Blocked :type Boolean))
  (return `Damage In` false))

(fn `OnRep_Is_Aiming`
  (`self.OnRep_Is_Aiming_Execution`))

(fn `OnRep_Is_Aiming_Execution`)

(fn `OnRep_Should Zoom`
  (`self.OnRep_Should Zoom_Execution`))

(fn `OnRep_Should Zoom_Execution`)

(fn `Spawn Hit Damage Text`
  (params (`Spawn Transform Location` :type "Vector Structure") (`Hit Text` :type Text)))

(fn `Spawn Projectile`
  (params (Class :type "Object Class Reference") (`Static Mesh` :type "StaticMesh Object Reference") (Weapon_Info :type "/Game/Hyper/Core/Equipment_Manager/Datamodel/Structures/Main_Structs/Struct_Equipment Structure") (`Initial Projectile Speed` :type "Float (single-precision)") (Time_Active :type "Float (double-precision)") (Transform :type "Transform Structure") (`Used Ammo` :type "DataTableRowHandle Structure") (Velocity :type "Vector Structure")))

(fn `Try Create Crosshair`
  (params (`Equipment info` :type "/Game/Hyper/Core/Equipment_Manager/Datamodel/Structures/Main_Structs/Struct_Equipment Structure")))

(fn `Try Inflict Melee Damage`
  (params (`Attack Type` :type "/Game/Hyper/Core/Equipment_Manager/Datamodel/Enumerations/Enum_Melee_Attack_Types Enum" :default "NewEnumerator0"))
  (locals (`Local hits` :type "Array of HitResult Structure") (`Local Hit` :type "HitResult Structure") (`Local Hit Actor` :type "Actor Object Reference") (`Local actors prevsouly hitted` :type "Array of Actor Object Reference") (`Local Hit Location` :type "Vector Structure" :default (0.0 0.0 0.0))))

(fn `Try_Remove_Crosshair`)

(fn `Update Crosshair`)

(fn `Update_Quiver_Amount`)

(fn `Which weapon to use for blocking`
  (returns (`Able to block` :type Boolean) (`Weapon found that can block` :type "/Game/Hyper/Core/Equipment_Manager/Datamodel/Structures/Main_Structs/Struct_Equipment Structure") (`Equipment slot used to block` :type "/Game/Hyper/Core/Equipment_Manager/Datamodel/Enumerations/Enum_Equipment_Slots Enum") (`Defend attributes` :type "/Game/Hyper/Core/Equipment_Manager/Datamodel/Structures/Sub_Structs/Struct_CombatAttributes_Defend Structure")))