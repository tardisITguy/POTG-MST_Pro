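; Abstract building-system component that defines the interface for placing, repairing and interacting with buildables in the combat system.
; Its events and functions are mostly empty stubs covering build modes, ghost mesh rotation, spline building, radial menu selection, server spawning and spawning from saves.
; The only real logic matches an inventory item to a DT_Buildables row by row name.
; Default stubs authorize every player and report no spline buildable.
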(event `Event: Spawn Spline on server`
  (params (`Builable Struct` :type "/Game/Hyper/Core/BuildingSystem/Datamodel/Structures/Struct_Buildable_Info Structure") (`Buildable Data Table Row` :type "DataTableRowHandle Structure") (`Spline point locations` :type "Array of Vector Structure (by ref)")))

(event `Event: Check and Try Repair`
  (params (`Actor trying to repair` :type "Actor Object Reference") (Component :type "PrimitiveComponent Object Reference")))

(event `Event: Stop Spline Build Mode`)

(event `Event: Initialize Spline Build Mode`)

(event `Event: Flip Rotation of Spline`)

(event `Event: Remove Last Spline Point`)

(event `Event: Add Spline Point`)

(event `Event: Set Active Spline Point Location`)

(event `Event: Stop Build Mode`)

(event `Event: Start Build Mode`
  (params (`Buildable Data Table Row Hanlde` :type "DataTableRowHandle Structure")))

(event `Event: Start Build mode from inventory slot`
  (params (`Inventory Slot` :type "/Game/Hyper/Core/Inventory/Datamodel/Structures/Main_Item_Slot_Structs/Struct_Inventory_Slot_Item Structure")))

(event `Event: Switch Buildmode`)

(event `Event: Start Rotate Ghost Mesh`
  (params (Clockwise :type Boolean) (`Rotation Muliplier` :type "Float (double-precision)")))

(event `Event: Stop Rotate Ghost Mesh`)

(event `Event: Try mode functionality`
  (params (Mode :type "/Game/Hyper/Core/BuildingSystem/Datamodel/Enumerations/Enum_Build_Actions Enum" :default "NewEnumerator0") (`Looked at buildable` :type "/Game/Hyper/Core/BuildingSystem/Blueprints/BP_Buildable_Abstract Object Reference")))

(event `Event: Start Progressbar`)

(event `Radial Menu Open`)

(event `Radial Menu Close`)

(event `Event: Spawn Buildable`
  (params (`Is buildmode on` :type Boolean) (`Can Build` :type Boolean) (transform :type "Transform Structure") (`selected buildable` :type "/Game/Hyper/Core/BuildingSystem/Datamodel/Structures/Struct_Buildable_Info Structure") (`hit actor` :type "Actor Object Reference") (`buildable data table row` :type "DataTableRowHandle Structure") (`Inventory Ref` :type "/Game/Hyper/Core/Inventory/Blueprints/AC_Inventory_Abstract Object Reference")))

(event `Event: Try Interact with Buildable`
  (params (Controller :type "Controller Object Reference")))

(event `Event: spawn buildables from save`)

(fn `Close_Radial_Menu_And_Select_Segment`)

(fn `Get Buildables Of Category`
  (params (`Categories to find` :type "Array of /Game/Hyper/Core/BuildingSystem/Datamodel/Enumerations/Enum_Buildable_Categories Enum") (`Categories to ignore` :type "Array of /Game/Hyper/Core/BuildingSystem/Datamodel/Enumerations/Enum_Buildable_Categories Enum"))
  (returns (` Buildables found in categories` :type "Array of /Game/Hyper/Core/BuildingSystem/Datamodel/Structures/Struct_Buildable_Info Structure") (`datatable rows found in category` :type "Array of DataTableRowHandle Structure"))
  (locals (`Local buildables found in category` :type "Array of /Game/Hyper/Core/BuildingSystem/Datamodel/Structures/Struct_Buildable_Info Structure") (`Local datatable rows found in category` :type "Array of DataTableRowHandle Structure") (`Local item should be ignored` :type Boolean :default false)))

(fn `Get Coupled Buildable Master From Spline`
  (params (`Potential Spline Buildable` :type "Actor Object Reference") (`Spline Mesh` :type "SplineMeshComponent Object Reference"))
  (returns (`Coupled Buildable` :type "/Game/Hyper/Core/BuildingSystem/Blueprints/BP_Buildable_Abstract Object Reference") (`Is Spline` :type Boolean))
  (return null false))

(fn `Is Player Authorized With Buildable`
  (params (Buildable :type "/Game/Hyper/Core/BuildingSystem/Blueprints/BP_Buildable_Abstract Object Reference"))
  (returns (Authorized :type Boolean))
  (return true))

(fn `Match Inventory Item with Buildable`
  (params (`Inventory Slot` :type "/Game/Hyper/Core/Inventory/Datamodel/Structures/Main_Item_Slot_Structs/Struct_Inventory_Slot_Item Structure"))
  (returns (`Out Row` :type "DataTableRowHandle Structure") (Match :type Boolean))
  (bind (_datatable _rowname) (break `DataTableRowHandle` (`.Item_2_C7967C054AE750B79BB1FDB9058FE0B3` (break `/Game/Hyper/Core/Inventory/Datamodel/Structures/Main_Item_Slot_Structs/Struct_Inventory_Slot_Item` `Inventory Slot`))))
  ;[0.05127 0.05127 0.05127] Matches inventory item to buildable by same row name
  (`|GetDataTableRow` "/Game/Hyper/Core/BuildingSystem/Datamodel/Datatables/DT_Buildables.DT_Buildables" _rowname
    (:`then`
      (return (make `DataTableRowHandle` "/Game/Hyper/Core/BuildingSystem/Datamodel/Datatables/DT_Buildables.DT_Buildables" _rowname) true))
    (:`RowNotFound`
      (`KismetSystemLibrary.PrintString` "Intentory item row name is not matching with selected buildable to try to match. Please match the row names.")
      (return (struct) false))))

(fn `spawn_buildables_from_save`
  (locals (`local save` :type "/Game/Hyper/BuildingSystem/Save/BP_Save_Buildings Object Reference") (`local spawned buildables` :type "Array of /Game/Hyper/Core/BuildingSystem/Blueprints/BP_Buildable_Abstract Object Reference") (Local_GUID_to_Actor :type "Map of String to Actor Object Reference") (`local spawned splines` :type "Array of Actor Object Reference")))