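; Abstract actor component defining the interface for extended character movement: movement and grounded modes, strafe or forward-facing orientation, camera modes, jetpack and linked animation layers.
; Nearly all events and functions are empty stubs, presumably for a child component to implement.
; Most OnReps forward to overridable Execution functions, since replicated state lives here.
; Only root-motion physics rotation has real logic: a server event sets it, and its OnRep applies it to CharacterMovement.
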(event `Server: Set Active Camera Mode`
  (params (`Active Camera Mode` :type "/Game/Hyper/Core/Locomotion/Datamodel/Enumerations/Enum_Camera_Mode Enum" :default "NewEnumerator0")))

(event `Disable movement on Client`
  (params (`Disable Movement` :type Boolean)))

(event `On Movement Input Changed`)

(event `Server: Set Jetpack Active`
  (params (Jetpack_Active :type Boolean)))

(event `Event: Initialize Change Movement Mode`
  (params (`Movement Mode` :type "EMovementMode Enum" :default "MOVE_None")))

(event `Event: Initialize Change Grounded Movement Mode`
  (params (`Grounded movement mode` :type "/Game/Hyper/Core/Locomotion/Datamodel/Enumerations/Enum_Grounded_MovementModes Enum" :default "NewEnumerator0")))

(event `Play Timeline`
  (params (`Timeline Play Rate` :type "Float (double-precision)" :default 1.0) (`Play from start` :type Boolean :default false) (`Reverse from end` :type Boolean) (`Play Reversed` :type Boolean)))

(event `Event: Move Character into local direction`
  (params (`Manual Direction` :type "/Game/Hyper/Locomotion/Chars/Mannequin_UE5/Anims/Enum_AnimEnum_CardinalDirection Enum" :default "NewEnumerator0") (`Override with desired input direction?` :type Boolean)))

(event `Server Allow Physics Rotation During Anim Root Motion`
  (params (`Allow Physics Rotation During Anim Root Motion` :type Boolean))
  (set `self.Allow Physics Rotation During Anim Root Motion` `Allow Physics Rotation During Anim Root Motion`))

(fn `Get Camera Components`
  (params (`Get By Tag` :type Boolean))
  (returns (`Third Person Camera` :type "CameraComponent Object Reference") (`First person camera` :type "CameraComponent Object Reference") (`Rear Facing Camera` :type "CameraComponent Object Reference") (`All cameras are valid` :type Boolean) (`All Cameras` :type "Array of CameraComponent Object Reference"))
  (locals (`Local Third Person Camera` :type "CameraComponent Object Reference") (`Local First person camera` :type "CameraComponent Object Reference") (`Local rear facing Camera` :type "CameraComponent Object Reference"))
  ;[0.05127 0.05127 0.05127] This is based on prediction.
  ; Nearly all camera's that are attached to a springarm are third person camera's.
  ; Nearly all cameras that are attached to a skeletal mesh are first person camera's
  ; In my case my other camera is the backwards facing camera
)

(fn `Get_Active_Camera_Component`
  (returns (`active camera` :type "CameraComponent Object Reference") (`Attached to this springarm` :type "SpringArmComponent Object Reference") (`Is Attached to springarm` :type Boolean) (`Is attached to skeletal mesh` :type Boolean) (`attached to this skeletal Mesh` :type "SkeletalMeshComponent Object Reference"))
  (locals (`local active camera` :type "CameraComponent Object Reference") (`Local Attached to this springarm` :type "SpringArmComponent Object Reference") (`Local Is Attached to springarm` :type Boolean) (`Local attached to this skeletal Mesh` :type "SkeletalMeshComponent Object Reference") (`Local is attached to skeletal mesh` :type Boolean))
  ;[0.05127 0.05127 0.05127] Nearly all camera's that are attached to a springarm are third person camera's.
  ; Nearly all cameras that are attached to a skeletal mesh are first person camera's
)

(fn `Jetpack_Toggle`
  (params (Reset :type Boolean) (Activate :type Boolean)))

(fn `Move Character into local direction`
  (params (Selection :type "/Game/Hyper/Locomotion/Chars/Mannequin_UE5/Anims/Enum_AnimEnum_CardinalDirection Enum" :default "NewEnumerator0")))

(fn `OnRep_Active Camera Mode`
  (`self.OnRep_Active Camera Mode_Execution`))

(fn `OnRep_Active Camera Mode_Execution`)

(fn `OnRep_Active Grounded Movement Mode`
  (`self.OnRep_Active Grounded Movement Mode_Execution`))

(fn `OnRep_Active Grounded Movement Mode_Execution`)

(fn `OnRep_Active Movement Mode`
  (`self.OnRep_Active Movement Mode_Execution`))

(fn `OnRep_Active Movement Mode_Execution`)

(fn `OnRep_Allow Physics Rotation During Anim Root Motion`
  (set `CharacterMovementComponent.bAllowPhysicsRotationDuringAnimRootMotion` (`self.Allow Physics Rotation During Anim Root Motion`) (`/Game/Hyper/Core/Generic/BlueprintMacroLibrary/BML_Generic_Component.Get Character Movement`)))

(fn `OnRep_Jetpack_Active`
  (`self.OnRep_Jetpack_Active_Execution`))

(fn `OnRep_Jetpack_Active_Execution`)

(fn `OnRep_Linked_Animation_Layer`
  (`self.OnRep_Linked_Animation_Layer_Execution`))

(fn `OnRep_Linked_Animation_Layer_Execution`)

(fn `OnRep_Override Global Orientation`
  (`self.OnRep_Override_Global_Orientation_Execution`))

(fn `OnRep_Override_Global_Orientation_Execution`)

(fn `Set to forward Facing Movement`)

(fn `Set to Original global Orientation`)

(fn `Set to Strafe Movement`)

(fn `Switch_Active_Camera_Mode`
  (params (`Switch to this camera mode` :type "/Game/Hyper/Core/Locomotion/Datamodel/Enumerations/Enum_Camera_Mode Enum" :default "NewEnumerator0")))

(fn `Trace from Active Camera`
  (params (TraceChannel :type "ETraceTypeQuery Enum" :default "TraceTypeQuery1") (`Front offset start position` :type "Float (double-precision)") (`Trace Lenght` :type "Float (double-precision)") (ActorsToIgnore :type "Array of Actor Object Reference (by ref)"))
  (returns (OutHit :type "HitResult Structure") (Hit :type Boolean) (HitActor :type "Actor Object Reference") (HitComponent :type "PrimitiveComponent Object Reference") (Location :type "Vector Structure")))