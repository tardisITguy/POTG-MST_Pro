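; Impact effect master actor, spawned on the server with an expose-on-spawn hit, that runs its impact logic on BeginPlay.
; The hit's surface type selects an optional decal, Niagara system (fed the impact position through an array) and sound.
; Sound goes through the owner controller's replication component and emits pawn noise.
; The sound lookup supports per-weapon variants but is called with None, and many surface entries are unset.
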(event `self.ReceiveBeginPlay`
  ;[0.05127 0.05127 0.05127] Excecute impact logic directly on spawn.
  ; the hit is set via expose on spawn.
  ; This actor is spawned on the server, so to replicate it back to the clients the hit data should also be replicated
  (`self.Excecute Impact` (`self.Hit`)))

(event `Event: Excecute Impact`
  (params (Hit :type "HitResult Structure (by ref)")))

(fn `Excecute Impact`
  (params (Hit :type "HitResult Structure (by ref)") (`Spawn Decal` :type Boolean :default true) (`Spawn Sound` :type Boolean :default true) (`Spawn Emitter` :type Boolean :default true))
  (locals (`Surface Type` :type "EPhysicalSurface Enum" :default "SurfaceType_Default") (Location :type "Vector Structure" :default (0.0 0.0 3158.663562)))
  (bind (_controller _bsuccess) (`/Game/Hyper/Core/Generic/BlueprintMacroLibrary/BML_Generic_Actor.Get Controller`))
  (bind _location (`local.Location`))
  (bind (_component _is_valid) (`/Game/Hyper/Core/ReplicationSubSystem/BlueprintMacroLibrary/BML_Replication_Controller.Get Replication` _controller))
  (set `local.Surface Type` (`GameplayStatics.GetSurfaceType` Hit))
  (set `local.Location` (`.Location` (`GameplayStatics.BreakHitResult` Hit)))
  (`|ExecutionSequence`
    (:`then_0`
      ;[0.05127 0.05127 0.05127] Decal
      (if (`local.Spawn Decal`)
        (bind _returnvalue (`GameplayStatics.SpawnDecalAtLocation` (`self.Get Bullet Decal Based On Surface Type` (`local.Surface Type`)) (7.0 7.0 7.0) (`local.Location`) (`KismetMathLibrary.Conv_VectorToRotator` (`.ImpactNormal` (`GameplayStatics.BreakHitResult` (`self.Hit`)))) 15.0))
        (`/Engine/EditorBlueprintResources/StandardMacros.IsValid` _returnvalue
          (:`Is Valid`
            (`DecalComponent.SetFadeScreenSize` _returnvalue 0.001)))))
    (:`then_1`
      ;[0.05127 0.05127 0.05127] Location
      (if (`local.Spawn Emitter`)
        (bind _returnvalue_2 (`NiagaraFunctionLibrary.SpawnSystemAtLocation` (`self.Get Impact Niagara System Based On Surface Type` (`local.Surface Type`)) _location (`KismetMathLibrary.Conv_VectorToRotator` (`.ImpactNormal` (`GameplayStatics.BreakHitResult` (`self.Hit`)))) (1.0 1.0 1.0) true true "AutoRelease"))
        ;[0.05127 0.05127 0.05127] The impact niagara system uses an array for impact positions
        (`/Engine/EditorBlueprintResources/StandardMacros.IsValid` _returnvalue_2
          (:`Is Valid`
            (if (not (`|EnumEquality` (`local.Surface Type`) "SurfaceType10"))
              (`NiagaraDataInterfaceArrayFunctionLibrary.SetNiagaraArrayPosition` _returnvalue_2 "ImpactPositions" (`|MakeArray` _location)))))))
    (:`then_2`
      ;[0.05127 0.05127 0.05127] Spawn Sound
      (if (`local.Spawn Sound`)
        (`/Engine/EditorBlueprintResources/StandardMacros.IsValid` _controller
          (:`Is Valid`
            (if (and _bsuccess _is_valid)
              (`/Engine/EditorBlueprintResources/StandardMacros.IsValid` _component
                (:`Is Valid`
                  ;;[0.05127 0.05127 0.05127] This extra check solves a timing issue when character is dying while just spwaning the effect
                  (cast `Character` (`self.GetOwner`))
                  (`/Game/Hyper/Core/ReplicationSubSystem/Blueprints/AC_Replication_Abstract.Initialize Spawn Sound At Location` _component (`self.Get Impact Sound Based On Surface Type` (`local.Surface Type`)) (`local.Location`) false 0.0 "/Game/Hyper/ResourcePack/Audio/AttenuationPresets/ATT_Default.ATT_Default")
                  (`Pawn.PawnMakeNoise` (`/Game/Hyper/Core/Generic/BlueprintMacroLibrary/BML_Generic_Actor.Get Character`) 0.5 (0.0 0.0 0.0) true self))))))))))

(fn `Get Bullet Decal Based On Surface Type`
  (params (`Surface Type` :type "EPhysicalSurface Enum" :default "SurfaceType_Default"))
  (returns (ReturnValue :type "MaterialInterface Object Reference"))
  (return (select `EPhysicalSurface` `Surface Type` :`SurfaceType_Default` (`KismetArrayLibrary.Array_Random` (`|MakeArray` "/Game/Hyper/CombatSystem/Decal/Decals/MI_Decal_Concrete_1.MI_Decal_Concrete_1" "/Game/Hyper/CombatSystem/Decal/Decals/MI_Decal_Concrete_2.MI_Decal_Concrete_2" "/Game/Hyper/CombatSystem/Decal/Decals/MI_Decal_Concrete_3.MI_Decal_Concrete_3" "/Game/Hyper/CombatSystem/Decal/Decals/MI_Decal_Concrete_4.MI_Decal_Concrete_4" :!type "MaterialInterface Object Reference")) :`SurfaceType8` (`KismetArrayLibrary.Array_Random` (`|MakeArray` "/Game/Hyper/CombatSystem/Decal/Decals/MI_Decal_Concrete_1.MI_Decal_Concrete_1" "/Game/Hyper/CombatSystem/Decal/Decals/MI_Decal_Concrete_2.MI_Decal_Concrete_2" "/Game/Hyper/CombatSystem/Decal/Decals/MI_Decal_Concrete_3.MI_Decal_Concrete_3" "/Game/Hyper/CombatSystem/Decal/Decals/MI_Decal_Concrete_4.MI_Decal_Concrete_4" :!type "MaterialInterface Object Reference")) :`SurfaceType10` "/Game/Hyper/CombatSystem/Decal/Decals/MI_Decal_Concrete_1.MI_Decal_Concrete_1")))

(fn `Get Impact Niagara System Based On Surface Type`
  (params (`Surface Type` :type "EPhysicalSurface Enum" :default "SurfaceType_Default"))
  (returns (ReturnValue :type "NiagaraSystem Object Reference"))
  (return (select `EPhysicalSurface` `Surface Type` :`SurfaceType_Default` "/Game/Hyper/ResourcePack/Effects/Particles/Impacts/NS_ImpactConcrete.NS_ImpactConcrete" :`SurfaceType8` "/Game/Hyper/ResourcePack/Effects/Particles/Impacts/NS_ImpactConcrete.NS_ImpactConcrete" :`SurfaceType10` "/Game/Hyper/ResourcePack/Effects/Particles/Blood/Niagara/NS_Blood.NS_Blood" :!type "NiagaraSystem Object Reference")))

(fn `Get Impact Sound Based On Surface Type`
  (params (`Surface Type` :type "EPhysicalSurface Enum" :default "SurfaceType_Default") (`Weapon Type` :type "/Game/Hyper/Core/Equipment_Manager/Datamodel/Enumerations/Enum_Equipment_Type Enum" :default "NewEnumerator14"))
  (returns (ReturnValue :type "MetaSoundSource Object Reference"))
  (bind _returnvalue (select `EPhysicalSurface` (`local.Surface Type`) :`SurfaceType_Default` "/Game/Hyper/ResourcePack/Audio/MetaSounds/sfx_Weapon_BaseImpact_nl_metaPreset.sfx_Weapon_BaseImpact_nl_metaPreset" :`SurfaceType1` "/Game/Hyper/ResourcePack/Audio/MetaSounds/sfx_Weapon_BaseImpact_nl_metaPreset.sfx_Weapon_BaseImpact_nl_metaPreset" :`SurfaceType2` "/Game/Hyper/ResourcePack/Audio/MetaSounds/sfx_Weapon_BaseImpact_nl_metaPreset.sfx_Weapon_BaseImpact_nl_metaPreset" :`SurfaceType3` "/Game/Hyper/ResourcePack/Audio/MetaSounds/sfx_Weapon_BaseImpact_nl_metaPreset.sfx_Weapon_BaseImpact_nl_metaPreset" :`SurfaceType4` "/Game/Hyper/ResourcePack/Audio/MetaSounds/sfx_Weapon_BaseImpact_nl_metaPreset.sfx_Weapon_BaseImpact_nl_metaPreset" :`SurfaceType5` "/Game/Hyper/ResourcePack/Audio/MetaSounds/sfx_Weapon_BaseImpact_nl_metaPreset.sfx_Weapon_BaseImpact_nl_metaPreset" :`SurfaceType6` "/Game/Hyper/ResourcePack/Audio/MetaSounds/sfx_Weapon_BaseImpact_nl_metaPreset.sfx_Weapon_BaseImpact_nl_metaPreset" :`SurfaceType7` "/Game/Hyper/ResourcePack/Audio/MetaSounds/sfx_Weapon_BaseImpact_nl_metaPreset.sfx_Weapon_BaseImpact_nl_metaPreset" :`SurfaceType8` "/Game/Hyper/ResourcePack/Audio/MetaSounds/sfx_ImpactPlaster_nl_meta.sfx_ImpactPlaster_nl_meta" :`SurfaceType9` "/Game/Hyper/ResourcePack/Audio/MetaSounds/sfx_Weapon_BaseImpact_nl_metaPreset.sfx_Weapon_BaseImpact_nl_metaPreset" :`SurfaceType10` "/Game/Hyper/ResourcePack/Audio/MetaSounds/sfx_Weapon_BaseImpact_nl_metaPreset.sfx_Weapon_BaseImpact_nl_metaPreset" :`SurfaceType11` "/Game/Hyper/ResourcePack/Audio/MetaSounds/sfx_Weapon_BaseImpact_nl_metaPreset.sfx_Weapon_BaseImpact_nl_metaPreset" :`SurfaceType12` "/Game/Hyper/ResourcePack/Audio/MetaSounds/sfx_Weapon_BaseImpact_nl_metaPreset.sfx_Weapon_BaseImpact_nl_metaPreset" :`SurfaceType13` "/Game/Hyper/ResourcePack/Audio/MetaSounds/sfx_Weapon_BaseImpact_nl_metaPreset.sfx_Weapon_BaseImpact_nl_metaPreset" :!type "MetaSoundSource Object Reference"))
  (bind _returnvalue_2 (select `EPhysicalSurface` (`local.Surface Type`) :`SurfaceType_Default` "/Game/Hyper/ResourcePack/Audio/MetaSounds/sfx_Weapon_BaseImpact_nl_metaPreset.sfx_Weapon_BaseImpact_nl_metaPreset" :`SurfaceType1` "/Game/Hyper/ResourcePack/Audio/MetaSounds/sfx_Weapon_BaseImpact_nl_metaPreset.sfx_Weapon_BaseImpact_nl_metaPreset" :`SurfaceType2` "/Game/Hyper/ResourcePack/Audio/MetaSounds/sfx_Weapon_BaseImpact_nl_metaPreset.sfx_Weapon_BaseImpact_nl_metaPreset" :`SurfaceType3` "/Game/Hyper/ResourcePack/Audio/MetaSounds/sfx_Weapon_BaseImpact_nl_metaPreset.sfx_Weapon_BaseImpact_nl_metaPreset" :`SurfaceType4` "/Game/Hyper/ResourcePack/Audio/MetaSounds/sfx_Weapon_BaseImpact_nl_metaPreset.sfx_Weapon_BaseImpact_nl_metaPreset" :`SurfaceType5` "/Game/Hyper/ResourcePack/Audio/MetaSounds/sfx_Weapon_BaseImpact_nl_metaPreset.sfx_Weapon_BaseImpact_nl_metaPreset" :`SurfaceType6` "/Game/Hyper/ResourcePack/Audio/MetaSounds/sfx_Weapon_BaseImpact_nl_metaPreset.sfx_Weapon_BaseImpact_nl_metaPreset" :`SurfaceType7` "/Game/Hyper/ResourcePack/Audio/MetaSounds/sfx_Weapon_BaseImpact_nl_metaPreset.sfx_Weapon_BaseImpact_nl_metaPreset" :`SurfaceType8` "/Game/Hyper/ResourcePack/Audio/MetaSounds/sfx_ImpactPlaster_nl_meta.sfx_ImpactPlaster_nl_meta" :`SurfaceType9` "/Game/Hyper/ResourcePack/Audio/MetaSounds/sfx_Weapon_BaseImpact_nl_metaPreset.sfx_Weapon_BaseImpact_nl_metaPreset" :`SurfaceType10` "/Game/Hyper/ResourcePack/Audio/MetaSounds/sfx_Weapon_BaseImpact_nl_metaPreset.sfx_Weapon_BaseImpact_nl_metaPreset" :`SurfaceType11` "/Game/Hyper/ResourcePack/Audio/MetaSounds/sfx_Weapon_BaseImpact_nl_metaPreset.sfx_Weapon_BaseImpact_nl_metaPreset" :`SurfaceType12` "/Game/Hyper/ResourcePack/Audio/MetaSounds/sfx_Weapon_BaseImpact_nl_metaPreset.sfx_Weapon_BaseImpact_nl_metaPreset" :`SurfaceType13` "/Game/Hyper/ResourcePack/Audio/MetaSounds/sfx_Weapon_BaseImpact_nl_metaPreset.sfx_Weapon_BaseImpact_nl_metaPreset" :!type "MetaSoundSource Object Reference"))
  (return (select `/Game/Hyper/Core/Equipment_Manager/Datamodel/Enumerations/Enum_Equipment_Type` (`local.Weapon Type`) :`NewEnumerator14` _returnvalue_2 :`NewEnumerator8` _returnvalue :`NewEnumerator7` _returnvalue :`NewEnumerator11` _returnvalue :`NewEnumerator9` _returnvalue :`NewEnumerator3` _returnvalue_2 :`NewEnumerator0` _returnvalue_2 :`NewEnumerator1` _returnvalue_2 :`NewEnumerator6` _returnvalue_2 :`NewEnumerator2` _returnvalue_2 :`NewEnumerator15` _returnvalue_2 :`NewEnumerator4` _returnvalue_2 :`NewEnumerator5` _returnvalue_2 :`NewEnumerator10` _returnvalue_2 :`NewEnumerator12` _returnvalue_2 :`NewEnumerator13` _returnvalue_2)))

(fn `UserConstructionScript`)