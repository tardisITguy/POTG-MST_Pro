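; Basic combat component that forwards primary-action input to equipped items and handles melee hits, damage and death ragdolls.
; Melee notifies pass a locally-controlled check before a server RPC box-traces from camera or character, sized by equipment override or type defaults.
; Each unique hit actor, optionally tag-filtered, takes attribute-based point damage and spawns an impact actor.
; The damage handler triggers server ragdoll when health would run out, except while swimming.
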(event `EnhancedInput|/Game/Hyper/Locomotion/Input/Interaction/IA_Primary_Action`
  (params (ActionValue :type Boolean) (ElapsedSeconds :type "Float (double-precision)") (TriggeredSeconds :type "Float (double-precision)") (InputAction :type "InputAction Object Reference" :default "/Game/Hyper/Locomotion/Input/Interaction/IA_Primary_Action.IA_Primary_Action"))
  ;[0.05127 0.05127 0.05127] Primary Action
  (:`Started`
    (`self.Event: Try Start Primary Action`))
  (:`Completed`
    (`self.Event: Try Stop Primary Action`)))

(event `self.Event: Try Start Primary Action`
  ;[0.05127 0.05127 0.05127] Primary Action
  (set `self.Receiving_Primary_Input` true)
  (bind _asbp_equipment_abstract (cast `/Game/Hyper/Core/Equipment_Manager/Blueprints/BP_Equipment_Abstract` (`.AttachedActor_5_6148DDC14889969E604D59A54A548813` (break `/Game/Hyper/Core/Equipment_Manager/Datamodel/Structures/Main_Structs/Struct_Attached_Equipment` (`.attached struct found` (`/Game/Hyper/Core/Equipment_Manager/Blueprints/AC_Equipment_Manager_Abstract.Find Attached Equipment slot in equipment array` (`/Game/Hyper/Core/Equipment_Manager/BlueprintMacroLibrary/BML_Equipment_Component.Get Equipment Manager`) "NewEnumerator8"))))))
  (`/Game/Hyper/Core/Equipment_Manager/Blueprints/BP_Equipment_Abstract.Event: Try Primary Input` _asbp_equipment_abstract))

(event `self.Event: Try Stop Primary Action`
  ;[0.05127 0.05127 0.05127] Primary Action
  (set `self.Receiving_Primary_Input` false)
  (bind _asbp_equipment_abstract (cast `/Game/Hyper/Core/Equipment_Manager/Blueprints/BP_Equipment_Abstract` (`.AttachedActor_5_6148DDC14889969E604D59A54A548813` (break `/Game/Hyper/Core/Equipment_Manager/Datamodel/Structures/Main_Structs/Struct_Attached_Equipment` (`.attached struct found` (`/Game/Hyper/Core/Equipment_Manager/Blueprints/AC_Equipment_Manager_Abstract.Find Attached Equipment slot in equipment array` (`/Game/Hyper/Core/Equipment_Manager/BlueprintMacroLibrary/BML_Equipment_Component.Get Equipment Manager`) "NewEnumerator8"))))))
  (`/Game/Hyper/Core/Equipment_Manager/Blueprints/BP_Equipment_Abstract.Event: Stop Primary Input` _asbp_equipment_abstract))

(event `Server Event: Try inflict Melee damage`
  (params (`Attack Type` :type "/Game/Hyper/Core/Equipment_Manager/Datamodel/Enumerations/Enum_Melee_Attack_Types Enum" :default "NewEnumerator0"))
  ;[0.05127 0.05127 0.05127] Inflict Melee Damage
  (`self.Try Inflict Melee Damage` `Attack Type`))

(event `self.Event: Initialize Try Inflict Melee Damage`
  (params (`Attack Type` :type "/Game/Hyper/Core/Equipment_Manager/Datamodel/Enumerations/Enum_Melee_Attack_Types Enum" :default "NewEnumerator0"))
  ;[0.05127 0.05127 0.05127] Inflict Melee Damage
  ;;[0.05127 0.05127 0.05127] Makes sure to only continue when is locally triggered.
  ;; This is required due to this event is triggered by an animation notify. This notify is sometimes triggered multiple times when it is multicasted
  (if (`Pawn.IsLocallyControlled` (`/Game/Hyper/Core/Generic/BlueprintMacroLibrary/BML_Generic_Component.Get Character`))
    (`self.Server Event: Try inflict Melee damage` `Attack Type`)))

(event `self.Event: Spawn Impact`
  (params (SpawnTransform :type "Transform Structure") (Hit :type "HitResult Structure") (Instigator :type "Pawn Object Reference") (Owner :type "Actor Object Reference"))
  (bind _impact_class_to_use (`self.Impact Class To Use`))
  ;[0.05127 0.05127 0.05127] Spawn impact effect via server call
  (if (`KismetSystemLibrary.IsValidClass` _impact_class_to_use)
    (`|SpawnActorFromClass` _impact_class_to_use SpawnTransform "AlwaysSpawn" "OverrideRootScale" Owner Hit Instigator)))

(fn `Apply_Damage`
  (params (`Hit Actor` :type "Actor Object Reference") (`Hit info` :type "HitResult Structure") (`Attack Type` :type "/Game/Hyper/Core/Equipment_Manager/Datamodel/Enumerations/Enum_Melee_Attack_Types Enum" :default "NewEnumerator0") (`Override Damage Amount` :type "Float (double-precision)"))
  (returns (`Damage Applied` :type "Float (single-precision)") (`health is zero after this hit` :type Boolean))
  (locals (`Local Damage` :type "Float (single-precision)" :default 15.0))
  (bind (_component _is_valid) (`/Game/Hyper/Core/Attribute_System/BlueprintMacroLibrary/BML_Attribute_Component.Get Attribute Manager`))
  (bind _hit_info (`local.Hit info`))
  (bind _hit_info_2 (`local.Hit info`))
  (bind (_bblockinghit _binitialoverlap _time _distance _location _impactpoint _normal _impactnormal) (`GameplayStatics.BreakHitResult` _hit_info_2))
  (bind _returnvalue (`Controller.K2_GetPawn` (`/Game/Hyper/Core/Generic/BlueprintMacroLibrary/BML_Generic_Component.Get Controller`)))
  (bind _total (`/Game/Hyper/Core/Attribute_System/FunctionLibraries/BFL_Attribute.Get Float Attribute Total` (`/Game/Hyper/Core/Attribute_System/Blueprints/AC_Attribute_Manager_Abstact.Get Generic Combat Attribute` _component "NewEnumerator12")))
  (`|ExecutionSequence`
    (:`then_0`
      (if (== (`local.Override Damage Amount`) 0.0)
        (if _is_valid
          (if (> _total 0.0)
            (set `local.Local Damage` _total)))
        (else
          (set `local.Local Damage` (`local.Override Damage Amount`)))))
    (:`then_1`
      (bind _returnvalue_2 (`GameplayStatics.ApplyPointDamage` (`local.Hit Actor`) (`local.Local Damage`) (`.Location` (`GameplayStatics.BreakHitResult` _hit_info)) _hit_info (`/Game/Hyper/Core/Generic/BlueprintMacroLibrary/BML_Generic_Component.Get Controller`) (`self.GetOwner`) "/Script/Engine.DamageType"))
      (`|ExecutionSequence`
        (:`then_0`
          (`self.Event: Spawn Impact` (`KismetMathLibrary.MakeTransform` _location (`KismetMathLibrary.Conv_VectorToRotator` _impactnormal)) _hit_info_2 _returnvalue _returnvalue))
        (:`then_1`
          (return _returnvalue_2 false))))))

(fn `Handle Take Damage`
  (params (`Damage In` :type "Float (double-precision)") (`Damage Type` :type "DamageType Object Reference") (`Instigated By` :type "Controller Object Reference") (`Damage Causer` :type "Actor Object Reference"))
  (returns (`Damage Out` :type "Float (double-precision)") (Blocked :type Boolean))
  (bind (_component _is_valid) (`/Game/Hyper/Core/Ragdoll/BlueprintMacroLibrary/BML_Ragdoll_Component.Get Ragdoll`))
  (`|ExecutionSequence`
    (:`then_0`
      (if (<= (- (`/Game/Hyper/Core/Attribute_System/Blueprints/AC_Attribute_Manager_Abstact.Get Non- Persistent Character Attribute` (`/Game/Hyper/Core/Attribute_System/BlueprintMacroLibrary/BML_Attribute_Component.Get Attribute Manager`) "NewEnumerator5") `Damage In`) 0.0)
        (if (`NavMovementComponent.IsSwimming` (`/Game/Hyper/Core/Generic/BlueprintMacroLibrary/BML_Generic_Component.Get Character Movement`))
          _
          (elif _is_valid
            (`/Game/Hyper/Core/Ragdoll/Blueprints/AC_Ragdoll_Abstract.Server To Ragdoll` _component true)))))
    (:`then_1`
      (return (`local.Damage In`) false))))

(fn `Try Inflict Melee Damage`
  (params (`Attack Type` :type "/Game/Hyper/Core/Equipment_Manager/Datamodel/Enumerations/Enum_Melee_Attack_Types Enum" :default "NewEnumerator0"))
  (locals (`Local hits` :type "Array of HitResult Structure") (`Local Hit Location` :type "Vector Structure") (`Local Hit` :type "HitResult Structure") (`Local Hit Actor` :type "Actor Object Reference") (`Local actors prevsouly hitted` :type "Array of Actor Object Reference") (`Local Character` :type "Character Object Reference") (`Local Trace Forward` :type "Vector Structure") (`Local Trace Start` :type "Vector Structure") (`Local Trace Orientation` :type "Rotator Structure") (`Local Hit Actors` :type "Array of Actor Object Reference") (`Local Trace End` :type "Vector Structure") (`Local Trace Half Size` :type "Vector Structure"))
  (bind _local_character (`local.Local Character`))
  (bind _tags_to_check_before_applying_damage (`self.tags to check before applying damage`))
  (bind _active_camera (`/Game/Hyper/Core/Locomotion/Blueprints/AC_Extended_Movement_Abstract.Get_Active_Camera_Component` (`/Game/Hyper/Core/Locomotion/BlueprintMacroLibrary/Generic/BML_ExtendedMovement_Component.Get ExtendedMovement`)))
  (bind _active_camera_2 (`/Game/Hyper/Core/Locomotion/Blueprints/AC_Extended_Movement_Abstract.Get_Active_Camera_Component` (`/Game/Hyper/Core/Locomotion/BlueprintMacroLibrary/Generic/BML_ExtendedMovement_Component.Get ExtendedMovement`)))
  (bind _array (`|MakeArray` (`local.Local Character`) :!type "Actor Object Reference"))
  (bind ((`Generic_41_F38D1B334B6B5DEFCF41708F1350F138` _generic) (`Melee_11_2D18FAC1420140F3EC39B68B3B62B313` _melee)) (break `/Game/Hyper/Core/Equipment_Manager/Datamodel/Structures/Main_Structs/Struct_Equipment` (`/Game/Hyper/Core/Inventory/FunctionLibraries/BFL_InventoryCrafting.Get Equipment info from Inventory Slot` (`.item found in equipment slot` (`/Game/Hyper/Core/Equipment_Manager/Blueprints/AC_Equipment_Manager_Abstract.Get Equipment slot in equipment array` (`/Game/Hyper/Core/Equipment_Manager/BlueprintMacroLibrary/BML_Equipment_Component.Get Equipment Manager`) "NewEnumerator8")))))
  (bind ((`OverrideBoxTraceBounds_59_AFB1ABC74F94887DA76199807F1F1C55` _overrideboxtracebounds) (`TraceBounds_63_AB3446D04F0B4AB2E664B889B50F2764` _tracebounds)) (break `/Game/Hyper/Core/Equipment_Manager/Datamodel/Structures/Sub_Structs/Struct_CombatAttributes_Melee` _melee))
  (set `local.Local Character` (`/Game/Hyper/Core/Generic/BlueprintMacroLibrary/BML_Generic_Component.Get Character`))
  (`|ExecutionSequence`
    (:`then_0`
      ;[0.05098 0.05098 0.05098] Set Start, Forward and Rotation Based on Camera Mode
      (if (`|EnumEquality` (`/Game/Hyper/Core/Locomotion/Blueprints/AC_Extended_Movement_Abstract.Active Camera Mode` (`/Game/Hyper/Core/Locomotion/BlueprintMacroLibrary/Generic/BML_ExtendedMovement_Component.Get ExtendedMovement`)) "NewEnumerator0")
        (set `local.Local Trace Start` (`SceneComponent.K2_GetComponentLocation` _active_camera_2))
        (set `local.Local Trace Forward` (`SceneComponent.GetForwardVector` _active_camera_2))
        (set `local.Local Trace Orientation` (`SceneComponent.K2_GetComponentRotation` _active_camera_2))
        (else
          (set `local.Local Trace Start` (+ (`Actor.K2_GetActorLocation` _local_character) (* (`Actor.GetActorForwardVector` _local_character) (`self.Third Person Attack Box Offset`))))
          (if (`Pawn.IsPlayerControlled` (`local.Local Character`))
            (set `local.Local Trace Forward` (`SceneComponent.GetForwardVector` _active_camera))
            (set `local.Local Trace Orientation` (`SceneComponent.K2_GetComponentRotation` _active_camera))
            (else
              (set `local.Local Trace Forward` (`Actor.GetActorForwardVector` (`local.Local Character`)))
              (set `local.Local Trace Orientation` (`Actor.K2_GetActorRotation` (`local.Local Character`))))))))
    (:`then_1`
      ;[0.05098 0.05098 0.05098] Calculate end location
      (set `local.Local Trace End` (+ (`local.Local Trace Start`) (* (`local.Local Trace Forward`) (.x (select `bool` _overrideboxtracebounds :`false` (`KismetMathLibrary.MakeVector` (select `/Game/Hyper/Core/Equipment_Manager/Datamodel/Enumerations/Enum_Equipment_Type` (`.EquipmentType_3_705F99114DCF7C5CF212D1B88F42334C` (break `/Game/Hyper/Core/Equipment_Manager/Datamodel/Structures/Sub_Structs/Struct_Combat_Attributes_Generic` _generic)) :`NewEnumerator14` 150.0 :`NewEnumerator8` 100.0 :`NewEnumerator7` 150.0 :`NewEnumerator20` 100.0 :`NewEnumerator11` 100.0 :`NewEnumerator9` 100.0 :`NewEnumerator3` 150.0 :`NewEnumerator0` 150.0 :`NewEnumerator1` 250.0 :`NewEnumerator17` 250.0 :`NewEnumerator6` 150.0 :`NewEnumerator2` 250.0 :`NewEnumerator15` 100.0 :`NewEnumerator21` 150.0 :`NewEnumerator22` 150.0 :`NewEnumerator16` 100.0 :`NewEnumerator18` 100.0 :`NewEnumerator4` 150.0 :`NewEnumerator5` 150.0 :`NewEnumerator19` 100.0 :`NewEnumerator10` 100.0 :`NewEnumerator12` 100.0 :`NewEnumerator13` 100.0 :`NewEnumerator23` 150.0) 120.0 120.0) :`true` _tracebounds)))))
      (set `local.Local Trace Half Size` (/ (`KismetMathLibrary.MakeVector` 0.0 (.y (select `bool` _overrideboxtracebounds :`false` (`KismetMathLibrary.MakeVector` (select `/Game/Hyper/Core/Equipment_Manager/Datamodel/Enumerations/Enum_Equipment_Type` (`.EquipmentType_3_705F99114DCF7C5CF212D1B88F42334C` (break `/Game/Hyper/Core/Equipment_Manager/Datamodel/Structures/Sub_Structs/Struct_Combat_Attributes_Generic` _generic)) :`NewEnumerator14` 150.0 :`NewEnumerator8` 100.0 :`NewEnumerator7` 150.0 :`NewEnumerator20` 100.0 :`NewEnumerator11` 100.0 :`NewEnumerator9` 100.0 :`NewEnumerator3` 150.0 :`NewEnumerator0` 150.0 :`NewEnumerator1` 250.0 :`NewEnumerator17` 250.0 :`NewEnumerator6` 150.0 :`NewEnumerator2` 250.0 :`NewEnumerator15` 100.0 :`NewEnumerator21` 150.0 :`NewEnumerator22` 150.0 :`NewEnumerator16` 100.0 :`NewEnumerator18` 100.0 :`NewEnumerator4` 150.0 :`NewEnumerator5` 150.0 :`NewEnumerator19` 100.0 :`NewEnumerator10` 100.0 :`NewEnumerator12` 100.0 :`NewEnumerator13` 100.0 :`NewEnumerator23` 150.0) 120.0 120.0) :`true` _tracebounds)) (.z (select `bool` _overrideboxtracebounds :`false` (`KismetMathLibrary.MakeVector` (select `/Game/Hyper/Core/Equipment_Manager/Datamodel/Enumerations/Enum_Equipment_Type` (`.EquipmentType_3_705F99114DCF7C5CF212D1B88F42334C` (break `/Game/Hyper/Core/Equipment_Manager/Datamodel/Structures/Sub_Structs/Struct_Combat_Attributes_Generic` _generic)) :`NewEnumerator14` 150.0 :`NewEnumerator8` 100.0 :`NewEnumerator7` 150.0 :`NewEnumerator20` 100.0 :`NewEnumerator11` 100.0 :`NewEnumerator9` 100.0 :`NewEnumerator3` 150.0 :`NewEnumerator0` 150.0 :`NewEnumerator1` 250.0 :`NewEnumerator17` 250.0 :`NewEnumerator6` 150.0 :`NewEnumerator2` 250.0 :`NewEnumerator15` 100.0 :`NewEnumerator21` 150.0 :`NewEnumerator22` 150.0 :`NewEnumerator16` 100.0 :`NewEnumerator18` 100.0 :`NewEnumerator4` 150.0 :`NewEnumerator5` 150.0 :`NewEnumerator19` 100.0 :`NewEnumerator10` 100.0 :`NewEnumerator12` 100.0 :`NewEnumerator13` 100.0 :`NewEnumerator23` 150.0) 120.0 120.0) :`true` _tracebounds))) 2.0))
      (bind _outhits (`KismetSystemLibrary.BoxTraceMultiForObjects` (`local.Local Trace Start`) (`local.Local Trace End`) (`local.Local Trace Half Size`) (`local.Local Trace Orientation`) (`|MakeArray` "ObjectTypeQuery3" "ObjectTypeQuery6" "ObjectTypeQuery7" :!type "EObjectTypeQuery Enum") false _array))
      (set `local.Local hits` _outhits)
      (bind _outhit (`KismetSystemLibrary.BoxTraceSingle` (`local.Local Trace Start`) (`local.Local Trace End`) (`local.Local Trace Half Size`) (`local.Local Trace Orientation`) "TraceTypeQuery1" false _array))
      (`KismetArrayLibrary.Array_Add` (`local.Local hits`) _outhit)
      (for _array_element (`local.Local hits`)
        (bind _output_get (set `local.Local Hit` _array_element))
        (if (`self.Use Tag Check to apply damage`)
          (bind (_bblockinghit _binitialoverlap _time _distance _location _impactpoint _normal _impactnormal _physmat _hitactor _hitcomponent) (`GameplayStatics.BreakHitResult` _output_get))
          (if (or (`/Game/Hyper/Core/Generic/FunctionLibraries/BFL_Generic.Does actor contain any of the tags?` _hitactor _tags_to_check_before_applying_damage) (`/Game/Hyper/Core/Generic/FunctionLibraries/BFL_Generic.Does Component contain any of the tags?` _hitcomponent _tags_to_check_before_applying_damage))
            (if (and _bblockinghit (not (`KismetArrayLibrary.Array_Contains` (`local.Local Hit Actors`) _hitactor))) :!label _label
              (`KismetArrayLibrary.Array_AddUnique` (`local.Local Hit Actors`) _hitactor)
              (`self.Apply_Damage` _hitactor (`local.Local Hit`) (`local.Attack Type`))))
          (else
            (goto _label))))
      (return))))