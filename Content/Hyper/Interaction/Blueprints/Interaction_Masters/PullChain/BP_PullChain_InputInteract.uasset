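; Pull chain interactable that a player triggers through an interact input, under the PullChain interaction masters.
; Interact calls MoveChain, which is not defined in this Blueprint, with a true argument.
; Overrides supply the "Pull Chain" prompt, a text location offset below the origin, a grab montage chosen for left or right hand by controller, and a clinging pickup sound.
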(event `/Game/Hyper/Core/Interaction/Interfaces/BPI_Interact.Interact`
  (params (`Owning Controller` :type "Controller Object Reference"))
  (`self.Move chain` true))

(fn `Get Interact Animation`
  (params (`Owning Controller` :type "Controller Object Reference"))
  (returns (`Anim Montage` :type "AnimMontage Object Reference"))
  (return (`/Game/Hyper/Core/Interaction/FunctionLibraries/BFL_Interaction.Select Interaction Animation` `Owning Controller` "/Game/Hyper/Locomotion/Chars/Mannequin_UE5/Anims/Actions/Grab/Anim_grab_item_mirrored_Montage.Anim_grab_item_mirrored_Montage" "/Game/Hyper/Locomotion/Chars/Mannequin_UE5/Anims/Actions/Grab/Anim_grab_item_Montage.Anim_grab_item_Montage")))

(fn `Get Interact Sound`
  (returns (`Interact Sound` :type "SoundBase Object Reference"))
  (return "/Game/Hyper/ResourcePack/Sounds/UI_Sounds/pickup_clinging_Cue.pickup_clinging_Cue"))

(fn `Get Interact Text`
  (params (`Owning Controller` :type "PlayerController Object Reference"))
  (returns (`Interact Text` :type Text) (`Secondary Interact Text` :type Text))
  (return "Pull Chain" ""))

(fn `Get Relative Interact Text Location`
  (returns (`Relative Location` :type "Vector Structure"))
  (return (0.0 0.0 -90.0)))

(fn `UserConstructionScript`
  (`parent.UserConstructionScript`))