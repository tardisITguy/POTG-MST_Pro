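; Master interactable valve crank whose wheel turns by player drag or automatically, driving triggers.
; UpdateCrankRotation dots drag direction with the wheel's right vector, smooths it via FInterpTo and accumulates a clamped roll.
; FlipCrankRotation plays or reverses the SetCrankRotation timeline based on TriggerIsDown.
; Both paths rotate the wheel, then set TriggerIsDown from a sign-aware threshold and call ExecuteTriggers on either result, throttled by a delayed DoOnce reset.
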(event `Flip Crank Rotation`
  (bind _rotation_required_before_trigger (`self.Rotation Required before trigger`))
  (bind _amount_rotated (`self.Amount Rotated`))
  ;[0.05127 0.05127 0.05127] Automated
  (if (`self.Trigger is down`)
    (bind (_direction _rotation) (`Timeline|Set Crank Rotation` :!via `Reverse` :!label _label)
      (:`Update`
        (set `self.Amount Rotated` (select `bool` (< (`self.Rotation Required before trigger`) 0.0) :`false` _rotation :`true` (* _rotation -1.0) :!type "Float (double-precision)"))
        (`SceneComponent.K2_SetRelativeRotation` (`self.Wheel`) (`KismetMathLibrary.MakeRotator` (`self.Amount Rotated`)) false false :!label _label_2)
        ;[0.05127 0.05127 0.05127] If it has reached a certain threshold, execute a trigger
        (`/Engine/EditorBlueprintResources/StandardMacros.DoOnce` false :!label _label_3
          (:`Completed`
            (if (select `bool` (< (`self.Rotation Required before trigger`) 0.0) :`false` (>= _amount_rotated _rotation_required_before_trigger) :`true` (<= _amount_rotated _rotation_required_before_trigger))
              (set `self.Trigger is down` true)
              (`self.Execute Triggers` null)
              (else
                (set `self.Trigger is down` false)
                (`self.Execute Triggers` null)))
            (`KismetSystemLibrary.Delay` 0.2)
            (goto _label_3 :!via `Reset`)))))
    (else
      (goto _label))))

(event `Update Crank Rotation`
  ;[0.05127 0.05127 0.05127] Rotate Crank manually via grab
  (set `self.Rotation value` (`KismetMathLibrary.FInterpTo` (`self.Rotation value`) (* (`KismetMathLibrary.Dot_VectorVector` (`self.Player drag direction`) (`KismetMathLibrary.GetRightVector` (`SceneComponent.RelativeRotation` (`self.Wheel`)))) -10.0) (`GameplayStatics.GetWorldDeltaSeconds`) 4.0)) ; Smoothly increase/decrease a float representing how much the wheel will turn
  (set `self.Amount Rotated` (`KismetMathLibrary.FClamp` (+ (`self.Amount Rotated`) (`self.Rotation value`)) (`self.Minimum Rotation`) (`self.Maximum Rotation`)))
  (goto _label_2))

(fn `Can Interact`
  (params (`Owning Controller` :type "Controller Object Reference"))
  (returns (True :type Boolean))
  (return true))

(fn `Get Interact Animation`
  (params (`Owning Controller` :type "Controller Object Reference"))
  (returns (`Anim Montage` :type "AnimMontage Object Reference"))
  (return null))

(fn `Get Interact Sound`
  (returns (`Interact Sound` :type "SoundBase Object Reference"))
  (return null))

(fn `Get Interact Text`
  (params (`Owning Controller` :type "PlayerController Object Reference"))
  (returns (`Interact Text` :type Text) (`Secondary Interact Text` :type Text))
  (return "" ""))

(fn `Get Relative Interact Text Location`
  (returns (`Relative Location` :type "Vector Structure"))
  (return (0.0 0.0 0.0)))

(fn `Should get other Actor to Interact with`
  (params (`Based on this Component` :type "PrimitiveComponent Object Reference"))
  (returns (True :type Boolean) (`Actor To Interact With` :type "Actor Object Reference"))
  (return false null))

(fn `Should server control the interact`
  (returns (`Server should excecute interact call` :type Boolean))
  (return true))

(fn `UserConstructionScript`)