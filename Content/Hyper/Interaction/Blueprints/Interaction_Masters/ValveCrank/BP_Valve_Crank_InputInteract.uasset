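; BP_Valve_Crank_InputInteract is the interaction point for a valve crank, prompting "Turn Crank".
; Its Interact event calls FlipCrankRotation to flip the crank's rotation.
; It supplies a left- or right-handed grab montage chosen from the interacting controller, with a zero relative text offset and no interact sound specified.
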(event `/Game/Hyper/Core/Interaction/Interfaces/BPI_Interact.Interact`
  (params (`Owning Controller` :type "Controller Object Reference"))
  (`self.Flip Crank Rotation`))

(fn `Get Interact Animation`
  (params (`Owning Controller` :type "Controller Object Reference"))
  (returns (`Anim Montage` :type "AnimMontage Object Reference"))
  (return (`/Game/Hyper/Core/Interaction/FunctionLibraries/BFL_Interaction.Select Interaction Animation` `Owning Controller` "/Game/Hyper/Locomotion/Chars/Mannequin_UE5/Anims/Actions/Grab/Anim_grab_item_mirrored_Montage.Anim_grab_item_mirrored_Montage" "/Game/Hyper/Locomotion/Chars/Mannequin_UE5/Anims/Actions/Grab/Anim_grab_item_Montage.Anim_grab_item_Montage")))

(fn `Get Interact Sound`
  (returns (`Interact Sound` :type "SoundBase Object Reference"))
  (return null))

(fn `Get Interact Text`
  (params (`Owning Controller` :type "PlayerController Object Reference"))
  (returns (`Interact Text` :type Text) (`Secondary Interact Text` :type Text))
  (return "Turn Crank" ""))

(fn `Get Relative Interact Text Location`
  (returns (`Relative Location` :type "Vector Structure"))
  (return (0.0 0.0 0.0)))

(fn `UserConstructionScript`
  (`parent.UserConstructionScript`))