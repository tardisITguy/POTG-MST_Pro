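; Grabbable switch interactive that the player flips by holding to grab it and dragging up or down.
; Grab compares the vertical grab offset against a threshold and the current TriggerIsDown state, calling FlipSwitch only when the drag opposes that state.
; It returns the handle's "Focus target" socket location and never requests that the grab stop.
; BeginPlay and construction defer to the parent, and FlipSwitch plays a timeline defined outside these graphs.
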(event `self.ReceiveBeginPlay`
  (`parent.ReceiveBeginPlay`))

(fn `Get Interact Text`
  (params (`Owning Controller` :type "PlayerController Object Reference"))
  (returns (`Interact Text` :type Text) (`Secondary Interact Text` :type Text))
  (return "Hold to Grab Switch" ""))

(fn `Grab`
  (params (GrabOffset :type "Vector2D Structure") (Dragging :type Boolean) (`Owning Controller` :type "Controller Object Reference"))
  (returns (`Focus Target` :type "Vector Structure"))
  (bind (_x _y) (`KismetMathLibrary.BreakVector2D` GrabOffset))
  (if (or (and (not (`self.Trigger is down`)) (>= _y 0.5)) (and (<= _y -0.5) (`self.Trigger is down`)))
    (`self.Flip switch`) ; Fire a custom event that plays a timeline
  )
  (return (`SceneComponent.GetSocketLocation` (`self.Switch handle`) "Focus target")))

(fn `ShouldStopGrab`
  (returns (ShouldStopGrab :type Boolean))
  (return false))

(fn `UserConstructionScript`
  (`parent.UserConstructionScript`))