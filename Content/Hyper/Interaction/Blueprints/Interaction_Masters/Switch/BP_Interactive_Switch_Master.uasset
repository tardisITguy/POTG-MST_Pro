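; Master Blueprint for an interactive switch that offers a "Flip Switch" prompt and fires triggers when toggled.
; Flipswitch plays or reverses the RotateSwitch timeline based on TriggerIsDown, pitching the handle between up and down.
; When the timeline finishes, TriggerIsDown is set from its direction and ExecuteTriggers runs.
; The construction script pre-poses a switch that starts down, and interaction is always allowed and server-controlled.
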(event `self.ReceiveBeginPlay`
  (`parent.ReceiveBeginPlay`))

(event `Flip switch`
  ;[0.05127 0.05127 0.05127] Animate the Switch
  (if (`self.Trigger is down`)
    (bind (_direction _pitch_value) (`Timeline|Rotate switch` :!via `Reverse` :!label _label) ; Timeline blends from 30 to -30
      (:`Update`
        (`SceneComponent.K2_SetRelativeRotation` (`self.Switch handle`) (`KismetMathLibrary.MakeRotator` 0.0 _pitch_value) false false) ; Move the switch handle into the up/down position
      )
      (:`Finished`
        ;[0.05127 0.05127 0.05127] When timeline is finished, the switch is down
        (set `self.Trigger is down` (`|EnumEquality` _direction "Forward"))
        (`self.Execute Triggers` null)))
    (else
      (goto _label))))

(fn `Can Interact`
  (params (`Owning Controller` :type "Controller Object Reference"))
  (returns (True :type Boolean))
  (return true))

(fn `Get Interact Animation`
  (params (`Owning Controller` :type "Controller Object Reference"))
  (returns (`Anim Montage` :type "AnimMontage Object Reference"))
  (return null))

(fn `Get Interact Sound`
  (returns (`Interact Sound` :type "SoundBase Object Reference"))
  (return null))

(fn `Get Interact Text`
  (params (`Owning Controller` :type "PlayerController Object Reference"))
  (returns (`Interact Text` :type Text) (`Secondary Interact Text` :type Text))
  (return "Flip Switch" ""))

(fn `Get Relative Interact Text Location`
  (returns (`Relative Location` :type "Vector Structure"))
  (return (0.0 0.0 0.0)))

(fn `Should get other Actor to Interact with`
  (params (`Based on this Component` :type "PrimitiveComponent Object Reference"))
  (returns (True :type Boolean) (`Actor To Interact With` :type "Actor Object Reference"))
  (return false null))

(fn `Should server control the interact`
  (returns (`Server should excecute interact call` :type Boolean))
  (return true))

(fn `UserConstructionScript`
  (`parent.UserConstructionScript`)
  (if (`self.Trigger is down`)
    (`SceneComponent.K2_SetRelativeRotation` (`self.Switch handle`) (`KismetMathLibrary.MakeRotator` 0.0 -30.0) false false) ; Move the switch handle into the up/down position
  ))