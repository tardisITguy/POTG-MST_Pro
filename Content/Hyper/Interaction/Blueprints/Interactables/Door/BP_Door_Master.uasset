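; BP_Door_Master is a base interactable door that swings open and closed around its yaw axis.
; A RotateDoor timeline drives the relative rotation of the SMDoor mesh, with InverseDoor negating the angle to flip the swing direction.
; Interactwithdoor toggles by playing or reversing the timeline based on DoorIsOpen, which updates from the timeline's direction when it finishes.
; OpenDoor and CloseDoor events drive the timeline directly.
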(event `Interact with door`
  (if (`self.Door is open`)
    (bind (_direction _rotate) (`Timeline|Rotate Door` :!via `Reverse` :!label _label)
      (:`Update`
        (`SceneComponent.K2_SetRelativeRotation` (`self.SM_Door`) (`KismetMathLibrary.MakeRotator` 0.0 0.0 (select `bool` (`self.Inverse door`) :`false` _rotate :`true` (* _rotate -1.0) :!type "Float (single-precision)")) false false))
      (:`Finished`
        (set `self.Door is open` (`|EnumEquality` _direction "Forward"))))
    (else
      (goto _label))))

(event `Open Door`
  (goto _label))

(event `Close Door`
  (goto _label :!via `Reverse`))

(fn `UserConstructionScript`)