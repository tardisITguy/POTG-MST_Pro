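; BP_Door_Interactable is a door that players open and close through the interaction system.
; The Interact event calls InteractWithDoor, and the prompt switches between open and close text based on DoorIsOpen.
; Its interaction functions always allow interaction, mark it as server-controlled, place the prompt at a raised offset, and supply no animation or sound.
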(event `/Game/Hyper/Core/Interaction/Interfaces/BPI_Interact.Interact`
  (params (`Owning Controller` :type "Controller Object Reference"))
  (`self.Interact with door`))

(fn `Can Interact`
  (params (`Owning Controller` :type "Controller Object Reference"))
  (returns (True :type Boolean))
  (return true))

(fn `Get Interact Animation`
  (params (`Owning Controller` :type "Controller Object Reference"))
  (returns (`Anim Montage` :type "AnimMontage Object Reference"))
  (return null))

(fn `Get Interact Sound`
  (returns (`Interact Sound` :type "SoundBase Object Reference"))
  (return null))

(fn `Get Interact Text`
  (params (`Owning Controller` :type "PlayerController Object Reference"))
  (returns (`Interact Text` :type Text) (`Secondary Interact Text` :type Text))
  (return (select `bool` (`self.Door is open`) :`false` "open Door" :`true` "Close Door" :!type "Text") ""))

(fn `Get Relative Interact Text Location`
  (returns (`Relative Location` :type "Vector Structure"))
  (return (0.0 0.0 125.0)))

(fn `Should get other Actor to Interact with`
  (params (`Based on this Component` :type "PrimitiveComponent Object Reference"))
  (returns (True :type Boolean) (`Actor To Interact With` :type "Actor Object Reference"))
  (return false null))

(fn `Should server control the interact`
  (returns (`Server should excecute interact call` :type Boolean))
  (return true))

(fn `UserConstructionScript`
  (`parent.UserConstructionScript`))