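; BP_Fire is an interactable fireplace fire that players can toggle on and off through a "Toggle Fire" prompt.
; Interact flips the IsActive flag, and a separate Toggle event sets it directly.
; The interaction is server-controlled, and the flag's OnRep activates or deactivates the Niagara gas-torch effect on replication.
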(event `/Game/Hyper/Core/Interaction/Interfaces/BPI_Interact.Interact`
  (params (`Owning Controller` :type "Controller Object Reference"))
  (set `self.Is Active` (not (`self.Is Active`))))

(event `/Game/Hyper/Core/Interaction/Interfaces/BPI_Toggle.Toggle`
  (params (`On/Off` :type Boolean) (`Owning Controller` :type "Controller Object Reference"))
  (set `self.Is Active` `On/Off`))

(fn `Can Interact`
  (params (`Owning Controller` :type "Controller Object Reference"))
  (returns (True :type Boolean))
  (return true))

(fn `Get Interact Animation`
  (params (`Owning Controller` :type "Controller Object Reference"))
  (returns (`Anim Montage` :type "AnimMontage Object Reference"))
  (return null))

(fn `Get Interact Sound`
  (returns (`Interact Sound` :type "SoundBase Object Reference"))
  (return null))

(fn `Get Interact Text`
  (params (`Owning Controller` :type "PlayerController Object Reference"))
  (returns (`Interact Text` :type Text) (`Secondary Interact Text` :type Text))
  (return "Toggle Fire" ""))

(fn `Get Relative Interact Text Location`
  (returns (`Relative Location` :type "Vector Structure"))
  (return (0.0 0.0 50.0)))

(fn `OnRep_Is Active`
  (`ActorComponent.SetActive` (`self.NS_2DGasTorch`) (`self.Is Active`) false))

(fn `Should get other Actor to Interact with`
  (params (`Based on this Component` :type "PrimitiveComponent Object Reference"))
  (returns (True :type Boolean) (`Actor To Interact With` :type "Actor Object Reference"))
  (return false null))

(fn `Should server control the interact`
  (returns (`Server should excecute interact call` :type Boolean))
  (return true))

(fn `UserConstructionScript`)