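; Advanced interaction component that extends a parent to add radius icons and grab interactions.
; A looping timer sphere-traces around the character, attaching dot icons to actors that pass CanInteract and removing those out of range.
; Interact input dispatches on the target's interface, preferring Grab over basic Interact.
; Grabbing loops through a delayed gate, locking look input, feeding it to the target locally and by server events, and steering the camera toward it.
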(event `self.ReceiveBeginPlay`
  (`parent.ReceiveBeginPlay`))

(event `self.Initialize`
  (`parent.Initialize`)
  (`self.Initialize Interactables in radius timer`))

(event `Initialize Interactables in radius timer`
  ;[0.05127 0.05127 0.05127] Can interact trace in RADIUS. Continously is checking for potential interactions in a radius and set the InteractableInRadius Icon
  ;;[0.05127 0.05127 0.05127] Starts the timer by event on begin play. Not on tick, this is less expensive
  (`KismetSystemLibrary.K2_SetTimerDelegate` (delegate `Check Interactables in radius`) 0.1 true))

(event `Check Interactables in radius`
  ;[0.05127 0.05127 0.05127] Can interact trace in RADIUS. Continously is checking for potential interactions in a radius and set the InteractableInRadius Icon
  ;;[0.05127 0.05127 0.05127] Traces hit actors by forward vector of the camera
  (`self.Check For Interactables In Radius`))

(event `self.Start Try Interact`
  (bind (_interaction_method _no_interaction_method_found) (`self.Get Interaction Method`))
  (bind _component (`/Game/Hyper/Core/Locomotion/BlueprintMacroLibrary/Generic/BML_ExtendedMovement_Component.Get ExtendedMovement`))
  (bind _component_2 (`/Game/Hyper/Core/Locomotion/BlueprintMacroLibrary/Generic/BML_ExtendedMovement_Component.Get ExtendedMovement`))
  (bind _controller (`/Game/Hyper/Core/Generic/BlueprintMacroLibrary/BML_Generic_Component.Get Controller`))
  (bind _asplayer_controller (`/Game/Hyper/Core/Generic/BlueprintMacroLibrary/BML_Generic_Component.Get Player Controller`))
  (bind _returnvalue (`KismetMathLibrary.MakeVector2D` (`/Game/Hyper/Core/Locomotion/Blueprints/AC_Extended_Movement_Abstract.Turn_ActionValue` _component) (`/Game/Hyper/Core/Locomotion/Blueprints/AC_Extended_Movement_Abstract.Lookup_ActionValue` _component)))
  ;[0.05127 0.05127 0.05127] Get current interactable, and switch on interaction type. Easy to add any interaction type to your liking
  (if (not _no_interaction_method_found)
    (switch `/Game/Hyper/Core/Interaction/Datamodel/Enumerations/Enum_Interaction_Methods` _interaction_method
      (:`NewEnumerator0`
        (`self.Start Basic Interact`))
      (:`NewEnumerator2`
        (set `/Game/Hyper/Core/Locomotion/Blueprints/AC_Extended_Movement_Abstract.Disable_Turn_Input` true _component_2)
        (set `/Game/Hyper/Core/Locomotion/Blueprints/AC_Extended_Movement_Abstract.Disable_LookUp_Input` true _component_2)
        (`|ExecutionSequence`
          (:`then_0`
            (goto _label :!via `Open`))
          (:`then_1`
            (`/Engine/EditorBlueprintResources/StandardMacros.Gate` false :!label _label
              (:`Exit`
                (set `self.Is Grabbing` true)
                (`KismetSystemLibrary.Delay` (`GameplayStatics.GetWorldDeltaSeconds`))
                (bind _able_to_interact_with_this_actor (`self.Able to interact with this actor`)
                  (:`then`
                    (`self.Server: Grab` _able_to_interact_with_this_actor _returnvalue true _controller)
                    (bind _focus_target (message `/Game/Hyper/Core/Interaction/Interfaces/BPI_Grab.Grab` _able_to_interact_with_this_actor _returnvalue true _controller))
                    (`Controller.SetControlRotation` _asplayer_controller (`KismetMathLibrary.RInterpTo` (`Controller.GetControlRotation` _asplayer_controller) (`KismetMathLibrary.FindLookAtRotation` (`PlayerCameraManager.GetCameraLocation` (`/Game/Hyper/Core/Generic/BlueprintMacroLibrary/BML_Generic_Component.Get Player Camera Manager`)) _focus_target) (`GameplayStatics.GetWorldDeltaSeconds`) 15.0)) ; Rotate the player's view to focus on the interactive Blueprint
                    (bind _able_to_interact_with_this_actor_2 (`self.Able to interact with this actor`)
                      (:`then`
                        (`self.Server: Should stop grab` _able_to_interact_with_this_actor_2)
                        (bind _shouldstopgrab (message `/Game/Hyper/Core/Interaction/Interfaces/BPI_Grab.ShouldStopGrab` _able_to_interact_with_this_actor_2))
                        (if _shouldstopgrab
                          (`self.Event: Stop Grabbing`))
                        (`|ExecutionSequence`
                          (:`then_0`
                            (goto _label_3 :!via `Reset`))
                          (:`then_1`
                            (goto _label))))
                      (:`else`)))
                  (:`else`))))))))))

(event `Server: Grab`
  (params (Target :type "Object Object Reference") (GrabOffset :type "Vector2D Structure") (Dragging :type Boolean) (`Owning Controller` :type "Controller Object Reference"))
  ;[0.05127 0.05127 0.05127] Get current interactable, and switch on interaction type. Easy to add any interaction type to your liking
  (message `/Game/Hyper/Core/Interaction/Interfaces/BPI_Grab.Grab` Target GrabOffset Dragging `Owning Controller`))

(event `Server: Should stop grab`
  (params (Target :type "Object Object Reference"))
  ;[0.05127 0.05127 0.05127] Get current interactable, and switch on interaction type. Easy to add any interaction type to your liking
  (message `/Game/Hyper/Core/Interaction/Interfaces/BPI_Grab.ShouldStopGrab` Target))

(event `self.Stop Try Interact`
  (bind _component (`/Game/Hyper/Core/Locomotion/BlueprintMacroLibrary/Generic/BML_ExtendedMovement_Component.Get ExtendedMovement`))
  ;[0.05127 0.05127 0.05127] Get current interactable, and switch on interaction type. Easy to add any interaction type to your liking
  (set `self.Is Grabbing` false :!label _label_2)
  (set `/Game/Hyper/Core/Locomotion/Blueprints/AC_Extended_Movement_Abstract.Disable_Turn_Input` false _component)
  (set `/Game/Hyper/Core/Locomotion/Blueprints/AC_Extended_Movement_Abstract.Disable_LookUp_Input` false _component)
  (`|ExecutionSequence`
    (:`then_0`
      (goto _label :!via `Close`))
    (:`then_1`
      (`/Engine/EditorBlueprintResources/StandardMacros.DoOnce` true :!label _label_3
        (:`Completed`
          (bind _able_to_interact_with_this_actor (`self.Able to interact with this actor`)
            (:`then`
              (`self.Server: Grab` _able_to_interact_with_this_actor (0.0 0.0) false (`/Game/Hyper/Core/Generic/BlueprintMacroLibrary/BML_Generic_Component.Get Controller`))
              (`KismetSystemLibrary.PrintString` "move up"))
            (:`else`)))))))

(event `self.Event: Stop Grabbing`
  ;[0.05127 0.05127 0.05127] Get current interactable, and switch on interaction type. Easy to add any interaction type to your liking
  (goto _label_2))

(fn `Check For Interactables In Radius`
  (locals (`Local Interactables in radius` :type "Array of Actor Object Reference"))
  (bind _returnvalue (`Actor.K2_GetActorLocation` (`/Game/Hyper/Core/Generic/BlueprintMacroLibrary/BML_Generic_Component.Get Character`)))
  (bind (_outhits _returnvalue_2) (`KismetSystemLibrary.SphereTraceMulti` _returnvalue _returnvalue (`self.Check for interactables in this radius`) "TraceTypeQuery3" false (`|MakeArray` null :!type "Actor Object Reference")))
  (if _returnvalue_2
    (for _array_element _outhits
      (bind (_bblockinghit _binitialoverlap _time _distance _location _impactpoint _normal _impactnormal _physmat _hitactor) (`GameplayStatics.BreakHitResult` _array_element))
      ;[0.05127 0.05127 0.05127] Add every interactable in radius with implemented can interact interface
      (if (`KismetSystemLibrary.DoesImplementInterface` _hitactor "/Game/Hyper/Core/Interaction/Interfaces/BPI_CanInteract.BPI_CanInteract_C")
        ;;[0.05127 0.05127 0.05127] Don't show if can interact returns false
        (bind _true (message `/Game/Hyper/Core/Interaction/Interfaces/BPI_CanInteract.Can Interact` _hitactor (`/Game/Hyper/Core/Generic/BlueprintMacroLibrary/BML_Generic_Component.Get Controller`)))
        (if _true
          (`KismetArrayLibrary.Array_AddUnique` (`local.Local Interactables in radius`) _hitactor)
          ;[0.05127 0.05127 0.05127] Does the hitted actor already has an in radius icon attached? If so, do nothing
          (if (not (`BlueprintMapLibrary.Map_Contains` (`self.Actors that has In radius icons attached`) _hitactor))
            ;[0.05127 0.05127 0.05127] Spawn and attach the in radius icon to the found interactable with an optional tweak on relative locaiton
            (bind _relative_location (message `/Game/Hyper/Core/Interaction/Interfaces/BPI_CanInteract.Get Relative Interact Text Location` _hitactor))
            (bind _returnvalue_3 (`|SpawnActorFromClass` "/Game/Hyper/UI/Widgets/Specific/Interaction/InteractInRadiusIcon/BP_InteractableInRadiusIcon.BP_InteractableInRadiusIcon_C" (`KismetMathLibrary.MakeTransform` _relative_location) "AlwaysSpawn" "OverrideRootScale" null "/Game/Hyper/ResourcePack/UI_Elements/Interaction/T_Dot_OuterGlow.T_Dot_OuterGlow" null))
            (`BlueprintMapLibrary.Map_Add` (`self.Actors that has In radius icons attached`) _hitactor _returnvalue_3)
            (`Actor.K2_AttachToActor` _returnvalue_3 _hitactor "None" "KeepRelative" "KeepRelative" "KeepRelative" true))))))
  ;[0.05127 0.05127 0.05127] Actors that has icons attached, is it in the current radius?
  ; 	False > Remove from actors in interact radius
  ; 	True > Do nothing
  (bind _keys (`BlueprintMapLibrary.Map_Keys` (`self.Actors that has In radius icons attached`)))
  (for _array_element_2 _keys
    (if (not (`KismetArrayLibrary.Array_Contains` (`local.Local Interactables in radius`) _array_element_2))
      (bind (_value _returnvalue_4) (`BlueprintMapLibrary.Map_Find` (`self.Actors that has In radius icons attached`) _array_element_2))
      (if _returnvalue_4
        (`Actor.K2_DestroyActor` _value)
        (`BlueprintMapLibrary.Map_Remove` (`self.Actors that has In radius icons attached`) _array_element_2)))))

(fn `Get Interaction Method`
  (returns (`Interaction Method` :type "/Game/Hyper/Core/Interaction/Datamodel/Enumerations/Enum_Interaction_Methods Enum") (`No interaction method found` :type Boolean))
  ;[0.05127 0.05127 0.05127] Determines which interact interface is available on the interacting component. Each interactable can only have one type available
  (bind _able_to_interact_with_this_actor (`self.Able to interact with this actor`)
    (:`then`
      (if (`KismetSystemLibrary.DoesImplementInterface` _able_to_interact_with_this_actor "/Game/Hyper/Core/Interaction/Interfaces/BPI_Grab.BPI_Grab_C")
        (return "NewEnumerator2" false)
        (elif (`KismetSystemLibrary.DoesImplementInterface` _able_to_interact_with_this_actor "/Game/Hyper/Core/Interaction/Interfaces/BPI_Interact.BPI_Interact_C")
          (return "NewEnumerator0" false)
          (else
            (return "NewEnumerator3" true)))))
    (:`else`
      (return "NewEnumerator3" true))))