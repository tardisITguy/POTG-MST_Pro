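; Basic interaction component that lets a locally controlled pawn detect and use actors implementing BPI_CanInteract.
; A looping timer, used instead of Tick, traces from the active camera to pick the target, which can redirect to another actor, then outlines it and attaches a prompt button.
; Interact input rechecks the target, plays optional montage and sound, then calls interact on server or client as the target specifies, waiting for the montage notify if animated.
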(fn `Can Interact Trace`
  (locals (`Local Should interact on diverted actor` :type Boolean :default false))
  (bind _component (`/Game/Hyper/Core/Locomotion/BlueprintMacroLibrary/Generic/BML_ExtendedMovement_Component.Get ExtendedMovement`))
  (bind _front_offset_start_position (`self.Front Offset Start Position`))
  (bind _returnvalue (+ _front_offset_start_position (`/Game/Hyper/Core/Locomotion/Blueprints/AC_Extended_Movement_Abstract.Spring Arm Lengt` _component)))
  (bind (_outhit _hit _hitactor _hitcomponent) (`/Game/Hyper/Core/Generic/FunctionLibraries/BFL_Generic.Trace From Active Camera` (`/Game/Hyper/Core/Generic/BlueprintMacroLibrary/BML_Generic_Component.Get Player Controller`) "TraceTypeQuery3" (`|MakeArray` null :!type "Actor Object Reference") (select `/Game/Hyper/Core/Locomotion/Datamodel/Enumerations/Enum_Camera_Mode` (`/Game/Hyper/Core/Locomotion/Blueprints/AC_Extended_Movement_Abstract.Active Camera Mode` _component) :`NewEnumerator1` _returnvalue :`NewEnumerator3` _returnvalue :`NewEnumerator4` _returnvalue :`NewEnumerator6` _front_offset_start_position) (`self.Can Interact Trace length Distance`)))
  ;[0.05127 0.05127 0.05127] As long as is grabbing, do not trace for new interactions
  (if (not (`self.Is Grabbing`))
    ;[0.05127 0.05127 0.05127] Trace and check if hitted actor has implemented BPI Interact Interface
    (`self.Handle Interact Logic` _hit _hitactor _hitcomponent)))

(fn `Cancel Can Interact`
  (params (`Continue When Able To Interact Is Not Valid` :type Boolean))
  (bind (_component _is_valid) (`/Game/Hyper/Core/Outliner_System/BlueprintMacroLibrary/BML_Outliner_Component.Get Outliner Manager`))
  (bind (_value _returnvalue) (`BlueprintMapLibrary.Map_Find` (`self.Actors that has In radius icons attached`) (`self.Able to interact with this actor`)))
  ;[0.05127 0.05127 0.05127] Cancel Can Interact
  (bind _able_to_interact_with_this_actor (`self.Able to interact with this actor`)
    (:`then`
      (message `/Game/Hyper/Core/Interaction/Interfaces/BPI_CanInteract.Cancel Can Interact` _able_to_interact_with_this_actor (`/Game/Hyper/Core/Generic/BlueprintMacroLibrary/BML_Generic_Component.Get Controller`))
      ;;[0.05127 0.05127 0.05127] Add switch outline on actor: Disable
      (if _is_valid
        (`/Game/Hyper/Core/Outliner_System/Blueprints/AC_Outliner_Abstract.Switch Outline On Actor` _component (`self.Able to interact with this actor`) "NewEnumerator0" false "NewEnumerator0"))
      ;;[0.05127 0.05127 0.05127] Switch the visibility of in radius icon
      (if _returnvalue
        (`SceneComponent.SetVisibility` (`/Game/Hyper/UI/Widgets/Specific/Interaction/InteractInRadiusIcon/BP_InteractableInRadiusIcon.Widget` _value) true false))
      ;;[0.05127 0.05127 0.05127] Destroy the button and empty references
      (set `self.Able to interact with this actor` null)
      (set `self.Able To Interact With This Component` null))
    (:`else`
      _))
  (bind _active_interact_button_reference (`self.Active_Interact_Button_Reference`)
    (:`then`
      (`Actor.K2_DestroyActor` _active_interact_button_reference)
      (set `self.Active_Interact_Button_Reference` null :!label _label))
    (:`else`
      (if (`local.Continue When Able To Interact Is Not Valid`)
        (goto _label)))))

(fn `Handle Interact Logic`
  (params (Hit :type Boolean) (`Hit Actor` :type "Actor Object Reference") (`Hit Component` :type "PrimitiveComponent Object Reference"))
  (locals (`Local Should interact on diverted actor` :type Boolean))
  (bind (_component _is_valid) (`/Game/Hyper/Core/Outliner_System/BlueprintMacroLibrary/BML_Outliner_Component.Get Outliner Manager`))
  (bind _able_to_interact_with_this_actor (`self.Able to interact with this actor`))
  (bind (_value _returnvalue) (`BlueprintMapLibrary.Map_Find` (`self.Actors that has In radius icons attached`) (`self.Able to interact with this actor`)))
  ;[0.05098 0.05098 0.05098] This function will handle the interact logic. It does the following things:
  ;
  ; - Set 'Able To Interact With Actor' to the correct actor. (Empty if none )
  ; - Check if should use diverted actor and set that one.
  ; - Set the correct interact text based on hit actor.
  (if Hit
    (if (`KismetSystemLibrary.DoesImplementInterface` `Hit Actor` "/Game/Hyper/Core/Interaction/Interfaces/BPI_CanInteract.BPI_CanInteract_C")
      (bind (_true _actor_to_interact_with) (message `/Game/Hyper/Core/Interaction/Interfaces/BPI_CanInteract.Should get other Actor to Interact with` (`local.Hit Actor`) (`local.Hit Component`)))
      (bind _output_get (set `local.Local Should interact on diverted actor` _true))
      (if _output_get
        (bind _true_2 (message `/Game/Hyper/Core/Interaction/Interfaces/BPI_CanInteract.Can Interact` _actor_to_interact_with (`/Game/Hyper/Core/Generic/BlueprintMacroLibrary/BML_Generic_Component.Get Controller`)))
        (if _true_2
          (bind _able_to_interact_with_this_actor_2 (`self.Able to interact with this actor`)
            (:`then`
              (if (== _able_to_interact_with_this_actor_2 _actor_to_interact_with)
                (bind (_interact_text _secondary_interact_text) (message `/Game/Hyper/Core/Interaction/Interfaces/BPI_CanInteract.Get Interact Text` (`self.Able to interact with this actor`) (`/Game/Hyper/Core/Generic/BlueprintMacroLibrary/BML_Generic_Component.Get Player Controller`) :!label _label))
                (bind _active_interact_button_reference (`self.Active_Interact_Button_Reference`)
                  (:`then`
                    (bind _asui_can_interact_button (cast `/Game/Hyper/UI/Widgets/Specific/Interaction/Can_Interact/UI_CanInteractButton` (`WidgetComponent.GetUserWidgetObject` (`/Game/Hyper/UI/Widgets/Specific/Interaction/Can_Interact/BP_CanInteract_Button.Widget` _active_interact_button_reference))))
                    (`/Game/Hyper/UI/Widgets/Specific/Interaction/Can_Interact/UI_CanInteractButton.Set Values` _asui_can_interact_button _interact_text _secondary_interact_text))
                  (:`else`))
                (else
                  ;;[0.05098 0.05098 0.05098] The top one will cancel interact on the current actor, and after that enable interact with the given actor. The bottom cancel interact will only cancel the interact
                  (`/Engine/EditorBlueprintResources/StandardMacros.DoOnce` false :!label _label_2
                    (:`Completed`
                      (`self.Cancel Can Interact` true)
                      (if (`local.Local Should interact on diverted actor`) :!label _label_3
                        (message `/Game/Hyper/Core/Interaction/Interfaces/BPI_CanInteract.Can Interact` _actor_to_interact_with (`/Game/Hyper/Core/Generic/BlueprintMacroLibrary/BML_Generic_Component.Get Controller`))
                        (set `self.Able to interact with this actor` _actor_to_interact_with)
                        (else
                          (message `/Game/Hyper/Core/Interaction/Interfaces/BPI_CanInteract.Can Interact` (`local.Hit Actor`) (`/Game/Hyper/Core/Generic/BlueprintMacroLibrary/BML_Generic_Component.Get Controller`))
                          (set `self.Able to interact with this actor` (`local.Hit Actor`))))
                      (if _is_valid
                        (`/Game/Hyper/Core/Outliner_System/Blueprints/AC_Outliner_Abstract.Switch Outline On Actor` _component (`self.Able to interact with this actor`) "NewEnumerator0" true "NewEnumerator0"))
                      (bind (_interact_text_2 _secondary_interact_text_2) (message `/Game/Hyper/Core/Interaction/Interfaces/BPI_CanInteract.Get Interact Text` _able_to_interact_with_this_actor (`/Game/Hyper/Core/Generic/BlueprintMacroLibrary/BML_Generic_Component.Get Player Controller`)))
                      (bind _relative_location (message `/Game/Hyper/Core/Interaction/Interfaces/BPI_CanInteract.Get Relative Interact Text Location` _able_to_interact_with_this_actor))
                      (bind _returnvalue_2 (`|SpawnActorFromClass` "/Game/Hyper/UI/Widgets/Specific/Interaction/Can_Interact/BP_CanInteract_Button.BP_CanInteract_Button_C" (`KismetMathLibrary.MakeTransform` _relative_location) "AlwaysSpawn" "OverrideRootScale" null _interact_text_2 _secondary_interact_text_2 null))
                      (bind _output_get_2 (set `self.Active_Interact_Button_Reference` _returnvalue_2))
                      (`Actor.K2_AttachToActor` _output_get_2 (`self.Able to interact with this actor`) "None" "KeepRelative" "KeepRelative" "KeepRelative" true)
                      (if _returnvalue
                        (`SceneComponent.SetVisibility` (`/Game/Hyper/UI/Widgets/Specific/Interaction/InteractInRadiusIcon/BP_InteractableInRadiusIcon.Widget` _value) false false))
                      (`|ExecutionSequence`
                        (:`then_0`
                          (goto _label_2 :!via `Reset`))
                        (:`then_1`
                          (goto _label_5 :!via `Reset`))))))))
            (:`else`
              (bind _active_interact_button_reference_2 (`self.Active_Interact_Button_Reference` :!label _label_4)
                (:`then`
                  (`Actor.K2_DestroyActor` _active_interact_button_reference_2)
                  (set `self.Active_Interact_Button_Reference` null)
                  (goto _label_3))
                (:`else`
                  (goto _label_3)))))
          (else
            (`/Engine/EditorBlueprintResources/StandardMacros.DoOnce` false :!label _label_5
              (:`Completed`
                (`self.Cancel Can Interact` false)))))
        (else
          (bind _true_3 (message `/Game/Hyper/Core/Interaction/Interfaces/BPI_CanInteract.Can Interact` (`local.Hit Actor`) (`/Game/Hyper/Core/Generic/BlueprintMacroLibrary/BML_Generic_Component.Get Controller`)))
          (if _true_3
            (bind _able_to_interact_with_this_actor_3 (`self.Able to interact with this actor`)
              (:`then`
                (if (== _able_to_interact_with_this_actor_3 (`local.Hit Actor`))
                  (goto _label)
                  (else
                    (goto _label_2))))
              (:`else`
                (goto _label_4)))
            (else
              (goto _label_5)))))
      (else
        (goto _label_5)))
    (else
      (goto _label_5))))

(fn `Link_InputMapping_Context`
  (bind _asplayer_controller (`/Game/Hyper/Core/Generic/BlueprintMacroLibrary/BML_Generic_Component.Get Player Controller`))
  ;[0.05127 0.05127 0.05127] We use the Enhanced Input System. I've categorized the mapping systems.
  ; After the mapping context is added to the player controller, the IA(Input actions) are receiving input.
  ; Please be aware that the enhanced input plugin needs to be enabled and in the project input settings it should be set
  (`/Engine/EditorBlueprintResources/StandardMacros.IsValid` _asplayer_controller
    (:`Is Valid`
      (`EnhancedInputSubsystemInterface.AddMappingContext` (pcsubsystem `EnhancedInputLocalPlayerSubsystem` _asplayer_controller) "/Game/Hyper/Locomotion/Input/InputMappings/IM_Interaction.IM_Interaction" 0 (struct)))))

(fn `Try Play Interact Animation`
  (returns (`Playing latent montage` :type Boolean))
  (bind _able_to_interact_with_this_actor (`self.Able to interact with this actor`)
    (:`then`
      ;[0.05127 0.05127 0.05127] Play optional animation
      (bind _anim_montage (message `/Game/Hyper/Core/Interaction/Interfaces/BPI_CanInteract.Get Interact Animation` _able_to_interact_with_this_actor (`/Game/Hyper/Core/Generic/BlueprintMacroLibrary/BML_Generic_Component.Get Controller`)))
      (`/Engine/EditorBlueprintResources/StandardMacros.IsValid` _anim_montage
        (:`Is Valid`
          (`/Game/Hyper/Core/ReplicationSubSystem/Blueprints/AC_Replication_Abstract.Initialize Multicast Latent Montage` (`/Game/Hyper/Core/ReplicationSubSystem/BlueprintMacroLibrary/BML_Replication_Component.Get Replication`) _anim_montage (`|MakeArray` "interact" :!type "Name") true null 1.0)
          (return true))
        (:`Is Not Valid`
          _)))
    (:`else`
      _))
  (return false))

(fn `Try Play Interact Sound`
  ;[0.05098 0.05098 0.05098] Check if we're interacting with an actor
  (bind _able_to_interact_with_this_actor (`self.Able to interact with this actor`)
    (:`then`
      ;[0.05127 0.05127 0.05127] Play Optional Interact Sound
      (bind _interact_sound (message `/Game/Hyper/Core/Interaction/Interfaces/BPI_CanInteract.Get Interact Sound` _able_to_interact_with_this_actor))
      (`/Engine/EditorBlueprintResources/StandardMacros.IsValid` _interact_sound
        (:`Is Valid`
          (`/Game/Hyper/Core/ReplicationSubSystem/Blueprints/AC_Replication_Abstract.Initialize Spawn Sound At Location` (`/Game/Hyper/Core/ReplicationSubSystem/BlueprintMacroLibrary/BML_Replication_Component.Get Replication`) _interact_sound (`Actor.K2_GetActorLocation` _able_to_interact_with_this_actor) false 0.0 "/Game/Hyper/ResourcePack/Audio/AttenuationPresets/ATT_Default.ATT_Default"))
        (:`Is Not Valid`
          _))
      (return))
    (:`else`
      (return))))

(fn `Try Press Button Animation`
  ;[0.05127 0.05127 0.05127] Press animation
  (bind _active_interact_button_reference (`self.Active_Interact_Button_Reference`)
    (:`then`
      (`/Game/Hyper/UI/Widgets/Specific/Interaction/Can_Interact/BP_CanInteract_Button.Play pressed animation` _active_interact_button_reference))
    (:`else`
      _))
  (return))