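; Placeable building cabinet that keeps a list of authorized builders for nearby buildables.
; Once built, a server-controlled interact toggles the player's name in that list, with interact text to match.
; A sphere sized by AuthorizationRange makes it the owning cabinet of finished buildables it begins overlapping.
; Unfinished buildables instead track it as an overlapping cabinet until the overlap ends.
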(event `self.ReceiveBeginPlay`
  (`parent.ReceiveBeginPlay`))

(event `/Game/Hyper/Core/Interaction/Interfaces/BPI_Interact.Interact`
  (params (`Owning Controller` :type "Controller Object Reference"))
  (bind _authorized_builders (`self.Authorized Builders`))
  (bind _returnvalue (`PlayerState.GetPlayerName` (`Controller.PlayerState` `Owning Controller`)))
  (`parent.Interact` `Owning Controller`)
  (if (`self.Is Building Finished`)
    (if (`KismetArrayLibrary.Array_Contains` (`self.Authorized Builders`) _returnvalue)
      (`KismetArrayLibrary.Array_RemoveItem` _authorized_builders _returnvalue)
      (else
        (`KismetArrayLibrary.Array_AddUnique` _authorized_builders _returnvalue)))))

(event `self.Sphere.OnComponentBeginOverlap`
  (params (OverlappedComponent :type "PrimitiveComponent Object Reference") (OtherActor :type "Actor Object Reference") (OtherComp :type "PrimitiveComponent Object Reference") (OtherBodyIndex :type Integer) (bFromSweep :type Boolean) (SweepResult :type "HitResult Structure (by ref)"))
  (if (not (== OtherActor self))
    (bind _asbp_buildable_abstract (cast `/Game/Hyper/Core/BuildingSystem/Blueprints/BP_Buildable_Abstract` OtherActor))
    (if (`/Game/Hyper/Core/BuildingSystem/Blueprints/BP_Buildable_Abstract.Is Building Finished` _asbp_buildable_abstract)
      (set `/Game/Hyper/Core/BuildingSystem/Blueprints/BP_Buildable_Abstract.Owning Cabinet` self _asbp_buildable_abstract)
      (else
        (`KismetArrayLibrary.Array_AddUnique` (`/Game/Hyper/Core/BuildingSystem/Blueprints/BP_Buildable_Abstract.Overlapping Cabinets` _asbp_buildable_abstract) self)))))

(event `self.Sphere.OnComponentEndOverlap`
  (params (OverlappedComponent :type "PrimitiveComponent Object Reference") (OtherActor :type "Actor Object Reference") (OtherComp :type "PrimitiveComponent Object Reference") (OtherBodyIndex :type Integer))
  (bind _asbp_buildable_abstract (cast `/Game/Hyper/Core/BuildingSystem/Blueprints/BP_Buildable_Abstract` OtherActor))
  (`KismetArrayLibrary.Array_RemoveItem` (`/Game/Hyper/Core/BuildingSystem/Blueprints/BP_Buildable_Abstract.Overlapping Cabinets` _asbp_buildable_abstract) self))

(fn `Get Interact Text`
  (params (`Owning Controller` :type "PlayerController Object Reference"))
  (returns (`Interact Text` :type Text) (`Secondary Interact Text` :type Text))
  (if (`self.Is Building Finished`)
    (return (select `bool` (`KismetArrayLibrary.Array_Contains` (`self.Authorized Builders`) (`PlayerState.GetPlayerName` (`Controller.PlayerState` `Owning Controller`))) :`false` (`self.Authorize Text`) :`true` (`self.Deauthorize Text`)) "")
    (else
      (bind (_interact_text _secondary_interact_text) (`parent.Get Interact Text` (`local.Owning Controller`)))
      (return _interact_text _secondary_interact_text))))

(fn `Should server control the interact`
  (returns (`Server should excecute interact call` :type Boolean))
  (return true))

(fn `UserConstructionScript`
  (`parent.UserConstructionScript`)
  (`SphereComponent.SetSphereRadius` (`self.Sphere`) (`self.Authorization Range`) true))