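; Modular buildable door for the building system that swings open and closed on interact once construction is finished, as a single or double door.
; A timeline offsets yaw from the rotations saved at BeginPlay, mirroring the second leaf, flipping for OpenOutwards and ignoring toggles while moving.
; An attached lock, re-snapped after a delay on BeginPlay, restricts use to players whose names it authorizes.
; Interaction is flagged as server-controlled.
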(event `self.ReceiveBeginPlay`
  (bind _attached_buildings (`self.Attached_Buildings`))
  (`parent.ReceiveBeginPlay`)
  (`|ExecutionSequence`
    (:`then_0`
      ;[1 1 1] set default rot
      (set `self.Start_Rotation_Left` (`SceneComponent.K2_GetComponentRotation` (`self.StaticMeshComponent`)))
      (set `self.Start_Rotation_Right` (`SceneComponent.K2_GetComponentRotation` (`self.Secondary`))))
    (:`then_1`
      ;[1 1 1] Attach the lock to the door on begin play (if there is a lock from a save)
      (`KismetSystemLibrary.Delay` 1.0)
      (if (`KismetArrayLibrary.Array_IsValidIndex` _attached_buildings)
        (bind _asbp_buildable_lock (cast `/Game/Hyper/BuildingSystem/Blueprints_Buildables/Modular/BP_Buildable_Lock` (`|GetArrayItem` _attached_buildings)))
        (bind _output_get (set `self.Door_Lock_Reference` _asbp_buildable_lock))
        (`self.K2_AttachToComponent` _output_get (`self.Lock_Snap`) "None" "SnapToTarget" "SnapToTarget" "SnapToTarget" true)))))

(event `/Game/Hyper/Core/Interaction/Interfaces/BPI_Interact.Interact`
  (params (`Owning Controller` :type "Controller Object Reference"))
  (bind (_start_rotation_right_roll _start_rotation_right_pitch _start_rotation_right_yaw) (`KismetMathLibrary.BreakRotator` (`self.Start_Rotation_Right`)))
  (bind (_start_rotation_left_roll _start_rotation_left_pitch _start_rotation_left_yaw) (`KismetMathLibrary.BreakRotator` (`self.Start_Rotation_Left`)))
  ;[1 1 1] Call the master event of interact. This handles the default interaction requirements
  (`self.Process Interaction` `Owning Controller`)
  ;[1 1 1] Check if building is finished. If not, dont process
  (if (`self.Is Building Finished`)
    (`|ExecutionSequence`
      (:`then_0`
        ;[1 1 1] If there is a lock, check if the player is authorized. If not, continue
        ;;[1 1 1] Index 0 of attached buildings should be a lock
        (bind _asbp_buildable_lock (cast `/Game/Hyper/BuildingSystem/Blueprints_Buildables/Modular/BP_Buildable_Lock` (`|GetArrayItem` (`self.Attached_Buildings`)))
          (:`then`
            (set `self.Door_Lock_Reference` _asbp_buildable_lock)
            (bind _authorized (`self.Check if is authorized` `Owning Controller`))
            (if _authorized
              ;[1 1 1] Rotate door
              (if (`self.Is Opening`) :!label _label
                _
                (elif (`self.IsOpen`)
                  (set `self.IsOpen` false)
                  (bind (_direction _newtrack_0) (`Timeline|Timeline_0` :!via `ReverseFromEnd` :!label _label_2)
                    (:`Update`
                      ;;[1 1 1] Left
                      (set `self.Is Opening` true)
                      (bind _returnvalue (select `bool` (`self.Open Outwards`) :`false` _newtrack_0 :`true` (* _newtrack_0 -1.0) :!type "Float (double-precision)"))
                      (`SceneComponent.K2_SetWorldRotation` (`self.StaticMeshComponent`) (`KismetMathLibrary.MakeRotator` _start_rotation_left_roll _start_rotation_left_pitch (+ _returnvalue _start_rotation_left_yaw)) false false)
                      ;;[1 1 1] Right
                      (`SceneComponent.K2_SetWorldRotation` (`self.Secondary`) (`KismetMathLibrary.MakeRotator` _start_rotation_right_roll _start_rotation_right_pitch (+ (* _returnvalue -1.0) _start_rotation_right_yaw)) false false))
                    (:`Finished`
                      (set `self.Is Opening` false)))
                  (else
                    (set `self.IsOpen` true)
                    (goto _label_2 :!via `PlayFromStart`))))))
          (:`CastFailed`
            (goto _label))))
      (:`then_1`
        ;[1 1 1] Set to build state once
        (`/Engine/EditorBlueprintResources/StandardMacros.DoOnce` false
          (:`Completed`
            (`self.Set buildable to Build State`)))))))

(fn `Check if is authorized`
  (params (controller :type "Controller Object Reference"))
  (returns (authorized :type Boolean))
  (bind _door_lock_reference (`self.Door_Lock_Reference`))
  ;[1 1 1] Check if has a lock attached
  (`/Engine/EditorBlueprintResources/StandardMacros.IsValid` _door_lock_reference
    (:`Is Valid`
      (return (`KismetArrayLibrary.Array_Contains` (`/Game/Hyper/BuildingSystem/Blueprints_Buildables/Masters/BP_Buildable_Advanced.Authorized Players` _door_lock_reference) (`PlayerState.GetPlayerName` (`Controller.PlayerState` controller)))))))

(fn `Should server control the interact`
  (returns (`Server should excecute interact call` :type Boolean))
  (return true))

(fn `UserConstructionScript`
  (`parent.UserConstructionScript`)
  (if (`self.Is_Double_Door`)
    (`StaticMeshComponent.SetStaticMesh` (`self.Secondary`) (`self.Buildable Mesh`))))