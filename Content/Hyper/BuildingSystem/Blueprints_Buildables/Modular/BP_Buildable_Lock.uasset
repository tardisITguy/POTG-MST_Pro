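; Buildable password lock for the modular building system that keeps a saved list of authorized player names.
; Server-controlled interaction sets the interacting controller as owner so the UI opens on that client, or runs normal interaction processing while unfinished.
; The lock widget's correct-password unlock adds the player to the list via a server event.
; A password reset stores the new password, clears the list and re-authorizes only the resetter.
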(event `Event: Reset password`
  (params (`new password` :type Text) (controller :type "Controller Object Reference"))
  ;[0.05098 0.05098 0.05098] On server:
  ; On password reset, clear authorized list and add the one to the autohorized list that resetted the password
  (set `self.Password` `new password`)
  (`KismetArrayLibrary.Array_Clear` (`self.Authorized Players`))
  (`self.Add to authorized players` controller))

(event `/Game/Hyper/Core/Interaction/Interfaces/BPI_Interact.Interact`
  (params (`Owning Controller` :type "Controller Object Reference"))
  (bind (_asplayer_controller _bsuccess) (`/Game/Hyper/Core/Generic/BlueprintMacroLibrary/BML_Generic_ControllerInput.Get Player Controller` `Owning Controller`))
  ;[0.05098 0.05098 0.05098] The interact is called via server. However, we want to do some things on the owning client. E.g. opening UI. That is why we also set owner so we can call logic on the interacting player (openening/closing UI)
  (`self.SetOwner` `Owning Controller`)
  (if (`self.Is Building Finished`)
    ;[0.05098 0.05098 0.05098] Open UI on owning client
    (if _bsuccess
      (`self.Open UI` _asplayer_controller))
    (else
      ;[0.05098 0.05098 0.05098] Call the master event of interact. This handles the default interaction requirements
      (`self.Process Interaction` `Owning Controller`))))

(event `OnButtonBaseClicked_Event_0`
  (params (Button :type "CommonButtonBase Object Reference"))
  (bind _ui_lock_password_reset (`/Game/Hyper/UI/Widgets/Specific/Building/Lock/UI_Lock_Master.UI_Lock_Password_Reset` (`self.Active UI lock widget`)))
  ;[0.05098 0.05098 0.05098] If entered password is correct, allow the reset password and set the password to the new variable
  (bind _correct (`/Game/Hyper/UI/Widgets/Specific/Building/Lock/UI_Lock_Password_Reset.Check if password is correct` _ui_lock_password_reset))
  (if _correct
    (`self.Event: Reset password` (`EditableTextBox.GetText` (`/Game/Hyper/UI/Widgets/Specific/Building/Lock/UI_Lock_Password_Reset.EditableTextBox_NewPass` _ui_lock_password_reset)) (`self.Player Controller interacting`))
    (`self.Close widget`)))

(event `Open UI`
  (params (`Player Controller interacting` :type "PlayerController Object Reference"))
  (bind _player_controller_interacting (`self.Player Controller interacting`))
  ;[0.05098 0.05098 0.05098] Create the lock widget on interaction. Also set the password in that widget
  (bind _output_get (set `self.Player Controller interacting` `Player Controller interacting`))
  (bind _returnvalue (`|CreateWidget` "/Game/Hyper/UI/Widgets/Specific/Building/Lock/UI_Lock_Master.UI_Lock_Master_C" _output_get (`self.Password`)))
  (bind _output_get_2 (set `self.Active UI lock widget` _returnvalue))
  (`UserWidget.AddToViewport` _output_get_2 0)
  (`WidgetBlueprintLibrary.SetInputMode_UIOnlyEx` _player_controller_interacting (`self.Active UI lock widget`) "LockAlways")
  (set `PlayerController.bShowMouseCursor` true _player_controller_interacting)
  (if (`self.Is Building Finished`)
    ;[0.05098 0.05098 0.05098] Binding the buttons in the UI
    (add `CommonButtonBase.OnButtonBaseClicked` (`/Game/Hyper/UI/Widgets/Specific/Building/Lock/UI_Lock_Password.UI_Button_Unlock` (`/Game/Hyper/UI/Widgets/Specific/Building/Lock/UI_Lock_Master.UI_Lock_Password` (`self.Active UI lock widget`))) (delegate `OnButtonBaseClicked_Event`))
    (add `CommonButtonBase.OnButtonBaseClicked` (`/Game/Hyper/UI/Widgets/Specific/Building/Lock/UI_Lock_Password_Reset.UI_Button_Reset` (`/Game/Hyper/UI/Widgets/Specific/Building/Lock/UI_Lock_Master.UI_Lock_Password_Reset` (`self.Active UI lock widget`))) (delegate `OnButtonBaseClicked_Event_0`))))

(event `Close widget`
  (bind _player_controller_interacting (`self.Player Controller interacting`))
  ;[0.05098 0.05098 0.05098] Close widget
  (`Widget.RemoveFromParent` (`self.Active UI lock widget`))
  (`WidgetBlueprintLibrary.SetInputMode_GameOnly` _player_controller_interacting)
  (set `PlayerController.bShowMouseCursor` false _player_controller_interacting))

(event `OnButtonBaseClicked_Event`
  (params (Button :type "CommonButtonBase Object Reference"))
  ;[0.05098 0.05098 0.05098] IF entered password is correct. Add the interacting player to the authorized players list
  (bind _correct (`/Game/Hyper/UI/Widgets/Specific/Building/Lock/UI_Lock_Password.Check if password is correct` (`/Game/Hyper/UI/Widgets/Specific/Building/Lock/UI_Lock_Master.UI_Lock_Password` (`self.Active UI lock widget`))))
  (if _correct
    (`self.Event add to authorized players` (`self.Player Controller interacting`))
    (`self.Close widget`)))

(event `Event add to authorized players`
  (params (controller :type "Controller Object Reference"))
  ;[0.05098 0.05098 0.05098] Set authorized player on server
  (`self.Add to authorized players` controller))

(fn `Add to authorized players`
  (params (controller :type "Controller Object Reference"))
  (`KismetArrayLibrary.Array_AddUnique` (`self.Authorized Players`) (`PlayerState.GetPlayerName` (`Controller.PlayerState` controller)))
  (`self.Save_Buildable_Actor`))

(fn `Should server control the interact`
  (returns (`Server should excecute interact call` :type Boolean))
  (return true))

(fn `UserConstructionScript`
  (`parent.UserConstructionScript`))