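; Master actor for spline-placed buildables, laying a mesh repeatedly along a spline as a ghost preview during placement.
; On finish, it spawns a BP_Buildable_Advanced per group of meshes, scaling resource cost for a short last group.
; These coupled buildables receive redirected interaction and damage, while the spline handles segment materials, collision and destruction.
; Clients rebuild the spline from replicated point locations, and state saves to the BuildSave slot.
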(event `self.ReceiveBeginPlay`
  (bind _object (`/Game/Hyper/Core/Generic/BlueprintMacroLibrary/BML_AssetLoading.Async Load Asset Checked` (`.Mesh_149_A56D2E784235667052B95EB56B8DC96F` (break `/Game/Hyper/Core/BuildingSystem/Datamodel/Structures/Struct_Buildable_Info` (`self.Builable Struct`))))
    (:`Completed`
      (bind _asstatic_mesh (cast `StaticMesh` _object))
      (set `self.Buildable Mesh` _asstatic_mesh)
      ;[0.2449 1 0] We need the length of the spline mesh to calulate when to place a mesh in the spline caluclation
      (`self.Calculate Spline Mesh Length`)
      ;[1 1 1] Stores the GUID if GUID is empty
      (if (not (> (`KismetStringLibrary.Len` (`self.GUID_Buildable_Spline`)) 0))
        (set `self.GUID_Buildable_Spline` (`KismetGuidLibrary.Conv_GuidToString` (`KismetGuidLibrary.NewGuid`)))))))

(event `Event: Update Spline`
  (bind _amount_of_meshes_needed_based_on_spline_length (`self.Calculate Amount Of Meshes Needed Based On Spline Length`))
  (bind _spline_mesh_components (`self.Spline Mesh Components`))
  (bind _returnvalue (`KismetArrayLibrary.Array_Length` (`self.Spline Mesh Components`)))
  ;[0.05098 0.05098 0.05098] Update the spline
  ; Continously destroy all created spline meshes and recalculate how the spline meshes should be positioned
  ;;[0.05098 0.05098 0.05098] Only run is spline is not yet finished
  (if (not (`self.Spline Building placement is finished`))
    ;;[0.05098 0.05098 0.05098] Do we have too many spline meshes?
    (if (< _amount_of_meshes_needed_based_on_spline_length _returnvalue)
      ;;[0.05098 0.05098 0.05098] Remove excess spline components
      (for _index (range _amount_of_meshes_needed_based_on_spline_length _returnvalue)
        (bind _output (`|GetArrayItem` _spline_mesh_components _index))
        (`/Engine/EditorBlueprintResources/StandardMacros.IsValid` _output
          (:`Is Valid`
            (`ActorComponent.K2_DestroyComponent` _output))))
      (`KismetArrayLibrary.Array_Resize` _spline_mesh_components _amount_of_meshes_needed_based_on_spline_length))
    (`self.Create Spline Meshes` false)))

(event `Event: Destroy Spline Mesh Component`
  (params (`Segment Indexes` :type "Array of Integer"))
  (bind _spline_mesh_components (`self.Spline Mesh Components`))
  ;[1 1 1] Destroy the spline mesh component. Via The component reference itself or via index
  ;;[1 1 1] We are multicasting this untill I've found a better solution to replicate the destroy nicely on the clients. It seems the the spline segments are hard to properly replicate
  (if (`KismetArrayLibrary.Array_IsValidIndex` `Segment Indexes`)
    (for _array_element `Segment Indexes`
      (`KismetArrayLibrary.Array_AddUnique` (`self.Destroyed spline mesh segment indexes`) _array_element)
      (if (`KismetArrayLibrary.Array_IsValidIndex` _spline_mesh_components)
        (`self.Destroy Spline Mesh Component` (`|GetArrayItem` _spline_mesh_components _array_element))))
    (`self.Save Buildable Spline Actor`)))

(event `/Game/Hyper/Core/BuildingSystem/Interfaces/BPI_Buildable.Set_Spline_Build_Ghost_Mesh_Color`
  (params (`Can Build` :type Boolean))
  ;[1 1 1] Set the ghost mesh color to can build: Green or red
  ; If this does not seem to work, check if the material has the setting: "Used with spline" is enabled
  (if `Can Build`
    (set `self.Ghost_Material` "/Game/Hyper/ResourcePack/Tileable_Materials/Glass/M_Glass_Inst_Green.M_Glass_Inst_Green")
    (else
      (set `self.Ghost_Material` "/Game/Hyper/ResourcePack/Tileable_Materials/Glass/M_Glass_Inst_Red.M_Glass_Inst_Red"))))

(event `Event: Set Spline to Finished and ghost`
  ;[1 1 1] For each spline mesh segment, determine where to spawn the buildable and couple it to the segments
  (`self.Set the complete spline to finished spline and couple buildable actors to the segments`)
  (`self.Save Buildable Spline Actor`))

(event `Event: Set Segment to Build State`
  (params (`Segment Index` :type Integer) (`Segment Indexes` :type "Array of Integer"))
  (bind _spline_mesh_components (`self.Spline Mesh Components`))
  ;[1 1 1] Set specific segment to build state via index.
  ; This is called via the "coupled" buildable master.
  ; The buildable is the onte that handles all the logic of a buildable. When all resources are added to that buildable, set the segment to build state of the spline
  (if (`KismetArrayLibrary.Array_IsValidIndex` `Segment Indexes`)
    (for _array_element `Segment Indexes`
      (`KismetArrayLibrary.Array_AddUnique` (`self.Segment Indexes set to build state`) _array_element)
      (if (`KismetArrayLibrary.Array_IsValidIndex` _spline_mesh_components _array_element)
        (`self.Set Spline segment to Build State` (`|GetArrayItem` _spline_mesh_components _array_element))))))

(event `Event: Interact with segment`
  (params (ItemToFind :type "PrimitiveComponent Object Reference (by ref)") (`Player Controller` :type "PlayerController Object Reference"))
  ;[1 1 1] Interact with specific segment
  ; The segment is coupled with a buildable master.
  ; The buildable is the one that handles all the logic of a buildable.
  ; When we hit this segment, we want to interact with the coupled buildable master to handle resource management
  (bind _asspline_mesh_component (cast `SplineMeshComponent` ItemToFind))
  (bind _coupled_buildable_master (`self.Get Coupled buildable master to spline mesh` _asspline_mesh_component))
  (`/Engine/EditorBlueprintResources/StandardMacros.IsValid` _coupled_buildable_master
    (:`Is Valid`
      (message `/Game/Hyper/Core/Interaction/Interfaces/BPI_Interact.Interact` _coupled_buildable_master `Player Controller`))))

(event `self.ReceivePointDamage`
  (params (Damage :type "Float (single-precision)") (DamageType :type "DamageType Object Reference") (HitLocation :type "Vector Structure") (HitNormal :type "Vector Structure") (HitComponent :type "PrimitiveComponent Object Reference") (BoneName :type Name) (ShotFromDirection :type "Vector Structure") (InstigatedBy :type "Controller Object Reference") (DamageCauser :type "Actor Object Reference") (HitInfo :type "HitResult Structure (by ref)"))
  (bind (_bblockinghit _binitialoverlap _time _distance _location _impactpoint _normal _impactnormal _physmat _hitactor _hitcomponent _hitbonename _bonename _hititem _elementindex _faceindex _tracestart _traceend) (`GameplayStatics.BreakHitResult` HitInfo))
  ;[1 1 1] When hitting this segement (via trace), propegate the damage to the coupled buildable master
  (bind _outhit (`KismetSystemLibrary.LineTraceSingle` _tracestart (+ _traceend (* (`KismetMathLibrary.GetDirectionUnitVector` _tracestart _traceend) 100.0)) "TraceTypeQuery1" false (`|MakeArray` DamageCauser (`Controller.K2_GetPawn` InstigatedBy) :!type "Actor Object Reference") "None" false))
  (bind _asspline_mesh_component (cast `SplineMeshComponent` (`.HitComponent` (`GameplayStatics.BreakHitResult` _outhit))))
  (`GameplayStatics.ApplyPointDamage` (`self.Get Coupled buildable master to spline mesh` _asspline_mesh_component) Damage ShotFromDirection _outhit InstigatedBy DamageCauser))

(fn `Calculate Amount Of Meshes Needed Based On Spline Length`
  (returns (`Amount of meshes needed based on spline length` :type Integer))
  (return (`KismetMathLibrary.FTrunc` (/ (`SplineComponent.GetSplineLength` (`self.Spline`)) (`self.Spline_Mesh_Length`)))))

(fn `Calculate Spline Mesh Length`
  (bind _buildable_mesh (`self.Buildable Mesh`))
  (`/Engine/EditorBlueprintResources/StandardMacros.IsValid` _buildable_mesh
    (:`Is Valid`
      ;[1 1 1] Set the spline mesh lenght. We need this so we can determine when a new mesh needs to be placed in the spline
      (set `self.Spline_Mesh_Length` (* (select `ESplineMeshAxis` (`self.Spline Mesh Forward Axis`) :`X` (.x (`.BoxExtent` (`KismetMathLibrary.BreakBoxSphereBounds` (`StaticMesh.GetBounds` _buildable_mesh)))) :`Y` (.y (`.BoxExtent` (`KismetMathLibrary.BreakBoxSphereBounds` (`StaticMesh.GetBounds` _buildable_mesh)))) :`Z` (.z (`.BoxExtent` (`KismetMathLibrary.BreakBoxSphereBounds` (`StaticMesh.GetBounds` _buildable_mesh))))) 2.0)))))

(fn `Can Interact`
  (params (`Owning Controller` :type "Controller Object Reference"))
  (returns (True :type Boolean))
  (return false))

(fn `Create Spline Meshes`
  (params (Recreate :type Boolean))
  (locals (`New Mesh Count` :type Integer :default 0) (`Current Index` :type Integer))
  (bind _spline (`self.Spline`))
  (bind _spline_mesh_length (`self.Spline_Mesh_Length`))
  (bind _spline_2 (`self.Spline`))
  (bind _spline_mesh_length_2 (`self.Spline_Mesh_Length`))
  (bind _current_index (`local.Current Index`))
  (bind _returnvalue (* _current_index (`self.Spline_Mesh_Length`)))
  (bind (_relativelocation_x _relativelocation_y _relativelocation_z) (`KismetMathLibrary.BreakVector` (`SceneComponent.RelativeLocation` (`self.Spline Mesh Component Reference`))))
  (bind _returnvalue_2 (`SplineComponent.GetLocationAtDistanceAlongSpline` _spline_2 _returnvalue "World"))
  (bind _returnvalue_3 (* (+ _current_index 1) (`self.Spline_Mesh_Length`)))
  (bind _returnvalue_4 (`KismetMathLibrary.ClampVectorSize` (`SplineComponent.GetTangentAtDistanceAlongSpline` _spline_2 _returnvalue "World") _spline_mesh_length_2 _spline_mesh_length_2))
  (set `local.New Mesh Count` (`self.Calculate Amount Of Meshes Needed Based On Spline Length`))
  ;[0.05098 0.05098 0.05098] Clear array if recreating
  (if (`local.Recreate`)
    (`KismetArrayLibrary.Array_Clear` (`self.Spline Mesh Components`)))
  ;[0.05098 0.05098 0.05098] Loop the amount of meshes that are needed based on the spline length
  (for _index (range (+ (`local.New Mesh Count`) 1))
    (set `local.Current Index` _index)
    ;[0.05098 0.05098 0.05098] if no spline mesh exists at the current index, create it (when mesh count is greater than the lenght of the mesh component array)
    (if (`KismetArrayLibrary.Array_IsValidIndex` (`self.Spline Mesh Components`) (`local.Current Index`))
      ;[0.05098 0.05098 0.05098] Update reference that gets used when updating the current spline mesh
      (set `self.Spline Mesh Component Reference` (`|GetArrayItem` (`self.Spline Mesh Components`) (`local.Current Index`)))
      (else
        ;[1 1 1] Add spline mesh, and set its mesh and forward axis. Also add it to the array for later references
        ;;[1 1 1] Has to be mobility to moveable
        (bind _returnvalue_5 (`AddComponent|NODE_AddSplineMeshComponent-0`))
        (bind _output_get (set `self.Spline Mesh Component Reference` _returnvalue_5))
        (`/Engine/EditorBlueprintResources/StandardMacros.IsValid` (`self.Buildable Mesh`)
          (:`Is Valid`
            _)
          (:`Is Not Valid`
            (bind _object (`/Game/Hyper/Core/Generic/BlueprintMacroLibrary/BML_AssetLoading.Load Asset Blocking Checked` (`.Mesh_149_A56D2E784235667052B95EB56B8DC96F` (break `/Game/Hyper/Core/BuildingSystem/Datamodel/Structures/Struct_Buildable_Info` (`self.Builable Struct`))))
              (:`Is Valid`
                (bind _asstatic_mesh (cast `StaticMesh` _object))
                (bind _output_get_2 (set `self.Buildable Mesh` _asstatic_mesh))))))
        (`StaticMeshComponent.SetStaticMesh` _output_get _output_get_2)
        ;;[1 1 1] Set the mesh to ghost
        (`self.Set Spline Mesh To Ghost` _returnvalue_5 (`self.Ghost_Material`))
        (`SplineMeshComponent.SetForwardAxis` _output_get (`self.Spline Mesh Forward Axis`) false)
        (`SceneComponent.K2_SetRelativeRotation` (`self.Spline Mesh Component Reference`) (`KismetMathLibrary.MakeRotator` 0.0 0.0 (+ _relativelocation_z (select `bool` (`self.Flip Rotation of Spline Mesh`) :`true` 180.0))) false false)
        (`KismetArrayLibrary.Array_AddUnique` (`self.Spline Mesh Components`) (`self.Spline Mesh Component Reference`))))
    ;[1 1 1] Set the start end end position of the spline mesh component of this index in the loop.
    (if (== (`SplineComponent.GetNumberOfSplinePoints` (`self.Spline`)) 1)
      (`SplineMeshComponent.SetStartAndEnd` (`self.Spline Mesh Component Reference`) _returnvalue_2 _returnvalue_4 (+ _returnvalue_2 (`KismetMathLibrary.MakeVector` (`self.Spline_Mesh_Length`))) _returnvalue_4 true)
      (else
        (`SplineMeshComponent.SetStartAndEnd` (`self.Spline Mesh Component Reference`) _returnvalue_2 _returnvalue_4 (`SplineComponent.GetLocationAtDistanceAlongSpline` _spline _returnvalue_3 "World") (`KismetMathLibrary.ClampVectorSize` (`SplineComponent.GetTangentAtDistanceAlongSpline` _spline _returnvalue_3 "World") _spline_mesh_length _spline_mesh_length) true)))))

(fn `Destroy Spline Mesh Component`
  (params (`Spline Mesh Component to destroy` :type "SplineMeshComponent Object Reference (by ref)"))
  (`/Engine/EditorBlueprintResources/StandardMacros.IsValid` `Spline Mesh Component to destroy`
    (:`Is Valid`
      ;[1 1 1] Check if the segment to destroy, is in this spline
      (if (`KismetArrayLibrary.Array_Contains` (`self.Spline Mesh Components`) `Spline Mesh Component to destroy`)
        ;[1 1 1] Remove the segment from the array and destroy that segment
        (`ActorComponent.K2_DestroyComponent` (`local.Spline Mesh Component to destroy`))
        ;[1 1 1] If the are no meshes anymore, destroy the complete actor
        (if (not (`KismetArrayLibrary.Array_IsValidIndex` (`self.Spline Mesh Components`)))
          (`self.K2_DestroyActor`))))))

(fn `Get Coupled buildable master to spline mesh`
  (params (`Spline mesh` :type "SplineMeshComponent Object Reference (by ref)"))
  (returns (`Coupled buildable master` :type "/Game/Hyper/BuildingSystem/Blueprints_Buildables/Masters/BP_Buildable_Advanced Object Reference"))
  (bind _coupled_buildable_master (`self.Coupled Buildable Master`))
  (bind _returnvalue (`KismetMathLibrary.FFloor` (/ (`KismetMathLibrary.Conv_IntToDouble` (`KismetArrayLibrary.Array_Find` (`self.Spline Mesh Components`) `Spline mesh`)) (`KismetMathLibrary.Conv_IntToDouble` (`self.Segment Size`)))))
  (if (`KismetArrayLibrary.Array_IsValidIndex` (`self.Spline Mesh Components`))
    (if (`KismetArrayLibrary.Array_IsValidIndex` _coupled_buildable_master _returnvalue)
      (return (`|GetArrayItem` _coupled_buildable_master _returnvalue)))))

(fn `Get Interact Animation`
  (params (`Owning Controller` :type "Controller Object Reference"))
  (returns (`Anim Montage` :type "AnimMontage Object Reference"))
  (return null))

(fn `Get Interact Sound`
  (returns (`Interact Sound` :type "SoundBase Object Reference"))
  (return null))

(fn `Get Interact Text`
  (params (`Owning Controller` :type "PlayerController Object Reference"))
  (returns (`Interact Text` :type Text) (`Secondary Interact Text` :type Text))
  (return "" ""))

(fn `Get Relative Interact Text Location`
  (returns (`Relative Location` :type "Vector Structure"))
  (return (0.0 0.0 0.0)))

(fn `IsBuildFinsihed`
  (returns (Finished :type Boolean))
  (return false))

(fn `OnRep_current Segment Index to destroy`
  (`self.Destroy Spline Mesh Component` (`|GetArrayItem` (`self.Spline Mesh Components`))))

(fn `OnRep_Current spline mesh component to destriy`)

(fn `OnRep_Destroyed spline mesh segment indexes`
  (if (not (`KismetSystemLibrary.IsServer`))
    (`self.Event: Destroy Spline Mesh Component` (`self.Destroyed spline mesh segment indexes`))))

(fn `OnRep_Segment Indexes set to build state`
  (`self.Event: Set Segment to Build State` 0 (`self.Segment Indexes set to build state`)))

(fn `OnRep_Spline Building placement is finished`
  ;[1 1 1] If it is not a server:
  ; Recreate the spline on the client by using the replicated spline point locations. It seems that in UE there is a bug that the spline is not replicated that is why we are doind this manually.
  ; First set the index 0 to the first location (otherwise it will be set at 0,0,0) since index 0 already exist there
  ; After setting the spline point locations, create the spline meshes along that spline
  (if (or (not (`KismetSystemLibrary.IsServer`)) (`KismetSystemLibrary.IsDedicatedServer`))
    (`self.Re-Create Spline based on spline point locations` (`self.spline point locations`))))

(fn `OnRep_Spline Mesh Components`)

(fn `Re-Create Spline based on spline point locations`
  (params (Array :type "Array of Vector Structure"))
  (bind _spline (`self.Spline`))
  ;[1 1 1] Recreate the spline on the by using the replicated spline point locations. It seems that in UE there is a bug that the spline is not replicated that is why we are doind this manually.
  ; First set the index 0 to the first location (otherwise it will be set at 0,0,0) since index 0 already exist there
  ; After setting the spline point locations, create the spline meshes along that spline
  (if (`KismetArrayLibrary.Array_IsValidIndex` Array)
    (for (_array_element _array_index) Array
      (if (== _array_index 0)
        (`SplineComponent.SetLocationAtSplinePoint` _spline 0 _array_element "World" true)
        (else
          (`SplineComponent.AddSplinePoint` _spline _array_element "World" true))))
    (`self.Create Spline Meshes` true)))

(fn `Return Build ID`
  (returns (`Build ID` :type Integer))
  (return 0))

(fn `Save Buildable Spline Actor`
  (locals (`local save object` :type "SaveGame Object Reference"))
  (bind _struct_saved_buildables (make `/Game/Hyper/BuildingSystem/Save/Struct_Saved_Buildables` :`Actor` (`GameplayStatics.GetObjectClass` self) :`Buildable Struct` (`self.Builable Struct`) :`Transform` (`self.GetTransform`) :`Upgrading_Struct_Buildable` (struct :`TraceChannel` "TraceTypeQuery1" :`CanbeDamaged` true :`MaximumDurability` 100.0 :`CanbeRepaired` true :`RepairFactor` 1.0 :`FinishedbuildcanbeRefurbished` true :`FinishedbuildRefurbishRate` 0.75 :`GhostBuildCanbeRefurbished` true :`Ghostbuildrefurbishrate` 1.0 :`CanbeUpgraded` true :`Upgradetothisbuilding` (struct :`DataTable` "/Script/Engine.DataTable'/Game/Hyper/Core/BuildingSystem/Datamodel/Datatables/DT_Buildables.DT_Buildables'") :`CanonlybebuildatSnappingPoint` true :`Canberotatedwhilesnapped` true :`RotationStepSizewhenSnapped` 90.0 :`Maximumacceptableangle` 25.0 :`MaxBuildHeight` 200.0 :`UseSelectedMeshinspawnedactor` true :`Tier` "NewEnumerator3" :`BuildableType` "NewEnumerator24" :`ConnectedDatatableRow` (struct) :`CanInteractText` "NSLOCTEXT(\"\", \"7549DBC54678241DBC19D985679B6DFA\", \"False\")") :`Buildable Data Table Row` (`self.Buildable Data Table Row`) :`GUID_Buildable` (`self.GUID_Buildable_Spline`) :`Spline Point Locations` (`self.spline point locations`) :`Coupled Buildables Masters to Spline GUIDS` (`self.Coupled Buildable Masters GUIDS`) :`Destroyed spline mesh segment indexes` (`self.Destroyed spline mesh segment indexes`)))
  ;[1 1 1] Ovveride to Don't save
  (if (not (`.DontSaveinBuildingsave_140_5E1F585F43283C8297F1A8B8AC19B8FD` (break `/Game/Hyper/Core/BuildingSystem/Datamodel/Structures/Struct_Buildable_Info` (`self.Builable Struct`))))
    ;[1 1 1] Check if save exist, if not create, if so load.
    (bind _returnvalue (`GameplayStatics.DoesSaveGameExist` "BuildSave"))
    (if _returnvalue
      (bind _returnvalue_2 (`GameplayStatics.LoadGameFromSlot` "BuildSave"))
      (set `local.local save object` _returnvalue_2)
      (else
        (bind _returnvalue_3 (`GameplayStatics.CreateSaveGameObject` "/Game/Hyper/BuildingSystem/Save/BP_Save_Buildings.BP_Save_Buildings_C"))
        (set `local.local save object` _returnvalue_3)))
    (bind _asbp_save_buildings (cast `/Game/Hyper/BuildingSystem/Save/BP_Save_Buildings` (`local.local save object`)))
    (bind (_array_element _found _index) (`/Game/Hyper/BuildingSystem/Save/BP_Save_Buildings.Find_Buildable` _asbp_save_buildings "/Script/Engine.Actor" (`self.GetTransform`) (`self.spline point locations`) (`self.GUID_Buildable_Spline`)))
    (if _found
      (bind _buildables (`/Game/Hyper/BuildingSystem/Save/BP_Save_Buildings.Buildables` _asbp_save_buildings))
      (`KismetArrayLibrary.Array_Set` _buildables _index _struct_saved_buildables)
      (else
        (`KismetArrayLibrary.Array_Add` _buildables _struct_saved_buildables)))
    (`GameplayStatics.SaveGameToSlot` _asbp_save_buildings "BuildSave")))

(fn `Set Spline Mesh To Ghost`
  (params (Target :type "MeshComponent Object Reference") (Material :type "MaterialInterface Object Reference"))
  (bind _target (`local.Target`))
  (bind _returnvalue (`MeshComponent.GetMaterials` (`local.Target`)))
  (bind _returnvalue_2 (`MeshComponent.GetMaterials` (`local.Target`)))
  (`/Engine/EditorBlueprintResources/StandardMacros.IsValid` Target
    (:`Is Valid`
      (bind _asstatic_mesh_component (cast `StaticMeshComponent` Target))
      ;[0.05127 0.05127 0.05127] Ghost material is glass. No translucent materials allowed on nanite
      (set `StaticMeshComponent.bDisallowNanite` true _asstatic_mesh_component)
      ;[1 1 1] Get materials so we can set it later when it is being build
      ; (From ghost material, when it is placed, but not finished)
      ;;[1 1 1] Only set finished state materials once
      (if (`KismetArrayLibrary.Array_IsEmpty` (`self.Finished_State_Materials`))
        ;[1 1 1] Save the materials of the mesh for later use
        ; Set the Materials of the mesh to the ghost material
        ; Set the collision to ignore, but make sure it is traceable for linetrace
        (if (`KismetArrayLibrary.Array_IsNotEmpty` _returnvalue)
          (set `self.Finished_State_Materials` _returnvalue)
          (if (`KismetArrayLibrary.Array_IsValidIndex` _returnvalue_2) :!label _label
            (for (_ _array_index) _returnvalue_2
              ;;[1 1 1] Set the mesh to ghost color
              (`PrimitiveComponent.SetMaterial` (`local.Target`) _array_index (`local.Material`)))
            ;;[1 1 1] Ignore all, but respond to visibility trace (So can build)
            (`PrimitiveComponent.SetCollisionResponseToAllChannels` _target "ECR_Ignore")
            (`PrimitiveComponent.SetCollisionResponseToChannel` _target "ECC_Visibility" "ECR_Block")
            (if (`self.Spline Building placement is finished`)
              (`PrimitiveComponent.SetCollisionEnabled` (`local.Target`) "QueryOnly")
              ;[0.05127 0.05127 0.05127] Set to can interact
              (`PrimitiveComponent.SetCollisionResponseToChannel` (`local.Target`) "ECC_GameTraceChannel1" "ECR_Block"))))
        (else
          (goto _label))))))

(fn `Set Spline segment to Build State`
  (params (`Spline Mesh` :type "PrimitiveComponent Object Reference"))
  (`/Engine/EditorBlueprintResources/StandardMacros.IsValid` `Spline Mesh`
    (:`Is Valid`
      (for (_array_element _array_index) (`self.Finished_State_Materials`)
        (`PrimitiveComponent.SetMaterial` `Spline Mesh` _array_index _array_element))
      (`PrimitiveComponent.SetCollisionEnabled` `Spline Mesh` "QueryAndPhysics")
      ;[1 1 1] Block all again when is build
      (`PrimitiveComponent.SetCollisionResponseToAllChannels` `Spline Mesh` "ECR_Block"))))

(fn `Set the complete spline to finished spline and couple buildable actors to the segments`
  (locals (Last_Segment_Is_Incomplete :type Boolean :default false) (Remaining_Segments_that_not_fit_in_Complete_Segment :type Integer :default 0) (Local_Array_Index :type Integer))
  (bind _local_array_index (`local.Local_Array_Index`))
  (bind _spline_mesh_components (`self.Spline Mesh Components`))
  (bind _spline (`self.Spline`))
  (bind _returnvalue (- (`KismetArrayLibrary.Array_Length` _spline_mesh_components) 1))
  (bind _returnvalue_2 (mod (+ (`local.Local_Array_Index`) 1) (`self.Segment Size`)))
  (bind _returnvalue_3 (== _returnvalue (`local.Local_Array_Index`)))
  (bind _output (`|GetArrayItem` (`self.Spline Mesh Components`) (- (`local.Local_Array_Index`) (`KismetMathLibrary.Round` (/ (`KismetMathLibrary.Conv_IntToDouble` (- (select `bool` (`local.Last_Segment_Is_Incomplete`) :`false` (`self.Segment Size`) :`true` (`local.Remaining_Segments_that_not_fit_in_Complete_Segment`)) 1)) 2.0)))))
  ;[1 1 1] Set to placement is finished
  (if (not (`self.Spline Building placement is finished`))
    ;[1 1 1] Removes the last spline point when finsihed building. This makes sure that only the latest manualt added splinepoint is placed.
    (`SplineComponent.RemoveSplinePoint` _spline (- (`SplineComponent.GetNumberOfSplinePoints` _spline) 1) true)
    (`self.Event: Update Spline`)
    ;[1 1 1] Store all locations of the spline points (on server) and replicate this array of location variables. This is used to recreate the spline on the clients
    (`self.Store Spline point locations`)
    ;[1 1 1] Set to finished and recreate the spline on the clients
    (set `self.Spline Building placement is finished` true)
    (if (`KismetArrayLibrary.Array_IsValidIndex` _spline_mesh_components)
      ;[1 1 1] For each spline mesh segment, determine where to spawn the buildable and couple it to the segments
      (for (_array_element _array_index) _spline_mesh_components
        (set `local.Local_Array_Index` _array_index)
        ;;[1 1 1] When the spline is placed, set to white ghost mesh
        (`self.Set Spline Mesh To Ghost` _array_element "/Game/Hyper/ResourcePack/Tileable_Materials/Glass/M_Glass_Inst_White.M_Glass_Inst_White")
        (if (== _returnvalue_2 0)
          (bind _returnvalue_4 (`|SpawnActorFromClass` :`Class` "/Game/Hyper/BuildingSystem/Blueprints_Buildables/Masters/BP_Buildable_Advanced.BP_Buildable_Advanced_C" :`SpawnTransform` (`KismetMathLibrary.Conv_VectorToTransform` (/ (+ (`SplineMeshComponent.GetStartPosition` _output) (`SplineMeshComponent.GetEndPosition` _output)) 2)) :`CollisionHandlingOverride` "AlwaysSpawn" :`TransformScaleMethod` "OverrideRootScale" :`Is Building Finished` false :`Password` "0000" :`Coupled Spline Master GUID` (`self.GUID_Buildable_Spline`) :`Is_Placed_In_world` true :`Buildable Data Table Row` (`self.Buildable Data Table Row`) :`Build By Player` null :`Instigator` null :!label _label))
          ;;[1 1 1] Spawn a buildable master for each segment in the spline. Add it to the list of coupled buildables
          (`KismetArrayLibrary.Array_Add` (`self.Coupled Buildable Master`) _returnvalue_4)
          ;;[1 1 1] Store coupled GUID
          (bind _output_get (`/Game/Hyper/BuildingSystem/Blueprints_Buildables/Masters/BP_Buildable_Advanced.Get GUID` _returnvalue_4))
          (`KismetArrayLibrary.Array_Add` (`self.Coupled Buildable Masters GUIDS`) _output_get)
          ;;[1 1 1] Store the coupled spline segments (and master) in the spawned buildable
          (set `/Game/Hyper/Core/BuildingSystem/Blueprints/BP_Buildable_Abstract.Coupled Spline Master` self _returnvalue_4)
          (for _index (range (- _local_array_index (- (`self.Segment Size`) 1)) (+ _local_array_index 1))
            (`KismetArrayLibrary.Array_Add` (`/Game/Hyper/Core/BuildingSystem/Blueprints/BP_Buildable_Abstract.Coupled Spline Segments` _returnvalue_4) _index))
          ;[1 1 1] This enforces to recalculate the required resourced. May also be done by expose on spawn
          (if (`local.Last_Segment_Is_Incomplete`)
            (set `/Game/Hyper/Core/BuildingSystem/Blueprints/BP_Buildable_Abstract.Resource Required Multiplier` (* (`/Game/Hyper/Core/BuildingSystem/Blueprints/BP_Buildable_Abstract.Resource Required Multiplier` _returnvalue_4) (/ (`KismetMathLibrary.Conv_IntToDouble` (`local.Remaining_Segments_that_not_fit_in_Complete_Segment`)) (`KismetMathLibrary.Conv_IntToDouble` (`self.Segment Size`)))) _returnvalue_4)
            (bind _struct_buildable (`/Game/Hyper/Core/BuildingSystem/Blueprints/BP_Buildable_Abstract.Struct Buildable` _returnvalue_4))
            (`/Game/Hyper/BuildingSystem/Blueprints_Buildables/Masters/BP_Buildable_Advanced.Calculate and set the amount of resources required to build` _returnvalue_4 _struct_buildable)
            (`/Game/Hyper/BuildingSystem/Blueprints_Buildables/Masters/BP_Buildable_Advanced.Set_Resources_Text` _returnvalue_4 _struct_buildable))
          (elif (`KismetArrayLibrary.Array_IsValidIndex` _spline_mesh_components _returnvalue)
            (if _returnvalue_3
              (set `local.Remaining_Segments_that_not_fit_in_Complete_Segment` _returnvalue_2)
              (set `local.Last_Segment_Is_Incomplete` _returnvalue_3)
              (goto _label))))))))

(fn `Should get other Actor to Interact with`
  (params (`Based on this Component` :type "PrimitiveComponent Object Reference"))
  (returns (True :type Boolean) (`Actor To Interact With` :type "Actor Object Reference"))
  ;[0.05127 0.05127 0.05127] Redirect the actor to interact with
  ; Interact with specific segment
  ; The segment is coupled with a buildable master.
  ; The buildable is the one that handles all the logic of a buildable.
  ; When we hit this segment, we want to interact with the coupled buildable master to handle resource management
  (bind _asspline_mesh_component (cast `SplineMeshComponent` `Based on this Component`))
  (bind _coupled_buildable_master (`self.Get Coupled buildable master to spline mesh` _asspline_mesh_component))
  (`/Engine/EditorBlueprintResources/StandardMacros.IsValid` _coupled_buildable_master
    (:`Is Valid`
      (return true _coupled_buildable_master))))

(fn `Should server control the interact`
  (returns (`Server should excecute interact call` :type Boolean))
  (return false))

(fn `Store Spline point locations`
  (returns (`spline point locations` :type "Array of Vector Structure"))
  (bind _spline (`self.Spline`))
  (bind _returnvalue (`SplineComponent.GetNumberOfSplinePoints` _spline))
  (if (> _returnvalue 0)
    ;[1 1 1] Store all locations of the spline points (on server) and replicate this array of location variables. This is used to recreate the spline on the clients
    (for _index (range _returnvalue)
      (`KismetArrayLibrary.Array_Add` (`self.spline point locations`) (`SplineComponent.GetLocationAtSplinePoint` _spline _index "World")))
    (return (`self.spline point locations`))))

(fn `UserConstructionScript`)