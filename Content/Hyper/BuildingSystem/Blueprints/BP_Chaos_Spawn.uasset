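; Spawns and plays the Chaos fracture destruction of a building piece, then removes itself.
; On BeginPlay it adds a Geometry Collection by Tier (thatch, wood, stone) and piece Type, hard-coded per combination because the collection can't be set dynamically.
; It registers a child anchor field, spawns a weapon-impact actor and triggers a child cluster-strain field to shatter every part.
; A delayed destroy clears the debris to protect performance.
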(event `Destroy geometry`
  (`KismetSystemLibrary.Delay` (`self.Delay before fractures are destroyed after meeting threshold`))
  (`ActorComponent.K2_DestroyComponent` (`self.GeometryCollection`))
  (`self.K2_DestroyActor` :!label _label))

(event `self.ReceiveBeginPlay`
  (bind _geometrycollection (`self.GeometryCollection`))
  ;[1 1 1] Since we can't set the geomerty dynamicly, I've added all geometries manualy untill Epic exposes it to blueprints. If someone knows a better workarround feel free to contact me
  (switch `/Game/Hyper/Core/BuildingSystem/Datamodel/Enumerations/Enum_Buildable_Tiers` (`self.Tier`)
    (:`NewEnumerator3`
      (goto _label))
    (:`NewEnumerator0`
      (switch `/Game/Hyper/Core/BuildingSystem/Datamodel/Enumerations/Enum_Buildable_Modular_Type` (`self.Type`)
        (:`NewEnumerator0`
          (bind _returnvalue (`AddComponent|NODE_AddGeometryCollectionComponent-21`))
          (set `self.GeometryCollection` _returnvalue))
        (:`NewEnumerator1`
          (bind _returnvalue_2 (`AddComponent|NODE_AddGeometryCollectionComponent-22`))
          (set `self.GeometryCollection` _returnvalue_2))
        (:`NewEnumerator2`
          (bind _returnvalue_3 (`AddComponent|NODE_AddGeometryCollectionComponent-23`))
          (set `self.GeometryCollection` _returnvalue_3))
        (:`NewEnumerator23`
          (bind _returnvalue_4 (`AddComponent|NODE_AddGeometryCollectionComponent-24`))
          (set `self.GeometryCollection` _returnvalue_4))
        (:`NewEnumerator3`
          (bind _returnvalue_5 (`AddComponent|NODE_AddGeometryCollectionComponent-25`))
          (set `self.GeometryCollection` _returnvalue_5))
        (:`NewEnumerator4`
          (bind _returnvalue_6 (`AddComponent|NODE_AddGeometryCollectionComponent-26`))
          (set `self.GeometryCollection` _returnvalue_6))
        (:`NewEnumerator5`
          (bind _returnvalue_7 (`AddComponent|NODE_AddGeometryCollectionComponent-27`))
          (set `self.GeometryCollection` _returnvalue_7))
        (:`NewEnumerator6`
          (bind _returnvalue_8 (`AddComponent|NODE_AddGeometryCollectionComponent-28`))
          (set `self.GeometryCollection` _returnvalue_8))
        (:`NewEnumerator7`
          (bind _returnvalue_9 (`AddComponent|NODE_AddGeometryCollectionComponent-29`))
          (set `self.GeometryCollection` _returnvalue_9))
        (:`NewEnumerator8`
          (bind _returnvalue_10 (`AddComponent|NODE_AddGeometryCollectionComponent-30`))
          (set `self.GeometryCollection` _returnvalue_10))
        (:`NewEnumerator9`
          (bind _returnvalue_11 (`AddComponent|NODE_AddGeometryCollectionComponent-31`))
          (set `self.GeometryCollection` _returnvalue_11))
        (:`NewEnumerator10`
          (bind _returnvalue_12 (`AddComponent|NODE_AddGeometryCollectionComponent-32`))
          (set `self.GeometryCollection` _returnvalue_12))
        (:`NewEnumerator11`
          (bind _returnvalue_13 (`AddComponent|NODE_AddGeometryCollectionComponent-33`))
          (set `self.GeometryCollection` _returnvalue_13))
        (:`NewEnumerator12`
          (bind _returnvalue_14 (`AddComponent|NODE_AddGeometryCollectionComponent-34`))
          (set `self.GeometryCollection` _returnvalue_14))
        (:`NewEnumerator13`
          (bind _returnvalue_15 (`AddComponent|NODE_AddGeometryCollectionComponent-35`))
          (set `self.GeometryCollection` _returnvalue_15))
        (:`NewEnumerator14`
          (bind _returnvalue_16 (`AddComponent|NODE_AddGeometryCollectionComponent-36`))
          (set `self.GeometryCollection` _returnvalue_16))
        (:`NewEnumerator15`
          (bind _returnvalue_17 (`AddComponent|NODE_AddGeometryCollectionComponent-37`))
          (set `self.GeometryCollection` _returnvalue_17))
        (:`NewEnumerator16`
          (bind _returnvalue_18 (`AddComponent|NODE_AddGeometryCollectionComponent-38`))
          (set `self.GeometryCollection` _returnvalue_18))
        (:`NewEnumerator17`
          (bind _returnvalue_19 (`AddComponent|NODE_AddGeometryCollectionComponent-39`))
          (set `self.GeometryCollection` _returnvalue_19))
        (:`NewEnumerator18`
          (bind _returnvalue_20 (`AddComponent|NODE_AddGeometryCollectionComponent-40`))
          (set `self.GeometryCollection` _returnvalue_20))))
    (:`NewEnumerator1`
      (switch `/Game/Hyper/Core/BuildingSystem/Datamodel/Enumerations/Enum_Buildable_Modular_Type` (`self.Type`)
        (:`NewEnumerator0`
          (bind _returnvalue_21 (`AddComponent|NODE_AddGeometryCollectionComponent-41`))
          (set `self.GeometryCollection` _returnvalue_21))
        (:`NewEnumerator1`
          (bind _returnvalue_22 (`AddComponent|NODE_AddGeometryCollectionComponent-42`))
          (set `self.GeometryCollection` _returnvalue_22))
        (:`NewEnumerator2`
          (bind _returnvalue_23 (`AddComponent|NODE_AddGeometryCollectionComponent-43`))
          (set `self.GeometryCollection` _returnvalue_23))
        (:`NewEnumerator23`
          (bind _returnvalue_24 (`AddComponent|NODE_AddGeometryCollectionComponent-44`))
          (set `self.GeometryCollection` _returnvalue_24))
        (:`NewEnumerator3`
          (bind _returnvalue_25 (`AddComponent|NODE_AddGeometryCollectionComponent-45`))
          (set `self.GeometryCollection` _returnvalue_25))
        (:`NewEnumerator4`
          (bind _returnvalue_26 (`AddComponent|NODE_AddGeometryCollectionComponent-46`))
          (set `self.GeometryCollection` _returnvalue_26))
        (:`NewEnumerator5`
          (bind _returnvalue_27 (`AddComponent|NODE_AddGeometryCollectionComponent-47`))
          (set `self.GeometryCollection` _returnvalue_27))
        (:`NewEnumerator6`
          (bind _returnvalue_28 (`AddComponent|NODE_AddGeometryCollectionComponent-48`))
          (set `self.GeometryCollection` _returnvalue_28))
        (:`NewEnumerator7`
          (bind _returnvalue_29 (`AddComponent|NODE_AddGeometryCollectionComponent-49`))
          (set `self.GeometryCollection` _returnvalue_29))
        (:`NewEnumerator8`
          (bind _returnvalue_30 (`AddComponent|NODE_AddGeometryCollectionComponent-50`))
          (set `self.GeometryCollection` _returnvalue_30))
        (:`NewEnumerator9`
          (bind _returnvalue_31 (`AddComponent|NODE_AddGeometryCollectionComponent-51`))
          (set `self.GeometryCollection` _returnvalue_31))
        (:`NewEnumerator10`
          (bind _returnvalue_32 (`AddComponent|NODE_AddGeometryCollectionComponent-52`))
          (set `self.GeometryCollection` _returnvalue_32))
        (:`NewEnumerator11`
          (bind _returnvalue_33 (`AddComponent|NODE_AddGeometryCollectionComponent-53`))
          (set `self.GeometryCollection` _returnvalue_33))
        (:`NewEnumerator12`
          (bind _returnvalue_34 (`AddComponent|NODE_AddGeometryCollectionComponent-54`))
          (set `self.GeometryCollection` _returnvalue_34))
        (:`NewEnumerator13`
          (bind _returnvalue_35 (`AddComponent|NODE_AddGeometryCollectionComponent-55`))
          (set `self.GeometryCollection` _returnvalue_35))
        (:`NewEnumerator14`
          (bind _returnvalue_36 (`AddComponent|NODE_AddGeometryCollectionComponent-56`))
          (set `self.GeometryCollection` _returnvalue_36))
        (:`NewEnumerator15`
          (bind _returnvalue_37 (`AddComponent|NODE_AddGeometryCollectionComponent-57`))
          (set `self.GeometryCollection` _returnvalue_37))
        (:`NewEnumerator16`
          (bind _returnvalue_38 (`AddComponent|NODE_AddGeometryCollectionComponent-58`))
          (set `self.GeometryCollection` _returnvalue_38))
        (:`NewEnumerator17`
          (bind _returnvalue_39 (`AddComponent|NODE_AddGeometryCollectionComponent-59`))
          (set `self.GeometryCollection` _returnvalue_39))
        (:`NewEnumerator18`
          (bind _returnvalue_40 (`AddComponent|NODE_AddGeometryCollectionComponent-60`))
          (set `self.GeometryCollection` _returnvalue_40))
        (:`NewEnumerator20`
          (bind _returnvalue_41 (`AddComponent|NODE_AddGeometryCollectionComponent-61`))
          (set `self.GeometryCollection` _returnvalue_41))
        (:`NewEnumerator21`
          (bind _returnvalue_42 (`AddComponent|NODE_AddGeometryCollectionComponent-63`))
          (set `self.GeometryCollection` _returnvalue_42))
        (:`NewEnumerator22`
          (bind _returnvalue_43 (`AddComponent|NODE_AddGeometryCollectionComponent-62`))
          (set `self.GeometryCollection` _returnvalue_43))))
    (:`NewEnumerator2`
      (switch `/Game/Hyper/Core/BuildingSystem/Datamodel/Enumerations/Enum_Buildable_Modular_Type` (`self.Type`)
        (:`NewEnumerator0`
          (bind _returnvalue_44 (`AddComponent|NODE_AddGeometryCollectionComponent-84`))
          (set `self.GeometryCollection` _returnvalue_44))
        (:`NewEnumerator1`
          (bind _returnvalue_45 (`AddComponent|NODE_AddGeometryCollectionComponent-85`))
          (set `self.GeometryCollection` _returnvalue_45))
        (:`NewEnumerator2`
          (bind _returnvalue_46 (`AddComponent|NODE_AddGeometryCollectionComponent-86`))
          (set `self.GeometryCollection` _returnvalue_46))
        (:`NewEnumerator23`
          (bind _returnvalue_47 (`AddComponent|NODE_AddGeometryCollectionComponent-87`))
          (set `self.GeometryCollection` _returnvalue_47))
        (:`NewEnumerator3`
          (bind _returnvalue_48 (`AddComponent|NODE_AddGeometryCollectionComponent-88`))
          (set `self.GeometryCollection` _returnvalue_48))
        (:`NewEnumerator4`
          (bind _returnvalue_49 (`AddComponent|NODE_AddGeometryCollectionComponent-89`))
          (set `self.GeometryCollection` _returnvalue_49))
        (:`NewEnumerator5`
          (bind _returnvalue_50 (`AddComponent|NODE_AddGeometryCollectionComponent-90`))
          (set `self.GeometryCollection` _returnvalue_50))
        (:`NewEnumerator6`
          (bind _returnvalue_51 (`AddComponent|NODE_AddGeometryCollectionComponent-91`))
          (set `self.GeometryCollection` _returnvalue_51))
        (:`NewEnumerator7`
          (bind _returnvalue_52 (`AddComponent|NODE_AddGeometryCollectionComponent-92`))
          (set `self.GeometryCollection` _returnvalue_52))
        (:`NewEnumerator8`
          (bind _returnvalue_53 (`AddComponent|NODE_AddGeometryCollectionComponent-93`))
          (set `self.GeometryCollection` _returnvalue_53))
        (:`NewEnumerator9`
          (bind _returnvalue_54 (`AddComponent|NODE_AddGeometryCollectionComponent-94`))
          (set `self.GeometryCollection` _returnvalue_54))
        (:`NewEnumerator10`
          (bind _returnvalue_55 (`AddComponent|NODE_AddGeometryCollectionComponent-95`))
          (set `self.GeometryCollection` _returnvalue_55))
        (:`NewEnumerator11`
          (bind _returnvalue_56 (`AddComponent|NODE_AddGeometryCollectionComponent-96`))
          (set `self.GeometryCollection` _returnvalue_56))
        (:`NewEnumerator12`
          (bind _returnvalue_57 (`AddComponent|NODE_AddGeometryCollectionComponent-97`))
          (set `self.GeometryCollection` _returnvalue_57))
        (:`NewEnumerator13`
          (bind _returnvalue_58 (`AddComponent|NODE_AddGeometryCollectionComponent-98`))
          (set `self.GeometryCollection` _returnvalue_58))
        (:`NewEnumerator14`
          (bind _returnvalue_59 (`AddComponent|NODE_AddGeometryCollectionComponent-99`))
          (set `self.GeometryCollection` _returnvalue_59))
        (:`NewEnumerator15`
          (bind _returnvalue_60 (`AddComponent|NODE_AddGeometryCollectionComponent-100`))
          (set `self.GeometryCollection` _returnvalue_60))
        (:`NewEnumerator16`
          (bind _returnvalue_61 (`AddComponent|NODE_AddGeometryCollectionComponent-101`))
          (set `self.GeometryCollection` _returnvalue_61))
        (:`NewEnumerator17`
          (bind _returnvalue_62 (`AddComponent|NODE_AddGeometryCollectionComponent-102`))
          (set `self.GeometryCollection` _returnvalue_62))
        (:`NewEnumerator18`
          (bind _returnvalue_63 (`AddComponent|NODE_AddGeometryCollectionComponent-103`))
          (set `self.GeometryCollection` _returnvalue_63)))))
  ;[1 1 1] When spawning the object dynamicly, the construction script does not seem to be excecuted properly and the anchor does not work. The geometry will move unless it is static. So we made the geometry static by default, and make it dynamic on begin play
  ;;[1 1 1] Add the Anchorfield to the initialization field of the Chaos Gemeometry Collection. This makes sure it is "Anchored" and does not fall, etc.
  (bind _asfield_system_actor (cast `FieldSystemActor` (`ChildActorComponent.ChildActor` (`self.BP_Chaos_AnchorField`))))
  (`KismetArrayLibrary.Array_Add` (`GeometryCollectionComponent.InitializationFields` _geometrycollection) _asfield_system_actor)
  ;[1 1 1] Make sure it is not hidden, is vsible and is active
  (`SceneComponent.SetHiddenInGame` _geometrycollection false false)
  (`SceneComponent.SetVisibility` _geometrycollection true false)
  (`ActorComponent.SetActive` _geometrycollection true false)
  ;[1 1 1] Damage Impact
  (`|SpawnActorFromClass` "/Game/Hyper/ResourcePack/Chaos/BP_Chaos_WeaponImpact.BP_Chaos_WeaponImpact_C" (`self.GetTransform`) "AlwaysSpawn" "MultiplyWithRoot" null 45000.0 4.0 true null)
  ;[1 1 1] This actor is a clusterstrainfield. This makes sure to destory ALL the components which gives a nice effect and cleans up all parts
  (bind _asbp_chaos_cluster_strain_field (cast `/Game/Hyper/ResourcePack/Chaos/BP_Chaos_ClusterStrainField` (`ChildActorComponent.ChildActor` (`self.BP_Chaos_ClusterStrainField`))))
  (`/Game/Hyper/ResourcePack/Chaos/BP_Chaos_ClusterStrainField.Activate Clusterstrainfield` _asbp_chaos_cluster_strain_field)
  (`KismetSystemLibrary.Delay` (`self.Delay before fractures are destroyed after meeting threshold`))
  (`self.K2_DestroyActor`))

(fn `UserConstructionScript`)