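; Base equipment actor for melee weapons and farming tools, configured by WeaponInfo.
; BeginPlay requests async loads of animations, meshes and damage types, then sets the mesh and default fire mode.
; Primary input switches on equipment type into light melee or farming actions; secondary switches are empty.
; Melee plays multicast montages with optional duration-matched play rate, while a polling timer re-enables root-motion rotation and opens the next combo at set playback percentages.
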(event `self.ReceiveBeginPlay`
  (bind ((`VisualAmmoActor_101_C121E28544B30095D45AAB89E7CC0568` _visualammoactor) (`AnimationLayertouse_114_F0B7F268487A71A0B99A82B4D4D5B8DF` _animationlayertouse) (`StaticMesh_94_E994802D45EA27F3D460D5944D8A3C63` _staticmesh) (`UsesSkeletalMesh_23_49F0D3AE4D41EFEC6341DDB41F39EB8B` _usesskeletalmesh) (`SkeletalMesh_100_BBEFA81F47EA9FA57E336FA954BE288A` _skeletalmesh)) (break `/Game/Hyper/Core/Equipment_Manager/Datamodel/Structures/Sub_Structs/Struct_CombatAttributes_Equip` (`.Equip_2_81FA71E840D3624FE8414082BDC1BC0C` (break `/Game/Hyper/Core/Equipment_Manager/Datamodel/Structures/Main_Structs/Struct_Equipment` (`self.Weapon_Info`)))))
  (bind (_damagetype _usesecondairydamagetypeforheavyattack _secondairydamagetype) (break `/Game/Hyper/Core/Equipment_Manager/Datamodel/Structures/Sub_Structs/Struct_Combat_Attributes_Damage_Types` (`.DamageTypes_54_C61AE785415D03E88392F695F1081AD5` (break `/Game/Hyper/Core/Equipment_Manager/Datamodel/Structures/Main_Structs/Struct_Equipment` (`self.Weapon_Info`)))))
  (bind ((`HasMelee_2_03899E8046469B45BE3E318D709F2701` _hasmelee) (`LightAttacks_13_8DD8C46A442BF24F97899D847DC4C733` _lightattacks) (`HeavyAttacks_16_B7FAB5854A9324F14361D5A1FA4C2D6B` _heavyattacks)) (break `/Game/Hyper/Core/Equipment_Manager/Datamodel/Structures/Sub_Structs/Struct_CombatAttributes_Melee` (`.Melee_11_2D18FAC1420140F3EC39B68B3B62B313` (break `/Game/Hyper/Core/Equipment_Manager/Datamodel/Structures/Main_Structs/Struct_Equipment` (`self.Weapon_Info`)))))
  (if _hasmelee
    (for _array_element _lightattacks
      (`/Game/Hyper/Core/Generic/BlueprintMacroLibrary/BML_AssetLoading.Async Load Asset Checked` (`.Animation_26_ACD52F5E43D3AAEC234150B43A6C2DE1` (break `/Game/Hyper/Core/Equipment_Manager/Datamodel/Structures/Sub_Structs/Struct_Melee_Combo_Instance` _array_element))))
    (for _array_element_2 _heavyattacks
      (`/Game/Hyper/Core/Generic/BlueprintMacroLibrary/BML_AssetLoading.Async Load Asset Checked` (`.Animation_26_ACD52F5E43D3AAEC234150B43A6C2DE1` (break `/Game/Hyper/Core/Equipment_Manager/Datamodel/Structures/Sub_Structs/Struct_Melee_Combo_Instance` _array_element_2)))))
  (if _usesskeletalmesh
    (bind _object (`/Game/Hyper/Core/Generic/BlueprintMacroLibrary/BML_AssetLoading.Async Load Asset Checked` _skeletalmesh)
      (:`Completed`
        (bind _asskeletal_mesh (cast `SkeletalMesh` _object))
        (set `self.Equipment Skel Mesh` _asskeletal_mesh)))
    (else
      (bind _object_2 (`/Game/Hyper/Core/Generic/BlueprintMacroLibrary/BML_AssetLoading.Async Load Asset Checked` _staticmesh)
        (:`Completed`
          (bind _asstatic_mesh (cast `StaticMesh` _object_2))
          (set `self.Equipment Mesh` _asstatic_mesh)))))
  (`|ExecutionSequence`
    (:`then_0`
      (`/Game/Hyper/Core/Generic/BlueprintMacroLibrary/BML_AssetLoading.Async Load Class Asset Checked` _damagetype
        (:`then`
          (if _usesecondairydamagetypeforheavyattack
            (`/Game/Hyper/Core/Generic/BlueprintMacroLibrary/BML_AssetLoading.Async Load Class Asset Checked` _secondairydamagetype)))))
    (:`then_1`
      (`self.Initialize Weapon`))))

(event `self.Event: Switch Visibility of weapon`
  (params (bNewVisibility :type Boolean))
  ;[0.05127 0.05127 0.05127] Switch visibility of weapon
  (`SceneComponent.SetVisibility` (`self.StaticMesh`) bNewVisibility false)
  (`SceneComponent.SetVisibility` (`self.SkeletalMesh`) bNewVisibility false))

(event `self.Event: Try Primary Input`
  (bind _equipment (`/Game/Hyper/Core/Equipment_Manager/BlueprintMacroLibrary/BML_Equipment_Actor.Get Equipment Manager`))
  ;[0.05127 0.05127 0.05127] Primary
  (switch `/Game/Hyper/Core/Equipment_Manager/Datamodel/Enumerations/Enum_Equipment_Type` (`.EquipmentType_3_705F99114DCF7C5CF212D1B88F42334C` (break `/Game/Hyper/Core/Equipment_Manager/Datamodel/Structures/Sub_Structs/Struct_Combat_Attributes_Generic` (`.Generic_41_F38D1B334B6B5DEFCF41708F1350F138` (break `/Game/Hyper/Core/Equipment_Manager/Datamodel/Structures/Main_Structs/Struct_Equipment` (`self.Weapon_Info`)))))
    (:`NewEnumerator0`
      (`self.Event: Try Melee` "NewEnumerator0" :!label _label))
    (:`NewEnumerator1`
      (goto _label))
    (:`NewEnumerator17`
      (goto _label))
    (:`NewEnumerator6`
      (goto _label))
    (:`NewEnumerator2`
      (goto _label))
    (:`NewEnumerator21`
      (goto _label))
    (:`NewEnumerator22`
      (goto _label))
    (:`NewEnumerator16`
      (goto _label))
    (:`NewEnumerator4`
      (goto _label))
    (:`NewEnumerator5`
      (goto _label))
    (:`NewEnumerator12`
      (goto _label))
    (:`NewEnumerator23`
      (goto _label))
    (:`NewEnumerator25`
      (`/Game/Hyper/Core/Equipment_Manager/Blueprints/AC_Equipment_Manager_Abstract.Try Add Water` _equipment)
      (`/Game/Hyper/Core/ReplicationSubSystem/Blueprints/AC_Replication_Abstract.Initialize Multicast Latent Montage` :`self` (`/Game/Hyper/Core/ReplicationSubSystem/BlueprintMacroLibrary/BML_Replication_Actor.Get Replication`) :`Montage To Play` "/Game/Hyper/Locomotion/Chars/Mannequin_UE5/Anims/Actions/Grab/Anim_grab_item_mirrored_Montage.Anim_grab_item_mirrored_Montage" :!label _label_2))
    (:`NewEnumerator26`
      (`/Game/Hyper/Core/Equipment_Manager/Blueprints/AC_Equipment_Manager_Abstract.Try Add Fertilizer` _equipment)
      (goto _label_2))
    (:`NewEnumerator27`
      (`/Game/Hyper/Core/Equipment_Manager/Blueprints/AC_Equipment_Manager_Abstract.Try Cure Plant` _equipment)
      (goto _label_2))))

(event `self.Event: Try Secondary Input`
  (switch `/Game/Hyper/Core/Equipment_Manager/Datamodel/Enumerations/Enum_Equipment_Type` (`.EquipmentType_3_705F99114DCF7C5CF212D1B88F42334C` (break `/Game/Hyper/Core/Equipment_Manager/Datamodel/Structures/Sub_Structs/Struct_Combat_Attributes_Generic` (`.Generic_41_F38D1B334B6B5DEFCF41708F1350F138` (break `/Game/Hyper/Core/Equipment_Manager/Datamodel/Structures/Main_Structs/Struct_Equipment` (`self.Weapon_Info`)))))))

(event `self.Event: Stop Secondary Input`
  (switch `/Game/Hyper/Core/Equipment_Manager/Datamodel/Enumerations/Enum_Equipment_Type` (`.EquipmentType_3_705F99114DCF7C5CF212D1B88F42334C` (break `/Game/Hyper/Core/Equipment_Manager/Datamodel/Structures/Sub_Structs/Struct_Combat_Attributes_Generic` (`.Generic_41_F38D1B334B6B5DEFCF41708F1350F138` (break `/Game/Hyper/Core/Equipment_Manager/Datamodel/Structures/Main_Structs/Struct_Equipment` (`self.Weapon_Info`)))))))

(event `Event: Try Melee`
  (params (`Attack Type` :type "/Game/Hyper/Core/Equipment_Manager/Datamodel/Enumerations/Enum_Melee_Attack_Types Enum" :default "NewEnumerator0"))
  (bind (_component _is_valid) (`/Game/Hyper/Core/CombatSystem/BlueprintMacroLibrary/BML_Combat_Actor.Get Combat Manager`))
  (bind _component_2 (`/Game/Hyper/Core/ReplicationSubSystem/BlueprintMacroLibrary/BML_Replication_Actor.Get Replication`))
  (bind (_component_3 _is_valid_2) (`/Game/Hyper/Core/ReplicationSubSystem/BlueprintMacroLibrary/BML_Replication_Actor.Get Replication`))
  (bind _combo_check_timer (`self.Combo check Timer`))
  (bind ((`LightAttacks_13_8DD8C46A442BF24F97899D847DC4C733` _lightattacks) (`HeavyAttacks_16_B7FAB5854A9324F14361D5A1FA4C2D6B` _heavyattacks)) (break `/Game/Hyper/Core/Equipment_Manager/Datamodel/Structures/Sub_Structs/Struct_CombatAttributes_Melee` (`.Melee_11_2D18FAC1420140F3EC39B68B3B62B313` (break `/Game/Hyper/Core/Equipment_Manager/Datamodel/Structures/Main_Structs/Struct_Equipment` (`self.Weapon_Info`)))))
  (bind _returnvalue (select `/Game/Hyper/Core/Equipment_Manager/Datamodel/Enumerations/Enum_Melee_Attack_Types` `Attack Type` :`NewEnumerator0` _lightattacks :`NewEnumerator1` _heavyattacks))
  (bind ((`Animation_26_ACD52F5E43D3AAEC234150B43A6C2DE1` _animation) (`UseTimebetweenattackinsteadofanimationTime_25_56FDEDD6417925A6F30160AF19D449DB` _usetimebetweenattackinsteadofanimationtime) (`Timebetweenattack_9_D22D133843EA21CDE41C8FA5F6B840EC` _timebetweenattack)) (break `/Game/Hyper/Core/Equipment_Manager/Datamodel/Structures/Sub_Structs/Struct_Melee_Combo_Instance` (`|GetArrayItem` _returnvalue (`self.Combo Selection Index`))))
  (bind _output (`|ConvertAsset` _animation))
  ;[0.05127 0.05127 0.05127] Melee: Light and Heavy Attacks
  ;;[0.05127 0.05127 0.05127] Check if combo montage can already be played
  (if (`self.Can Play Combat Montage`)
    ;;[0.05127 0.05127 0.05127] If the index is not valid, use the last index
    (if (not (`KismetArrayLibrary.Array_IsValidIndex` _returnvalue (`self.Combo Selection Index`)))
      (set `self.Combo Selection Index` 0))
    ;;[0.05127 0.05127 0.05127] It can be that there is no attack sset, so only excecute if it is set
    (if (`KismetArrayLibrary.Array_IsValidIndex` _returnvalue (`self.Combo Selection Index`))
      ;;[0.05127 0.05127 0.05127] Lock the montage so it cannot play another combo
      (set `self.Can Play Combat Montage` false)
      ;;[0.05127 0.05127 0.05127] Add combo's played
      (`/Engine/EditorBlueprintResources/StandardMacros.IncrementInt` (`self.Combos played in a row`)
        (:`  `
          ;;[0.05127 0.05127 0.05127] Play montage
          (if _is_valid_2
            (`/Game/Hyper/Core/ReplicationSubSystem/Blueprints/AC_Replication_Abstract.Initialize Multicast Latent Montage` _component_3 _output (`|MakeArray` "None" :!type "Name") true null (select `bool` (not _usetimebetweenattackinsteadofanimationtime) :`false` (/ (`AnimationAsset.GetPlayLength` _output) _timebetweenattack) :`true` 1.0 :!type "Float (single-precision)"))
            (`/Game/Hyper/Core/Locomotion/Blueprints/AC_Extended_Movement_Abstract.Server Allow Physics Rotation During Anim Root Motion` (`/Game/Hyper/Core/Locomotion/BlueprintMacroLibrary/Generic/BML_ExtendedMovement_Actor.Get ExtendedMovement`) false)
            ;;[0.05127 0.05127 0.05127] If timer already exists, unpause it
            ;; Otherwise initialize it
            (set `self.Is_Attacking` true)
            ;;;[0.05127 0.05127 0.05127] When attacking, don't block
            (if _is_valid
              (`/Game/Hyper/Core/CombatSystem/Blueprints/AC_Combat_Abstract.Event: Try stop Blocking` _component))
            (if (`KismetSystemLibrary.K2_IsValidTimerHandle` _combo_check_timer)
              (`KismetSystemLibrary.K2_UnPauseTimerHandle` _combo_check_timer)
              (else
                (bind _returnvalue_2 (`KismetSystemLibrary.K2_SetTimerDelegate` (delegate `Check if next combo can be played`) 0.02 true))
                (set `self.Combo check Timer` _returnvalue_2)))
            ;;[0.05127 0.05127 0.05127] If the montage is intertupted or finished, also set to can play combat montage true
            ;; and set the combo index to 0 so it resets the combo
            (add `/Game/Hyper/Core/ReplicationSubSystem/Blueprints/AC_Replication_Abstract.Montage Finished` _component_2 (delegate `Montage Finished_Event_0`))
            (add `/Game/Hyper/Core/ReplicationSubSystem/Blueprints/AC_Replication_Abstract.Montage Interupted` _component_2 (delegate `Montage Interupted_Event_0`)))))
      (else
        (`KismetSystemLibrary.PrintString` "Trying to excectute heavy or light melee attack but none assigned." false)))))

(event `Montage Finished_Event_0`
  ;[0.05127 0.05127 0.05127] Melee: Light and Heavy Attacks
  ;;[0.05127 0.05127 0.05127] If the montage is intertupted or finished, also set to can play combat montage true
  ;; and set the combo index to 0 so it resets the combo
  (set `self.Can Play Combat Montage` true)
  (set `self.Combo Selection Index` 0)
  (set `self.Combos played in a row` 0)
  (set `self.Is_Attacking` false))

(event `Montage Interupted_Event_0`
  ;[0.05127 0.05127 0.05127] Melee: Light and Heavy Attacks
  ;;[0.05127 0.05127 0.05127] If the montage is intertupted or finished, also set to can play combat montage true
  ;; and set the combo index to 0 so it resets the combo
)

(event `Check if next combo can be played`
  (bind ((`LightAttacks_13_8DD8C46A442BF24F97899D847DC4C733` _lightattacks) (`HeavyAttacks_16_B7FAB5854A9324F14361D5A1FA4C2D6B` _heavyattacks)) (break `/Game/Hyper/Core/Equipment_Manager/Datamodel/Structures/Sub_Structs/Struct_CombatAttributes_Melee` (`.Melee_11_2D18FAC1420140F3EC39B68B3B62B313` (break `/Game/Hyper/Core/Equipment_Manager/Datamodel/Structures/Main_Structs/Struct_Equipment` (`self.Weapon_Info`)))))
  ;[0.05127 0.05127 0.05127] Melee: Light and Heavy Attacks
  ;;[0.05127 0.05127 0.05127] Check if any montage is playing
  ;;;[0.05127 0.05127 0.05127] If not, pause timer
  (if (`AnimInstance.IsAnyMontagePlaying` (`/Game/Hyper/Core/Generic/BlueprintMacroLibrary/BML_Generic_Actor.Get Anim Instance`))
    ;;[0.05127 0.05127 0.05127] If montage is playing, get the montage
    (bind _current_active_montage (`/Game/Hyper/Core/ReplicationSubSystem/Blueprints/AC_Replication_Abstract.Current Active Montage` (`/Game/Hyper/Core/ReplicationSubSystem/BlueprintMacroLibrary/BML_Replication_Actor.Get Replication`))
      (:`then`
        (bind _returnvalue (/ (`AnimInstance.Montage_GetPosition` (`/Game/Hyper/Core/Generic/BlueprintMacroLibrary/BML_Generic_Actor.Get Anim Instance`) _current_active_montage) (`AnimationAsset.GetPlayLength` _current_active_montage)))
        (bind ((`Animation_26_ACD52F5E43D3AAEC234150B43A6C2DE1` _animation) (`PercentageRequiredtobeplayedbeforebeingabletostartnextattack_5_D0FF057F4423D2FDCB61499448769A7E` _percentagerequiredtobeplayedbeforebeingabletostartnextattack)) (break `/Game/Hyper/Core/Equipment_Manager/Datamodel/Structures/Sub_Structs/Struct_Melee_Combo_Instance` (`|GetArrayItem` (select `/Game/Hyper/Core/Equipment_Manager/Datamodel/Enumerations/Enum_Melee_Attack_Types` (stale `Event: Try Melee` `Attack Type`) :`NewEnumerator0` _lightattacks :`NewEnumerator1` _heavyattacks) (`self.Combo Selection Index`))))
        ;[0.05127 0.05127 0.05127] If the next combo montage can be played minus 15%, enable root motion rotation
        (if (> _returnvalue (- _percentagerequiredtobeplayedbeforebeingabletostartnextattack (`self.Percentage before next montage is played to allow root motion rotation`)))
          (`|ExecutionSequence`
            (:`then_0`
              (`/Engine/EditorBlueprintResources/StandardMacros.DoOnce` false :!label _label
                (:`Completed`
                  (`/Game/Hyper/Core/Locomotion/Blueprints/AC_Extended_Movement_Abstract.Server Allow Physics Rotation During Anim Root Motion` (`/Game/Hyper/Core/Locomotion/BlueprintMacroLibrary/Generic/BML_ExtendedMovement_Actor.Get ExtendedMovement`) true))))
            (:`then_1`
              ;[0.05127 0.05127 0.05127] Has reached the required amount of the animation to be finished playing before being able to try next attack?
              (if (> _returnvalue _percentagerequiredtobeplayedbeforebeingabletostartnextattack)
                (`|ExecutionSequence`
                  (:`then_0`
                    (set `self.Is_Attacking` false)
                    (`KismetSystemLibrary.K2_PauseTimerHandle` (`self.Combo check Timer`))
                    ;[0.05127 0.05127 0.05127] Can play next combo
                    (set `self.Can Play Combat Montage` true)
                    (`/Engine/EditorBlueprintResources/StandardMacros.IncrementInt` (`self.Combo Selection Index`)))
                  (:`then_1`
                    (goto _label :!via `Reset`))))))))
      (:`else`))
    (else
      (`KismetSystemLibrary.K2_PauseTimerHandle` (`self.Combo check Timer`)))))

(fn `Initialize Weapon`
  (bind ((`IsRanged_47_03899E8046469B45BE3E318D709F2701` _isranged) (`FireAnimation_52_5E858D6348CA64C80E8538AE13279B6B` _fireanimation) (`Requireaimingtofire_38_9DF987AB413C039FE7AC929547DD36CA` _requireaimingtofire) (`Fireeffect_51_FDB6FEB24FE41FC27EE2FEA0609C5563` _fireeffect) (`Animationinequippedmesh_53_CD1823544ED7AA6C99EFAB82FE4620DF` _animationinequippedmesh) (`AcceptedFireModes_36_63E056FF4A19331802F9D79ED9668040` _acceptedfiremodes)) (break `/Game/Hyper/Core/Equipment_Manager/Datamodel/Structures/Sub_Structs/Struct_CombatAttributes_Ranged` (`.Ranged_17_32881AE6486E69C26C2C808512B0A238` (break `/Game/Hyper/Core/Equipment_Manager/Datamodel/Structures/Main_Structs/Struct_Equipment` (`self.Weapon_Info`)))))
  (`|ExecutionSequence`
    (:`then_0`
      ;[0.05127 0.05127 0.05127] Switch on skeletal or static mesh
      (if (`.UsesSkeletalMesh_23_49F0D3AE4D41EFEC6341DDB41F39EB8B` (break `/Game/Hyper/Core/Equipment_Manager/Datamodel/Structures/Sub_Structs/Struct_CombatAttributes_Equip` (`.Equip_2_81FA71E840D3624FE8414082BDC1BC0C` (break `/Game/Hyper/Core/Equipment_Manager/Datamodel/Structures/Main_Structs/Struct_Equipment` (`self.Weapon_Info`)))))
        (`SkinnedMeshComponent.SetSkinnedAssetAndUpdate` (`self.SkeletalMesh`) (`self.Equipment Skel Mesh`) true)
        (else
          (`StaticMeshComponent.SetStaticMesh` (`self.StaticMesh`) (`self.Equipment Mesh`)))))
    (:`then_1`
      ;[0.05127 0.05127 0.05127] Set the firemode to the first available.
      (if (`KismetArrayLibrary.Array_IsValidIndex` _acceptedfiremodes)
        (set `self.Active_Fire_Mode` (`|GetArrayItem` _acceptedfiremodes))))))

(fn `UserConstructionScript`
  (`parent.UserConstructionScript`))