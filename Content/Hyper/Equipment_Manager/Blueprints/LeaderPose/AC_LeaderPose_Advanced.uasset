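; Equipment component that drives a modular character's head, torso, hands, legs and feet meshes from the main mesh via leader pose.
; When the split-mesh flag is set, setup overrides main mesh materials with M_Full_Opacity, links parts fetched through an interface, copies the anim class and caches default meshes.
; Swapping synchronously loads the inventory item's skeletal mesh onto the slot's part, restoring the default when invalid or reset.
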(fn `Set Leader Pose Component`
  (bind _mesh (`/Game/Hyper/Core/Generic/BlueprintMacroLibrary/BML_Generic_Component.Get Character Mesh`))
  ;[0.05127 0.05127 0.05127] If the mesh is splitted into several skeletal meshes, set the boolean to true and it will automatically set the master pose component
  (if (`self.Mesh is splitted in skeletal meshes`)
    ;[0.05127 0.05127 0.05127] Set the mesh to full opacity
    (for (_ _array_index) (`MeshComponent.GetMaterials` _mesh)
      (`PrimitiveComponent.SetMaterial` _mesh _array_index "/Game/Hyper/ResourcePack/Tileable_Materials/Plain_Color/M_Full_Opacity.M_Full_Opacity"))
    ;[0.05127 0.05127 0.05127] Set all skeletal mesh parts to master pose component and the same anim instance as the master
    (bind (_head _torso_with_arms _hands _legs _feet) (message `/Game/Hyper/Core/Equipment_Manager/Interfaces/BPI_LeaderPose.Get Skeletal Mesh Components` (`/Game/Hyper/Core/Generic/BlueprintMacroLibrary/BML_Generic_Component.Get Character`)))
    (`SkinnedMeshComponent.SetLeaderPoseComponent` _head (`/Game/Hyper/Core/Generic/BlueprintMacroLibrary/BML_Generic_Component.Get Character Mesh`) true false)
    (`SkinnedMeshComponent.SetLeaderPoseComponent` _torso_with_arms (`/Game/Hyper/Core/Generic/BlueprintMacroLibrary/BML_Generic_Component.Get Character Mesh`) true false)
    (`SkinnedMeshComponent.SetLeaderPoseComponent` _hands (`/Game/Hyper/Core/Generic/BlueprintMacroLibrary/BML_Generic_Component.Get Character Mesh`) true false)
    (`SkinnedMeshComponent.SetLeaderPoseComponent` _legs (`/Game/Hyper/Core/Generic/BlueprintMacroLibrary/BML_Generic_Component.Get Character Mesh`) true false)
    (`SkinnedMeshComponent.SetLeaderPoseComponent` _feet (`/Game/Hyper/Core/Generic/BlueprintMacroLibrary/BML_Generic_Component.Get Character Mesh`) true false)
    (`SkeletalMeshComponent.SetAnimInstanceClass` _head (`GameplayStatics.GetObjectClass` (`/Game/Hyper/Core/Generic/BlueprintMacroLibrary/BML_Generic_Component.Get Anim Instance`)))
    (`SkeletalMeshComponent.SetAnimInstanceClass` _torso_with_arms (`GameplayStatics.GetObjectClass` (`/Game/Hyper/Core/Generic/BlueprintMacroLibrary/BML_Generic_Component.Get Anim Instance`)))
    (`SkeletalMeshComponent.SetAnimInstanceClass` _hands (`GameplayStatics.GetObjectClass` (`/Game/Hyper/Core/Generic/BlueprintMacroLibrary/BML_Generic_Component.Get Anim Instance`)))
    (`SkeletalMeshComponent.SetAnimInstanceClass` _legs (`GameplayStatics.GetObjectClass` (`/Game/Hyper/Core/Generic/BlueprintMacroLibrary/BML_Generic_Component.Get Anim Instance`)))
    (`SkeletalMeshComponent.SetAnimInstanceClass` _feet (`GameplayStatics.GetObjectClass` (`/Game/Hyper/Core/Generic/BlueprintMacroLibrary/BML_Generic_Component.Get Anim Instance`)))
    ;;[0.05127 0.05127 0.05127] Get the skeletal mesh components and set the skeletal mesh references. We assume that with what we start, it is the default
    (set `self.Default_Head` (`SkeletalMeshComponent.GetSkeletalMeshAsset` _head))
    (set `self.Default_Torso with Arms` (`SkeletalMeshComponent.GetSkeletalMeshAsset` _torso_with_arms))
    (set `self.Default_Hands` (`SkeletalMeshComponent.GetSkeletalMeshAsset` _hands))
    (set `self.Default_Legs` (`SkeletalMeshComponent.GetSkeletalMeshAsset` _legs))
    (set `self.Default_Feet` (`SkeletalMeshComponent.GetSkeletalMeshAsset` _feet))))

(fn `Swap Leader Posed Skeletal Mesh`
  (params (`Equipment Slot` :type "/Game/Hyper/Core/Equipment_Manager/Datamodel/Enumerations/Enum_Equipment_Slots Enum" :default "NewEnumerator13") (`Inventory Slot` :type "/Game/Hyper/Core/Inventory/Datamodel/Structures/Main_Item_Slot_Structs/Struct_Inventory_Slot_Item Structure") (`Set Slot To Default` :type Boolean))
  (bind _returnvalue (select `/Game/Hyper/Core/Equipment_Manager/Datamodel/Enumerations/Enum_Equipment_Slots` (`local.Equipment Slot`) :`NewEnumerator0` (`self.Default_Head`) :`NewEnumerator1` (`self.Default_Torso with Arms`) :`NewEnumerator2` (`self.Default_Hands`) :`NewEnumerator3` (`self.Default_Legs`) :`NewEnumerator4` (`self.Default_Feet`)))
  ;[0.05127 0.05127 0.05127] Get the skeletal mesh component of the owned character. The owned character should implement the Master Pose interface and return the skeletal mesh components.
  ; Based on the equipment slot input, we swap the mesh of the master posed skeletal mesh component.
  (bind (_head _torso_with_arms _hands _legs _feet) (message `/Game/Hyper/Core/Equipment_Manager/Interfaces/BPI_LeaderPose.Get Skeletal Mesh Components` (`/Game/Hyper/Core/Generic/BlueprintMacroLibrary/BML_Generic_Component.Get Character`)))
  ;;[0.05127 0.05127 0.05127] If set to empty, fall back to the default mesh
  (bind _object (`/Game/Hyper/Core/Generic/BlueprintMacroLibrary/BML_AssetLoading.Load Asset Blocking Checked` (`.SkeletalMesh_100_BBEFA81F47EA9FA57E336FA954BE288A` (break `/Game/Hyper/Core/Equipment_Manager/Datamodel/Structures/Sub_Structs/Struct_CombatAttributes_Equip` (`.Equip_2_81FA71E840D3624FE8414082BDC1BC0C` (break `/Game/Hyper/Core/Equipment_Manager/Datamodel/Structures/Main_Structs/Struct_Equipment` (`/Game/Hyper/Core/Inventory/FunctionLibraries/BFL_InventoryCrafting.Get Equipment info from Inventory Slot` (`local.Inventory Slot`)))))))
    (:`Is Not Valid`
      (bind _returnvalue_2 (select `/Game/Hyper/Core/Equipment_Manager/Datamodel/Enumerations/Enum_Equipment_Slots` (`local.Equipment Slot`) :`NewEnumerator0` _head :`NewEnumerator1` _torso_with_arms :`NewEnumerator2` _hands :`NewEnumerator3` _legs :`NewEnumerator4` _feet :!type "SkinnedMeshComponent Object Reference"))
      (`SkinnedMeshComponent.SetSkinnedAssetAndUpdate` _returnvalue_2 _returnvalue false))
    (:`Is Valid`
      (bind _asskeletal_mesh (cast `SkeletalMesh` _object))
      (`SkinnedMeshComponent.SetSkinnedAssetAndUpdate` _returnvalue_2 (select `bool` (`local.Set Slot To Default`) :`false` _asskeletal_mesh :`true` _returnvalue) false))))