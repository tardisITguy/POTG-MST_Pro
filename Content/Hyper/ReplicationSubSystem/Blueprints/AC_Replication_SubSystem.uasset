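; Character component that replicates montages, sounds and generic spawned actors in multiplayer.
; Montages and sounds play locally first, then route through server multicasts that generally skip the locally controlled client.
; Latent montages relay notify, finish and interrupt callbacks and support section jumps.
; The server spawns named, attachable mesh/Niagara/audio actors, toggling or destroying them by key; clients rebuild the name map from a replicated array via OnRep.
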(event `self.Initialize Multicast Montage`
  (params (`Montage To Play` :type "AnimMontage Object Reference") (`Target Is Mesh` :type Boolean) (`Optional Target` :type "AnimInstance Object Reference"))
  ;[0.05127 0.05127 0.05127] Animation logic.
  ;;[0.05127 0.05127 0.05127] play montage localy, and than on Server
  (`self.Play Montage event` `Montage To Play` `Target Is Mesh` `Optional Target`)
  (`self.Event play montage on server` `Montage To Play` `Target Is Mesh` `Optional Target`))

(event `self.Initialize Stop Multicast Montage`
  ;[0.05127 0.05127 0.05127] Animation logic.
  ;;[0.05127 0.05127 0.05127] stop montage localy, and than on Server
  (`self.Stop Montage`)
  (`self.Event: Stop Multicast Montage on server`))

(event `Event play montage on server`
  (params (`Montage to play` :type "AnimSequenceBase Object Reference") (`Target is Mesh` :type Boolean :default true) (`Optional Target` :type "AnimInstance Object Reference"))
  ;[0.05127 0.05127 0.05127] Animation logic.
  ;;[0.05127 0.05127 0.05127] At Input action, play axe animation montage
  ;;;[0.05127 0.05127 0.05127] First play animation on the server
  (`self.Event: Multicast montage to clients` `Montage to play` `Target is Mesh` `Optional Target`))

(event `Event: Stop Multicast Montage on server`
  ;[0.05127 0.05127 0.05127] Animation logic.
  ;;[0.05127 0.05127 0.05127] Stop animation on clients by multicast (Also runs on server)
  (`self.Event: Stop multicast montage`))

(event `Event: Multicast montage to clients`
  (params (`Montage to play` :type "AnimSequenceBase Object Reference") (`Target is Mesh` :type Boolean :default true) (`Optional Target` :type "AnimInstance Object Reference"))
  ;[0.05127 0.05127 0.05127] Animation logic.
  ;;[0.05127 0.05127 0.05127] At Input action, play axe animation montage
  ;;;[0.05127 0.05127 0.05127] Play animation montage on clients, but not on the locall client. Local client is Already triggered on direct input
  (if (not (`Pawn.IsLocallyControlled` (`/Game/Hyper/Core/Generic/BlueprintMacroLibrary/BML_Generic_Component.Get Character`)))
    (`self.Play Montage event` `Montage to play` `Target is Mesh` `Optional Target`)))

(event `Event: Stop multicast montage`
  ;[0.05127 0.05127 0.05127] Animation logic.
  ;;[0.05127 0.05127 0.05127] Stop animation montage on clients, but not on the locall client. Local client is Already triggered on direct input
  (if (not (`Pawn.IsLocallyControlled` (`/Game/Hyper/Core/Generic/BlueprintMacroLibrary/BML_Generic_Component.Get Character`)))
    (`self.Stop Montage`)))

(event `Play Montage event`
  (params (`Montage to play` :type "AnimSequenceBase Object Reference") (`Target is Mesh` :type Boolean :default true) (`Optional Target` :type "AnimInstance Object Reference"))
  (bind (_returnvalue _bsuccess) (`/Game/Hyper/Core/Generic/BlueprintMacroLibrary/BML_Generic_Component.Get Anim Instance`))
  ;[0.05127 0.05127 0.05127] Animation logic.
  ;;[0.05127 0.05127 0.05127] Play montage on Event
  (if _bsuccess
    (bind _returnvalue_2 (`AnimInstance.PlaySlotAnimationAsDynamicMontage` (select `bool` `Target is Mesh` :`false` `Optional Target` :`true` _returnvalue) `Montage to play` "DefaultSlot" 0.0 0.25 1.0 1 -1.0 0.0))
    (set `self.Current Active Montage` _returnvalue_2)))

(event `Stop Montage`
  ;[0.05127 0.05127 0.05127] Animation logic.
  ;;[0.05127 0.05127 0.05127] Stop Montage
  (bind _current_active_montage (`self.Current Active Montage`)
    (:`then`
      (`Character.StopAnimMontage` (`/Game/Hyper/Core/Generic/BlueprintMacroLibrary/BML_Generic_Component.Get Character`) _current_active_montage))
    (:`else`)))

(event `example bind receive notify 2` :!signature `self.Montage Notify Received`
  (params (Notify :type Name))
  ;[0.002935 0.05127 0] Example Usage
  ;;[0.05127 0.05127 0.05127] You can bind on the notifies that you have given to check for
  ;;;[0.05127 0.05127 0.05127] On notify receive Attach, do X
  (if (not (== Notify "Attach"))
    ;;;[0.05127 0.05127 0.05127] On notify receive Finished, do X
    (if (== Notify "Finish")
      _)))

(event `example bind finsihed 2`
  ;[0.002935 0.05127 0] Example Usage
  ;;[0.05127 0.05127 0.05127] On finsihed, do X
)

(event `self.Initialize Multicast Latent Montage`
  (params (`Montage To Play` :type "AnimMontage Object Reference") (`Notifies To Check` :type "Array of Name (by ref)") (`Play In Default Mesh` :type Boolean) (`Optional Mesh To Play In` :type "SkeletalMeshComponent Object Reference") (`Play Rate` :type "Float (double-precision)"))
  ;[0.05127 0.05127 0.05127] Play montage localy, and than on Server which multicasts it
  (`self.latent montage` `Montage To Play` `Notifies To Check` `Play In Default Mesh` `Optional Mesh To Play In` `Play Rate`)
  (`self.Event: server to multicast latent montage` `Montage To Play` `Notifies To Check` `Play In Default Mesh` `Optional Mesh To Play In`))

(event `self.Initialize Stop Multicast Latent Montage`
  ;[0.05127 0.05127 0.05127] Stop montage localy, and than on Server which multicasts it
  (`self.Stop Latent Montage`)
  (`self.Event: server to Multicast stop latent montage`))

(event `self.Initialize Multicast Play Next Montage Section`
  (`self.Play Next Montage Section`)
  (`self.Event: Server To Multicast Play Next Montage Section`))

(event `Event: server to multicast latent montage`
  (params (MontageToPlay :type "AnimMontage Object Reference") (`Notifies to check` :type "Array of Name (by ref)") (`Play in default mesh` :type Boolean :default true) (`Optional Mesh to play in` :type "SkeletalMeshComponent Object Reference") (PlayRate :type "Float (single-precision)" :default 1.0))
  ;[0.05127 0.05127 0.05127] Server call which initializes the multicast
  (`self.Event: Multicast Latent Montage` MontageToPlay `Notifies to check` `Play in default mesh` `Optional Mesh to play in` PlayRate))

(event `Event: Server To Multicast Stop Latent Montage`
  ;[0.05127 0.05127 0.05127] Server call which initializes the multicast
  (`self.Event: Multicast stop latent montage`))

(event `Event: Server To Multicast Play Next Montage Section`
  (`self.Event: Multicast Play Next Montage Section`))

(event `Event: Multicast Latent Montage`
  (params (MontageToPlay :type "AnimMontage Object Reference") (`Notifies to check` :type "Array of Name (by ref)") (`Play in default mesh` :type Boolean :default true) (`Optional Mesh to play in` :type "SkeletalMeshComponent Object Reference") (PlayRate :type "Float (single-precision)" :default 1.0))
  ;[0.05127 0.05127 0.05127] Multicast: Play animation montage on clients, but not on the locall client. Local client is Already triggered on direct input
  (if (not (`Pawn.IsLocallyControlled` (`/Game/Hyper/Core/Generic/BlueprintMacroLibrary/BML_Generic_Component.Get Character`)))
    (`self.latent montage` MontageToPlay `Notifies to check` `Play in default mesh` `Optional Mesh to play in` PlayRate)))

(event `Event: Multicast Stop Latent Montage`
  ;[0.05127 0.05127 0.05127] Multicast: stop animation montage on clients, but not on the locall client. Local client is Already triggered on direct input
  (if (not (`Pawn.IsLocallyControlled` (`/Game/Hyper/Core/Generic/BlueprintMacroLibrary/BML_Generic_Component.Get Character`)))
    (`self.Stop Latent Montage`)))

(event `Event: Multicast Play Next Montage Section`
  (if (not (`Pawn.IsLocallyControlled` (`/Game/Hyper/Core/Generic/BlueprintMacroLibrary/BML_Generic_Component.Get Character`)))
    (`self.Play Next Montage Section`)))

(event `Stop Latent Montage`
  (bind (_returnvalue _bsuccess) (`/Game/Hyper/Core/Generic/BlueprintMacroLibrary/BML_Generic_Component.Get Anim Instance`))
  ;[0.05127 0.05127 0.05127] Play and stop the multicasted montages
  ;;[0.05127 0.05127 0.05127] Stop Latent Montage
  (if _bsuccess
    (`AnimInstance.Montage_Stop` _returnvalue 0.2 (`AnimInstance.GetCurrentActiveMontage` _returnvalue))))

(event `latent montage`
  (params (MontageToPlay :type "AnimMontage Object Reference") (`Notifies to check` :type "Array of Name") (`Play in default mesh` :type Boolean :default true) (`Optional Mesh to play in` :type "SkeletalMeshComponent Object Reference") (PlayRate :type "Float (single-precision)" :default 1.0))
  (bind (_mesh _bsuccess) (`/Game/Hyper/Core/Generic/BlueprintMacroLibrary/BML_Generic_Component.Get Character Mesh`))
  (bind (_returnvalue _bsuccess_2) (`/Game/Hyper/Core/Generic/BlueprintMacroLibrary/BML_Generic_Component.Get Anim Instance`))
  ;[0.05127 0.05127 0.05127] Play and stop the multicasted montages
  ;;[0.05127 0.05127 0.05127] Play a montage on the client.
  ;; This montage is a latent function. So we can't use it in rep notify or in any other function.
  ;; We still want info like on completed, interrupted, etc.
  (set `self.Notifies to check` `Notifies to check`)
  (set `self.Play Rate` PlayRate)
  (if _bsuccess
    (bind _notifyname (`|PlayMontage` (select `bool` `Play in default mesh` :`false` `Optional Mesh to play in` :`true` _mesh) MontageToPlay PlayRate)
      (:`then`
        ;;[0.05127 0.05127 0.05127] Set current active latent montage
        (if _bsuccess_2
          (set `self.Current Active Montage` (`AnimInstance.GetCurrentActiveMontage` _returnvalue))))
      (:`OnCompleted`
        ;;[0.05127 0.05127 0.05127] When the montage is completed, we want to clear the montage reference so we are able to call a new notify with the same montage
        (set `self.Current Active Montage` null)
        (`self.Montage Finished`))
      (:`OnInterrupted`
        ;;[0.05127 0.05127 0.05127] On montage interrupted
        (set `self.Current Active Montage` null)
        (`self.Montage Interupted`))
      (:`OnNotifyBegin`
        ;;[0.05127 0.05127 0.05127] Check if a specific notify is reached in the montage
        (if (`KismetArrayLibrary.Array_Contains` (`self.Notifies To Check`) _notifyname)
          (`self.Montage Notify Received` _notifyname))))))

(event `self.Initialize Spawn Sound At Location`
  (params (Sound :type "SoundBase Object Reference") (Location :type "Vector Structure") (`Delay New Sound` :type Boolean) (`Delay Amount` :type "Float (double-precision)") (`Attenuation Settings` :type "SoundAttenuation Object Reference"))
  ;[0.05127 0.05127 0.05127] Play Sound at Locaiton
  ;;[0.05127 0.05127 0.05127] Play sound localy, and than on Server which multicasts it
  (if `Delay New Sound`
    ;;;[0.05127 0.05127 0.05127] Only can play new sound if delay has finished
    (`/Engine/EditorBlueprintResources/StandardMacros.DoOnce` false :!label _label
      (:`Completed`
        (`|ExecutionSequence`
          (:`then_0`
            _)
          (:`then_1`
            (`KismetSystemLibrary.Delay` `Delay Amount`)
            (goto _label :!via `Reset`))))))
  (`self.Event: Spawn Sound at location` Sound Location `Attenuation Settings`)
  (`self.Server to multicast spawn sound at location` Sound Location `Attenuation Settings` (or (`KismetSystemLibrary.IsDedicatedServer`) (`KismetSystemLibrary.IsServer`))))

(event `self.Initialize Attach Sound`
  (params (Sound :type "SoundBase Object Reference") (`Attach To Component` :type "SceneComponent Object Reference") (`Attach Point Name` :type Name) (LocationType :type "EAttachLocation Enum" :default "KeepRelativeOffset") (`Stop When Attached To Destroyed` :type Boolean) (`Attenuation Settings` :type "SoundAttenuation Object Reference") (`Concurrency Settings` :type "SoundConcurrency Object Reference"))
  ;[0.05127 0.05127 0.05127] Spawn Sound attached
  ;;[0.05127 0.05127 0.05127] Play  localy, and than on Server which multicasts it
  (`self.Event: Attach Sound` Sound `Attach To Component` `Attach Point Name` LocationType `Stop When Attached To Destroyed` `Attenuation Settings` `Concurrency Settings`)
  (if (`Pawn.IsLocallyControlled` (`/Game/Hyper/Core/Generic/BlueprintMacroLibrary/BML_Generic_Component.Get Character`))
    (`self.Server to multicast  attach sound` Sound `Attach To Component` `Attach Point Name` LocationType `Stop When Attached To Destroyed` `Attenuation Settings` `Concurrency Settings` (or (`KismetSystemLibrary.IsDedicatedServer`) (`KismetSystemLibrary.IsServer`)))))

(event `self.Initialize Stop Attached Sound`
  (params (Sound :type "AudioComponent Object Reference"))
  ;[0.05127 0.05127 0.05127] stop an attached sound
  (`self.stop attach sound` Sound)
  (if (`Pawn.IsLocallyControlled` (`/Game/Hyper/Core/Generic/BlueprintMacroLibrary/BML_Generic_Component.Get Pawn`))
    (`self.server to multicast stop attach sound` Sound (or (`KismetSystemLibrary.IsDedicatedServer`) (`KismetSystemLibrary.IsServer`)))))

(event `Server to multicast spawn sound at location`
  (params (Sound :type "SoundBase Object Reference") (Location :type "Vector Structure") (AttenuationSettings :type "SoundAttenuation Object Reference") (`Instigated from server` :type Boolean))
  ;[0.05127 0.05127 0.05127] Play Sound at Locaiton
  ;;[0.05127 0.05127 0.05127] Initialize from server the multicast
  (`self.Multicast spawn sound at location` Sound Location AttenuationSettings `Instigated from server`))

(event `Server to multicast  attach sound`
  (params (Sound :type "SoundBase Object Reference") (AttachToComponent :type "SceneComponent Object Reference") (AttachPointName :type Name) (LocationType :type "EAttachLocation Enum" :default "KeepRelativeOffset") (bStopWhenAttachedToDestroyed :type Boolean) (AttenuationSettings :type "SoundAttenuation Object Reference") (ConcurrencySettings :type "SoundConcurrency Object Reference") (`Instigated from server` :type Boolean))
  ;[0.05127 0.05127 0.05127] Spawn Sound attached
  ;;[0.05127 0.05127 0.05127] Initialize from server the multicast
  (`self.multicast  attach sound` Sound AttachToComponent AttachPointName LocationType bStopWhenAttachedToDestroyed AttenuationSettings ConcurrencySettings `Instigated from server`))

(event `server to multicast stop attach sound`
  (params (Sound :type "AudioComponent Object Reference") (`instiageted from server` :type Boolean))
  ;[0.05127 0.05127 0.05127] stop an attached sound
  (`self.multicast stop attach sound` Sound `instiageted from server`))

(event `Multicast spawn sound at location`
  (params (Sound :type "SoundBase Object Reference") (Location :type "Vector Structure") (AttenuationSettings :type "SoundAttenuation Object Reference") (`Instigated from server` :type Boolean))
  ;[0.05127 0.05127 0.05127] Play Sound at Locaiton
  ;;[0.05127 0.05127 0.05127] Mutlicast the sound
  (if `Instigated from server`
    (`self.Event: Spawn Sound at location` Sound Location AttenuationSettings :!label _label_2)
    (elif (not (`Pawn.IsLocallyControlled` (`/Game/Hyper/Core/Generic/BlueprintMacroLibrary/BML_Generic_Component.Get Character`)))
      (goto _label_2))))

(event `multicast  attach sound`
  (params (Sound :type "SoundBase Object Reference") (AttachToComponent :type "SceneComponent Object Reference") (AttachPointName :type Name) (LocationType :type "EAttachLocation Enum" :default "KeepRelativeOffset") (bStopWhenAttachedToDestroyed :type Boolean) (AttenuationSettings :type "SoundAttenuation Object Reference") (ConcurrencySettings :type "SoundConcurrency Object Reference") (`Instigated from server` :type Boolean))
  ;[0.05127 0.05127 0.05127] Spawn Sound attached
  ;;[0.05127 0.05127 0.05127] Multicast: Play on clients, but not on the locall client. Local client is Already triggered on direct input
  (if (not (`Pawn.IsLocallyControlled` (`/Game/Hyper/Core/Generic/BlueprintMacroLibrary/BML_Generic_Component.Get Character`)))
    (`self.Event: Attach Sound` Sound AttachToComponent AttachPointName LocationType bStopWhenAttachedToDestroyed AttenuationSettings ConcurrencySettings)))

(event `multicast stop attach sound`
  (params (Sound :type "AudioComponent Object Reference") (`Is instigated from server` :type Boolean))
  ;[0.05127 0.05127 0.05127] stop an attached sound
  (if (not (`Pawn.IsLocallyControlled` (`/Game/Hyper/Core/Generic/BlueprintMacroLibrary/BML_Generic_Component.Get Character`)))
    (`self.stop attach sound` Sound)))

(event `Event: Spawn Sound at location`
  (params (Sound :type "SoundBase Object Reference") (Location :type "Vector Structure") (AttenuationSettings :type "SoundAttenuation Object Reference"))
  ;[0.05127 0.05127 0.05127] Play Sound at Locaiton
  ;;[0.05127 0.05127 0.05127] Spawn the actual sound
  (`GameplayStatics.SpawnSoundAtLocation` Sound Location (struct) 1.0 1.0 0.0 AttenuationSettings null))

(event `Event: Attach Sound`
  (params (Sound :type "SoundBase Object Reference") (AttachToComponent :type "SceneComponent Object Reference") (AttachPointName :type Name) (LocationType :type "EAttachLocation Enum" :default "KeepRelativeOffset") (bStopWhenAttachedToDestroyed :type Boolean) (AttenuationSettings :type "SoundAttenuation Object Reference") (ConcurrencySettings :type "SoundConcurrency Object Reference"))
  ;[0.05127 0.05127 0.05127] Spawn Sound attached
  ;;[0.05127 0.05127 0.05127] Spawn the actual sound
  (bind _returnvalue (`GameplayStatics.SpawnSoundAttached` Sound AttachToComponent AttachPointName (0.0 0.0 0.0) (struct) LocationType bStopWhenAttachedToDestroyed 1.0 1.0 0.0 AttenuationSettings ConcurrencySettings))
  (bind _output_get (set `self.Attached Sound` _returnvalue))
  (`self.Sound Attached` _output_get))

(event `self.Initialize Spawn Sound At Location On Owning Client`
  (params (Sound :type "SoundBase Object Reference") (Location :type "Vector Structure") (`Delay New Sound` :type Boolean) (`Delay Amount` :type "Float (double-precision)") (`Attenuation Settings` :type "SoundAttenuation Object Reference"))
  ;[0.05127 0.05127 0.05127] Play Sound at Locaiton
  (if `Delay New Sound`
    ;;[0.05127 0.05127 0.05127] Only can play new sound if delay has finished
    (`/Engine/EditorBlueprintResources/StandardMacros.DoOnce` false :!label _label_3
      (:`Completed`
        (`|ExecutionSequence`
          (:`then_0`
            _)
          (:`then_1`
            (`KismetSystemLibrary.Delay` `Delay Amount`)
            (goto _label_3 :!via `Reset`))))))
  (`self.Event: Spawn Sound at location` Sound Location `Attenuation Settings`))

(event `stop attach sound`
  (params (Sound :type "AudioComponent Object Reference"))
  ;[0.05127 0.05127 0.05127] stop an attached sound
  (`/Engine/EditorBlueprintResources/StandardMacros.IsValid` Sound
    (:`Is Valid`
      (`AudioComponent.Stop` Sound)
      (`self.K2_DestroyComponent` Sound))))

(event `self.Server: Spawn Actor`
  (params (`Static Mesh` :type "StaticMesh Object Reference") (`Static Mesh Relative Transform` :type "Transform Structure") (`Skeletal Mesh` :type "SkeletalMesh Object Reference") (`Skeletal Mesh Relative Location` :type "Transform Structure") (`Niagara System` :type "NiagaraSystem Object Reference") (`Niagara Relative Transform` :type "Transform Structure") (Sound :type "SoundBase Object Reference") (`Attach To actor` :type Boolean) (`Target Actor` :type "Actor Object Reference") (`Attach To Component` :type Boolean) (`Target Component` :type "SceneComponent Object Reference") (`Target Socket Name` :type Name) (`Spawned Actor Name` :type "Name (by ref)") (Actor :type "/Game/Hyper/Locomotion/Blueprints/Actor_Spawn/BP_Generic_Actor_Spawn Class Reference") (Amount :type "Float (double-precision)"))
  ;[0.05127 0.05127 0.05127] You can use this to spawn a generic replicated actor from an owning connection.
  ; It has basic functionality to spawn effects, meshes, skeletal meshes and/or audio which can be attached to any actor or component.
  ;
  ; This is perfect for testing basic stuff in networked games. I am using this as an example to spawn the Jetpack. If you want you can include jetpack functionality in the equipment/combat system. However, I've not intended the current jetpack like that. You can choose to change it however you see fit.
  ;;[0.05127 0.05127 0.05127] The actual event logic to excecute
  ;;;[0.05127 0.05127 0.05127] If it already exists with same name, do not spawn
  (if (`BlueprintMapLibrary.Map_Contains` (`self.Spawned Actors`) `Spawned Actor Name`)
    (`/Game/Hyper/Core/Debugging/BFL_Debug.Debug` "NewEnumerator17" (`KismetStringLibrary.Concat_StrStr` "Trying to spawn actor: " (`KismetStringLibrary.Conv_NameToString` `Spawned Actor Name`) " but it already exists"))
    (else
      (bind _returnvalue (`|SpawnActorFromClass` Actor (`KismetMathLibrary.MakeTransform` (0.0 0.0 0.0)) "AlwaysSpawn" "SelectDefaultAtRuntime" null `Static Mesh` `Static Mesh Relative Transform` `Skeletal Mesh` `Skeletal Mesh Relative Location` `Niagara System` `Niagara Relative Transform` Sound `Spawned Actor Name` (`/Game/Hyper/Core/Generic/BlueprintMacroLibrary/BML_Generic_Component.Get Character`)))
      (`self.Add Spawned Actor` `Spawned Actor Name` _returnvalue)
      (if `Attach To actor`
        (`Actor.K2_AttachToActor` _returnvalue `Target Actor` `Target Socket Name` "SnapToTarget" "SnapToTarget" "SnapToTarget" true)
        (elif `Attach To Component`
          (`Actor.K2_AttachToComponent` _returnvalue `Target Component` `Target Socket Name` "SnapToTarget" "SnapToTarget" "SnapToTarget" true))))))

(event `self.Server: Set audio active in spawned mesh`
  (params (bNewActive :type Boolean) (Key :type "Name (by ref)"))
  (bind (_value _returnvalue) (`BlueprintMapLibrary.Map_Find` (`self.Spawned Actors`) Key))
  ;[0.05127 0.05127 0.05127] You can use this to spawn a generic replicated actor from an owning connection.
  ; It has basic functionality to spawn effects, meshes, skeletal meshes and/or audio which can be attached to any actor or component.
  ;
  ; This is perfect for testing basic stuff in networked games. I am using this as an example to spawn the Jetpack. If you want you can include jetpack functionality in the equipment/combat system. However, I've not intended the current jetpack like that. You can choose to change it however you see fit.
  ;;[0.05127 0.05127 0.05127] Find actor in mapping, and switch the audio and//or niagara effect
  (if _returnvalue
    (`/Game/Hyper/Locomotion/Blueprints/Actor_Spawn/BP_Generic_Actor_Spawn.Set Audio Active` _value bNewActive)
    (else
      (`/Game/Hyper/Core/Debugging/BFL_Debug.Debug` "NewEnumerator17" (`KismetStringLibrary.Concat_StrStr` "Setting audio: " (`KismetStringLibrary.Conv_NameToString` Key) " not found in mapping")))))

(event `self.Server: Set niagara active in spawned mesh`
  (params (bNewActive :type Boolean) (Key :type "Name (by ref)"))
  (bind (_value _returnvalue) (`BlueprintMapLibrary.Map_Find` (`self.Spawned Actors`) Key))
  ;[0.05127 0.05127 0.05127] You can use this to spawn a generic replicated actor from an owning connection.
  ; It has basic functionality to spawn effects, meshes, skeletal meshes and/or audio which can be attached to any actor or component.
  ;
  ; This is perfect for testing basic stuff in networked games. I am using this as an example to spawn the Jetpack. If you want you can include jetpack functionality in the equipment/combat system. However, I've not intended the current jetpack like that. You can choose to change it however you see fit.
  ;;[0.05127 0.05127 0.05127] Find actor in mapping, and switch the audio and//or niagara effect
  (if _returnvalue
    (`/Game/Hyper/Locomotion/Blueprints/Actor_Spawn/BP_Generic_Actor_Spawn.Set Niagara Active` _value bNewActive)
    (else
      (`/Game/Hyper/Core/Debugging/BFL_Debug.Debug` "NewEnumerator17" (`KismetStringLibrary.Concat_StrStr` "Setting niagara: " (`KismetStringLibrary.Conv_NameToString` Key) " not found in mapping")))))

(event `self.Server: Destroy Spawned actor`
  (params (Key :type "Name (by ref)"))
  (bind (_value _returnvalue) (`BlueprintMapLibrary.Map_Find` (`self.Spawned Actors`) Key))
  ;[0.05127 0.05127 0.05127] You can use this to spawn a generic replicated actor from an owning connection.
  ; It has basic functionality to spawn effects, meshes, skeletal meshes and/or audio which can be attached to any actor or component.
  ;
  ; This is perfect for testing basic stuff in networked games. I am using this as an example to spawn the Jetpack. If you want you can include jetpack functionality in the equipment/combat system. However, I've not intended the current jetpack like that. You can choose to change it however you see fit.
  ;;[0.05127 0.05127 0.05127] Destroy the spawned actor
  (if _returnvalue
    (`/Engine/EditorBlueprintResources/StandardMacros.IsValid` _value
      (:`Is Valid`
        (`Actor.K2_DestroyActor` _value))
      (:`Is Not Valid`
        _))
    (`self.Remove Spawned Actor` Key)
    (else
      (`/Game/Hyper/Core/Debugging/BFL_Debug.Debug` "NewEnumerator17" (`KismetStringLibrary.Concat_StrStr` "Destroying actor: " (`KismetStringLibrary.Conv_NameToString` Key) " not found in mapping")))))

(fn `Add Spawned Actor`
  (params (Key :type Name) (Actor :type "/Game/Hyper/Locomotion/Blueprints/Actor_Spawn/BP_Generic_Actor_Spawn Object Reference"))
  (`BlueprintMapLibrary.Map_Add` (`self.Spawned Actors`) (`local.Key`) (`local.Actor`))
  (`KismetArrayLibrary.Array_Add` (`self.Spawned Actor Names`) (`local.Key`))
  (`KismetArrayLibrary.Array_Add` (`self.Spawned Actor Objects`) (`local.Actor`))
  (`self.Actor Spawned` (`local.Key`) (`local.Actor`)))

(fn `Is Actor Spawned`
  (params (`Spawned Actor Name` :type Name))
  (returns (`Is Spawned` :type Boolean))
  (return (`KismetArrayLibrary.Array_Contains` (`self.Spawned Actor Names`) `Spawned Actor Name`)))

(fn `OnRep_Spawned Actor Objects_Execution`
  (locals (`Old Spawned Actors` :type "Map of Name to /Game/Hyper/Locomotion/Blueprints/Actor_Spawn/BP_Generic_Actor_Spawn Object Reference"))
  (set `local.Old Spawned Actors` (`self.Spawned Actors`))
  (`/Engine/EditorBlueprintResources/ActorComponentMacros.Switch Has Authority`
    (:`Remote`
      (`BlueprintMapLibrary.Map_Clear` (`self.Spawned Actors`))
      (for _array_element (`self.Spawned Actor Objects`)
        (bind _actor_name (`/Game/Hyper/Locomotion/Blueprints/Actor_Spawn/BP_Generic_Actor_Spawn.Actor Name` _array_element))
        (`BlueprintMapLibrary.Map_Add` (`self.Spawned Actors`) _actor_name _array_element)
        (bind (_value _returnvalue) (`BlueprintMapLibrary.Map_Find` (`local.Old Spawned Actors`) _actor_name))
        (if _returnvalue
          _
          (elif (not (`KismetSystemLibrary.IsValid` _value))
            (`self.Actor Spawned` _actor_name _array_element)))))))

(fn `Play Next Montage Section`
  (locals (`Local Anim Instance` :type "AnimInstance Object Reference"))
  (bind _returnvalue (`/Game/Hyper/Core/Generic/BlueprintMacroLibrary/BML_Generic_Component.Get Anim Instance`))
  (bind _returnvalue_2 (`AnimMontage.GetSectionIndex` (`self.Current Active Montage`) (`AnimInstance.Montage_GetCurrentSection` (`local.Local Anim Instance`) (`self.Current Active Montage`))))
  (set `local.Local Anim Instance` _returnvalue)
  ;[0.05098 0.05098 0.05098] Do we have a next sections
  (set `self.Current Active Montage` (`AnimInstance.GetCurrentActiveMontage` _returnvalue))
  (if (< _returnvalue_2 (- (`AnimMontage.GetNumSections` (`self.Current Active Montage`)) 1))
    (`AnimInstance.Montage_JumpToSection` (`local.Local Anim Instance`) (`AnimMontage.GetSectionName` (`self.Current Active Montage`) (+ _returnvalue_2 1)) (`self.Current Active Montage`))))

(fn `Remove Spawned Actor`
  (params (Key :type Name))
  (bind (_value _returnvalue) (`BlueprintMapLibrary.Map_Find` (`self.Spawned Actors`) (`local.Key`)))
  (if _returnvalue
    (`KismetArrayLibrary.Array_RemoveItem` (`self.Spawned Actor Objects`) _value))
  (`BlueprintMapLibrary.Map_Remove` (`self.Spawned Actors`) (`local.Key`))
  (`KismetArrayLibrary.Array_RemoveItem` (`self.Spawned Actor Names`) (`local.Key`)))