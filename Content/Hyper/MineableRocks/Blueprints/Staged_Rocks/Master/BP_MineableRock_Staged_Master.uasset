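; Master Blueprint for a mineable rock that breaks away in three stages and spawns ore, extending a parent rock class.
; Point damage from an accepted equipment type lowers durability through a server event and restarts an inactivity timer.
; Each durability threshold destroys a mesh layer, plays a sound and spawns ores at random child points, capped by a counter never reset here.
; The final stage destroys the actor and checks respawn.
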(event `Server CanRockDestructBasedOnDurability`
  (params (Damage :type "Float (double-precision)") (Instigator :type "Controller Object Reference"))
  ;[0.05127 0.05127 0.05127] process the hit on the server
  (`self.CanRockDestructBasedOnDurability` Damage Instigator))

(event `self.ReceivePointDamage`
  (params (Damage :type "Float (single-precision)") (DamageType :type "DamageType Object Reference") (HitLocation :type "Vector Structure") (HitNormal :type "Vector Structure") (HitComponent :type "PrimitiveComponent Object Reference") (BoneName :type Name) (ShotFromDirection :type "Vector Structure") (InstigatedBy :type "Controller Object Reference") (DamageCauser :type "Actor Object Reference") (HitInfo :type "HitResult Structure (by ref)"))
  (bind _returnvalue (`self.GetComponentByClass` DamageCauser "/Game/Hyper/Core/Equipment_Manager/Blueprints/AC_Equipment_Manager_Abstract.AC_Equipment_Manager_Abstract_C"))
  ;[0.05127 0.05127 0.05127] process the hit on the server
  ;;[0.05127 0.05127 0.05127] Does the instigator has the required equipment to inflict damage?
  (`/Engine/EditorBlueprintResources/StandardMacros.IsValid` _returnvalue
    (:`Is Valid`
      (if (`/Game/Hyper/Core/Equipment_Manager/Blueprints/AC_Equipment_Manager_Abstract.Does actor has required equipmenttype in slot?` _returnvalue (`self.Accepted Equipment Type to inflict Damage`) "NewEnumerator8")
        (`self.Server CanRockDestructBasedOnDurability` Damage InstigatedBy)
        ;;[0.05127 0.05127 0.05127] On every hit, restart inactivity timer
        (`self.Start inactivity timer`)))))

(event `self.ReceiveBeginPlay`
  (`parent.ReceiveBeginPlay`)
  (`self.Set Static Mesh stages`))

(fn `CanRockDestructBasedOnDurability`
  (params (Damage :type "Float (double-precision)") (Instigator :type "Controller Object Reference"))
  ;[0.05127 0.05127 0.05127] Set durability/health
  (set `self.Durability` (- (`self.Durability`) Damage))
  (`|ExecutionSequence`
    (:`then_0`
      ;[0.05127 0.05127 0.05127] Stage one
      (if (and (<= (`self.Durability`) (* (`self.MaxDurability`) (`self.Stage 1 threshold factor`))) (not (`self.DestructedStage1`)))
        (`self.Process Hit on Stage` (`self.Stage_01`) (`local.Instigator`))
        (set `self.DestructedStage1` true)
        (`KismetSystemLibrary.PrintString` "stage 1 destructed" false)))
    (:`then_1`
      ;[0.05127 0.05127 0.05127] stage 2
      (if (and (<= (`self.Durability`) (* (`self.MaxDurability`) (`self.Stage 2 threshold factor`))) (not (`self.DestructedStage2`)))
        (`self.Process Hit on Stage` (`self.Stage_02`) (`local.Instigator`))
        (set `self.DestructedStage2` true)
        (`KismetSystemLibrary.PrintString` "stage 2 destructed" false)))
    (:`then_2`
      ;[0.05127 0.05127 0.05127] stage 3
      (if (and (<= (`self.Durability`) (* (`self.MaxDurability`) (`self.Stage 3 threshold factor`))) (not (`self.DestructedStage3`)))
        (set `self.DestructedStage3` true)
        (`self.Process Hit on Stage` (`self.Stage_03`) (`local.Instigator`))
        (`KismetSystemLibrary.PrintString` "stage 3 destructed" false)))))

(fn `Process Hit on Stage`
  (params (Component :type "PrimitiveComponent Object Reference") (Instigator :type "Controller Object Reference"))
  (bind (_component _is_valid) (`/Game/Hyper/Core/ReplicationSubSystem/BlueprintMacroLibrary/BML_Replication_Controller.Get Replication` Instigator))
  ;[0.05127 0.05127 0.05127] Destroy the staged layer, spawn a sound and spawn the ores
  (`ActorComponent.K2_DestroyComponent` Component)
  (`self.SpawnOres`)
  (if _is_valid
    (`/Game/Hyper/Core/ReplicationSubSystem/Blueprints/AC_Replication_Abstract.Initialize Spawn Sound At Location` _component (`self.RockDestructionSound`) (`self.K2_GetActorLocation`) false 0.0 "/Game/Hyper/ResourcePack/Sounds/Attenuations/SA_Generic.SA_Generic"))
  ;[0.05127 0.05127 0.05127] If final stages is destructed. Make sure to check respawn
  (if (`self.DestructedStage3`)
    (`self.Destroy Actor And Check Respawn`)))

(fn `Set Static Mesh stages`
  (bind _static_mesh (`self.Static Mesh`))
  ;[0.05127 0.05127 0.05127] Set static mesh stages
  (`StaticMeshComponent.SetStaticMesh` (`self.Stage_01`) _static_mesh)
  (`StaticMeshComponent.SetStaticMesh` (`self.Stage_02`) _static_mesh)
  (`StaticMeshComponent.SetStaticMesh` (`self.Stage_03`) _static_mesh))

(fn `SpawnOres`
  (locals (`stones spawned` :type Integer))
  (bind _children (`SceneComponent.GetChildrenComponents` (`self.Ores`) false))
  (bind (_returnvalue_location _returnvalue_rotation) (`KismetMathLibrary.BreakTransform` (`SceneComponent.K2_GetComponentToWorld` (`KismetArrayLibrary.Array_Random` _children))))
  ;[0.05127 0.05127 0.05127] Loop over child components and spawn log on location of scene components under Tree Top
  (for _ _children
    (`|SpawnActorFromClass` (`self.OreToSpawn`) (`KismetMathLibrary.MakeTransform` _returnvalue_location _returnvalue_rotation) "Undefined" "SelectDefaultAtRuntime" null null)
    (bind _result (`/Engine/EditorBlueprintResources/StandardMacros.IncrementInt` (`local.stones spawned`))
      (:`  `
        (set `local.stones spawned` _result)
        (if (>= (`local.stones spawned`) (`self.max stones spawned per layer`))
          (break))))))

(fn `UserConstructionScript`
  (`self.Set Static Mesh stages`))