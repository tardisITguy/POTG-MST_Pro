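; Master Blueprint for a Chaos-based mineable rock that breaks apart under tool hits, drops ores and hands off to respawn logic.
; Point damage from accepted equipment spawns a damage-scaled impact field on the anchored, kinematic-field-activated geometry collection.
; Server-side break events accumulate broken mass, spawning ores at even thresholds and setting HasBroken at the limit.
; Its OnRep triggers cluster-strain shattering and geometry cleanup, while an optional static base mesh takes separate post-break damage.
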(event `Play Sound On Clients`
  (params (Sound :type "SoundBase Object Reference"))
  ;[0.05098 0.05098 0.05098] Multicast break sound to clients and spawn sound at location
  (`GameplayStatics.PlaySoundAtLocation` Sound (`self.K2_GetActorLocation`) (struct) 1.0 1.0 0.0 null null null null))

(event `Destroy geometry`
  ;[0.05098 0.05098 0.05098] Logic for letting object break
  (`ActorComponent.K2_DestroyComponent` (`self.CollionCapsuleForOres`))
  (`KismetSystemLibrary.DelayUntilNextTick`)
  (bind _geometrycollection (`self.GeometryCollection`)
    (:`then`
      (`ActorComponent.K2_DestroyComponent` (`self.BP_Chaos_AnchorField`))
      (`ActorComponent.K2_DestroyComponent` (`self.BP_Chaos_ClusterStrainField`))
      (`ActorComponent.K2_DestroyComponent` _geometrycollection))
    (:`else`)))

(event `self.GeometryCollection.OnChaosBreakEvent`
  (params (BreakEvent :type "ChaosBreakEvent Structure (by ref)"))
  ;[0.05098 0.05098 0.05098] Logic for letting object break
  (`/Engine/EditorBlueprintResources/ActorMacros.Switch Has Authority`
    (:`Authority`
      (`self.Calculate mass chopped and check if has met threshold to spawn ore` BreakEvent)
      (if (>= (`self.Total Mass Broken`) (`self.Mass required to be chopped before breaking`))
        (`/Engine/EditorBlueprintResources/StandardMacros.DoOnce` false
          (:`Completed`
            (set `self.Has Broken` true)
            (`self.Destroy Actor And Check Respawn`)))))))

(event `self.ReceivePointDamage`
  (params (Damage :type "Float (single-precision)") (DamageType :type "DamageType Object Reference") (HitLocation :type "Vector Structure") (HitNormal :type "Vector Structure") (HitComponent :type "PrimitiveComponent Object Reference") (BoneName :type Name) (ShotFromDirection :type "Vector Structure") (InstigatedBy :type "Controller Object Reference") (DamageCauser :type "Actor Object Reference") (HitInfo :type "HitResult Structure (by ref)"))
  (bind _returnvalue (`self.GetComponentByClass` DamageCauser "/Game/Hyper/Core/Equipment_Manager/Blueprints/AC_Equipment_Manager_Abstract.AC_Equipment_Manager_Abstract_C"))
  (bind _force_mutliplier (`self.Force Mutliplier`))
  (bind _returnvalue_2 (+ (* Damage 0.01) 1.0))
  (`/Engine/EditorBlueprintResources/StandardMacros.IsValid` DamageCauser
    (:`Is Valid`
      (`/Engine/EditorBlueprintResources/StandardMacros.IsValid` _returnvalue
        (:`Is Valid`
          (if (`/Game/Hyper/Core/Equipment_Manager/Blueprints/AC_Equipment_Manager_Abstract.Does actor has required equipmenttype in slot?` _returnvalue (`self.Accepted Equipment Type to inflict Damage`) "NewEnumerator8")
            (`self.Set Dynamic`)
            (`self.Base Mesh Logic` HitComponent Damage)
            (`|SpawnActorFromClass` "/Game/Hyper/ResourcePack/Chaos/BP_Chaos_WeaponImpact.BP_Chaos_WeaponImpact_C" (`KismetMathLibrary.MakeTransform` (`.Location` (`GameplayStatics.BreakHitResult` HitInfo))) "Undefined" "MultiplyWithRoot" null (* (* 25000.0 _returnvalue_2) _force_mutliplier) (* (* 1.35 _returnvalue_2) _force_mutliplier) true null)
            (`self.Start inactivity timer`)))))))

(event `self.ReceiveBeginPlay`
  (`parent.ReceiveBeginPlay`)
  (`|ExecutionSequence`
    (:`then_0`
      (bind _asfield_system_actor (cast `FieldSystemActor` (`ChildActorComponent.ChildActor` (`self.BP_Chaos_AnchorField`))))
      (`KismetArrayLibrary.Array_Add` (`GeometryCollectionComponent.InitializationFields` (`self.GeometryCollection`)) _asfield_system_actor)
      (`self.Set Dynamic`))
    (:`then_1`
      (if (`self.Spawn Base Mesh`)
        (`StaticMeshComponent.SetStaticMesh` (`self.Base_Mesh`) null)))))

(event `Set Dynamic`
  (bind _geometrycollection (`self.GeometryCollection`))
  (`GeometryCollectionComponent.ApplyKinematicField` _geometrycollection 220.0 (`SceneComponent.K2_GetComponentLocation` _geometrycollection)))

(fn `Base Mesh Logic`
  (params (A :type "Object Object Reference") (Damage :type "Float (double-precision)"))
  ;[0.05098 0.05098 0.05098] I would prefer to use an CHAOS based trunk. However I do not seem to be able to set the "Object State" dynamicly. This is a proper alternative for now.
  ;;[0.05098 0.05098 0.05098] Check if the trunk is hit, if so, destroy it
  (if (and (== A (`self.Base_Mesh`)) (`self.Has Broken`))
    ;;[0.05098 0.05098 0.05098] If trunk has met damage threshold, destroy the trunk component and call the destroy treeecutting actor
    (bind _met_damage_threshold (`self.Calculate damage done to trunk` Damage))
    (if _met_damage_threshold
      (set `self.Base Mesh Is Destroyed` true)
      ;;[0.05098 0.05098 0.05098] Spawn item when trunk is destroyed
      (if (`self.Spawn item when base mesh is destroyed`)
        (`|SpawnActorFromClass` (`self.Spawn this item when base is destroyed`) (`SceneComponent.K2_GetComponentToWorld` (`self.Base_Mesh`)) "AdjustIfPossibleButAlwaysSpawn" "SelectDefaultAtRuntime" null null)
        ;;[0.05098 0.05098 0.05098] Spawn trunk sound
        (`GameplayStatics.PlaySoundAtLocation` (`self.Base Mesh destruct sound`) (`self.K2_GetActorLocation`) (struct) 1.0 1.0 0.0 null null null null))
      (`ActorComponent.K2_DestroyComponent` (`self.Base_Mesh`))
      (`self.Destroy Actor And Check Respawn`))))

(fn `Calculate Break Layers`
  ;[1 1 1] E.g.
  ; Total mass to be break down = 10
  ; Total ores = 5
  ; Fraction per ore spawn = 2
  ; Thresholds =  Ore spawn index * Fraction
  ;    1* 2 =2
  ;    2*2 = 4
  ;    3*2 = 6
  ;    etc.
  (for _index (range 1 (+ (`self.Amount of ores to spawn`) 1))
    (`KismetArrayLibrary.Array_Add` (`self.Spawn ore Thresholds`) (* (`self.Fraction off mass required to an ore to spawn`) (`KismetMathLibrary.Conv_IntToDouble` _index)))))

(fn `Calculate damage done to trunk`
  (params (Damage :type "Float (double-precision)"))
  (returns (`Met damage threshold` :type Boolean))
  (bind _output_get (set `self.Damage done to base Mesh` (+ (`self.Damage done to base Mesh`) Damage)))
  (`self.Calculate Break Layers`)
  (return (>= _output_get (`self.Damage required to destroy base mesh`))))

(fn `Calculate mass chopped and check if has met threshold to spawn ore`
  (params (ChaosBreakEvent :type "ChaosBreakEvent Structure (by ref)"))
  (bind ((`Location` _location) (`Mass` _mass)) (break `ChaosBreakEvent` ChaosBreakEvent))
  ;[1 1 1] Get mass from break event and add it to total mass variable
  (bind _output_get (set `self.Total Mass Broken` (+ (`self.Total Mass Broken`) _mass)))
  ;[1 1 1] Optionally print total mass chopped down
  (if (`self.Print Mass Chopped Down`)
    (`KismetSystemLibrary.PrintString` (`KismetStringLibrary.Concat_StrStr` "Total mass chopped down: " (`KismetStringLibrary.Conv_DoubleToString` _output_get)) true true (struct :`G` 0.66 :`B` 1.0 :`A` 1.0) 5.0))
  ;[1 1 1] check if total mass broken has met threshold value to spawn ore
  (if (>= (`self.Total Mass Broken`) (`self. Current mass required to spawn ore`))
    ;[1 1 1] When a threshold is met, reculculate  new mass required to spawn an ore
    (set `self. Current mass required to spawn ore` (+ (`self. Current mass required to spawn ore`) (`self.Fraction off mass required to an ore to spawn`)))
    ;[1 1 1] Check if the maximum of ores has been spawned
    (if (not (>= (`self.Ores spawned`) (`self.Amount of ores to spawn`)))
      ;[1 1 1] Spawn an ore at the break location
      (`|SpawnActorFromClass` (`self.Ore to Spawn`) (`KismetMathLibrary.MakeTransform` (+ _location (10.0 10.0 250.0))) "AdjustIfPossibleButAlwaysSpawn" "SelectDefaultAtRuntime" null null)
      (`self.Play Sound On Clients` (`self.Break Sound`))
      ;[1 1 1] Increment amount of ores spawned
      (set `self.Ores spawned` (+ (`self.Ores spawned`) 1))
      (return)
      (else
        (return)))
    (else
      (return))))

(fn `OnRep_Has Broken_Execution`
  (params (`Override Initialization Check` :type Boolean))
  ;[0.05098 0.05098 0.05098] break sound on hit location
  (`GameplayStatics.PlaySoundAtLocation` (`self.Break Sound`) (`self.K2_GetActorLocation`) (struct) 1.0 1.0 0.0 null null null null)
  ;[0.05098 0.05098 0.05098] This actor is a clusterstrainfield. This makes sure to destory ALL the components which gives a nice effect and cleans up all parts
  (bind _asbp_chaos_cluster_strain_field (cast `/Game/Hyper/ResourcePack/Chaos/BP_Chaos_ClusterStrainField` (`ChildActorComponent.ChildActor` (`self.BP_Chaos_ClusterStrainField`))))
  (`/Game/Hyper/ResourcePack/Chaos/BP_Chaos_ClusterStrainField.Activate Clusterstrainfield` _asbp_chaos_cluster_strain_field)
  (`self.Destroy geometry`))

(fn `UserConstructionScript`
  (`|ExecutionSequence`
    (:`then_0`
      (bind _output_get (set `self.Fraction off mass required to an ore to spawn` (/ (`self.Mass required to be chopped before breaking`) (`KismetMathLibrary.Conv_IntToDouble` (`self.Amount of ores to spawn`)))))
      (set `self. Current mass required to spawn ore` _output_get))
    (:`then_1`
      (`self.Calculate Break Layers`)
      (if (`self.Print Threshold calucalation`)
        (for (_array_element _array_index) (`self.Spawn ore Thresholds`)
          (`KismetSystemLibrary.PrintString` (`KismetStringLibrary.Concat_StrStr` "Threshold Calculations: \nIndex: " (`KismetStringLibrary.Conv_IntToString` _array_index) "Threshold: " (`KismetStringLibrary.Conv_DoubleToString` _array_element)) true true (struct :`G` 0.66 :`B` 1.0 :`A` 1.0) 10.0))))))