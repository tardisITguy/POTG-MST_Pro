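; BP_ShallowWater_Trigger is a box trigger volume that marks characters as walking in shallow water for the footstep system.
; Begin and end overlap find the footstep manager through the instigator's controller and toggle its CharacterIsWalkingInShallowWater flag.
; The flag bypasses visibility traces on the water surface, which would otherwise make foot IK stand on it.
; The one-shot entry splash logic is disconnected.
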(event `self.Box.OnComponentBeginOverlap`
  (params (OverlappedComponent :type "PrimitiveComponent Object Reference") (OtherActor :type "Actor Object Reference") (OtherComp :type "PrimitiveComponent Object Reference") (OtherBodyIndex :type Integer) (bFromSweep :type Boolean) (SweepResult :type "HitResult Structure (by ref)"))
  (bind _returnvalue (`self.GetInstigatorController` OtherActor))
  (bind (_component _is_valid) (`/Game/Hyper/Core/FootstepSystem/BlueprintMacroLibrary/BML_Footstep_Controller.Get Footstep Manager` _returnvalue))
  ;[0.05127 0.05127 0.05127] The footstep is doing a trace downwards on visibility.
  ; However, when we walk in shallow water, we want water footsteps as a sound.
  ; We are able to trace down and find the surface of the water is visibility is on block, BUT the IK trace of the feet are also checking the visibility trace which will place the feet on the water surface if that visibility is set to block.
  ; So for shallow water, we bypass it by setting this boolean on and off based on overlap with water with the ShallowWater Trigger BP.
  ; We also check for the location to spawn the water ripples
  (`/Engine/EditorBlueprintResources/StandardMacros.IsValid` _returnvalue
    (:`Is Valid`
      (if _is_valid
        (set `/Game/Hyper/Core/FootstepSystem/Blueprints/AC_Footsteps_Abstract.Character_Is_Walking_In_Shallow_Water` true _component)
        (if (`.bSuccess` (cast `Character` (`Controller.K2_GetPawn` _returnvalue) :!pure true))
          _)))))

(event `self.Box.OnComponentEndOverlap`
  (params (OverlappedComponent :type "PrimitiveComponent Object Reference") (OtherActor :type "Actor Object Reference") (OtherComp :type "PrimitiveComponent Object Reference") (OtherBodyIndex :type Integer))
  (bind _returnvalue (`self.GetInstigatorController` OtherActor))
  (bind (_component _is_valid) (`/Game/Hyper/Core/FootstepSystem/BlueprintMacroLibrary/BML_Footstep_Controller.Get Footstep Manager` _returnvalue))
  ;[0.05127 0.05127 0.05127] The footstep is doing a trace downwards on visibility.
  ; However, when we walk in shallow water, we want water footsteps as a sound.
  ; We are able to trace down and find the surface of the water is visibility is on block, BUT the IK trace of the feet are also checking the visibility trace which will place the feet on the water surface if that visibility is set to block.
  ; So for shallow water, we bypass it by setting this boolean on and off based on overlap with water with the ShallowWater Trigger BP.
  ; We also check for the location to spawn the water ripples
  (`/Engine/EditorBlueprintResources/StandardMacros.IsValid` _returnvalue
    (:`Is Valid`
      (if _is_valid
        (set `/Game/Hyper/Core/FootstepSystem/Blueprints/AC_Footsteps_Abstract.Character_Is_Walking_In_Shallow_Water` false _component)))))

(fn `UserConstructionScript`)