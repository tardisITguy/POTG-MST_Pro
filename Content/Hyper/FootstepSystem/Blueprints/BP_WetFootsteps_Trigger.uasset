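; BP_WetFootsteps_Trigger is a trigger volume that turns on water splash footstep sounds for characters inside it.
; On box overlap begin, it finds the footstep manager component through the overlapping actor's instigator controller and enables its water splash sound flag.
; On overlap end it disables the same flag, with validity checks on the controller and manager.
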(event `self.Box.OnComponentBeginOverlap`
  (params (OverlappedComponent :type "PrimitiveComponent Object Reference") (OtherActor :type "Actor Object Reference") (OtherComp :type "PrimitiveComponent Object Reference") (OtherBodyIndex :type Integer) (bFromSweep :type Boolean) (SweepResult :type "HitResult Structure (by ref)"))
  (bind _returnvalue (`self.GetInstigatorController` OtherActor))
  (bind (_component _is_valid) (`/Game/Hyper/Core/FootstepSystem/BlueprintMacroLibrary/BML_Footstep_Controller.Get Footstep Manager` _returnvalue))
  (`/Engine/EditorBlueprintResources/StandardMacros.IsValid` _returnvalue
    (:`Is Valid`
      (if _is_valid
        (set `/Game/Hyper/Core/FootstepSystem/Blueprints/AC_Footsteps_Abstract.footstep water splash sound enabled` true _component)))))

(event `self.Box.OnComponentEndOverlap`
  (params (OverlappedComponent :type "PrimitiveComponent Object Reference") (OtherActor :type "Actor Object Reference") (OtherComp :type "PrimitiveComponent Object Reference") (OtherBodyIndex :type Integer))
  (bind _returnvalue (`self.GetInstigatorController` OtherActor))
  (bind (_component _is_valid) (`/Game/Hyper/Core/FootstepSystem/BlueprintMacroLibrary/BML_Footstep_Controller.Get Footstep Manager` _returnvalue))
  (`/Engine/EditorBlueprintResources/StandardMacros.IsValid` _returnvalue
    (:`Is Valid`
      (if _is_valid
        (set `/Game/Hyper/Core/FootstepSystem/Blueprints/AC_Footsteps_Abstract.footstep water splash sound enabled` false _component)))))

(fn `UserConstructionScript`)