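; Character footstep component that plays surface-based sounds, decals and particles, and reports AI noise for each step.
; ExcecuteFootstepLogic traces down from a foot or root socket for the physical surface, using an object trace against the water trigger in shallow water.
; A hit drives sounds by step type with optional splash, sand or snow prints, and surface particles.
; Locally controlled characters send weight-scaled noise through a server PawnMakeNoise event.
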(event `Server: Pawn Make Noise`
  (params (Loudness :type "Float (double-precision)") (`Noise Location` :type "Vector Structure") (`Use Noise Maker Location` :type Boolean) (`Noise Maker` :type "Actor Object Reference"))
  (`Pawn.PawnMakeNoise` (`/Game/Hyper/Core/Generic/BlueprintMacroLibrary/BML_Generic_Component.Get Character`) Loudness `Noise Location` `Use Noise Maker Location` `Noise Maker`))

(fn `ExcecuteFootstepLogic`
  (params (`Skeletal Mesh Component` :type "SkeletalMeshComponent Object Reference") (`Footstep Type` :type "/Game/Hyper/Core/FootstepSystem/Datamodel/Enumerations/Enum_Walk_Types Enum" :default "NewEnumerator0") (`Notify Type` :type "/Game/Hyper/Core/FootstepSystem/Datamodel/Enumerations/Enum_Notify_Type Enum" :default "NewEnumerator0") (`Footstep Weight` :type "/Game/Hyper/Core/FootstepSystem/Datamodel/Enumerations/Enum_Footstep_Weight Enum" :default "NewEnumerator4"))
  ;[0.05127 0.05127 0.05127] Checks the surface based on line trace
  (bind (_has_hit_on_surface _surfacetype _stepimpactlocation) (`self.SurfaceTypeCheck` `Skeletal Mesh Component` `Notify Type`))
  ;[0.05127 0.05127 0.05127] Optionally print the footstep resuls for debugging
  (if (`self.Print_Debugging`)
    (`KismetSystemLibrary.PrintString` (`KismetTextLibrary.Conv_TextToString` (`|FormatText` "Footstep Type: {Footstep Type} \nNotify Type: {Notify Type:} \nFootstep Weight: {Footstep Weight} \nSurface Type Hit: {Surface Type Hit}" (`|GetEnumeratorNameAsString` `Footstep Type`) (`|GetEnumeratorNameAsString` `Notify Type`) (`|GetEnumeratorNameAsString` `Footstep Weight`) (`|GetEnumeratorNameAsString` _surfacetype)))))
  ;[0.05127 0.05127 0.05127] If there is a hit conintue
  (if _has_hit_on_surface
    (`|ExecutionSequence`
      (:`then_0`
        ;[0.05127 0.05127 0.05127] Play sound, spawn decal and spawn footstep particle. Easy to add more logic, add a pin in the sequence
        (`self.Play Footstep Sound` (`local.Footstep Type`) _surfacetype _stepimpactlocation (`local.Footstep Weight`)))
      (:`then_1`
        (`self.SpawnFootstepDecal` _stepimpactlocation _surfacetype (`local.Skeletal Mesh Component`) (`local.Notify Type`) (`local.Footstep Weight`)))
      (:`then_2`
        (`self.SpawnFootstepParticle` _stepimpactlocation _surfacetype (`local.Footstep Weight`)))
      (:`then_3`
        (if (`Pawn.IsLocallyControlled` (`/Game/Hyper/Core/Generic/BlueprintMacroLibrary/BML_Generic_Component.Get Character`))
          (`self.Server: Pawn Make Noise` (select `/Game/Hyper/Core/FootstepSystem/Datamodel/Enumerations/Enum_Footstep_Weight` (`local.Footstep Weight`) :`NewEnumerator4` 0.1 :`NewEnumerator0` 0.25 :`NewEnumerator1` 0.5 :`NewEnumerator2` 0.66 :`NewEnumerator3` 0.75) _stepimpactlocation))))))

(fn `Get Footstep Water Splash Sound Based On Footstep Type`
  (params (`Footstep type` :type "/Game/Hyper/Core/FootstepSystem/Datamodel/Enumerations/Enum_Walk_Types Enum" :default "NewEnumerator0"))
  (returns (`Run Sound` :type "SoundCue Object Reference"))
  (bind _run_footstep_sound_water (`self.Run Footstep Sound Water`))
  (return (select `/Game/Hyper/Core/FootstepSystem/Datamodel/Enumerations/Enum_Walk_Types` `Footstep type` :`NewEnumerator0` _run_footstep_sound_water :`NewEnumerator1` _run_footstep_sound_water :`NewEnumerator2` _run_footstep_sound_water :`NewEnumerator3` _run_footstep_sound_water :`NewEnumerator4` (`self.Jump Footstep Sound Water`) :`NewEnumerator5` (`self.Land Footstep Sound Water`))))

(fn `Get Jump Sound Based On SurfaceType`
  (params (`Physical surface Type` :type "EPhysicalSurface Enum" :default "SurfaceType_Default") (`Footstep Weight` :type "/Game/Hyper/Core/FootstepSystem/Datamodel/Enumerations/Enum_Footstep_Weight Enum" :default "NewEnumerator4"))
  (returns (`Run Sound` :type "SoundCue Object Reference"))
  (bind _returnvalue (select `EPhysicalSurface` (`local.Physical surface Type`) :`SurfaceType_Default` (`self.Jump Footstep Sound Default`) :`SurfaceType1` (`self.Jump Footstep Sound Grass`) :`SurfaceType2` (`self.Jump Footstep Sound Rock`) :`SurfaceType3` (`self.Jump Footstep Sound Wood`) :`SurfaceType4` (`self.Jump Footstep Sound Water`) :`SurfaceType5` (`self.Jump Footstep Sound Sand`) :`SurfaceType6` (`self.Jump Footstep Sound Snow`) :`SurfaceType7` (`self.Jump Footstep Sound Cloth`)))
  (return (select `/Game/Hyper/Core/FootstepSystem/Datamodel/Enumerations/Enum_Footstep_Weight` (`local.Footstep Weight`) :`NewEnumerator4` _returnvalue :`NewEnumerator0` _returnvalue :`NewEnumerator1` _returnvalue :`NewEnumerator2` _returnvalue :`NewEnumerator3` _returnvalue)))

(fn `Get Land Sound Based On SurfaceType`
  (params (`Physical surface Type` :type "EPhysicalSurface Enum" :default "SurfaceType_Default") (`Footstep Weight` :type "/Game/Hyper/Core/FootstepSystem/Datamodel/Enumerations/Enum_Footstep_Weight Enum" :default "NewEnumerator4"))
  (returns (`Run Sound` :type "SoundCue Object Reference"))
  (bind _returnvalue (select `EPhysicalSurface` (`local.Physical surface Type`) :`SurfaceType_Default` (`self.Land Footstep Sound Default`) :`SurfaceType1` (`self.Land Footstep Sound Grass`) :`SurfaceType2` (`self.Land Footstep Sound Rock`) :`SurfaceType3` (`self.Land Footstep Sound Wood`) :`SurfaceType4` (`self.Land Footstep Sound Water`) :`SurfaceType5` (`self.Land Footstep Sound Sand`) :`SurfaceType6` (`self.Land Footstep Sound Snow`) :`SurfaceType7` (`self.Land Footstep Sound Cloth`)))
  (return (select `/Game/Hyper/Core/FootstepSystem/Datamodel/Enumerations/Enum_Footstep_Weight` (`local.Footstep Weight`) :`NewEnumerator4` _returnvalue :`NewEnumerator0` _returnvalue :`NewEnumerator1` _returnvalue :`NewEnumerator2` _returnvalue :`NewEnumerator3` _returnvalue)))

(fn `Get Run Sound Based On SurfaceType`
  (params (`Physical surface Type` :type "EPhysicalSurface Enum" :default "SurfaceType_Default") (`Footstep Weight` :type "/Game/Hyper/Core/FootstepSystem/Datamodel/Enumerations/Enum_Footstep_Weight Enum" :default "NewEnumerator4"))
  (returns (`Run Sound` :type "SoundCue Object Reference"))
  (bind _returnvalue (select `EPhysicalSurface` (`local.Physical surface Type`) :`SurfaceType_Default` (`self.Run Footstep Sound Default`) :`SurfaceType1` (`self.Run Footstep Sound Grass`) :`SurfaceType2` (`self.Run Footstep Sound Rock`) :`SurfaceType3` (`self.Run Footstep Sound Wood`) :`SurfaceType4` (`self.Run Footstep Sound Water`) :`SurfaceType5` (`self.Run Footstep Sound Sand`) :`SurfaceType6` (`self.Run Footstep Sound Snow`) :`SurfaceType7` (`self.Run Footstep Sound Cloth`)))
  (return (select `/Game/Hyper/Core/FootstepSystem/Datamodel/Enumerations/Enum_Footstep_Weight` (`local.Footstep Weight`) :`NewEnumerator4` _returnvalue :`NewEnumerator0` _returnvalue :`NewEnumerator1` _returnvalue :`NewEnumerator2` _returnvalue :`NewEnumerator3` _returnvalue)))

(fn `GetNotifyLocationBasedOnSocket`
  (params (`Skeletal Mesh Component` :type "SkeletalMeshComponent Object Reference") (`Notify Type` :type "/Game/Hyper/Core/FootstepSystem/Datamodel/Enumerations/Enum_Notify_Type Enum" :default "NewEnumerator0"))
  (returns (ReturnValue :type "Vector Structure"))
  (switch `/Game/Hyper/Core/FootstepSystem/Datamodel/Enumerations/Enum_Notify_Type` `Notify Type`
    (:`NewEnumerator0`
      (return (`SceneComponent.GetSocketLocation` `Skeletal Mesh Component` "foot_l")))
    (:`NewEnumerator1`
      (return (`SceneComponent.GetSocketLocation` `Skeletal Mesh Component` "foot_r")))
    (:`NewEnumerator2`
      (return (`SceneComponent.GetSocketLocation` `Skeletal Mesh Component` "root")))))

(fn `GetWalkSoundBasedOnSurfaceType`
  (params (`Physical surface Type` :type "EPhysicalSurface Enum" :default "SurfaceType_Default") (`Footstep Weight` :type "/Game/Hyper/Core/FootstepSystem/Datamodel/Enumerations/Enum_Footstep_Weight Enum" :default "NewEnumerator4"))
  (returns (`Run Sound` :type "SoundCue Object Reference"))
  (bind _returnvalue (select `EPhysicalSurface` (`local.Physical surface Type`) :`SurfaceType_Default` (`self.Walk Footstep sounds default`) :`SurfaceType1` (`self.Walk Footstep sounds Grass`) :`SurfaceType2` (`self.Walk Footstep sounds  Rock`) :`SurfaceType3` (`self.Walk Footstep sounds Wood`) :`SurfaceType4` (`self.Walk Footstep sounds Water`) :`SurfaceType5` (`self.Walk Footstep sounds Sand`) :`SurfaceType6` (`self.Walk Footstep sounds Snow`) :`SurfaceType7` (`self.Walk Footstep sounds Cloth`)))
  (return (select `/Game/Hyper/Core/FootstepSystem/Datamodel/Enumerations/Enum_Footstep_Weight` (`local.Footstep Weight`) :`NewEnumerator4` _returnvalue :`NewEnumerator0` _returnvalue :`NewEnumerator1` _returnvalue :`NewEnumerator2` _returnvalue :`NewEnumerator3` _returnvalue)))

(fn `Play Footstep Sound`
  (params (`Footstep Type` :type "/Game/Hyper/Core/FootstepSystem/Datamodel/Enumerations/Enum_Walk_Types Enum" :default "NewEnumerator0") (`Physical surface Type` :type "EPhysicalSurface Enum" :default "SurfaceType_Default") (Location :type "Vector Structure") (`Footstep Weight` :type "/Game/Hyper/Core/FootstepSystem/Datamodel/Enumerations/Enum_Footstep_Weight Enum" :default "NewEnumerator4"))
  (bind _run_sound (`self.Get Footstep Water Splash Sound Based On Footstep Type` `Footstep Type`))
  (bind _concurrency_settings (`self.Concurrency Settings`))
  (bind _footstep_water_splash_sound_enabled (`self.footstep water splash sound enabled`))
  (bind _splash_sound_volume_multiplier (`self.Splash Sound volume multiplier`))
  (bind _volume_multiplier (`self.Volume Multiplier`))
  (bind _attenuation_settings (`self.Attenuation_Settings`))
  (switch `/Game/Hyper/Core/FootstepSystem/Datamodel/Enumerations/Enum_Walk_Types` `Footstep Type`
    (:`NewEnumerator0`
      (`GameplayStatics.PlaySoundAtLocation` (`self.GetWalkSoundBasedOnSurfaceType` `Physical surface Type` `Footstep Weight`) Location (struct) _volume_multiplier 1.0 0.0 _attenuation_settings _concurrency_settings null null)
      ;[0.05127 0.05127 0.05127] If surface type is same as water don't spawn water splash sound (otherwise double)
      (if (not (`|EnumEquality` `Physical surface Type` "SurfaceType4"))
        ;[0.05127 0.05127 0.05127] Only play water splash sound when this is enabled. For instance when wet or walking in puddles. This boolean can be set in from the character via the footstep component
        (if _footstep_water_splash_sound_enabled
          (`GameplayStatics.PlaySoundAtLocation` _run_sound Location (struct) 1.0 1.0 0.0 null null null null))))
    (:`NewEnumerator1`
      (`GameplayStatics.PlaySoundAtLocation` (`self.Get Run Sound Based On SurfaceType` `Physical surface Type` `Footstep Weight`) Location (struct) _volume_multiplier 1.0 0.0 _attenuation_settings _concurrency_settings null null :!label _label)
      (if (`|EnumEquality` `Physical surface Type` "SurfaceType4")
        _
        (elif _footstep_water_splash_sound_enabled
          (`GameplayStatics.PlaySoundAtLocation` _run_sound Location (struct) _splash_sound_volume_multiplier 1.0 0.0 null null null null))))
    (:`NewEnumerator2`
      (goto _label))
    (:`NewEnumerator3`
      (goto _label))
    (:`NewEnumerator4`
      (`GameplayStatics.PlaySoundAtLocation` (`self.Get Jump Sound Based On SurfaceType` `Physical surface Type` `Footstep Weight`) Location (struct) _volume_multiplier 1.0 0.0 _attenuation_settings _concurrency_settings null null)
      (if (`|EnumEquality` `Physical surface Type` "SurfaceType4")
        _
        (elif _footstep_water_splash_sound_enabled
          (`GameplayStatics.PlaySoundAtLocation` _run_sound Location (struct) _splash_sound_volume_multiplier 1.0 0.0 null null null null))))
    (:`NewEnumerator5`
      (`GameplayStatics.PlaySoundAtLocation` (`self.Get Land Sound Based On SurfaceType` `Physical surface Type` `Footstep Weight`) Location (struct) _volume_multiplier 1.0 0.0 _attenuation_settings _concurrency_settings null null)
      (if (`|EnumEquality` `Physical surface Type` "SurfaceType4")
        _
        (elif _footstep_water_splash_sound_enabled
          (`GameplayStatics.PlaySoundAtLocation` _run_sound Location (struct) _splash_sound_volume_multiplier 1.0 0.0 null null null null))))))

(fn `SpawnFootstepDecal`
  (params (NotifyLocation :type "Vector Structure") (`Physical Surface Type` :type "EPhysicalSurface Enum" :default "SurfaceType_Default") (`Skeletal Mesh Component` :type "SkeletalMeshComponent Object Reference") (`Notify Type` :type "/Game/Hyper/Core/FootstepSystem/Datamodel/Enumerations/Enum_Notify_Type Enum" :default "NewEnumerator0") (`Footstep Weight` :type "/Game/Hyper/Core/FootstepSystem/Datamodel/Enumerations/Enum_Footstep_Weight Enum" :default "NewEnumerator4"))
  (locals (`Local stored footstep Decal left` :type "MaterialInterface Object Reference") (`Local stored footstep Decal right` :type "MaterialInterface Object Reference"))
  (bind (_returnvalue_roll _returnvalue_pitch _returnvalue_yaw) (`KismetMathLibrary.BreakRotator` (`Actor.K2_GetActorRotation` (`self.GetOwner` `Skeletal Mesh Component`))))
  (switch `/Game/Hyper/Core/FootstepSystem/Datamodel/Enumerations/Enum_Notify_Type` `Notify Type`
    (:`NewEnumerator0`
      (switch `EPhysicalSurface` `Physical Surface Type`
        (:`SurfaceType5`
          ;[1 1 1] Switches decal based on surface type. If none defined, none spawned.
          (set `local.Local stored footstep Decal left` (`self.Sand footstep Decal left`)))
        (:`SurfaceType6`
          (set `local.Local stored footstep Decal left` (`self.Snow footstep decal left`))))
      (`GameplayStatics.SpawnDecalAtLocation` (`local.Local stored footstep Decal left`) (50.0 20.0 -20.0) NotifyLocation (`KismetMathLibrary.MakeRotator` -90.0 90.0 _returnvalue_yaw) (`self.Footstep decal life`)))
    (:`NewEnumerator1`
      (switch `EPhysicalSurface` `Physical Surface Type`
        (:`SurfaceType5`
          ;[1 1 1] Switches decal based on surface type. If none defined, none spawned.
          (set `local.Local stored footstep Decal right` (`self.Sand footstep Decal Right`)))
        (:`SurfaceType6`
          (set `local.Local stored footstep Decal right` (`self.Snow footstep Decal Right`))))
      (`GameplayStatics.SpawnDecalAtLocation` (`local.Local stored footstep Decal right`) (50.0 20.0 -20.0) NotifyLocation (`KismetMathLibrary.MakeRotator` -90.0 90.0 _returnvalue_yaw) (`self.Footstep decal life`)))))

(fn `SpawnFootstepParticle`
  (params (Location :type "Vector Structure") (`Physical Surface Type` :type "EPhysicalSurface Enum" :default "SurfaceType_Default") (`Footstep Weight` :type "/Game/Hyper/Core/FootstepSystem/Datamodel/Enumerations/Enum_Footstep_Weight Enum" :default "NewEnumerator4"))
  (locals (`Local footstep particle` :type "ParticleSystem Object Reference"))
  (bind _genericdust (`self.GenericDust`))
  (bind _grass_footstep_particle (`self.Grass footstep particle`))
  (bind _water_footstep_particle (`self.Water footstep particle`))
  (bind _sand_footstep_particle (`self.Sand footstep particle`))
  (bind _snow_footstep_particle (`self.Snow footstep particle`))
  (switch `EPhysicalSurface` `Physical Surface Type`
    (:`SurfaceType_Default`
      ;[0.05127 0.05127 0.05127] Default
      (set `local.Local footstep particle` (select `/Game/Hyper/Core/FootstepSystem/Datamodel/Enumerations/Enum_Footstep_Weight` (`local.Footstep Weight`) :`NewEnumerator4` _genericdust :`NewEnumerator0` _genericdust :`NewEnumerator1` _genericdust :`NewEnumerator2` _genericdust :`NewEnumerator3` _genericdust) :!label _label))
    (:`SurfaceType1`
      ;[0.05127 0.05127 0.05127] Grass
      (set `local.Local footstep particle` (select `/Game/Hyper/Core/FootstepSystem/Datamodel/Enumerations/Enum_Footstep_Weight` (`local.Footstep Weight`) :`NewEnumerator4` _grass_footstep_particle :`NewEnumerator0` _grass_footstep_particle :`NewEnumerator1` _grass_footstep_particle :`NewEnumerator2` _grass_footstep_particle :`NewEnumerator3` _grass_footstep_particle)))
    (:`SurfaceType2`
      (goto _label))
    (:`SurfaceType3`
      (goto _label))
    (:`SurfaceType4`
      ;[0.05127 0.05127 0.05127] Water
      (set `local.Local footstep particle` (select `/Game/Hyper/Core/FootstepSystem/Datamodel/Enumerations/Enum_Footstep_Weight` (`local.Footstep Weight`) :`NewEnumerator4` _water_footstep_particle :`NewEnumerator0` _water_footstep_particle :`NewEnumerator1` _water_footstep_particle :`NewEnumerator2` _water_footstep_particle :`NewEnumerator3` _water_footstep_particle)))
    (:`SurfaceType5`
      ;[0.05127 0.05127 0.05127] Sand
      (set `local.Local footstep particle` (select `/Game/Hyper/Core/FootstepSystem/Datamodel/Enumerations/Enum_Footstep_Weight` (`local.Footstep Weight`) :`NewEnumerator4` _sand_footstep_particle :`NewEnumerator0` _sand_footstep_particle :`NewEnumerator1` _sand_footstep_particle :`NewEnumerator2` _sand_footstep_particle :`NewEnumerator3` _sand_footstep_particle)))
    (:`SurfaceType6`
      ;[0.05127 0.05127 0.05127] Snow
      (set `local.Local footstep particle` (select `/Game/Hyper/Core/FootstepSystem/Datamodel/Enumerations/Enum_Footstep_Weight` (`local.Footstep Weight`) :`NewEnumerator4` _snow_footstep_particle :`NewEnumerator0` _snow_footstep_particle :`NewEnumerator1` _snow_footstep_particle :`NewEnumerator2` _snow_footstep_particle :`NewEnumerator3` _snow_footstep_particle))))
  ;[0.05127 0.05127 0.05127] Switches particle based on surface type. If none defined, none spawned.
  (`GameplayStatics.SpawnEmitterAtLocation` (`local.Local footstep particle`) Location))

(fn `SurfaceTypeCheck`
  (params (`Skeletal Mesh Component` :type "SkeletalMeshComponent Object Reference") (`Notify Type` :type "/Game/Hyper/Core/FootstepSystem/Datamodel/Enumerations/Enum_Notify_Type Enum" :default "NewEnumerator0"))
  (returns (`Has Hit On Surface` :type Boolean) (SurfaceType :type "EPhysicalSurface Enum") (StepImpactLocation :type "Vector Structure"))
  ;[1 1 1] Gets the location from foot socket position
  (bind _returnvalue (`self.GetNotifyLocationBasedOnSocket` `Skeletal Mesh Component` `Notify Type`))
  (if (`self.Character_Is_Walking_In_Shallow_Water`)
    (bind _returnvalue_2 (+ _returnvalue (0.0 0.0 55.0)))
    (bind _returnvalue_3 (- _returnvalue (0.0 0.0 45.0)))
    ;[0.05127 0.05127 0.05127] The footstep is doing a trace downwards on visibility.
    ; However, when we walk in shallow water, we want water footsteps as a sound.
    ; We are able to trace down and find the surface of the water is visibility is on block, BUT the IK trace of the feet are also checking the visibility trace which will place the feet on the water surface if that visibility is set to block.
    ; So for shallow water, we bypass it by setting this boolean on and off based on overlap with water with the ShallowWater Trigger BP.
    ; We also check for the location to spawn the water ripples
    (bind (_outhit _returnvalue_4) (`KismetSystemLibrary.LineTraceSingleForObjects` _returnvalue_2 (- _returnvalue_3 (0.0 0.0 75.0)) (`|MakeArray` "ObjectTypeQuery2" :!type "EObjectTypeQuery Enum")))
    (if _returnvalue_4
      (bind (_bblockinghit _binitialoverlap _time _distance _location _impactpoint _normal _impactnormal _physmat _hitactor) (`GameplayStatics.BreakHitResult` _outhit))
      (cast `/Game/Hyper/FootstepSystem/Blueprints/BP_ShallowWater_Trigger` _hitactor
        (:`then`
          ;;[1 1 1] If there is a hit, return water surface
          (return true "SurfaceType4" _location))
        (:`CastFailed`
          _)))
    ;;[1 1 1] If there is no hit, return false
    (return false "SurfaceType_Default" (0.0 0.0 0.0))
    (else
      ;[1 1 1] Line trace from the foot location.
      ; We want to know the surface type on which the foot hits. This can be found in the physical material reference.
      ; We also want to know the location of the hit for particle and print effects.
      (bind (_outhit_2 _returnvalue_5) (`KismetSystemLibrary.LineTraceSingle` _returnvalue_2 _returnvalue_3 "TraceTypeQuery1"))
      (if _returnvalue_5
        ;[1 1 1] If there is a hit, return the surface type, location and true state
        (return true (`GameplayStatics.GetSurfaceType` _outhit_2) (`.Location` (`GameplayStatics.BreakHitResult` _outhit_2)))
        (else
          ;[1 1 1] If there is no hit, return false
          (return false "SurfaceType_Default" (0.0 0.0 0.0)))))))