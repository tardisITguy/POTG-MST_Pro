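; Trigger pad that switches the voice of a character entering its interact sphere.
; On overlap, it stops any playing voice by destroying the current voice sound, then has the cast third-person voice-system character remove its existing voice component.
; It then adds the configured component class to the character and plays a fixed dialogue through the controller's Character Voice Manager, interrupting existing dialogue.
; The construction script runs InitializeItem.
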(event `self.Interact_Area_Sphere.OnComponentBeginOverlap`
  (params (OverlappedComponent :type "PrimitiveComponent Object Reference") (OtherActor :type "Actor Object Reference") (OtherComp :type "PrimitiveComponent Object Reference") (OtherBodyIndex :type Integer) (bFromSweep :type Boolean) (SweepResult :type "HitResult Structure (by ref)"))
  (bind _returnvalue (`self.GetInstigatorController` OtherActor))
  (bind (_component _is_valid) (`/Game/Hyper/Core/Character_Voice/BlueprintMacroLibrary/BML_CharacterVoice_Controller.Get Character Voice Manager` _returnvalue))
  ;[0.05127 0.05127 0.05127] If there is a voice playing, destroy it first
  (`/Engine/EditorBlueprintResources/StandardMacros.IsValid` _returnvalue
    (:`Is Valid`
      (if _is_valid
        (bind _current_voice_sound_playing (`/Game/Hyper/Core/Character_Voice/Blueprints/AC_Character_Voice_System_Abstract.Current Voice Sound Playing` _component)
          (:`then`
            (`ActorComponent.K2_DestroyComponent` _current_voice_sound_playing))
          (:`else`
            _))
        ;[0.05127 0.05127 0.05127] Remove Existing Voice Component
        (bind _asbp_basic_third_person_character_character_voice_system (cast `/Game/Hyper/Locomotion/Chars/Mannequin_UE5/Blueprints/ExampleSystemCharacters/BP_Basic_ThirdPersonCharacter_CharacterVoiceSystem` OtherActor))
        (`/Game/Hyper/Locomotion/Chars/Mannequin_UE5/Blueprints/ExampleSystemCharacters/BP_Basic_ThirdPersonCharacter_CharacterVoiceSystem.Event Destroy Component` _asbp_basic_third_person_character_character_voice_system)
        ;[0.05127 0.05127 0.05127] Add new voice, and directly play a diaglogue
        ;;[0.05127 0.05127 0.05127] Add new voice component
        (`|AddComponentByClass` OtherActor (`self.Comppnent To Add`))
        (`/Game/Hyper/Core/Character_Voice/Blueprints/AC_Character_Voice_System_Abstract.Play Fixed Dialogue` (`/Game/Hyper/Core/Character_Voice/BlueprintMacroLibrary/BML_CharacterVoice_Controller.Get Character Voice Manager` (`self.GetInstigatorController` OtherActor)) (`self.Dialogue To Play`) true false)))))

(fn `UserConstructionScript`
  (`self.Initialize item`))