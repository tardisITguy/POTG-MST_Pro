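; Trigger pad Blueprint that plays a configured fixed dialogue when a character enters its interaction sphere.
; On overlap, it continues only if the actor's instigator controller is valid and local, so the dialogue triggers just for that local player.
; It passes the dialogue and its stop/same-dialogue flags to that controller's Character Voice Manager.
; The construction script runs InitializeItem to set up the pad.
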(event `self.Interact_Area_Sphere.OnComponentBeginOverlap`
  (params (OverlappedComponent :type "PrimitiveComponent Object Reference") (OtherActor :type "Actor Object Reference") (OtherComp :type "PrimitiveComponent Object Reference") (OtherBodyIndex :type Integer) (bFromSweep :type Boolean) (SweepResult :type "HitResult Structure (by ref)"))
  (bind _returnvalue (`self.GetInstigatorController` OtherActor))
  ;[0.05127 0.05127 0.05127] If there is a voice playing, destroy it first
  (`/Engine/EditorBlueprintResources/StandardMacros.IsValid` _returnvalue
    (:`Is Valid`
      (if (`Controller.IsLocalController` _returnvalue)
        ;;[0.05127 0.05127 0.05127] play a dialogue
        (`/Game/Hyper/Core/Character_Voice/Blueprints/AC_Character_Voice_System_Abstract.Play Fixed Dialogue` (`/Game/Hyper/Core/Character_Voice/BlueprintMacroLibrary/BML_CharacterVoice_Controller.Get Character Voice Manager` _returnvalue) (`self.Dialogue To Play`) (`self.Should Stop Existing Dialogues`) (`self.Should Not Stop When It Is The Same Dialogue`))))))

(fn `UserConstructionScript`
  (`self.Initialize item`))