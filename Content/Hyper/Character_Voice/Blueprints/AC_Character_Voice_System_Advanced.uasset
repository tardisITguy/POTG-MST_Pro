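; Character voice component that plays fixed dialogue lines, such as pain, taunts, kills and status barks, on the character mesh's head.
; A dialogue enum selects the sound, which a replication component attaches with shared attenuation and dialogue concurrency.
; Optionally, it stops the current line first, skipping requests for the same sound.
; A DoOnce gates these interrupting requests and resets when a new sound attaches or audio finishes.
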(event `self.Play Fixed Dialogue`
  (params (`Dialogue to play` :type "/Game/Hyper/Core/Character_Voice/Datamodel/Enumerations/Enum_Fixed_Dialogue Enum" :default "NewEnumerator0") (`Should stop existing Dialogues` :type Boolean) (`Should not stop when it is the same Dialogue` :type Boolean))
  (bind _sound (`self.Get Character Dialogue` `Dialogue to play`))
  (bind _component (`/Game/Hyper/Core/ReplicationSubSystem/BlueprintMacroLibrary/BML_Replication_Component.Get Replication`))
  ;[0.05127 0.05127 0.05127] Should stop current dialogues?
  (if `Should stop existing Dialogues`
    (`/Engine/EditorBlueprintResources/StandardMacros.DoOnce` false :!label _label
      (:`Completed`
        ;[0.05127 0.05127 0.05127] Should stop when new sound to play is the existing one?
        (bind _current_voice_sound_playing (`self.Current Voice Sound Playing`)
          (:`then`
            (if (and `Should not stop when it is the same Dialogue` (== (`AudioComponent.Sound` _current_voice_sound_playing) _sound))
              (`KismetSystemLibrary.PrintString` "Already playing this dialogue")
              (else
                ;[0.05127 0.05127 0.05127] If there is something playing, first stop it
                (`/Game/Hyper/Core/ReplicationSubSystem/Blueprints/AC_Replication_Abstract.Initialize Stop Attached Sound` (`/Game/Hyper/Core/ReplicationSubSystem/BlueprintMacroLibrary/BML_Replication_Component.Get Replication`) _current_voice_sound_playing)
                ;[0.05127 0.05127 0.05127] Always attach a dialogue to a character mesh. If you get an error here, think of on what you want to attach the dialogue sound
                (add `/Game/Hyper/Core/ReplicationSubSystem/Blueprints/AC_Replication_Abstract.Sound Attached` _component (delegate `Sound Attached_Event_0`) :!label _label_2)
                (`/Game/Hyper/Core/ReplicationSubSystem/Blueprints/AC_Replication_Abstract.Initialize Attach Sound` _component _sound (`/Game/Hyper/Core/Generic/BlueprintMacroLibrary/BML_Generic_Component.Get Character Mesh`) "head" "KeepRelativeOffset" true "/Game/Hyper/ResourcePack/Audio/AttenuationPresets/ATT_Default.ATT_Default" "/Game/Hyper/ResourcePack/Audio/Concurrency/SCON_Dialogues.SCON_Dialogues"))))
          (:`else`
            (goto _label_2)))))
    (else
      (goto _label_2))))

(event `Reset Do Once`
  ;[0.05127 0.05127 0.05127] Should stop current dialogues?
  (goto _label :!via `Reset`))

(event `Sound Attached_Event_0`
  (params (Sound :type "AudioComponent Object Reference"))
  ;[0.05127 0.05127 0.05127] Always attach a dialogue to a character mesh. If you get an error here, think of on what you want to attach the dialogue sound
  (bind _output_get (set `self.Current Voice Sound Playing` Sound))
  (`/Engine/EditorBlueprintResources/StandardMacros.IsValid` _output_get
    (:`Is Valid`
      (add `AudioComponent.OnAudioFinished` _output_get (delegate `On Audio Finished`))
      (`self.Reset Do Once`))))

(event `On Audio Finished`
  ;[0.05127 0.05127 0.05127] Always attach a dialogue to a character mesh. If you get an error here, think of on what you want to attach the dialogue sound
  (`self.Reset Do Once`))

(fn `Get Character Dialogue`
  (params (Dialogue :type "/Game/Hyper/Core/Character_Voice/Datamodel/Enumerations/Enum_Fixed_Dialogue Enum" :default "NewEnumerator0"))
  (returns (Sound :type "SoundBase Object Reference"))
  (return (select `/Game/Hyper/Core/Character_Voice/Datamodel/Enumerations/Enum_Fixed_Dialogue` (`local.Dialogue`) :`NewEnumerator0` (`self.Jump Land`) :`NewEnumerator1` (`self.Jump Land Heavy`) :`NewEnumerator2` (`self.Health Low `) :`NewEnumerator3` (`self.Death`) :`NewEnumerator4` (`self.Breathing Low Health `) :`NewEnumerator5` (`self.Health Critical`) :`NewEnumerator6` (`self.Health Saved`) :`NewEnumerator7` (`self.Revive`) :`NewEnumerator8` (`self.Healed`) :`NewEnumerator9` (`self.Buffed`) :`NewEnumerator10` (`self.Suffered Critical Hit`) :`NewEnumerator11` (`self.Killed Enemy`) :`NewEnumerator12` (`self.Killed Enemy First Blood`) :`NewEnumerator13` (`self.Killed Enemy Revenge`) :`NewEnumerator14` (`self.Killed Enemy Streak`) :`NewEnumerator15` (`self.Killed Enemy Shut Down`) :`NewEnumerator16` (`self.Level Up`) :`NewEnumerator17` (`self.Enough To Spent`) :`NewEnumerator18` (`self.Block`) :`NewEnumerator19` (`self.Attack`) :`NewEnumerator20` (`self.Taunt`) :`NewEnumerator21` (`self.Catchphrase`) :`NewEnumerator22` (`self.Cheer`) :`NewEnumerator23` (`self.Frustration`) :`NewEnumerator24` (`self.Laugh`) :`NewEnumerator25` (`self.Celebrate`) :`NewEnumerator26` (`self.Pain`) :`NewEnumerator27` (`self.Pain Heavy`) :`NewEnumerator28` (`self.Low Mana`) :`NewEnumerator29` (`self.No`) :`NewEnumerator30` (`self.Made a choice`) :`NewEnumerator31` (`self.Selecting an Option`) :`NewEnumerator32` (`self.Confirm`) :`NewEnumerator33` (`self.Bought Item`) :`NewEnumerator34` (`self.Need More Time`) :`NewEnumerator35` (`self.Used Last One`) :`NewEnumerator36` (`self.Breathing Run`) :`NewEnumerator37` (`self.Danger`) :`NewEnumerator38` (`self.Defeat`) :`NewEnumerator39` (`self.Idle`) :`NewEnumerator40` (`self.I will Return`) :`NewEnumerator41` (`self.Team Dead`) :`NewEnumerator42` (`self.Team Victory`) :`NewEnumerator43` (`self.Effort Primary`) :`NewEnumerator50` (`self.Effort Heavy`) :`NewEnumerator44` (`self.Enage`) :`NewEnumerator45` (`self.Ability 01`) :`NewEnumerator46` (`self.Ability 02`) :`NewEnumerator47` (`self.Ability 03`) :`NewEnumerator48` (`self.Ability 04`) :`NewEnumerator49` (`self.Ability 05`) :`NewEnumerator51` (`self.Thirsty`) :`NewEnumerator52` (`self.Hungry`) :`NewEnumerator53` (`self.Drowning`) :`NewEnumerator54` (`self.Sleepy`) :`NewEnumerator55` (`self.Low Magic`))))