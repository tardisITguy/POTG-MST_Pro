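; AI controller for humanoid NPCs that runs their behavior tree and respawns them after death.
; Once a valid pawn is possessed, it caches the pawn's class, starts BT_Humanoid_Basic, notifies the humanoid master pawn and binds to the attribute manager's death event.
; On death it stops logic, waits a random delay, spawns the same class at a random reachable nearby point, then destroys the old pawn and itself.
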(event `self.ReceiveBeginPlay`
  (`/Engine/EditorBlueprintResources/StandardMacros.IsValid` (`self.K2_GetPawn`)
    (:`Is Valid`
      (`self.Initialize`))
    (:`Is Not Valid`
      (add `self.OnPossessedPawnChanged` (delegate `On Pawn Changed`)))))

(event `On Pawn Changed` :!signature `self.OnPossessedPawnChanged`
  (params (OldPawn :type "Pawn Object Reference") (NewPawn :type "Pawn Object Reference"))
  (`/Engine/EditorBlueprintResources/StandardMacros.IsValid` NewPawn
    (:`Is Valid`
      (`self.Initialize`))))

(event `Initialize`
  (set `self.Class To Spawn` (`GameplayStatics.GetObjectClass` (`self.K2_GetPawn`)))
  (`self.RunBehaviorTree` "/Game/Hyper/AI/Humannoid_Basic/BT_Humanoid_Basic.BT_Humanoid_Basic")
  (bind _asbp_ai_humanoid_master (cast `/Game/Hyper/AI/Master/BP_AI_Humanoid_Master` (`self.K2_GetPawn`)))
  (`/Game/Hyper/AI/Master/BP_AI_Humanoid_Master.On Run Behaviour Tree` _asbp_ai_humanoid_master)
  ;[0.05127 0.05127 0.05127] On die, stop behavior tree
  (add `/Game/Hyper/Core/Attribute_System/Blueprints/AC_Attribute_Manager_Abstact.On Die` (`/Game/Hyper/Core/Attribute_System/BlueprintMacroLibrary/BML_Attribute__Controller.Get Attribute Manager` self) (delegate `On Die_Event`)))

(event `On Die_Event`
  ;[0.05127 0.05127 0.05127] On die, stop behavior tree
  (bind _braincomponent (`self.BrainComponent`)
    (:`then`
      (`BrainComponent.StopLogic` _braincomponent "Died")
      (`KismetSystemLibrary.Delay` (`KismetMathLibrary.RandomFloatInRange` 10.0 15.0))
      (`|SpawnActorFromClass` (`self.Class To Spawn`) (`KismetMathLibrary.MakeTransform` (`NavigationSystemV1.K2_GetRandomReachablePointInRadius` (`self.K2_GetActorLocation` (`self.K2_GetPawn`)) (`self.Respawn Radius`) null null)) "AdjustIfPossibleButAlwaysSpawn" "MultiplyWithRoot" null null)
      (`self.K2_DestroyActor` (`self.K2_GetPawn`))
      (`self.K2_DestroyActor`))
    (:`else`)))

(fn `UserConstructionScript`
  (`self.RunBehaviorTree` "/Game/Hyper/AI/Humannoid_Basic/BT_Humanoid_Basic.BT_Humanoid_Basic"))