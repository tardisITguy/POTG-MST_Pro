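; Deer AI creature that senses threats through sight, sound and damage, with flee behaviour driven by its behaviour tree.
; Seeds the blackboard with wander, follow and flee settings and walks slowly when the tree starts.
; With no valid threat held, a sensed pawn or attacker becomes the threat, updating the blackboard, raising speed and calling Spotted.
; Also has a server-only attack that damages overlapping characters through their attribute manager.
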(event `self.ReceiveBeginPlay`
  (`/Engine/EditorBlueprintResources/ActorMacros.Switch Has Authority`
    (:`Authority`
      (`PawnSensingComponent.SetSensingInterval` (`self.PawnSensing`) 0.1)
      (`PawnSensingComponent.SetSensingUpdatesEnabled` (`self.PawnSensing`) true))))

(event `On Run Behaviour Tree`
  (bind (_blackboard _blackboard_key_name_return) (`self.BB Data` "FleeDistance"))
  (bind (_blackboard_2 _blackboard_key_name_return_2) (`self.BB Data` "StartingLocation"))
  (bind (_blackboard_3 _blackboard_key_name_return_3) (`self.BB Data` "MaxFollowDistance"))
  (bind (_blackboard_4 _blackboard_key_name_return_4) (`self.BB Data` "WanderDistance"))
  (bind (_blackboard_5 _blackboard_key_name_return_5) (`self.BB Data` "FleeRange"))
  (bind (_blackboard_6 _blackboard_key_name_return_6) (`self.BB Data` "ShouldFlee"))
  (`/Engine/EditorBlueprintResources/StandardMacros.IsValid` (`AIBlueprintHelperLibrary.GetBlackboard` (`AIBlueprintHelperLibrary.GetAIController` self))
    (:`Is Valid`
      ;[0.05098 0.05098 0.05098] Set all blackboard values
      (`BlackboardComponent.SetValueAsFloat` _blackboard_4 _blackboard_key_name_return_4 (`self.Maximum Wander Distance`))
      (`BlackboardComponent.SetValueAsBool` _blackboard_6 _blackboard_key_name_return_6 (`self.Should Flee`))
      (`BlackboardComponent.SetValueAsVector` _blackboard_2 _blackboard_key_name_return_2 (`self.K2_GetActorLocation`))
      (`BlackboardComponent.SetValueAsFloat` _blackboard_3 _blackboard_key_name_return_3 (`self.Max Follow Distance`))
      (`BlackboardComponent.SetValueAsFloat` _blackboard_5 _blackboard_key_name_return_5 (`self.Flee Range`))
      (`BlackboardComponent.SetValueAsFloat` _blackboard _blackboard_key_name_return (`self.Flee Distance`))
      (set `CharacterMovementComponent.MaxWalkSpeed` 150.0 (`self.CharacterMovement`)))))

(event `self.PawnSensing.OnHearNoise`
  (params (Instigator :type "Pawn Object Reference") (Location :type "Vector Structure (by ref)") (Volume :type "Float (single-precision)"))
  (bind (_blackboard _blackboard_key_name_return) (`self.BB Data` "WasAttacked"))
  (bind (_blackboard_2 _blackboard_key_name_return_2) (`self.BB Data` "Threat"))
  (`/Engine/EditorBlueprintResources/StandardMacros.IsValid` (`self.Threat Pawn`)
    (:`Is Not Valid`
      (set `self.Threat Pawn` Instigator)
      (`BlackboardComponent.SetValueAsObject` _blackboard_2 _blackboard_key_name_return_2 (`self.Threat Pawn`) :!label _label)
      (set `CharacterMovementComponent.MaxWalkSpeed` 750.0 (`self.CharacterMovement`))
      (`self.Spotted`)
      (`BlackboardComponent.SetValueAsBool` _blackboard _blackboard_key_name_return (`self.Was Attacked`)))))

(event `self.PawnSensing.OnSeePawn`
  (params (Pawn :type "Pawn Object Reference"))
  (set `self.Was Attacked` false)
  (`/Engine/EditorBlueprintResources/StandardMacros.IsValid` (`self.Threat Pawn`)
    (:`Is Not Valid`
      (set `self.Threat Pawn` Pawn)
      (goto _label))))

(event `self.ReceiveAnyDamage`
  (params (Damage :type "Float (single-precision)") (DamageType :type "DamageType Object Reference") (InstigatedBy :type "Controller Object Reference") (DamageCauser :type "Actor Object Reference"))
  (set `self.Was Attacked` true)
  (`/Engine/EditorBlueprintResources/StandardMacros.IsValid` (`self.Threat Pawn`)
    (:`Is Not Valid`
      (set `self.Threat Pawn` (`Controller.K2_GetPawn` InstigatedBy))
      (goto _label))))

(fn `BB Data`
  (params (`Blackboard Key Name` :type Name))
  (returns (Blackboard :type "BlackboardComponent Object Reference") (`Blackboard Key Name Return` :type Name))
  (return (`AIBlueprintHelperLibrary.GetBlackboard` (`AIBlueprintHelperLibrary.GetAIController` self)) (`KismetSystemLibrary.MakeLiteralName` `Blackboard Key Name`)))

(fn `Do Attack`
  (`/Engine/EditorBlueprintResources/ActorMacros.Switch Has Authority`
    (:`Authority`
      (for _array_element (`PrimitiveComponent.GetOverlappingActors` (`self.Sphere`) "/Script/Engine.Character")
        (bind _returnvalue (`self.GetComponentByClass` _array_element "/Game/Hyper/Core/Attribute_System/Blueprints/AC_Attribute_Manager_Abstact.AC_Attribute_Manager_Abstact_C"))
        (`/Engine/EditorBlueprintResources/StandardMacros.IsValid` _returnvalue
          (:`Is Valid`
            (`/Game/Hyper/Core/Attribute_System/Blueprints/AC_Attribute_Manager_Abstact.On Take Damage` _returnvalue _array_element (`self.Damage`) null (`AIBlueprintHelperLibrary.GetAIController` self) self)))))))

(fn `Get_PawnName`
  (returns (PawnName :type Name))
  (return "Deer"))

(fn `Get_Relative_Widget_Position`
  (returns (`Relative Location` :type "Vector Structure"))
  (return (0.0 0.0 100.0)))

(fn `Should_Receive_Pawn_Info`
  (returns (True :type Boolean))
  (return true))

(fn `UserConstructionScript`)