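; AI controller for the deer creature that runs its behavior tree and handles death and respawn.
; It initializes on BeginPlay, or when possession changes, recording the pawn's class, starting BT_Deer and binding to the attribute manager's death event.
; On death it stops the brain, waits a random delay, spawns a replacement at a random reachable point nearby, then destroys the pawn and itself.
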(event `self.ReceiveBeginPlay`
  (`/Engine/EditorBlueprintResources/StandardMacros.IsValid` (`self.K2_GetPawn`)
    (:`Is Valid`
      (`self.Initialize`))
    (:`Is Not Valid`
      (add `self.OnPossessedPawnChanged` (delegate `On Possessed Pawn Changed`)))))

(event `On Possessed Pawn Changed` :!signature `self.OnPossessedPawnChanged`
  (params (OldPawn :type "Pawn Object Reference") (NewPawn :type "Pawn Object Reference"))
  (`/Engine/EditorBlueprintResources/StandardMacros.IsValid` NewPawn
    (:`Is Valid`
      (`self.Initialize`))))

(event `Initialize`
  (set `self.Class To Spawn` (`GameplayStatics.GetObjectClass` (`self.K2_GetPawn`)))
  (`self.RunBehaviorTree` "/Game/Hyper/AI/Creature/Deer/BT_Deer.BT_Deer")
  (bind _asbp_ai_deer (cast `/Game/Hyper/AI/Creature/Deer/BP_AI_Deer` (`self.K2_GetPawn`)))
  (`/Game/Hyper/AI/Creature/Deer/BP_AI_Deer.On Run Behaviour Tree` _asbp_ai_deer)
  (add `/Game/Hyper/Core/Attribute_System/Blueprints/AC_Attribute_Manager_Abstact.On Die` (`/Game/Hyper/Core/Attribute_System/BlueprintMacroLibrary/BML_Attribute__Controller.Get Attribute Manager` self) (delegate `On Die`)))

(event `On Die`
  (`BrainComponent.StopLogic` (`self.BrainComponent`) "Died")
  (`KismetSystemLibrary.Delay` (`KismetMathLibrary.RandomFloatInRange` 10.0 15.0))
  (`|SpawnActorFromClass` (`self.Class To Spawn`) (`KismetMathLibrary.MakeTransform` (`NavigationSystemV1.K2_GetRandomReachablePointInRadius` (`self.K2_GetActorLocation` (`self.K2_GetPawn`)) (`self.Respawn Radius`) null null)) "AdjustIfPossibleButAlwaysSpawn" "MultiplyWithRoot" self null)
  (`self.K2_DestroyActor` (`self.K2_GetPawn`))
  (`self.K2_DestroyActor`))

(fn `UserConstructionScript`)