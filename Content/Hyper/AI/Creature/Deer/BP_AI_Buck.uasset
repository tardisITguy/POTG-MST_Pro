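; BP_AI_Buck is a child Blueprint for the male deer AI creature.
; Its construction script runs the parent's, then attaches a static mesh to the Antlers socket on the main mesh.
; Function overrides supply the name "Buck", opt in to receiving pawn info and set a relative widget position above the origin.
; The event graph holds only disabled placeholder events, so it adds no runtime logic of its own.
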(fn `Get_PawnName`
  (returns (PawnName :type Name))
  (return "Buck"))

(fn `Get_Relative_Widget_Position`
  (returns (`Relative Location` :type "Vector Structure"))
  (return (0.0 0.0 100.0)))

(fn `Should_Receive_Pawn_Info`
  (returns (True :type Boolean))
  (return true))

(fn `UserConstructionScript`
  (`parent.UserConstructionScript`)
  (`SceneComponent.K2_AttachToComponent` (`self.StaticMesh`) (`self.Mesh`) "Antlers" "KeepRelative" "KeepRelative" "KeepRelative" true))