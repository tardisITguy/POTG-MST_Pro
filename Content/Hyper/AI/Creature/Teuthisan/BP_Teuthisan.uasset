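; Teuthisan AI creature that wanders slowly until it acquires a threat, then speeds up and can deal area melee damage.
; When its behavior tree runs, it seeds blackboard limits and plays a replicated stand-up montage, flagging completion.
; Hearing, sight or damage sets the threat if none is valid, updating the blackboard and calling Spotted.
; DoAttack runs server-side, damaging sphere-overlapped characters through their attribute manager components.
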(event `self.ReceiveBeginPlay`
  (`/Engine/EditorBlueprintResources/ActorMacros.Switch Has Authority`
    (:`Authority`
      (`/Engine/EditorBlueprintResources/StandardMacros.IsValid` (`AIBlueprintHelperLibrary.GetAIController` self)
        (:`Is Not Valid`
          (`self.SpawnDefaultController`))))))

(event `On Run Behaviour Tree`
  (bind (_blackboard _blackboard_key_name_return) (`self.BB Data` "StartingLocation"))
  (bind (_blackboard_2 _blackboard_key_name_return_2) (`self.BB Data` "ShouldFlee"))
  (bind (_blackboard_3 _blackboard_key_name_return_3) (`self.BB Data` "WanderDistance"))
  (bind (_blackboard_4 _blackboard_key_name_return_4) (`self.BB Data` "MaxFollowDistance"))
  (bind _ac_replication_subsystem (`self.AC_Replication_SubSystem`))
  (`/Engine/EditorBlueprintResources/StandardMacros.IsValid` (`AIBlueprintHelperLibrary.GetBlackboard` (`AIBlueprintHelperLibrary.GetAIController` self))
    (:`Is Valid`
      (`BlackboardComponent.SetValueAsFloat` _blackboard_3 _blackboard_key_name_return_3 (`self.Maximum Wander Distance`))
      (`BlackboardComponent.SetValueAsVector` _blackboard _blackboard_key_name_return (`self.K2_GetActorLocation`))
      (`BlackboardComponent.SetValueAsFloat` _blackboard_4 _blackboard_key_name_return_4 (`self.Max Follow Distance`))
      (`BlackboardComponent.SetValueAsBool` _blackboard_2 _blackboard_key_name_return_2 false)
      (set `CharacterMovementComponent.MaxWalkSpeed` 150.0 (`self.CharacterMovement`))
      (`/Game/Hyper/Core/ReplicationSubSystem/Blueprints/AC_Replication_Abstract.Initialize Multicast Latent Montage` :`self` _ac_replication_subsystem :`Montage To Play` "/Game/Hyper/AI/Creature/Teuthisan/Animations/Anim_Teuthisan_Standup_Montage.Anim_Teuthisan_Standup_Montage")
      (add `/Game/Hyper/Core/ReplicationSubSystem/Blueprints/AC_Replication_Abstract.Montage Finished` _ac_replication_subsystem (delegate `Montage Finished_Event`)))))

(event `Montage Finished_Event`
  (bind (_blackboard _blackboard_key_name_return) (`self.BB Data` "IsStandupFinished"))
  (`BlackboardComponent.SetValueAsBool` _blackboard _blackboard_key_name_return true)
  (remove `/Game/Hyper/Core/ReplicationSubSystem/Blueprints/AC_Replication_Abstract.Montage Finished` (`self.AC_Replication_SubSystem`) (delegate `Montage Finished_Event`)))

(event `self.PawnSensing.OnHearNoise`
  (params (Instigator :type "Pawn Object Reference") (Location :type "Vector Structure (by ref)") (Volume :type "Float (single-precision)"))
  (bind (_blackboard _blackboard_key_name_return) (`self.BB Data` "Threat"))
  (`/Engine/EditorBlueprintResources/StandardMacros.IsValid` (`self.Threat Pawn`)
    (:`Is Not Valid`
      (set `self.Threat Pawn` Instigator)
      (set `CharacterMovementComponent.MaxWalkSpeed` 1250.0 (`self.CharacterMovement`) :!label _label)
      (`BlackboardComponent.SetValueAsObject` _blackboard _blackboard_key_name_return (`self.Threat Pawn`))
      (`self.Spotted`))))

(event `self.PawnSensing.OnSeePawn`
  (params (Pawn :type "Pawn Object Reference"))
  (`/Engine/EditorBlueprintResources/StandardMacros.IsValid` (`self.Threat Pawn`)
    (:`Is Not Valid`
      (set `self.Threat Pawn` Pawn)
      (goto _label))))

(event `self.ReceiveAnyDamage`
  (params (Damage :type "Float (single-precision)") (DamageType :type "DamageType Object Reference") (InstigatedBy :type "Controller Object Reference") (DamageCauser :type "Actor Object Reference"))
  (`/Engine/EditorBlueprintResources/StandardMacros.IsValid` (`self.Threat Pawn`)
    (:`Is Not Valid`
      (set `self.Threat Pawn` (`Controller.K2_GetPawn` InstigatedBy))
      (goto _label))))

(fn `BB Data`
  (params (`Blackboard Key Name` :type Name))
  (returns (Blackboard :type "BlackboardComponent Object Reference") (`Blackboard Key Name Return` :type Name))
  (return (`AIBlueprintHelperLibrary.GetBlackboard` (`AIBlueprintHelperLibrary.GetAIController` self)) (`KismetSystemLibrary.MakeLiteralName` `Blackboard Key Name`)))

(fn `Do Attack`
  (`/Engine/EditorBlueprintResources/ActorMacros.Switch Has Authority`
    (:`Authority`
      (for _array_element (`PrimitiveComponent.GetOverlappingActors` (`self.Sphere`) "/Script/Engine.Character")
        (bind _returnvalue (`self.GetComponentByClass` _array_element "/Game/Hyper/Core/Attribute_System/Blueprints/AC_Attribute_Manager_Abstact.AC_Attribute_Manager_Abstact_C"))
        (`/Engine/EditorBlueprintResources/StandardMacros.IsValid` _returnvalue
          (:`Is Valid`
            (`/Game/Hyper/Core/Attribute_System/Blueprints/AC_Attribute_Manager_Abstact.On Take Damage` _returnvalue _array_element (`self.Damage`) null (`AIBlueprintHelperLibrary.GetAIController` self) self)))))))

(fn `Get_PawnName`
  (returns (PawnName :type Name))
  (return "Teuthisan"))

(fn `Get_Relative_Widget_Position`
  (returns (`Relative Location` :type "Vector Structure"))
  (return (0.0 0.0 100.0)))

(fn `Should_Receive_Pawn_Info`
  (returns (True :type Boolean))
  (return true))

(fn `UserConstructionScript`)