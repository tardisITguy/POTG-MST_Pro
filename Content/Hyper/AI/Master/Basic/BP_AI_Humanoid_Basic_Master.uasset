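; Basic master Blueprint for humanoid AI characters that spawns them armed with a random melee weapon.
; On BeginPlay, after the parent logic, only the authority picks one of seven data table item entries (swords, longsword, dagger, knife).
; The basic equipment manager component equips it without animation, bypassing the equip-in-progress check.
; Iron sword and longsword each appear twice, doubling their odds.
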(event `self.ReceiveBeginPlay`
  ;[0.05127 0.05127 0.05127] Equip a weapon
  (`parent.ReceiveBeginPlay`)
  (`/Engine/EditorBlueprintResources/ActorMacros.Switch Has Authority`
    (:`Authority`
      (`/Game/Hyper/Equipment_Manager/Blueprints/AC_Equipment_Manager_Basic.Equip Weapon without animation` (`self.AC_Equipment_Manager_Basic`) (select `int` (`KismetMathLibrary.RandomIntegerInRange` 0 6) :`0` (make `/Game/Hyper/Core/Inventory/Datamodel/Structures/Main_Item_Slot_Structs/Struct_Inventory_Slot_Item` (make `DataTableRowHandle` "/Game/Hyper/Core/Inventory/Datamodel/Datatables/DT_Items.DT_Items" "Basic_Wooden_Sword") 1 0 false (struct :`CurrentDurability` 100.0 :`IsUseable` true) (struct :`Chanceofspawinginvendorinventory` 1.0 :`MinimalAmounttorestock` 1 :`MaximumAmounttorestock` 5 :`MaximumStock` 10) true null (struct :`Hotbarslotindex` 999 :`Inventoryslotindex` 999) (struct :`Linkedtothisequipmentslot` "NewEnumerator13" :`AmmoSlot` (struct :`AmmoDataTable` (struct :`DataTable` "/Script/Engine.DataTable'/Game/Hyper/Core/Equipment_Manager/Datamodel/Datatables/DT_Ammo.DT_Ammo'")))) :`1` (make `/Game/Hyper/Core/Inventory/Datamodel/Structures/Main_Item_Slot_Structs/Struct_Inventory_Slot_Item` (make `DataTableRowHandle` "/Game/Hyper/Core/Inventory/Datamodel/Datatables/DT_Items.DT_Items" "Basic_Iron_Sword") 1 0 false (struct :`CurrentDurability` 100.0 :`IsUseable` true) (struct :`Chanceofspawinginvendorinventory` 1.0 :`MinimalAmounttorestock` 1 :`MaximumAmounttorestock` 5 :`MaximumStock` 10) true null (struct :`Hotbarslotindex` 999 :`Inventoryslotindex` 999) (struct :`Linkedtothisequipmentslot` "NewEnumerator13" :`AmmoSlot` (struct :`AmmoDataTable` (struct :`DataTable` "/Script/Engine.DataTable'/Game/Hyper/Core/Equipment_Manager/Datamodel/Datatables/DT_Ammo.DT_Ammo'")))) :`2` (make `/Game/Hyper/Core/Inventory/Datamodel/Structures/Main_Item_Slot_Structs/Struct_Inventory_Slot_Item` (make `DataTableRowHandle` "/Game/Hyper/Core/Inventory/Datamodel/Datatables/DT_Items.DT_Items" "Basic_Iron_Longsword") 1 0 false (struct :`CurrentDurability` 100.0 :`IsUseable` true) (struct :`Chanceofspawinginvendorinventory` 1.0 :`MinimalAmounttorestock` 1 :`MaximumAmounttorestock` 5 :`MaximumStock` 10) true null (struct :`Hotbarslotindex` 999 :`Inventoryslotindex` 999) (struct :`Linkedtothisequipmentslot` "NewEnumerator13" :`AmmoSlot` (struct :`AmmoDataTable` (struct :`DataTable` "/Script/Engine.DataTable'/Game/Hyper/Core/Equipment_Manager/Datamodel/Datatables/DT_Ammo.DT_Ammo'")))) :`3` (make `/Game/Hyper/Core/Inventory/Datamodel/Structures/Main_Item_Slot_Structs/Struct_Inventory_Slot_Item` (make `DataTableRowHandle` "/Game/Hyper/Core/Inventory/Datamodel/Datatables/DT_Items.DT_Items" "Basic_Iron_Dagger") 1 0 false (struct :`CurrentDurability` 100.0 :`IsUseable` true) (struct :`Chanceofspawinginvendorinventory` 1.0 :`MinimalAmounttorestock` 1 :`MaximumAmounttorestock` 5 :`MaximumStock` 10) true null (struct :`Hotbarslotindex` 999 :`Inventoryslotindex` 999) (struct :`Linkedtothisequipmentslot` "NewEnumerator13" :`AmmoSlot` (struct :`AmmoDataTable` (struct :`DataTable` "/Script/Engine.DataTable'/Game/Hyper/Core/Equipment_Manager/Datamodel/Datatables/DT_Ammo.DT_Ammo'")))) :`4` (make `/Game/Hyper/Core/Inventory/Datamodel/Structures/Main_Item_Slot_Structs/Struct_Inventory_Slot_Item` (make `DataTableRowHandle` "/Game/Hyper/Core/Inventory/Datamodel/Datatables/DT_Items.DT_Items" "Basic_Iron_Longsword") 1 0 false (struct :`CurrentDurability` 100.0 :`IsUseable` true) (struct :`Chanceofspawinginvendorinventory` 1.0 :`MinimalAmounttorestock` 1 :`MaximumAmounttorestock` 5 :`MaximumStock` 10) true null (struct :`Hotbarslotindex` 999 :`Inventoryslotindex` 999) (struct :`Linkedtothisequipmentslot` "NewEnumerator13" :`AmmoSlot` (struct :`AmmoDataTable` (struct :`DataTable` "/Script/Engine.DataTable'/Game/Hyper/Core/Equipment_Manager/Datamodel/Datatables/DT_Ammo.DT_Ammo'")))) :`5` (make `/Game/Hyper/Core/Inventory/Datamodel/Structures/Main_Item_Slot_Structs/Struct_Inventory_Slot_Item` (make `DataTableRowHandle` "/Game/Hyper/Core/Inventory/Datamodel/Datatables/DT_Items.DT_Items" "Basic_Iron_Sword") 1 0 false (struct :`CurrentDurability` 100.0 :`IsUseable` true) (struct :`Chanceofspawinginvendorinventory` 1.0 :`MinimalAmounttorestock` 1 :`MaximumAmounttorestock` 5 :`MaximumStock` 10) true null (struct :`Hotbarslotindex` 999 :`Inventoryslotindex` 999) (struct :`Linkedtothisequipmentslot` "NewEnumerator13" :`AmmoSlot` (struct :`AmmoDataTable` (struct :`DataTable` "/Script/Engine.DataTable'/Game/Hyper/Core/Equipment_Manager/Datamodel/Datatables/DT_Ammo.DT_Ammo'")))) :`6` (make `/Game/Hyper/Core/Inventory/Datamodel/Structures/Main_Item_Slot_Structs/Struct_Inventory_Slot_Item` (make `DataTableRowHandle` "/Game/Hyper/Core/Inventory/Datamodel/Datatables/DT_Items.DT_Items" "Knife") 1 0 false (struct :`CurrentDurability` 100.0 :`IsUseable` true) (struct :`Chanceofspawinginvendorinventory` 1.0 :`MinimalAmounttorestock` 1 :`MaximumAmounttorestock` 5 :`MaximumStock` 10) true null (struct :`Hotbarslotindex` 999 :`Inventoryslotindex` 999) (struct :`Linkedtothisequipmentslot` "NewEnumerator13" :`AmmoSlot` (struct :`AmmoDataTable` (struct :`DataTable` "/Script/Engine.DataTable'/Game/Hyper/Core/Equipment_Manager/Datamodel/Datatables/DT_Ammo.DT_Ammo'"))))) true))))

(fn `UserConstructionScript`
  (`parent.UserConstructionScript`))