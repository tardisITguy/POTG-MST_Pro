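; Master Blueprint for humanoid AI enemies that roam and react when they sense a player.
; On behaviour tree start it seeds the Blackboard with roaming range, default behaviour and start location, and sets a slow walk.
; Server-enabled PawnSensing locks onto the first seen or heard Player-tagged pawn as Enemy, speeds up movement and calls a Spotted hook for AI Blueprints.
; Sight also triggers a voice taunt when a voice manager exists.
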(event `self.ReceiveBeginPlay`
  (`/Engine/EditorBlueprintResources/ActorMacros.Switch Has Authority`
    (:`Authority`
      (`PawnSensingComponent.SetSensingInterval` (`self.PawnSensing`) 0.1)
      (`PawnSensingComponent.SetSensingUpdatesEnabled` (`self.PawnSensing`) true))))

(event `On Run Behaviour Tree`
  (bind (_blackboard _blackboard_key_name_return) (`self.BB Data` "Default_Behaviour"))
  (bind (_blackboard_2 _blackboard_key_name_return_2) (`self.BB Data` "Start_Location"))
  (bind (_blackboard_3 _blackboard_key_name_return_3) (`self.BB Data` "Roaming_Range"))
  (`/Engine/EditorBlueprintResources/StandardMacros.IsValid` (`AIBlueprintHelperLibrary.GetBlackboard` (`AIBlueprintHelperLibrary.GetAIController` self))
    (:`Is Valid`
      ;[0.05127 0.05127 0.05127] On initialize, set blackboard values
      (set `self.Start_Location` (`self.K2_GetActorLocation`))
      (`/Engine/EditorBlueprintResources/StandardMacros.IsValid` _blackboard_3
        (:`Is Valid`
          (`BlackboardComponent.SetValueAsFloat` _blackboard_3 _blackboard_key_name_return_3 (`self.Maximum_Wander_Distance`))
          (`BlackboardComponent.SetValueAsEnum` _blackboard _blackboard_key_name_return (`self.Default_Behaviour`))
          (`BlackboardComponent.SetValueAsVector` _blackboard_2 _blackboard_key_name_return_2 (`self.Start_Location`))
          (set `CharacterMovementComponent.MaxWalkSpeed` 100.0 (`self.CharacterMovement`)))))))

(event `self.PawnSensing.OnHearNoise`
  (params (Instigator :type "Pawn Object Reference") (Location :type "Vector Structure (by ref)") (Volume :type "Float (single-precision)"))
  (bind (_blackboard _blackboard_key_name_return) (`self.BB Data` "Enemy"))
  (if (`self.ActorHasTag` Instigator "Player")
    ;[0.05127 0.05127 0.05127] If there is no enemy pawn yet selected, set the pawn reference to the sensed pawn
    (`self.Enemy Pawn`
      (:`then`)
      (:`else`
        (set `self.Enemy Pawn` Instigator)
        ;[0.05127 0.05127 0.05127] Set the enemy object reference in the blackboard of the AI
        (`BlackboardComponent.SetValueAsObject` _blackboard _blackboard_key_name_return (`self.Enemy Pawn`) :!label _label)
        ;[0.05127 0.05127 0.05127] If an enemy is spotted, increase the walkspeed
        (set `CharacterMovementComponent.MaxWalkSpeed` 500.0 (`self.CharacterMovement`))
        ;[0.05127 0.05127 0.05127] Call event spotted, can be used in AI BP
        (`self.Spotted`)))))

(event `self.PawnSensing.OnSeePawn`
  (params (Pawn :type "Pawn Object Reference"))
  (bind (_component _is_valid) (`/Game/Hyper/Core/Character_Voice/BlueprintMacroLibrary/BML_CharacterVoice_Controller.Get Character Voice Manager` (`self.GetController`)))
  ;[0.05127 0.05127 0.05127] Check if the pawn that has been seen by the pawnsensing component = player
  (if (`self.ActorHasTag` Pawn "Player")
    ;[0.05127 0.05127 0.05127] If there is no enemy pawn yet selected, set the pawn reference to the sensed pawn
    (`self.Enemy Pawn`
      (:`then`)
      (:`else`
        (set `self.Enemy Pawn` Pawn)
        ;[0.05127 0.05127 0.05127] add taunt voice here
        (if _is_valid
          (`/Game/Hyper/Core/Character_Voice/Blueprints/AC_Character_Voice_System_Abstract.Play Fixed Dialogue` _component "NewEnumerator20" true false)
          (goto _label)
          (else
            (goto _label)))))))

(fn `BB Data`
  (params (`Blackboard Key Name` :type Name))
  (returns (Blackboard :type "BlackboardComponent Object Reference") (`Blackboard Key Name Return` :type Name))
  (return (`AIBlueprintHelperLibrary.GetBlackboard` (`AIBlueprintHelperLibrary.GetAIController` self)) (`KismetSystemLibrary.MakeLiteralName` `Blackboard Key Name`)))

(fn `Get_Blackboard_Key_Data_0`
  (params (`Blackboard Key Name` :type Name))
  (returns (Blackboard :type "BlackboardComponent Object Reference") (`Blackboard Key Name Return` :type Name))
  (return (`AIBlueprintHelperLibrary.GetBlackboard` (`AIBlueprintHelperLibrary.GetAIController` self)) (`KismetSystemLibrary.MakeLiteralName` `Blackboard Key Name`)))

(fn `Get_PawnName`
  (returns (PawnName :type Name))
  (return "Enemy"))

(fn `Get_Relative_Widget_Position`
  (returns (`Relative Location` :type "Vector Structure"))
  (return (0.0 0.0 125.0)))

(fn `Should_Receive_Pawn_Info`
  (returns (True :type Boolean))
  (return true))

(fn `UserConstructionScript`)