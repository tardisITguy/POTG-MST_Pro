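; Vendor component that runs item trades between player and vendor inventories, each found as the owner's inventory component.
; Trade actions map to quantities, then buy by slot index or automatically after checking buyer funds and seller stock, swapping items and price resource.
; Unit cost scales base sell price by the vendor's buy or sell multiplier and floored durability ratio.
; BeginPlay flags player ownership and warns non-players lacking an item allocator.
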(event `self.ReceiveBeginPlay`
  ;[0.05098 0.05098 0.05098] Set Is Player by linked inventory type, this is later used to determine which trade actions can be performed
  (bind _output_get (set `self.Is Player` (`|EnumEquality` (`/Game/Hyper/Core/Inventory/Blueprints/AC_Inventory_Abstract.Inventory Type` (`self.Get Vendor Inventory` self)) "NewEnumerator0")))
  (if (not _output_get)
    (`/Engine/EditorBlueprintResources/StandardMacros.IsValid` (`Actor.GetComponentByClass` (`self.GetOwner`) "/Game/Hyper/Core/ItemAllocator/Blueprints/AC_Item_Allocator_Abstract.AC_Item_Allocator_Abstract_C")
      (:`Is Not Valid`
        (`KismetSystemLibrary.PrintString` "Warning: Missing Item Allocator Component On Vendor")))))

(event `self.Event: Process Buy Item By Trade Action`
  (params (Seller :type "/Game/Hyper/Core/Vendor/Blueprints/AC_Vendor_Abstract Object Reference") (Buyer :type "/Game/Hyper/Core/Vendor/Blueprints/AC_Vendor_Abstract Object Reference") (`Trade Action` :type "/Game/Hyper/Core/Vendor/Datamodel/Enumerations/Enum_Trading_Action_Types Enum" :default "NewEnumerator7") (Item :type "/Game/Hyper/Core/Inventory/Datamodel/Structures/Main_Item_Slot_Structs/Struct_Inventory_Slot_Item Structure") (`Custom Amount` :type Integer) (`Slot Index` :type Integer))
  (`self.Process Buy Item By Trade Action` Seller Buyer `Trade Action` Item `Custom Amount` `Slot Index`))

(event `self.Event: Try Buy Item From Seller By Slot Index`
  (params (Seller :type "/Game/Hyper/Core/Vendor/Blueprints/AC_Vendor_Abstract Object Reference") (Buyer :type "/Game/Hyper/Core/Vendor/Blueprints/AC_Vendor_Abstract Object Reference") (Item :type "/Game/Hyper/Core/Inventory/Datamodel/Structures/Main_Item_Slot_Structs/Struct_Inventory_Slot_Item Structure") (Amount :type Integer) (`Slot Index` :type Integer))
  (`self.Try Buy Item From Seller By Slot Index` Seller Buyer Item Amount `Slot Index`))

(event `self.Event: Try To Automatically Buy Item From Seller`
  (params (Seller :type "/Game/Hyper/Core/Vendor/Blueprints/AC_Vendor_Abstract Object Reference") (Buyer :type "/Game/Hyper/Core/Vendor/Blueprints/AC_Vendor_Abstract Object Reference") (Item :type "/Game/Hyper/Core/Inventory/Datamodel/Structures/Main_Item_Slot_Structs/Struct_Inventory_Slot_Item Structure") (Amount :type Integer))
  (`self.Try To Automatically Buy Item From Seller` Seller Buyer Item Amount))

(fn `Calculate Sell Cost Of Single Item`
  (params (Seller :type "/Game/Hyper/Core/Vendor/Blueprints/AC_Vendor_Abstract Object Reference") (Buyer :type "/Game/Hyper/Core/Vendor/Blueprints/AC_Vendor_Abstract Object Reference") (Item :type "/Game/Hyper/Core/Inventory/Datamodel/Structures/Main_Item_Slot_Structs/Struct_Inventory_Slot_Item Structure"))
  (returns (Cost :type "Float (double-precision)") (`Rounded Cost` :type Integer) (Resource :type "/Game/Hyper/Core/Inventory/Datamodel/Structures/Main_Item_Slot_Structs/Struct_Inventory_Slot_Item Structure"))
  (bind _item (`local.Item`))
  (bind ((`BaseSellPrice_4_3768EC174F3117D4A0D57FBC4470C756` _basesellprice)) (break `/Game/Hyper/Core/Inventory/Datamodel/Structures/Sub_Structs_Attributes/Struct_Attributes_Sellable` (`.Sellable_Attributes_17_F8DD5673423CE0A266B8DA941969B77D` (break `/Game/Hyper/Core/Inventory/Datamodel/Structures/Main_Item_Slot_Structs/Struct_Item` (`/Game/Hyper/Core/Inventory/FunctionLibraries/BFL_InventoryCrafting.Get Inventory info from inventory slot` (`local.Item`))))))
  (bind (_hasdurability _maxdurability) (break `/Game/Hyper/Core/Inventory/Datamodel/Structures/Sub_Structs_Attributes/Struct_Attributes_Durability` (`.DurabilityAttributes_11_8BFC98204F44DCE1D7ADD68E766FA9F8` (break `/Game/Hyper/Core/Inventory/Datamodel/Structures/Main_Item_Slot_Structs/Struct_Item` (`/Game/Hyper/Core/Inventory/FunctionLibraries/BFL_InventoryCrafting.Get Inventory info from inventory slot` _item)))))
  (bind _returnvalue (* (`KismetMathLibrary.Conv_IntToDouble` (`.Amount_5_3D501FFE494086BDD8C291A969150384` (break `/Game/Hyper/Core/Inventory/Datamodel/Structures/Main_Item_Slot_Structs/Struct_Inventory_Slot_Item` _basesellprice))) (* (select `bool` (`|EnumEquality` (`/Game/Hyper/Core/Inventory/Blueprints/AC_Inventory_Abstract.Inventory Type` (`self.Get Vendor Inventory` (`local.Seller`))) "NewEnumerator5") :`false` (`/Game/Hyper/Core/Vendor/Blueprints/AC_Vendor_Abstract.Player Sell Multiplier` (`local.Buyer`)) :`true` (`/Game/Hyper/Core/Vendor/Blueprints/AC_Vendor_Abstract.Player Buy Multiplier` (`local.Seller`))) (select `bool` _hasdurability :`false` 1.0 :`true` (`KismetMathLibrary.FMax` (/ (`.CurrentDurability_8_EAC98CE74E6B1BA6EBE8DC86CE9A5442` (break `/Game/Hyper/Core/Inventory/Datamodel/Structures/Main_Item_Slot_Structs/Struct_Slot_Durability` (`.Durabilitydetails_24_1A7269D6428BC693FF3A859CFE819E71` (break `/Game/Hyper/Core/Inventory/Datamodel/Structures/Main_Item_Slot_Structs/Struct_Inventory_Slot_Item` _item)))) _maxdurability) 0.05)))))
  (return _returnvalue (`KismetMathLibrary.Round` _returnvalue) _basesellprice))

(fn `Can Buy All Items`
  (params (Seller :type "/Game/Hyper/Core/Vendor/Blueprints/AC_Vendor_Abstract Object Reference") (Buyer :type "/Game/Hyper/Core/Vendor/Blueprints/AC_Vendor_Abstract Object Reference") (Item :type "/Game/Hyper/Core/Inventory/Datamodel/Structures/Main_Item_Slot_Structs/Struct_Inventory_Slot_Item Structure") (Amount :type Integer))
  (returns (`Amount Buyer Can Buy` :type Integer) (`Buyable Amount` :type Integer) (`Buyer Has Sufficient Resources` :type Boolean) (`Seller Has Sufficient Amount` :type Boolean) (`Can Buy All` :type Boolean))
  (locals (`Local Buyable Amount` :type Integer) (`Local Amount In Inventory` :type Integer))
  (bind _local_buyable_amount (`local.Local Buyable Amount`))
  (bind _local_amount_in_inventory (`local.Local Amount In Inventory`))
  (bind _inventory (`self.Get Vendor Inventory` (`local.Seller`)))
  (bind _returnvalue (>= _local_amount_in_inventory (`local.Amount`)))
  ;[0.05098 0.05098 0.05098] Does buyer have enough resources
  (bind _output_get (set `local.Local Buyable Amount` (`self.Get Amount Buyer Can Buy` Seller Buyer Item)))
  (set `local.Local Amount In Inventory` (`/Game/Hyper/Core/Inventory/Blueprints/AC_Inventory_Abstract.How many of item in inventory` _inventory (`local.Item`) (`/Game/Hyper/Core/Inventory/Blueprints/AC_Inventory_Abstract.Inventory Slots` _inventory)))
  (bind _returnvalue_2 (>= _output_get (`local.Amount`)))
  (return (`local.Local Buyable Amount`) (select `bool` (> _local_buyable_amount _local_amount_in_inventory) :`false` _local_buyable_amount :`true` _local_amount_in_inventory) _returnvalue_2 _returnvalue (and _returnvalue_2 _returnvalue)))

(fn `Get Amount Buyer Can Buy`
  (params (Seller :type "/Game/Hyper/Core/Vendor/Blueprints/AC_Vendor_Abstract Object Reference") (Buyer :type "/Game/Hyper/Core/Vendor/Blueprints/AC_Vendor_Abstract Object Reference") (Item :type "/Game/Hyper/Core/Inventory/Datamodel/Structures/Main_Item_Slot_Structs/Struct_Inventory_Slot_Item Structure"))
  (returns (`Amount Buyer Can Buy` :type Integer))
  (bind (_cost _rounded_cost _resource) (`self.Calculate Sell Cost Of Single Item` Seller Buyer Item))
  (bind _inventory (`self.Get Vendor Inventory` (`local.Buyer`)))
  (return (`KismetMathLibrary.FFloor` (/ (`KismetMathLibrary.Conv_IntToDouble` (`/Game/Hyper/Core/Inventory/Blueprints/AC_Inventory_Abstract.How many of item in inventory` _inventory _resource (`/Game/Hyper/Core/Inventory/Blueprints/AC_Inventory_Abstract.Inventory Slots` _inventory))) (select `bool` (== _cost 0.0) :`false` _cost :`true` 1.0)))))

(fn `Get Vendor Inventory`
  (params (Vendor :type "/Game/Hyper/Core/Vendor/Blueprints/AC_Vendor_Abstract Object Reference"))
  (returns (Inventory :type "/Game/Hyper/Core/Inventory/Blueprints/AC_Inventory_Abstract Object Reference"))
  (return (`Actor.GetComponentByClass` (`self.GetOwner` Vendor) "/Game/Hyper/Core/Inventory/Blueprints/AC_Inventory_Abstract.AC_Inventory_Abstract_C")))

(fn `Process Buy Item By Trade Action`
  (params (Seller :type "/Game/Hyper/Core/Vendor/Blueprints/AC_Vendor_Abstract Object Reference") (Buyer :type "/Game/Hyper/Core/Vendor/Blueprints/AC_Vendor_Abstract Object Reference") (`Trade Action` :type "/Game/Hyper/Core/Vendor/Datamodel/Enumerations/Enum_Trading_Action_Types Enum" :default "NewEnumerator7") (Item :type "/Game/Hyper/Core/Inventory/Datamodel/Structures/Main_Item_Slot_Structs/Struct_Inventory_Slot_Item Structure") (`Custom Amount` :type Integer) (`Slot Index` :type Integer))
  (locals (`Local Amount` :type Integer))
  (bind _custom_amount (`local.Custom Amount`))
  (bind (_amount_buyer_can_buy _buyable_amount _buyer_has_sufficient_resources _seller_has_sufficient_amount _can_buy_all) (`self.Can Buy All Items` (`local.Seller`) (`local.Buyer`) (`local.Item`) _custom_amount))
  ;[0.05098 0.05098 0.05098] Is the item we are buying sellable?
  (if (`.IsSellable_1_5CA93FA548A9E6E022FB6F8637AC36AF` (break `/Game/Hyper/Core/Inventory/Datamodel/Structures/Sub_Structs_Attributes/Struct_Attributes_Sellable` (`.Sellable_Attributes_17_F8DD5673423CE0A266B8DA941969B77D` (break `/Game/Hyper/Core/Inventory/Datamodel/Structures/Main_Item_Slot_Structs/Struct_Item` (`/Game/Hyper/Core/Inventory/FunctionLibraries/BFL_InventoryCrafting.Get Inventory info from inventory slot` Item)))))
    (switch `/Game/Hyper/Core/Vendor/Datamodel/Enumerations/Enum_Trading_Action_Types` (`local.Trade Action`)
      (:`NewEnumerator0`
        ;[0.05098 0.05098 0.05098] Buy preset amount
        (set `local.Local Amount` 1)
        (`self.Try Buy Item From Seller By Slot Index` (`local.Seller`) (`local.Buyer`) (`local.Item`) (`local.Slot Index`) (`local.Local Amount`) :!label _label))
      (:`NewEnumerator1`
        (set `local.Local Amount` 5)
        (goto _label))
      (:`NewEnumerator2`
        (set `local.Local Amount` 10)
        (goto _label))
      (:`NewEnumerator6`
        (set `local.Local Amount` (`.Amount_5_3D501FFE494086BDD8C291A969150384` (break `/Game/Hyper/Core/Inventory/Datamodel/Structures/Main_Item_Slot_Structs/Struct_Inventory_Slot_Item` (`local.Item`))))
        (goto _label))
      (:`NewEnumerator3`
        ;[0.05098 0.05098 0.05098] Buy Calculated amount
        (set `local.Local Amount` _buyable_amount)
        (`self.Try To Automatically Buy Item From Seller` (`local.Seller`) (`local.Buyer`) (`local.Item`) (`local.Local Amount`) :!label _label_2))
      (:`NewEnumerator4`
        (set `local.Local Amount` (select `bool` _can_buy_all :`false` _buyable_amount :`true` _custom_amount))
        (goto _label_2)))))

(fn `Try Buy Item From Seller By Slot Index`
  (params (Seller :type "/Game/Hyper/Core/Vendor/Blueprints/AC_Vendor_Abstract Object Reference") (Buyer :type "/Game/Hyper/Core/Vendor/Blueprints/AC_Vendor_Abstract Object Reference") (Item :type "/Game/Hyper/Core/Inventory/Datamodel/Structures/Main_Item_Slot_Structs/Struct_Inventory_Slot_Item Structure") (`Slot Index` :type Integer) (Amount :type Integer))
  (bind ((`Item_2_C7967C054AE750B79BB1FDB9058FE0B3` _item) (`Durabilitydetails_24_1A7269D6428BC693FF3A859CFE819E71` _durabilitydetails) (`TradingandLootdetails_30_A4191A2D48AF499B2B301CAED61CB925` _tradingandlootdetails)) (break `/Game/Hyper/Core/Inventory/Datamodel/Structures/Main_Item_Slot_Structs/Struct_Inventory_Slot_Item` (`local.Item`)))
  (bind (_cost _rounded_cost _resource) (`self.Calculate Sell Cost Of Single Item` (`local.Seller`) (`local.Buyer`) (`local.Item`)))
  (bind _inventory (`self.Get Vendor Inventory` (`local.Buyer`)))
  (bind _inventory_2 (`self.Get Vendor Inventory` (`local.Seller`)))
  (bind ((`Item_2_C7967C054AE750B79BB1FDB9058FE0B3` _item_2) (`Durabilitydetails_24_1A7269D6428BC693FF3A859CFE819E71` _durabilitydetails_2) (`TradingandLootdetails_30_A4191A2D48AF499B2B301CAED61CB925` _tradingandlootdetails_2)) (break `/Game/Hyper/Core/Inventory/Datamodel/Structures/Main_Item_Slot_Structs/Struct_Inventory_Slot_Item` _resource))
  (bind _returnvalue (* _rounded_cost (`local.Amount`)))
  ;[0.05098 0.05098 0.05098] Remove cost from buyer inventory
  (if (`.Can Buy All` (`self.Can Buy All Items` Seller Buyer Item Amount))
    (`/Game/Hyper/Core/Inventory/Blueprints/AC_Inventory_Abstract.Remove Item From Inventory Automatically` _inventory _resource _returnvalue (`/Game/Hyper/Core/Inventory/Blueprints/AC_Inventory_Abstract.Inventory Slots` _inventory) false)
    ;[0.05098 0.05098 0.05098] Add cost to seller inventory
    (`/Game/Hyper/Core/Inventory/Blueprints/AC_Inventory_Abstract.Try Add Item to Inventory Automatically` _inventory_2 (make `/Game/Hyper/Core/Inventory/Datamodel/Structures/Main_Item_Slot_Structs/Struct_Inventory_Slot_Item` :`Item` _item_2 :`Amount` _returnvalue :`Durability details` _durabilitydetails_2 :`Trading and Loot details` _tradingandlootdetails_2) (`/Game/Hyper/Core/Inventory/Blueprints/AC_Inventory_Abstract.Inventory Slots` _inventory_2) false 0 true false true)
    ;[0.05098 0.05098 0.05098] Remove bought item from seller inventory
    (`/Game/Hyper/Core/Inventory/Blueprints/AC_Inventory_Abstract.Remove item at slot index` _inventory_2 (`local.Slot Index`) (`local.Amount`) (`/Game/Hyper/Core/Inventory/Blueprints/AC_Inventory_Abstract.Inventory Slots` _inventory_2) false false)
    ;[0.05098 0.05098 0.05098] Add Item to buyer inventory
    (`/Game/Hyper/Core/Inventory/Blueprints/AC_Inventory_Abstract.Try Add Item to Inventory Automatically` _inventory (make `/Game/Hyper/Core/Inventory/Datamodel/Structures/Main_Item_Slot_Structs/Struct_Inventory_Slot_Item` :`Item` _item :`Amount` (`local.Amount`) :`Durability details` _durabilitydetails :`Trading and Loot details` _tradingandlootdetails) (`/Game/Hyper/Core/Inventory/Blueprints/AC_Inventory_Abstract.Inventory Slots` _inventory) false 0 true false true)))

(fn `Try To Automatically Buy Item From Seller`
  (params (Seller :type "/Game/Hyper/Core/Vendor/Blueprints/AC_Vendor_Abstract Object Reference") (Buyer :type "/Game/Hyper/Core/Vendor/Blueprints/AC_Vendor_Abstract Object Reference") (Item :type "/Game/Hyper/Core/Inventory/Datamodel/Structures/Main_Item_Slot_Structs/Struct_Inventory_Slot_Item Structure") (Amount :type Integer))
  (bind ((`Item_2_C7967C054AE750B79BB1FDB9058FE0B3` _item) (`Durabilitydetails_24_1A7269D6428BC693FF3A859CFE819E71` _durabilitydetails) (`TradingandLootdetails_30_A4191A2D48AF499B2B301CAED61CB925` _tradingandlootdetails)) (break `/Game/Hyper/Core/Inventory/Datamodel/Structures/Main_Item_Slot_Structs/Struct_Inventory_Slot_Item` (`local.Item`)))
  (bind (_cost _rounded_cost _resource) (`self.Calculate Sell Cost Of Single Item` (`local.Seller`) (`local.Buyer`) (`local.Item`)))
  (bind _inventory (`self.Get Vendor Inventory` (`local.Buyer`)))
  (bind _inventory_2 (`self.Get Vendor Inventory` (`local.Seller`)))
  (bind ((`Item_2_C7967C054AE750B79BB1FDB9058FE0B3` _item_2) (`Durabilitydetails_24_1A7269D6428BC693FF3A859CFE819E71` _durabilitydetails_2) (`TradingandLootdetails_30_A4191A2D48AF499B2B301CAED61CB925` _tradingandlootdetails_2)) (break `/Game/Hyper/Core/Inventory/Datamodel/Structures/Main_Item_Slot_Structs/Struct_Inventory_Slot_Item` _resource))
  (bind _returnvalue (* _rounded_cost (`local.Amount`)))
  ;[0.05098 0.05098 0.05098 1 14] Can the buyer buy the amount of items they want to buy,
  ; Can the seller sell the amount the buyer wants to buy
  (if (`.Can Buy All` (`self.Can Buy All Items` Seller Buyer Item Amount))
    ;[0.05098 0.05098 0.05098] Remove cost from buyer inventory
    (`/Game/Hyper/Core/Inventory/Blueprints/AC_Inventory_Abstract.Remove Item From Inventory Automatically` _inventory _resource _returnvalue (`/Game/Hyper/Core/Inventory/Blueprints/AC_Inventory_Abstract.Inventory Slots` _inventory) false)
    ;[0.05098 0.05098 0.05098] Add cost to seller inventory
    (`/Game/Hyper/Core/Inventory/Blueprints/AC_Inventory_Abstract.Try Add Item to Inventory Automatically` _inventory_2 (make `/Game/Hyper/Core/Inventory/Datamodel/Structures/Main_Item_Slot_Structs/Struct_Inventory_Slot_Item` :`Item` _item_2 :`Amount` _returnvalue :`Durability details` _durabilitydetails_2 :`Trading and Loot details` _tradingandlootdetails_2) (`/Game/Hyper/Core/Inventory/Blueprints/AC_Inventory_Abstract.Inventory Slots` _inventory_2) false 0 true false true)
    ;[0.05098 0.05098 0.05098] Remove the item from seller inventory
    (`/Game/Hyper/Core/Inventory/Blueprints/AC_Inventory_Abstract.Remove Item From Inventory Automatically` _inventory_2 (`local.Item`) (`local.Amount`) (`/Game/Hyper/Core/Inventory/Blueprints/AC_Inventory_Abstract.Inventory Slots` _inventory_2) false)
    ;[0.05098 0.05098 0.05098] Add Item to buyer inventory
    (`/Game/Hyper/Core/Inventory/Blueprints/AC_Inventory_Abstract.Try Add Item to Inventory Automatically` _inventory (make `/Game/Hyper/Core/Inventory/Datamodel/Structures/Main_Item_Slot_Structs/Struct_Inventory_Slot_Item` :`Item` _item :`Amount` (`local.Amount`) :`Durability details` _durabilitydetails :`Trading and Loot details` _tradingandlootdetails) (`/Game/Hyper/Core/Inventory/Blueprints/AC_Inventory_Abstract.Inventory Slots` _inventory) false 0 true false true)))