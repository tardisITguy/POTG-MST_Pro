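; BP_Chaos_AnchorField is a Chaos field actor that anchors physics particles by setting their dynamic state to static within a box.
; The construction script resets the field system, then adds a single dynamic-state command built from a uniform integer culled outside a box falloff.
; The Cube component's world transform defines the box, and the event graph holds only disabled default events.
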(fn `UserConstructionScript`
  (bind _fieldsystemcomponent (`self.FieldSystemComponent`))
  ;[1 1 1] Removes all field components
  (`FieldSystemComponent.ResetFieldSystem` _fieldsystemcomponent)
  ;[1 1 1] dynamic state
  (`FieldSystemComponent.AddFieldCommand` _fieldsystemcomponent true "Field_DynamicState" null (`CullingField.SetCullingField` (`self.CullingField`) (`BoxFalloff.SetBoxFalloff` (`self.BoxFalloff`) 1.0 0.0 1.0 0.0 (`SceneComponent.K2_GetComponentToWorld` (`self.Cube`)) "Field_FallOff_None") (`UniformInteger.SetUniformInteger` (`self.UniformInteger`) (`KismetMathLibrary.Conv_ByteToInt` (`self.StaticState`))) "Field_Culling_Outside")))