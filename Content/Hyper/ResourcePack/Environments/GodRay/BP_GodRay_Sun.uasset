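; BP_GodRay_Sun is a placeable god ray light shaft effect, configured entirely in its construction script.
; It adds a mesh with a dynamic instance of either the animated or master god ray material, optionally copying the rotation of a referenced Sun actor.
; A spotlight flag selects the mask texture, and exposed shape, color, brightness and fade settings feed the material alongside a stream-seeded random value.
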(fn `UserConstructionScript`
  (bind _mid (`self.MID`))
  (bind _godraymesh (`self.GodRayMesh`))
  (bind _returnvalue (`AddComponent|NODE_AddStaticMeshComponent-0`))
  (set `self.GodRayMesh` _returnvalue)
  (if (`self.Animated`)
    (bind _returnvalue_2 (`PrimitiveComponent.CreateDynamicMaterialInstance` _godraymesh 0 "/Game/Hyper/ResourcePack/Environments/GodRay/Materials/M_GodRay_Animated.M_GodRay_Animated" "None"))
    (set `self.MID` _returnvalue_2)
    (else
      (bind _returnvalue_3 (`PrimitiveComponent.CreateDynamicMaterialInstance` _godraymesh 0 "/Game/Hyper/ResourcePack/Environments/GodRay/Materials/M_GodRay_MASTER.M_GodRay_MASTER" "None"))
      (set `self.MID` _returnvalue_3)))
  (`PrimitiveComponent.SetMaterial` (`self.GodRayMesh`) 0 (`self.MID`))
  (if (`self.UseSun`)
    (`SceneComponent.K2_SetRelativeRotation` (`self.GodRayMesh`) (`self.K2_GetActorRotation` (`self.Sun`)) true false))
  (if (`self.SpotLight`)
    (`MaterialInstanceDynamic.SetTextureParameterValue` _mid "Mask" "/Game/Hyper/ResourcePack/Environments/GodRay/Textures/T_GodRay_Mask02.T_GodRay_Mask02")
    (else
      (`MaterialInstanceDynamic.SetTextureParameterValue` _mid "Mask" "/Game/Hyper/ResourcePack/Environments/GodRay/Textures/T_GodRay_Mask01.T_GodRay_Mask01")))
  (`MaterialInstanceDynamic.SetScalarParameterValue` _mid "width" (`self.Width`))
  (`MaterialInstanceDynamic.SetScalarParameterValue` _mid "Length" (`self.Length`))
  (`MaterialInstanceDynamic.SetVectorParameterValue` _mid "color" (`self.Color`))
  (`MaterialInstanceDynamic.SetScalarParameterValue` _mid "Brightness" (`self.Brightness`))
  (`MaterialInstanceDynamic.SetScalarParameterValue` _mid "fadedistance" (`self.FadeDistance`))
  (`MaterialInstanceDynamic.SetScalarParameterValue` _mid "random" (`KismetMathLibrary.RandomFloatInRangeFromStream` (`self.RandomTime`) 0.0 100.0)))