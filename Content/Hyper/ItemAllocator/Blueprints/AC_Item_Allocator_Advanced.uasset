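; Item allocator component that stocks an inventory with vendor goods or loot, using the vendor's trade details when present, otherwise its own allocation list.
; It adds specific items and category matches from DT_Items, rolling chance and amount up to max stock, skipping excluded entries.
; Category fills write slots directly when the inventory starts empty.
; Optional one-second countdown timers drive repeated restocking and a full wipe-and-refill, whose timer stops after firing.
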(fn `Allocate Complete Category lists`
  (params (`auto include list` :type "Array of /Game/Hyper/Core/Vendor/Datamodel/Structures/Struct_Vendor_Sell_Categories_Details Structure (by ref)") (`Ignore categories` :type "Array of /Game/Hyper/Core/Inventory/Datamodel/Enumerations/Enum_Item_Categories Enum (by ref)"))
  (locals (`Local Next Slot Index` :type Integer) (`Local Current Row` :type Name) (`Local Current Categories` :type "Array of /Game/Hyper/Core/Inventory/Datamodel/Enumerations/Enum_Item_Categories Enum") (`Local Is Initialization` :type Boolean))
  ;[0.05098 0.05098 0.05098] Check if the inventory is empty so we can optimize the allocation process
  (set `local.Local Is Initialization` (`/Game/Hyper/Core/Inventory/FunctionLibraries/BFL_InventoryCrafting.Is Inventory Array Empty` (`/Game/Hyper/Core/Inventory/Blueprints/AC_Inventory_Abstract.Inventory Slots` (`/Game/Hyper/Core/Inventory/BlueprintMacroLibrary/BML_Inventory_Component.Get Inventory Manager`))))
  ;[0.05098 0.05098 0.05098] Loops over all items in the data table from the items to check if it has the same category. If it does, restock item.
  ;;[0.05098 0.05098 0.05098] Loop over all items and get each catagory
  (bind _outrownames (`DataTableFunctionLibrary.GetDataTableRowNames` "/Game/Hyper/Core/Inventory/Datamodel/Datatables/DT_Items.DT_Items"))
  (for _array_element _outrownames
    (bind _output_get (set `local.Local Current Row` _array_element))
    (bind _returnvalue (`|GetDataTableRow` "/Game/Hyper/Core/Inventory/Datamodel/Datatables/DT_Items.DT_Items" _output_get)
      (:`then`
        (bind ((`Categories_19_2BE791FB418EF8ED5C8F5BB16CFE96FE` _categories)) (break `/Game/Hyper/Core/Inventory/Datamodel/Structures/Sub_Structs_Attributes/Struct_Attributes_Generic` (`.GenericAttributes_2_ECBA8D824275F3AB65EED8A7E46C293F` (break `/Game/Hyper/Core/Inventory/Datamodel/Structures/Main_Item_Slot_Structs/Struct_Item` _returnvalue))))
        (if (`KismetArrayLibrary.Array_IsNotEmpty` _categories)
          (bind _output_get_2 (set `local.Local Current Categories` _categories))
          (for _array_element_2 _output_get_2
            (bind _returnvalue_2 (`KismetArrayLibrary.Array_Contains` (`local.Ignore categories`) _array_element_2))
            ;[0.05098 0.05098 0.05098] Check if the found category is one that we don't want to sell. If so we break, if we dont break the last result of the contains node will be false which means we will continue with the restock
            (if _returnvalue_2
              (break)))
          (if (not _returnvalue_2)
            ;[0.05098 0.05098 0.05098] If the item is in one of the sell categories, restock the item based on the restock settings for this category
            (for _array_element_3 (`local.auto include list`) :!label _label
              ;;[0.05098 0.05098 0.05098] Check if one of the accepted categories is one of the assigned towards the item
              (if (`KismetArrayLibrary.Array_Contains` (`local.Local Current Categories`) (break `/Game/Hyper/Core/Vendor/Datamodel/Structures/Struct_Vendor_Sell_Categories_Details` _array_element_3))
                (bind _new_next_index (`self.Try Allocate Item` (make `/Game/Hyper/Core/Inventory/Datamodel/Structures/Main_Item_Slot_Structs/Struct_Inventory_Slot_Item` :`Item` (make `DataTableRowHandle` "/Game/Hyper/Core/Inventory/Datamodel/Datatables/DT_Items.DT_Items" (`local.Local Current Row`)) :`Trading and Loot details` (`.TradingDetailsettingsforcategory_9_1BC4FF1D4F5F189DBA729C8DBEC21458` (break `/Game/Hyper/Core/Vendor/Datamodel/Structures/Struct_Vendor_Sell_Categories_Details` _array_element_3))) (`local.Local Is Initialization`) (`local.Local Next Slot Index`)))
                (set `local.Local Next Slot Index` _new_next_index)
                (break))))
          (else
            (goto _label)))))))

(fn `Allocate Items`
  (locals (`Local Allocation List` :type "/Game/Hyper/Core/Inventory/Datamodel/Structures/Loot_Struct/Struct_Loot Structure" :default (struct)))
  (bind (_component _is_valid) (`/Game/Hyper/Core/Vendor/BlueprintMacroLibrary/BML_Vendor_Component.Get Vendor Manager`))
  (bind (_local_allocation_list_specificitemstoaddtolootlist _local_allocation_list_categoriestoautomaticlyincludeinthelootlist _local_allocation_list_dontincludethesecategories) (break `/Game/Hyper/Core/Inventory/Datamodel/Structures/Loot_Struct/Struct_Loot` (`local.Local Allocation List`)))
  (bind (_vendor_trading_details_defaultforsalelistperitem _vendor_trading_details_notintrestedinthesespecificitems _vendor_trading_details_notintrestedinfollowingcategories _vendor_trading_details_selleverythinginthefollowingcategories _vendor_trading_details_dontsellfromthesecatagories) (break `/Game/Hyper/Core/Vendor/Datamodel/Structures/Struct_Vendor_TradingDetails` (`/Game/Hyper/Core/Vendor/FunctionLibraries/BFL_Vendor.Get Trade Details From Trade List` (`/Game/Hyper/Core/Vendor/Blueprints/AC_Vendor_Abstract.Trade List` _component))))
  (`|ExecutionSequence`
    (:`then_0`
      ;[0.05098 0.05098 0.05098] Select an allocation list to use. if we have a vendor component we get this info from the trade details, if not we use the assigned allocation list on this component
      (if _is_valid
        (set `local.Local Allocation List` (make `/Game/Hyper/Core/Inventory/Datamodel/Structures/Loot_Struct/Struct_Loot` _vendor_trading_details_defaultforsalelistperitem _vendor_trading_details_selleverythinginthefollowingcategories _vendor_trading_details_dontsellfromthesecatagories))
        (else
          (set `local.Local Allocation List` (`/Game/Hyper/Core/ItemAllocator/FunctionLibraries/BFL_ItemAllocator.Get Loot Details From Loot List` (`self.Allocation List`))))))
    (:`then_1`
      ;[0.05098 0.05098 0.05098] Allocate the categories and the individiual items
      (`|ExecutionSequence`
        (:`then_0`
          (if (`KismetArrayLibrary.Array_IsNotEmpty` _local_allocation_list_categoriestoautomaticlyincludeinthelootlist)
            (`self.Allocate Complete Category lists` _local_allocation_list_categoriestoautomaticlyincludeinthelootlist _local_allocation_list_dontincludethesecategories)))
        (:`then_1`
          (for _array_element _local_allocation_list_specificitemstoaddtolootlist
            (`self.Try Allocate Item` _array_element)))))))

(fn `Reset Inventory Allocation`
  (bind _component (`/Game/Hyper/Core/Inventory/BlueprintMacroLibrary/BML_Inventory_Component.Get Inventory Manager`))
  (bind _inventory_slots (`/Game/Hyper/Core/Inventory/Blueprints/AC_Inventory_Abstract.Inventory Slots` _component))
  ;[0.05098 0.05098 0.05098] Clear the existing item slots and create new slots, and fill them with items
  (for _array_element _inventory_slots
    (`KismetArrayLibrary.Array_RemoveItem` _inventory_slots _array_element))
  (for _ (range 1 (+ (`/Game/Hyper/Core/Inventory/Blueprints/AC_Inventory_Abstract.Amount of default inventory slots` _component) 1))
    (`/Game/Hyper/Core/Inventory/Blueprints/AC_Inventory_Abstract.Create Empty slot` (`/Game/Hyper/Core/Inventory/BlueprintMacroLibrary/BML_Inventory_Component.Get Inventory Manager`) _inventory_slots))
  (`self.Allocate Items`))

(fn `Should Item be Allocated`
  (params (Item :type "/Game/Hyper/Core/Inventory/Datamodel/Structures/Main_Item_Slot_Structs/Struct_Inventory_Slot_Item Structure"))
  (returns (`Should Be Allocated` :type Boolean))
  (return (not (`KismetArrayLibrary.Array_Contains` (`self.Never Allocate These Items`) (`.Item_2_C7967C054AE750B79BB1FDB9058FE0B3` (break `/Game/Hyper/Core/Inventory/Datamodel/Structures/Main_Item_Slot_Structs/Struct_Inventory_Slot_Item` Item))))))

(fn `Try Allocate Item`
  (params (`Item to restock` :type "/Game/Hyper/Core/Inventory/Datamodel/Structures/Main_Item_Slot_Structs/Struct_Inventory_Slot_Item Structure (by ref)") (`Is Initialization` :type Boolean) (`Slot Index` :type Integer))
  (returns (`New Next Index` :type Integer))
  (locals (`Local Item to be added` :type "/Game/Hyper/Core/Inventory/Datamodel/Structures/Main_Item_Slot_Structs/Struct_Inventory_Slot_Item Structure") (`Local Amount Of Item In Inventory` :type Integer :default 0) (`Local Random Amount To Restock` :type Integer :default 0) (`Local Final Amount To Restock` :type Integer))
  (bind _component (`/Game/Hyper/Core/Inventory/BlueprintMacroLibrary/BML_Inventory_Component.Get Inventory Manager`))
  (bind _component_2 (`/Game/Hyper/Core/Inventory/BlueprintMacroLibrary/BML_Inventory_Component.Get Inventory Manager`))
  (bind ((`Item_2_C7967C054AE750B79BB1FDB9058FE0B3` _item) (`Durabilitydetails_24_1A7269D6428BC693FF3A859CFE819E71` _durabilitydetails) (`TradingandLootdetails_30_A4191A2D48AF499B2B301CAED61CB925` _tradingandlootdetails)) (break `/Game/Hyper/Core/Inventory/Datamodel/Structures/Main_Item_Slot_Structs/Struct_Inventory_Slot_Item` (`local.Item to restock`)))
  (bind ((`MinimalAmounttorestock_21_BA2367A942C13C6A54AA508D309DA605` _minimalamounttorestock) (`MaximumAmounttorestock_23_C7C2305845A38A3A443C8B87E8598D47` _maximumamounttorestock)) (break `/Game/Hyper/Core/Inventory/Datamodel/Structures/Main_Item_Slot_Structs/Struct_SlotInfo_Trading_and_Loot_Details` (`.TradingandLootdetails_30_A4191A2D48AF499B2B301CAED61CB925` (break `/Game/Hyper/Core/Inventory/Datamodel/Structures/Main_Item_Slot_Structs/Struct_Inventory_Slot_Item` (`local.Item to restock`)))))
  (bind ((`MaximumStock_20_C773D3F74CB0350366977E9C7C072938` _maximumstock)) (break `/Game/Hyper/Core/Inventory/Datamodel/Structures/Main_Item_Slot_Structs/Struct_SlotInfo_Trading_and_Loot_Details` (`.TradingandLootdetails_30_A4191A2D48AF499B2B301CAED61CB925` (break `/Game/Hyper/Core/Inventory/Datamodel/Structures/Main_Item_Slot_Structs/Struct_Inventory_Slot_Item` (`local.Item to restock`)))))
  (bind ((`Chanceofspawinginvendorinventory_31_DFBA6D9B45C1E145B0A6A2BC8F065A28` _chanceofspawinginvendorinventory) (`MaximumStock_20_C773D3F74CB0350366977E9C7C072938` _maximumstock_2)) (break `/Game/Hyper/Core/Inventory/Datamodel/Structures/Main_Item_Slot_Structs/Struct_SlotInfo_Trading_and_Loot_Details` (`.TradingandLootdetails_30_A4191A2D48AF499B2B301CAED61CB925` (break `/Game/Hyper/Core/Inventory/Datamodel/Structures/Main_Item_Slot_Structs/Struct_Inventory_Slot_Item` (`local.Item to restock`)))))
  (if (`self.Should Item be Allocated` `Item to restock`)
    (set `local.Local Amount Of Item In Inventory` (`/Game/Hyper/Core/Inventory/Blueprints/AC_Inventory_Abstract.How many of item in inventory` _component (`local.Item to restock`) (`/Game/Hyper/Core/Inventory/Blueprints/AC_Inventory_Abstract.Inventory Slots` _component)))
    ;[0.05098 0.05098 0.05098] Check if item should be restocked based on random chance
    (if (<= (`KismetMathLibrary.RandomFloatInRange` 0.0 1.0) _chanceofspawinginvendorinventory)
      (if (< (`local.Local Amount Of Item In Inventory`) _maximumstock_2)
        (set `local.Local Random Amount To Restock` (`KismetMathLibrary.RandomIntegerInRange` _minimalamounttorestock _maximumamounttorestock))
        (set `local.Local Final Amount To Restock` (select `bool` (>= (+ (`local.Local Amount Of Item In Inventory`) (`local.Local Random Amount To Restock`)) _maximumstock) :`false` (`local.Local Random Amount To Restock`) :`true` (- _maximumstock (`local.Local Amount Of Item In Inventory`))))
        ;[0.05098 0.05098 0.05098] Create the item that we will be restocking so we dont have to duplicate the code in the next step
        (set `local.Local Item to be added` (make `/Game/Hyper/Core/Inventory/Datamodel/Structures/Main_Item_Slot_Structs/Struct_Inventory_Slot_Item` :`Item` _item :`Amount` (`local.Local Final Amount To Restock`) :`Durability details` _durabilitydetails :`Trading and Loot details` _tradingandlootdetails))
        (if (`local.Is Initialization`)
          ;[0.05098 0.05098 0.05098] Optimized way of restocking, when we are initializing we assume the inventory is empty meaning we can set the slot indices directly
          (setmembers `/Game/Hyper/Core/Inventory/Datamodel/Structures/Main_Item_Slot_Structs/Struct_Inventory_Slot_Item` :`StructRef` (`local.Local Item to be added`) :`Slot Index` (`local.Slot Index`))
          (`KismetArrayLibrary.Array_Set` (`/Game/Hyper/Core/Inventory/Blueprints/AC_Inventory_Abstract.Inventory Slots` (`/Game/Hyper/Core/Inventory/BlueprintMacroLibrary/BML_Inventory_Component.Get Inventory Manager`)) (`local.Slot Index`) (`local.Local Item to be added`) true)
          (return (+ (`local.Slot Index`) 1))
          (else
            ;[0.05098 0.05098 0.05098] Automatically add the item to the inventory. because we dont know if the inventory is empty, we cant optimize and need to use this function
            (`/Game/Hyper/Core/Inventory/Blueprints/AC_Inventory_Abstract.Try Add Item to Inventory Automatically` _component_2 (`local.Local Item to be added`) (`/Game/Hyper/Core/Inventory/Blueprints/AC_Inventory_Abstract.Inventory Slots` _component_2) true 1000000 false false true)))))))